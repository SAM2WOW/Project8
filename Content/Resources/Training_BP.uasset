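; Tutorial actor that walks the player through a list of control prompts, plus a dash hint triggered when attacked.
; StartTutorial or MsgInteract shows the first Tutorial_Widget hint; later MsgInteract calls advance it.
; Input events match the current step's action name, filling progress for holds.
; Completed steps post HUD console messages, add MemoryLog_DT entries and open a pausing log popup; finishing logs Dash and destroys the actor.
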(event `/Game/Resources/Characters/Interactables/interactable_interface.msg_interact`
  (bind (_output_text _output_button _output_action _output_is_hold) (break `/Game/Resources/Characters/Player/Blueprints/Tutorial/Tutorial_Struct` (`|GetArrayItem` (`self.List`) (`self.Index`))))
  (if (`self.main_tutorial`)
    (`self.Next`)
    (else
      (`KismetSystemLibrary.Delay` 0.2 :!label _label)
      (set `self.main_tutorial` true)
      (`self.SpawnHint` _output_text _output_is_hold (`KismetStringLibrary.Conv_StringToName` _output_action)))))

(event `StartTutorial`
  (goto _label))

(event `Attacked`
  (`self.SpawnHint` "SPACE" false "IA_Dashing")
  (set `self.initial_attacked` true))

(event `EnhancedInput|/Game/Resources/Characters/Player/Input/Actions/IA_Dashing`
  (params (ActionValue :type Boolean) (ElapsedSeconds :type "Float (double-precision)") (TriggeredSeconds :type "Float (double-precision)") (InputAction :type "InputAction Object Reference" :default "/Game/Resources/Characters/Player/Input/Actions/IA_Dashing.IA_Dashing"))
  (bind _hinttemp (`self.HintTemp`))
  (:`Started`
    (if (and (`KismetSystemLibrary.IsValid` _hinttemp) (`self.initial_attacked`))
      (`/Game/Resources/Widgets/Tutorial_Widget.Released` _hinttemp)
      (set `self.initial_attacked` false))))

(event `SpawnHint`
  (params (`Hint Text` :type Text) (`Is Hold` :type Boolean) (Action :type Name))
  (bind _hinttemp (`self.HintTemp`))
  (if (`KismetSystemLibrary.IsValid` _hinttemp)
    (`/Game/Resources/Widgets/Tutorial_Widget.Released` _hinttemp)
    (`KismetSystemLibrary.Delay` 0.5))
  (bind _returnvalue (`|CreateWidget` "/Game/Resources/Widgets/Tutorial_Widget.Tutorial_Widget_C" null `Hint Text` `Is Hold` Action))
  (`UserWidget.AddToViewport` _returnvalue 0)
  (set `self.HintTemp` _returnvalue))

(event `self.ReceiveTick`
  (params (DeltaSeconds :type "Float (single-precision)"))
  (if (`self.Holding`)
    (`/Game/Resources/Widgets/Tutorial_Widget.UpdateProgress` (`self.HintTemp`) (`self.temp_progress`))))

(event `EnhancedInput|/Game/Resources/Characters/Player/Input/Actions/IA_Deploy`
  (params (ActionValue :type Boolean) (ElapsedSeconds :type "Float (double-precision)") (TriggeredSeconds :type "Float (double-precision)") (InputAction :type "InputAction Object Reference" :default "/Game/Resources/Characters/Player/Input/Actions/IA_Deploy.IA_Deploy"))
  (bind _index (`self.Index`))
  (bind (_output_text _output_button _output_action) (break `/Game/Resources/Characters/Player/Blueprints/Tutorial/Tutorial_Struct` (`|GetArrayItem` (`self.List`) (`self.Index`))))
  (bind (_output_text_2 _output_button_2 _output_action_2 _output_is_hold) (break `/Game/Resources/Characters/Player/Blueprints/Tutorial/Tutorial_Struct` (`|GetArrayItem` (`self.List`) (`self.Index`))))
  (bind _returnvalue (- _index 1))
  (bind (_output_text_3 _output_button_3 _output_action_3 _output_is_hold_2 _output_tutoriallog) (break `/Game/Resources/Characters/Player/Blueprints/Tutorial/Tutorial_Struct` (`|GetArrayItem` (`self.List`) _returnvalue)))
  (:`Completed`
    (if (`KismetStringLibrary.EqualEqual_StrStr` (`KismetSystemLibrary.GetDisplayName` InputAction) _output_action)
      (if (`self.main_tutorial`) :!label _label_2
        (if _output_is_hold
          (if (>= (`self.temp_progress`) 1.0)
            (set `self.temp_progress` 0.0)
            (`/Game/Resources/Widgets/Tutorial_Widget.Released` (`self.HintTemp`) :!label _label_3)
            (`/Engine/EditorBlueprintResources/StandardMacros.IncrementInt` _index
              (:`  `
                (bind _asnew_game_mode_gm (cast `/Game/Resources/Characters/Player/Blueprints/NewGameMode_GM` (`GameplayStatics.GetGameMode`)))
                (`/Game/Resources/Widgets/HUD_Widget.Add Console` (`/Game/Resources/Characters/Player/Blueprints/NewGameMode_GM.HUD_ref` _asnew_game_mode_gm) (`|FormatText` "<RichText.Emphasis>{name}</> Calibrated" (`KismetTextLibrary.TextToUpper` _output_button_3)) "" 8.0 (select `int` _returnvalue :`0` "/Game/Resources/Widgets/Textures/Fast.Fast" :`1` "/Game/Resources/Widgets/Textures/Console/Confirm.Confirm" :`2` "/Game/Resources/Widgets/Textures/Console/Confirm.Confirm" :`3` "/Game/Resources/Widgets/Textures/Charged.Charged" :`4` "/Game/Resources/Widgets/Textures/Console/Confirm.Confirm" :!type "Texture2D Object Reference"))
                ;[1 0.9609 0] Add Logs
                (bind _returnvalue_2 (`|GetDataTableRow` "/Game/Resources/Characters/Interactables/MemoryLog_DT.MemoryLog_DT" _output_tutoriallog)
                  (:`then`
                    (bind _asnew_game_state_gs (cast `/Game/Resources/Characters/Player/Blueprints/NewGameState_GS` (`GameplayStatics.GetGameState`)))
                    (`BlueprintMapLibrary.Map_Add` (`/Game/Resources/Characters/Player/Blueprints/NewGameState_GS.LogEntries` _asnew_game_state_gs) _output_tutoriallog _returnvalue_2)
                    ;[0 0.1797 1] Intrusive Tutorials
                    (`GameplayStatics.SetGamePaused` true)
                    (bind _returnvalue_3 (`|CreateWidget` "/Game/Resources/Widgets/LogPopup_Widget.LogPopup_Widget_C" null _returnvalue_2 (`GameplayStatics.ProjectWorldToScreen` (`GameplayStatics.GetPlayerController` 0) (`self.K2_GetActorLocation` (`GameplayStatics.GetPlayerPawn` 0))) true))
                    (`UserWidget.AddToViewport` _returnvalue_3 0)))))
            (else
              (set `self.temp_progress` 0.0)
              (`/Game/Resources/Widgets/Tutorial_Widget.UpdateProgress` (`self.HintTemp`) 0.0)))
          (else
            (goto _label_3)))))))

(event `EnhancedInput|/Game/Resources/Characters/Player/Input/Actions/IA_HeavyAttack`
  (params (ActionValue :type Boolean) (ElapsedSeconds :type "Float (double-precision)") (TriggeredSeconds :type "Float (double-precision)") (InputAction :type "InputAction Object Reference" :default "/Game/Resources/Characters/Player/Input/Actions/IA_HeavyAttack.IA_HeavyAttack"))
  (bind (_output_text _output_button _output_action) (break `/Game/Resources/Characters/Player/Blueprints/Tutorial/Tutorial_Struct` (`|GetArrayItem` (`self.List`) (`self.Index`))))
  (bind _returnvalue (`KismetStringLibrary.EqualEqual_StrStr` (`KismetSystemLibrary.GetDisplayName` InputAction) _output_action))
  (:`Triggered`
    (if _returnvalue
      (bind _output_get (set `self.temp_progress` (`KismetMathLibrary.FMin` (+ (`self.temp_progress`) (* (`GameplayStatics.GetWorldDeltaSeconds`) 1.5)) 1.0)))
      (`/Game/Resources/Widgets/Tutorial_Widget.UpdateProgress` (`self.HintTemp`) _output_get)))
  (:`Completed`
    (if _returnvalue
      (goto _label_2))))

(event `Next`
  (bind _hinttemp (`self.HintTemp`))
  (bind (_output_text _output_button _output_action _output_is_hold) (break `/Game/Resources/Characters/Player/Blueprints/Tutorial/Tutorial_Struct` (`|GetArrayItem` (`self.List`) (`self.Index`))))
  (if (<= (`self.Index`) (`KismetArrayLibrary.Array_LastIndex` (`self.List`)))
    (`self.SpawnHint` _output_text _output_is_hold (`KismetStringLibrary.Conv_StringToName` _output_action))
    (elif (`KismetSystemLibrary.IsValid` _hinttemp)
      (`/Game/Resources/Widgets/Tutorial_Widget.Released` _hinttemp)
      ;[1 0 0.5156] Idoit
      (bind _asnew_game_mode_gm (cast `/Game/Resources/Characters/Player/Blueprints/NewGameMode_GM` (`GameplayStatics.GetGameMode`)))
      (bind _hud_ref (`/Game/Resources/Characters/Player/Blueprints/NewGameMode_GM.HUD_ref` _asnew_game_mode_gm))
      (`/Game/Resources/Widgets/HUD_Widget.Add Console` _hud_ref (`|FormatText` "<RichText.Emphasis>DASH</> Calibrated") "" 8.0 "/Game/Resources/Widgets/Textures/Console/Confirm.Confirm")
      (`/Game/Resources/Widgets/HUD_Widget.Add Console` _hud_ref "<RichText.Emphasis>TUTORIALS</> added to <RichText.Emphasis>LOGS</>" "PAUSE the game to open LOGS menu" 16.0 "/Game/Resources/Widgets/Textures/Console/Confirm.Confirm")
      ;[1 0.9609 0] Add Logs
      (bind _returnvalue (`|GetDataTableRow` "/Game/Resources/Characters/Interactables/MemoryLog_DT.MemoryLog_DT" "Dash")
        (:`then`
          (bind _asnew_game_state_gs (cast `/Game/Resources/Characters/Player/Blueprints/NewGameState_GS` (`GameplayStatics.GetGameState`)))
          (`BlueprintMapLibrary.Map_Add` (`/Game/Resources/Characters/Player/Blueprints/NewGameState_GS.LogEntries` _asnew_game_state_gs) "Dash" _returnvalue)
          ;[1 0.09375 0] Kill
          (`self.K2_DestroyActor`))))))

(event `EnhancedInput|/Game/Resources/Characters/Player/Input/Actions/IA_LightAttack`
  (params (ActionValue :type Boolean) (ElapsedSeconds :type "Float (double-precision)") (TriggeredSeconds :type "Float (double-precision)") (InputAction :type "InputAction Object Reference" :default "/Game/Resources/Characters/Player/Input/Actions/IA_LightAttack.IA_LightAttack"))
  (bind (_output_text _output_button _output_action) (break `/Game/Resources/Characters/Player/Blueprints/Tutorial/Tutorial_Struct` (`|GetArrayItem` (`self.List`) (`self.Index`))))
  (bind _returnvalue (`KismetStringLibrary.EqualEqual_StrStr` (`KismetSystemLibrary.GetDisplayName` InputAction) _output_action))
  (:`Triggered`
    (if _returnvalue
      (bind _output_get (set `self.temp_progress` (`KismetMathLibrary.FMin` (+ (`self.temp_progress`) (* (`GameplayStatics.GetWorldDeltaSeconds`) 1.5)) 1.0)))
      (`/Game/Resources/Widgets/Tutorial_Widget.UpdateProgress` (`self.HintTemp`) _output_get)))
  (:`Completed`
    (if _returnvalue
      (goto _label_2))))

(event `EnhancedInput|/Game/Resources/Characters/Player/Input/Actions/IA_Dashing`
  (params (ActionValue :type Boolean) (ElapsedSeconds :type "Float (double-precision)") (TriggeredSeconds :type "Float (double-precision)") (InputAction :type "InputAction Object Reference" :default "/Game/Resources/Characters/Player/Input/Actions/IA_Dashing.IA_Dashing"))
  (bind (_output_text _output_button _output_action) (break `/Game/Resources/Characters/Player/Blueprints/Tutorial/Tutorial_Struct` (`|GetArrayItem` (`self.List`) (`self.Index`))))
  (bind _returnvalue (`KismetStringLibrary.EqualEqual_StrStr` (`KismetSystemLibrary.GetDisplayName` InputAction) _output_action))
  (:`Triggered`
    (if _returnvalue
      (bind _output_get (set `self.temp_progress` (`KismetMathLibrary.FMin` (+ (`self.temp_progress`) (* (`GameplayStatics.GetWorldDeltaSeconds`) 1.5)) 1.0)))
      (`/Game/Resources/Widgets/Tutorial_Widget.UpdateProgress` (`self.HintTemp`) _output_get)))
  (:`Completed`
    (if _returnvalue
      (goto _label_2))))

(event `EnhancedInput|/Game/Resources/Characters/Player/Input/Actions/IA_EditMode`
  (params (ActionValue :type Boolean) (ElapsedSeconds :type "Float (double-precision)") (TriggeredSeconds :type "Float (double-precision)") (InputAction :type "InputAction Object Reference" :default "/Game/Resources/Characters/Player/Input/Actions/IA_EditMode.IA_EditMode"))
  (bind (_output_text _output_button _output_action) (break `/Game/Resources/Characters/Player/Blueprints/Tutorial/Tutorial_Struct` (`|GetArrayItem` (`self.List`) (`self.Index`))))
  (:`Completed`
    (if (`KismetStringLibrary.EqualEqual_StrStr` (`KismetSystemLibrary.GetDisplayName` InputAction) _output_action)
      (goto _label_2))))

(fn `UserConstructionScript`)