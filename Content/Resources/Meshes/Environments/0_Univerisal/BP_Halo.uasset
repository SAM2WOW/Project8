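; BP_Halo is an environment Blueprint that makes its Halo component bob up and down.
; While Looping is true, Tick sets the relative Z location from a sine of game time, using a random phase Offset chosen at BeginPlay so instances bob out of sync.
; An older Movement timeline that levitates the halo and toggles direction remains in the graph but never runs.
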(event `self.ReceiveBeginPlay`
  (set `self.Offset` (`KismetMathLibrary.RandomFloatInRange` 0.0 100.0)))

(event `self.ReceiveTick`
  (params (DeltaSeconds :type "Float (single-precision)"))
  (if (`self.Looping?`)
    (`SceneComponent.K2_SetRelativeLocation` (`self.Halo`) (`KismetMathLibrary.MakeVector` 0.0 0.0 (* (`KismetMathLibrary.Sin` (+ (`KismetSystemLibrary.GetGameTimeInSeconds`) (`self.Offset`))) 7.0)) false false)))

(fn `UserConstructionScript`)