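; Interactable double door that can start locked; interacting unlocks and opens it, then turns off further interaction and its UI.
; Once unlocked, a sphere trigger opens it when the player character enters and closes it when they leave.
; One timeline, played forward or reversed, swings both leaves in mirrored pitch rotations, while their Camera collision switches to ignore on opening and block on closing.
; An older sliding timeline remains unwired.
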(event `self.Interact`
  (`parent.Interact`)
  (if (`self.locked`)
    (set `self.locked` false)
    (`self.DoorOpen`)
    (set `self.ShowInteractUI?` false)
    (set `self.Interactable` false)))

(event `DoorOpen`
  (`PrimitiveComponent.SetCollisionResponseToChannel` (`self.Door`) "ECC_Camera" "ECR_Ignore")
  (`PrimitiveComponent.SetCollisionResponseToChannel` (`self.Door2`) "ECC_Camera" "ECR_Ignore")
  (bind (_direction _progress) (`Timeline|Door Open` :!label _label)
    (:`Update`
      (bind _returnvalue (`KismetMathLibrary.Lerp` 0.0 -90.0 _progress))
      (`SceneComponent.K2_SetRelativeRotation` (`self.Door`) (`KismetMathLibrary.MakeRotator` 0.0 _returnvalue) false false)
      (`SceneComponent.K2_SetRelativeRotation` (`self.Door2`) (`KismetMathLibrary.MakeRotator` 180.0 (* _returnvalue -1.0) 180.0) false false))))

(event `self.Sphere.OnComponentBeginOverlap`
  (params (OverlappedComponent :type "PrimitiveComponent Object Reference") (OtherActor :type "Actor Object Reference") (OtherComp :type "PrimitiveComponent Object Reference") (OtherBodyIndex :type Integer) (bFromSweep :type Boolean) (SweepResult :type "HitResult Structure (by ref)"))
  (if (not (`self.locked`))
    (cast `/Game/Resources/Characters/Player/Blueprints/BP_PlayerCharacter` OtherActor)
    (`self.DoorOpen`)))

(event `DoorClose`
  (`PrimitiveComponent.SetCollisionResponseToChannel` (`self.Door`) "ECC_Camera" "ECR_Block")
  (`PrimitiveComponent.SetCollisionResponseToChannel` (`self.Door2`) "ECC_Camera" "ECR_Block")
  (goto _label :!via `Reverse`))

(event `self.Sphere.OnComponentEndOverlap`
  (params (OverlappedComponent :type "PrimitiveComponent Object Reference") (OtherActor :type "Actor Object Reference") (OtherComp :type "PrimitiveComponent Object Reference") (OtherBodyIndex :type Integer))
  (cast `/Game/Resources/Characters/Player/Blueprints/BP_PlayerCharacter` OtherActor)
  (`self.DoorClose`))

(fn `UserConstructionScript`
  (`parent.UserConstructionScript`))