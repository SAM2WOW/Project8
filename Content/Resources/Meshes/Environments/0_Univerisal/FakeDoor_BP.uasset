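; FakeDoor_BP is a two-panel sliding environment door that starts open and closes when the player approaches.
; BeginPlay plays a Timeline that slides both door meshes, and a sphere overlap by BP_PlayerCharacter reverses it unless Locked is set.
; Ending the overlap does nothing, so the door does not reopen by itself.
; A separate FakeSpawn event forwards an interact message to the referenced FakeSpawner.
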(event `CustomEvent`)

(event `DoorOpen`
  (bind (_direction _doorslide _doorslide2) (`Timeline|Timeline` :!label _label)
    (:`Update`
      (`SceneComponent.K2_SetRelativeLocation` (`self.Door`) _doorslide false false)
      (`SceneComponent.K2_SetRelativeLocation` (`self.Door2`) _doorslide2 false false))))

(event `self.ReceiveBeginPlay`
  (`self.DoorOpen`))

(event `DoorClose`
  (goto _label :!via `Reverse`))

(event `self.Sphere.OnComponentBeginOverlap`
  (params (OverlappedComponent :type "PrimitiveComponent Object Reference") (OtherActor :type "Actor Object Reference") (OtherComp :type "PrimitiveComponent Object Reference") (OtherBodyIndex :type Integer) (bFromSweep :type Boolean) (SweepResult :type "HitResult Structure (by ref)"))
  (if (not (`self.locked`))
    (if (== (`GameplayStatics.GetObjectClass` OtherActor) "/Game/Resources/Characters/Player/Blueprints/BP_PlayerCharacter.BP_PlayerCharacter_C")
      (`self.DoorClose`))))

(event `self.Sphere.OnComponentEndOverlap`
  (params (OverlappedComponent :type "PrimitiveComponent Object Reference") (OtherActor :type "Actor Object Reference") (OtherComp :type "PrimitiveComponent Object Reference") (OtherBodyIndex :type Integer)))

(event `FakeSpawn`
  (message `/Game/Resources/Characters/Interactables/interactable_interface.msg_interact` (`self.fakeSpawner`)))

(fn `UserConstructionScript`)