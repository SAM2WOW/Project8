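; Test actor Blueprint that drives a Cube component through a PhysicsControl component, with no gameplay purpose shown.
; BeginPlay creates a control on the cube with a set angular strength and a body modifier that removes its gravity.
; Tick reapplies the control's target transform, multipliers and the body's kinematic target by name, with no computed inputs shown.
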(event `self.ReceiveBeginPlay`
  (`PhysicsControlComponent.MakeControl` :`self` (`self.PhysicsControl`) :`ChildMeshComponent` (`self.Cube`) :`ControlData` (make `PhysicsControlData` 1.0 1.0 0.0 0.0 2.0))
  (`PhysicsControlComponent.MakeBodyModifier` (`self.PhysicsControl`) (`self.Cube`) "None" "Simulated" "QueryAndPhysics" 0.0 true))

(event `self.ReceiveTick`
  (params (DeltaSeconds :type "Float (single-precision)"))
  (bind _physicscontrol (`self.PhysicsControl`))
  (`PhysicsControlComponent.SetControlTargetPositionAndOrientation` :`self` _physicscontrol :`Name` "0")
  (`PhysicsControlComponent.SetControlMultipliers` _physicscontrol "0" (make `PhysicsControlMultipliers` (1.0 1.0 1.0)) true)
  (`PhysicsControlComponent.SetBodyModifierKinematicTarget` :`self` _physicscontrol :`Name` "Body_0"))

(fn `UserConstructionScript`)