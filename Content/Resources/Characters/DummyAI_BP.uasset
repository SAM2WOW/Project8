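; DummyAI_BP is a dummy enemy that turns to face the player and periodically swings its weapon.
; Tick snaps the actor's yaw toward player pawn 0 and interpolates the weapon's relative rotation toward a target rotation.
; A looping timer calls Attack, which steps that target through wind-up, strike and return poses using delays.
; Damage it receives is only printed on screen with the causer and amount.
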(event `self.ReceiveBeginPlay`
  (`KismetSystemLibrary.K2_SetTimer` null "Attack" 3.0 true))

(event `self.ReceiveTick`
  (params (DeltaSeconds :type "Float (single-precision)"))
  (bind _weapon (`self.Weapon`))
  (bind (_returnvalue_roll _returnvalue_pitch _returnvalue_yaw) (`KismetMathLibrary.BreakRotator` (`KismetMathLibrary.FindLookAtRotation` (`self.K2_GetActorLocation`) (`self.K2_GetActorLocation` (`GameplayStatics.GetPlayerPawn` 0)))))
  (`self.K2_SetActorRotation` (`KismetMathLibrary.MakeRotator` 0.0 0.0 _returnvalue_yaw))
  (`SceneComponent.K2_SetRelativeRotation` _weapon (`KismetMathLibrary.RInterpTo` (`SceneComponent.RelativeRotation` _weapon) (`self.TargetRotation`) (`GameplayStatics.GetWorldDeltaSeconds`) 40.0) false false))

(event `self.ReceiveAnyDamage`
  (params (Damage :type "Float (single-precision)") (DamageType :type "DamageType Object Reference") (InstigatedBy :type "Controller Object Reference") (DamageCauser :type "Actor Object Reference"))
  (`KismetSystemLibrary.PrintString` (`KismetTextLibrary.Conv_TextToString` (`|FormatText` (`KismetSystemLibrary.GetDisplayName` self) "{self} got HIT by {name}! -{damge}" (`KismetSystemLibrary.GetDisplayName` DamageCauser) Damage)) true true (struct :`R` 1.0 :`B` 0.181067 :`A` 1.0)))

(event `Attack`
  (set `self.TargetRotation` (struct :`Pitch` 30.0))
  (`KismetSystemLibrary.Delay` 0.5)
  (set `self.TargetRotation` (struct :`Pitch` -80.0))
  (`KismetSystemLibrary.Delay` 0.5)
  (set `self.TargetRotation` (struct)))

(fn `UserConstructionScript`)