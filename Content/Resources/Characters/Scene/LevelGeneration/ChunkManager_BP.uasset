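; ChunkManager is a procedural level generation Blueprint that streams map chunks in at BeginPlay.
; It loads the R_Start level instance, then loops to load random picks from the Battle list in Chunkdata as visible level instances.
; Every random chunk is placed at the world origin, with no offset or duplicate check, and prints a debug message.
; An older CreateInstance streaming method and a delayed loop remain unconnected.
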(event `self.ReceiveBeginPlay`
  (bind (_chunkdata_end _chunkdata_special _chunkdata_battle) (break `/Game/Resources/Characters/Scene/LevelGeneration/ChunkData_Struct` (`self.Chunkdata`)))
  (`|ExecutionSequence`
    (:`then_0`
      (`LevelStreamingDynamic.LoadLevelInstance` "/Game/Resources/Maps/ProceduralLevels/R_Start" (0.0 0.0 0.0) (struct) "" null))
    (:`then_1`
      (for _ (range 6)
        (bind (_boutsuccess _returnvalue) (`LevelStreamingDynamic.LoadLevelInstance` (`KismetStringLibrary.Concat_StrStr` "/Game/Resources/Maps/ProceduralLevels/" (`KismetStringLibrary.Conv_NameToString` (`KismetArrayLibrary.Array_Random` _chunkdata_battle))) (0.0 0.0 0.0) (struct) "" null))
        (set `LevelStreaming.bShouldBeLoaded` true _returnvalue)
        (set `LevelStreaming.bShouldBeVisible` true _returnvalue)
        (`KismetSystemLibrary.PrintString` "I am new level" true true (struct :`R` 0.680672 :`G` 1.0 :`A` 1.0))))))

(fn `UserConstructionScript`)