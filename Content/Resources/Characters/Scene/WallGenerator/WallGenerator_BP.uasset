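; Wall generator Blueprint that builds a room's perimeter walls from its Roomdata, leaving gaps where doors are.
; The construction script walks all four edges across a fixed range of vertical levels, adding offset wall segments to an instanced static mesh on a grid.
; CheckDoor suppresses a segment when a door shares its cell and faces along that wall's axis.
; Skipped segments on the X-running edges print a debug message; event graph logic is inactive.
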(fn `Check Door`
  (params (`Facing Y` :type Boolean) (X :type Integer) (Y :type Integer) (Z :type Integer))
  (returns (Empty :type Boolean))
  (for _array_element (`RoomData.Doors` (`self.Roomdata`))
    (if (and (== (break `IntVector` (break `DoorDef` _array_element)) X) (== (`.Y` (break `IntVector` (break `DoorDef` _array_element))) Y) (== (`.Z` (break `IntVector` (break `DoorDef` _array_element))) Z))
      (if (`KismetArrayLibrary.Array_Contains` (select `bool` `Facing Y` :`false` (`|MakeArray` "East" "West" :!type "EDoorDirection Enum") :`true` (`|MakeArray` "North" "South" :!type "EDoorDirection Enum")) (`.Direction` (break `DoorDef` _array_element)))
        (return false))))
  (return true))

(fn `UserConstructionScript`
  (bind _roomdata (`self.Roomdata`))
  (bind _size_x (break `IntVector` (`RoomData.Size` (`self.Roomdata`))))
  (bind (_size_x_2 _size_y) (break `IntVector` (`RoomData.Size` (`self.Roomdata`))))
  (bind (_size_x_3 _size_y_2) (break `IntVector` (`RoomData.Size` _roomdata)))
  (bind (_size_x_4 _size_y_3) (break `IntVector` (`RoomData.Size` (`self.Roomdata`))))
  (`/Engine/EditorBlueprintResources/StandardMacros.IsValid` _roomdata
    (:`Is Valid`
      (for _index (range _size_x_3)
        (for _index_2 (range 2)
          (for _index_3 (range -10 21)
            (bind _returnvalue (* _index_2 (- _size_y_2 1)))
            (bind _empty (`self.Check Door` false _index _returnvalue _index_3))
            (if _empty
              (`InstancedStaticMeshComponent.AddInstance` (`self.InstancedStaticMesh`) (`KismetMathLibrary.MakeTransform` (+ (`KismetMathLibrary.MakeVector` (`KismetMathLibrary.Conv_IntToDouble` (* _index 1000)) (- (`KismetMathLibrary.Conv_IntToDouble` (* _size_y_3 1000 _index_2)) (* _index_2 100.0)) (`KismetMathLibrary.Conv_IntToDouble` (* _index_3 400))) (`self.Offset`))) false)
              (else
                (`KismetSystemLibrary.PrintString` (`KismetTextLibrary.Conv_TextToString` (`|FormatText` "NOT EMPTY {x} {y} {z}" _index _returnvalue _index_3)) true true (struct :`R` 1.0 :`G` 0.755162 :`A` 1.0) 10.0))))))
      (for _index_4 (range _size_y)
        (for _index_5 (range -10 21)
          (for _index_6 (range 2)
            (bind _empty_2 (`self.Check Door` true (* _index_6 (- _size_x_2 1)) _index_4 _index_5))
            (if _empty_2
              (`InstancedStaticMeshComponent.AddInstance` (`self.InstancedStaticMesh`) (`KismetMathLibrary.MakeTransform` (+ (`KismetMathLibrary.MakeVector` (+ (`KismetMathLibrary.Conv_IntToDouble` (* _size_x 1000 _index_6)) (* (`KismetMathLibrary.Abs_Int` (- _index_6 1)) 100.0)) (`KismetMathLibrary.Conv_IntToDouble` (* _index_4 1000)) (`KismetMathLibrary.Conv_IntToDouble` (* _index_5 400))) (`self.Offset`)) (struct :`Yaw` 90.0)) false))))))))