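; LightSwitcher Blueprint that toggles a list of lights through a ChangeLightVisibility event, acting only when the state changes.
; Switching on reveals the lights one by one through a delayed loop, playing a Lightswitch sound at each.
; Switching off hides them all at once.
; The RoomVisibility hookups on BeginPlay and visibility change are disconnected, so nothing in this graph triggers the switch.
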(event `self.ReceiveBeginPlay`)

(event `self.RoomVisibility.OnRoomVisibilityChanged`
  (params (Actor :type "Actor Object Reference") (IsInVisibleRoom :type Boolean)))

(event `ChangeLightVisibility`
  (params (On :type Boolean))
  (if (!= On (`self.On`))
    (bind _output_get (set `self.On` On))
    (if _output_get
      (`KismetSystemLibrary.PrintString` "Light Activated")
      (bind _index (`/Game/Resources/Characters/Player/Blueprints/NewActorMacroLibrary.ForLoopWithDelay` 0 (`KismetArrayLibrary.Array_LastIndex` (`self.Lights`)) 0.5)
        (:`Loop Body`
          (bind _output (`|GetArrayItem` (`self.Lights`) _index))
          (`SceneComponent.SetVisibility` (`Light.LightComponent` _output) true false)
          (`FMODBlueprintStatics.PlayEventAtLocation` "/Game/FMOD/Events/Sounds/Scene/Lightswitch.Lightswitch" (`KismetMathLibrary.MakeTransform` (`self.K2_GetActorLocation` _output)))))
      (else
        (for _array_element (`self.Lights`)
          (`SceneComponent.SetVisibility` (`Light.LightComponent` _array_element) false false))))))

(fn `UserConstructionScript`)