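; Payload actor that travels along the spline of a referenced track actor.
; Each Tick advances a distance value by Speed times delta time, wraps it to the spline length so movement loops, and moves the actor to that world-space location and rotation.
; The move is swept, so blocking collision along the path can stop it.
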(event `self.ReceiveTick`
  (params (DeltaSeconds :type "Float (single-precision)"))
  (bind _spline (`/Game/Resources/Characters/Scene/Payload/PayloadTrack_BP.Spline` (`self.Track_ref`)))
  (bind _output_get (set `self.Position` (+ (* DeltaSeconds (`self.Speed`)) (`self.Position`))))
  (bind (_returnvalue_location _returnvalue_rotation) (`KismetMathLibrary.BreakTransform` (`SplineComponent.GetTransformAtDistanceAlongSpline` _spline (`KismetMathLibrary.FWrap` _output_get 0.0 (`SplineComponent.GetSplineLength` _spline)) "World" false)))
  (`self.K2_SetActorTransform` (`KismetMathLibrary.MakeTransform` _returnvalue_location _returnvalue_rotation) true))

(fn `UserConstructionScript`)