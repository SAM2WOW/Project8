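; DemoEnd_BP is an interactable actor that ends the demo when it receives MsgInteract.
; It saves through NewGameState_GS, pauses the game and shows a "DEMO ENDED" log popup announcing a return to the hub, set to unpause when closed.
; It then randomizes the game state's Seed, waits until the next tick and kills the player character.
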(event `/Game/Resources/Characters/Interactables/interactable_interface.msg_interact`
  (bind _asnew_game_state_gs (cast `/Game/Resources/Characters/Player/Blueprints/NewGameState_GS` (`GameplayStatics.GetGameState`)))
  (`/Game/Resources/Characters/Player/Blueprints/NewGameState_GS.Save Game` _asnew_game_state_gs false)
  (`GameplayStatics.SetGamePaused` true)
  (bind _returnvalue (`|CreateWidget` "/Game/Resources/Widgets/LogPopup_Widget.LogPopup_Widget_C" (`GameplayStatics.GetPlayerController` 0) (make `/Game/Resources/Characters/Interactables/MemoryLog_Struct` "DEMO ENDED" "Thank you for playing the demo. \n \nYou'll be teleported back to the hub now. \n \nYou can start your free exploration from the hub -- there are more levels!." null "NewEnumerator1") (0.0 0.0) true))
  (`UserWidget.AddToViewport` _returnvalue 0)
  (bind _asnew_game_state_gs_2 (cast `/Game/Resources/Characters/Player/Blueprints/NewGameState_GS` (`GameplayStatics.GetGameState`)))
  (set `/Game/Resources/Characters/Player/Blueprints/NewGameState_GS.Seed` (`KismetMathLibrary.RandomInteger` 999999) _asnew_game_state_gs_2)
  (`KismetSystemLibrary.DelayUntilNextTick`)
  (bind _asbp_player_character (cast `/Game/Resources/Characters/Player/Blueprints/BP_PlayerCharacter` (`GameplayStatics.GetPlayerPawn` 0)))
  (`/Game/Resources/Characters/Player/Blueprints/BP_PlayerCharacter.Kill` _asbp_player_character))

(fn `UserConstructionScript`)