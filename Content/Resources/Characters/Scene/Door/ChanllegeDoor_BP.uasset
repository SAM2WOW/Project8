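; Interactable challenge door that locks the player into a challenge, optionally charging Scraps for entry.
; Entry plays a camera cutscene with timeline-swung doors, reveals lock props, teleports the player to SwordTarget and can swap in a preset loadout after saving theirs.
; Unlock, triggered by message or a title-keyed GameState flag on BeginPlay, charges an emissive material, explodes the lock, restores any swapped loadout and reopens the door.
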(event `self.ReceiveBeginPlay`
  (bind _asnew_game_state_gs (cast `/Game/Resources/Characters/Player/Blueprints/NewGameState_GS` (`GameplayStatics.GetGameState`)))
  (bind (_exist _value) (`/Game/Resources/Characters/Player/Blueprints/NewGameState_GS.Get Flag` _asnew_game_state_gs (`KismetStringLibrary.Conv_StringToName` (`KismetTextLibrary.Conv_TextToString` (`self.Title`)))))
  (if _value
    ;[0 0.2031 1] Unlock if beaten
    (`self.Unlock`)))

(event `self.Interact`
  (bind _cost (`self.Cost`))
  (`parent.Interact`)
  (if (`self.locked`)
    (if (> (`self.Cost`) 0)
      (bind _asnew_game_state_gs (cast `/Game/Resources/Characters/Player/Blueprints/NewGameState_GS` (`GameplayStatics.GetGameState`)))
      (bind _scraps (`/Game/Resources/Characters/Player/Blueprints/NewGameState_GS.Scraps` _asnew_game_state_gs))
      (if (>= _scraps _cost)
        (set `/Game/Resources/Characters/Player/Blueprints/NewGameState_GS.Scraps` (- _scraps _cost) _asnew_game_state_gs)
        (bind _asnew_game_mode_gm (cast `/Game/Resources/Characters/Player/Blueprints/NewGameMode_GM` (`GameplayStatics.GetGameMode`)))
        (`/Game/Resources/Widgets/HUD_Widget.ScrapConsumed` (`/Game/Resources/Characters/Player/Blueprints/NewGameMode_GM.HUD_ref` _asnew_game_mode_gm))
        (`self.Start Chanllege` :!label _label)
        (else
          (`FMODBlueprintStatics.PlayEvent2D` "/Game/FMOD/Events/Sounds/UI/UI_Error.UI_Error")))
      (else
        (goto _label)))))

(event `Start Chanllege`
  (bind (_returnvalue_location _returnvalue_rotation) (`KismetMathLibrary.BreakTransform` (`SceneComponent.K2_GetComponentToWorld` (`self.SwordTarget`))))
  (`self.DoorOpen`)
  (set `self.ShowInteractUI?` false)
  (set `self.Interactable` false)
  (set `self.locked` true)
  ;[0.6406 0 1] Sequence
  (`self.DisableInput` (`GameplayStatics.GetPlayerPawn` 0) (`GameplayStatics.GetPlayerController` 0))
  (`PlayerController.SetViewTargetWithBlend` (`GameplayStatics.GetPlayerController` 0) self 0.5 "VTBlend_EaseInOut" 3.0 false)
  (bind _asnew_game_mode_gm (cast `/Game/Resources/Characters/Player/Blueprints/NewGameMode_GM` (`GameplayStatics.GetGameMode`)))
  (`Widget.SetRenderOpacity` (`/Game/Resources/Characters/Player/Blueprints/NewGameMode_GM.HUD_ref` _asnew_game_mode_gm) 0.0)
  (bind _asbp_player_character (cast `/Game/Resources/Characters/Player/Blueprints/BP_PlayerCharacter` (`GameplayStatics.GetPlayerCharacter` 0)))
  (`|PlayMontage` (`Character.Mesh` _asbp_player_character) "/Game/Resources/Animations/NewSelf/Soccer_Spin_Montage.Soccer_Spin_Montage"
    (:`then`
      (`KismetSystemLibrary.Delay` 0.8)
      (`self.DoorClose`)
      (`KismetSystemLibrary.Delay` 0.38)
      (`|ExecutionSequence`
        (:`then_0`
          (if (`self.ChangeLoadout`)
            ;[0 1 0.3672] Save and Apply Loadout
            (bind _asnew_game_state_gs (cast `/Game/Resources/Characters/Player/Blueprints/NewGameState_GS` (`GameplayStatics.GetGameState`)))
            (`/Game/Resources/Characters/Player/Blueprints/NewGameState_GS.Save Loadout` _asnew_game_state_gs 4)
            (`/Game/Resources/Characters/Player/Blueprints/NewGameState_GS.Apply Loadout` _asnew_game_state_gs (`self.Loadout`))))
        (:`then_1`
          (`SceneComponent.SetHiddenInGame` (`self.Lab_Platform`) false false)
          (`SceneComponent.SetHiddenInGame` (`self.Cylinder`) false false)
          (`SceneComponent.SetHiddenInGame` (`self.Lab_Platform1`) false false))))
    (:`OnCompleted`
      (bind _asbp_player_character_2 (cast `/Game/Resources/Characters/Player/Blueprints/BP_PlayerCharacter` (`GameplayStatics.GetPlayerCharacter` 0)))
      (`self.K2_SetActorTransform` _asbp_player_character_2 (`KismetMathLibrary.MakeTransform` _returnvalue_location _returnvalue_rotation) false false)
      ;[0 0.625 1] Rotate Camera Facing
      (`Controller.SetControlRotation` (`GameplayStatics.GetPlayerController` 0) (`SceneComponent.K2_GetComponentRotation` (`self.SpringArm`)))
      (`PlayerController.SetViewTargetWithBlend` (`GameplayStatics.GetPlayerController` 0) (`GameplayStatics.GetPlayerPawn` 0) 1.0 "VTBlend_EaseInOut" 3.0 false)
      (`self.EnableInput` (`GameplayStatics.GetPlayerPawn` 0) (`GameplayStatics.GetPlayerController` 0))
      (bind _asnew_game_mode_gm_2 (cast `/Game/Resources/Characters/Player/Blueprints/NewGameMode_GM` (`GameplayStatics.GetGameMode`)))
      (`Widget.SetRenderOpacity` (`/Game/Resources/Characters/Player/Blueprints/NewGameMode_GM.HUD_ref` _asnew_game_mode_gm_2) 1.0))))

(event `DoorOpen`
  ;[0 0.5312 1] Animation
  (`FMODBlueprintStatics.PlayEventAtLocation` "/Game/FMOD/Events/Sounds/Scene/Door_Open.Door_Open" (`self.GetTransform`))
  (`PrimitiveComponent.SetCollisionResponseToChannel` (`self.Door`) "ECC_Camera" "ECR_Ignore")
  (`PrimitiveComponent.SetCollisionResponseToChannel` (`self.Door2`) "ECC_Camera" "ECR_Ignore")
  (bind (_direction _progress) (`Timeline|Door Open` :!label _label_2)
    (:`Update`
      (bind _returnvalue (`KismetMathLibrary.Lerp` 0.0 -90.0 _progress))
      (`SceneComponent.K2_SetRelativeRotation` (`self.Door`) (`KismetMathLibrary.MakeRotator` 0.0 _returnvalue) false false)
      (`SceneComponent.K2_SetRelativeRotation` (`self.Door2`) (`KismetMathLibrary.MakeRotator` 180.0 (* _returnvalue -1.0) 180.0) false false))))

(event `self.Sphere.OnComponentBeginOverlap`
  (params (OverlappedComponent :type "PrimitiveComponent Object Reference") (OtherActor :type "Actor Object Reference") (OtherComp :type "PrimitiveComponent Object Reference") (OtherBodyIndex :type Integer) (bFromSweep :type Boolean) (SweepResult :type "HitResult Structure (by ref)")))

(event `DoorClose`
  ;[0 0.5312 1] Animation
  (`FMODBlueprintStatics.PlayEventAtLocation` "/Game/FMOD/Events/Sounds/Scene/Door_Close.Door_Close" (`self.GetTransform`))
  (`PrimitiveComponent.SetCollisionResponseToChannel` (`self.Door`) "ECC_Camera" "ECR_Block")
  (`PrimitiveComponent.SetCollisionResponseToChannel` (`self.Door2`) "ECC_Camera" "ECR_Block")
  (goto _label_2 :!via `Reverse`))

(event `self.Sphere.OnComponentEndOverlap`
  (params (OverlappedComponent :type "PrimitiveComponent Object Reference") (OtherActor :type "Actor Object Reference") (OtherComp :type "PrimitiveComponent Object Reference") (OtherBodyIndex :type Integer)))

(event `/Game/Resources/Characters/Interactables/interactable_interface.msg_unlock`
  (bind (_returnvalue_location _returnvalue_rotation) (`KismetMathLibrary.BreakTransform` (`SceneComponent.K2_GetComponentToWorld` (`self.Lab_Platform`))))
  (`SceneComponent.K2_SetRelativeRotation` (`self.SpringArm`) (struct :`Yaw` -270.0) false false :!label _label_3)
  (`self.DisableInput` (`GameplayStatics.GetPlayerPawn` 0) (`GameplayStatics.GetPlayerController` 0))
  (`PlayerController.SetViewTargetWithBlend` (`GameplayStatics.GetPlayerController` 0) self 0.5 "VTBlend_EaseInOut" 3.0 false)
  (bind _asnew_game_mode_gm (cast `/Game/Resources/Characters/Player/Blueprints/NewGameMode_GM` (`GameplayStatics.GetGameMode`)))
  (`Widget.SetRenderOpacity` (`/Game/Resources/Characters/Player/Blueprints/NewGameMode_GM.HUD_ref` _asnew_game_mode_gm) 0.0)
  ;[1 0 0.9375] Comment
  (`FMODBlueprintStatics.PlayEventAtLocation` "/Game/FMOD/Events/Sounds/Others/Explode_Charging.Explode_Charging" (`self.GetTransform`))
  (bind _returnvalue (`PrimitiveComponent.CreateDynamicMaterialInstance` (`self.Lab_Platform`) 0 "/Game/Resources/Materials/Common/Transform_Mat.Transform_Mat" "None"))
  (bind _output_get (set `self.Transform_Mat` _returnvalue))
  (`PrimitiveComponent.SetMaterial` (`self.Lab_Platform`) 0 _output_get)
  (`PrimitiveComponent.SetMaterial` (`self.Lab_Platform1`) 0 _output_get)
  (bind (_direction _newtrack_0) (`Timeline|Timeline` :!via `PlayFromStart`)
    (:`Update`
      (`MaterialInstanceDynamic.SetScalarParameterValue` (`self.Transform_Mat`) "Emmisive" (`KismetMathLibrary.Lerp` 0.0 10.0 _newtrack_0)))
    (:`Finished`
      ;;[0.3828 1 0] Play Camera Shakes
      (`GameplayStatics.PlayWorldCameraShake` "/Game/Resources/Characters/Player/Blueprints/Camera/Big_CameraShake.Big_CameraShake_C" (`self.K2_GetActorLocation`) 500.0 3000.0)
      (`|SpawnActorFromClass` "/Game/Resources/Characters/Destructables/DestructableExploded_BP_DoorLock.DestructableExploded_BP_DoorLock_C" (`KismetMathLibrary.MakeTransform` _returnvalue_location _returnvalue_rotation) "Undefined" "OverrideRootScale" null (`KismetMathLibrary.RandomIntegerInRange` 2 5) null)
      (`ActorComponent.K2_DestroyComponent` (`self.Lab_Platform`))
      (`ActorComponent.K2_DestroyComponent` (`self.Lab_Platform1`))
      (`ActorComponent.K2_DestroyComponent` (`self.Cylinder`))
      (`|ExecutionSequence`
        (:`then_0`
          (if (`self.ChangeLoadout`)
            ;[0 1 0.3672] Restore Loadout
            (bind _asnew_game_state_gs (cast `/Game/Resources/Characters/Player/Blueprints/NewGameState_GS` (`GameplayStatics.GetGameState`)))
            (`/Game/Resources/Characters/Player/Blueprints/NewGameState_GS.Load Loadout` _asnew_game_state_gs 4)))
        (:`then_2`
          (`KismetSystemLibrary.Delay` 0.3)
          (`self.DoorOpen`)
          (`KismetSystemLibrary.Delay` 0.3)
          ;[0 0.625 1] Rotate Camera Facing
          (`Controller.SetControlRotation` (`GameplayStatics.GetPlayerController` 0) (`SceneComponent.K2_GetComponentRotation` (`self.SpringArm`)))
          (`PlayerController.SetViewTargetWithBlend` (`GameplayStatics.GetPlayerController` 0) (`GameplayStatics.GetPlayerPawn` 0) 1.0 "VTBlend_EaseInOut" 3.0 false)
          (`self.EnableInput` (`GameplayStatics.GetPlayerPawn` 0) (`GameplayStatics.GetPlayerController` 0))
          (bind _asnew_game_mode_gm_2 (cast `/Game/Resources/Characters/Player/Blueprints/NewGameMode_GM` (`GameplayStatics.GetGameMode`)))
          (`Widget.SetRenderOpacity` (`/Game/Resources/Characters/Player/Blueprints/NewGameMode_GM.HUD_ref` _asnew_game_mode_gm_2) 1.0))))))

(event `Unlock`
  (goto _label_3))

(fn `UserConstructionScript`
  (`parent.UserConstructionScript`))