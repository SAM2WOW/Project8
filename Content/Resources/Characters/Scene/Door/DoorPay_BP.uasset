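; DoorPay_BP is a paid double door that stays locked until the player spends Scraps, shown in the prompt as memories.
; Interact deducts Cost from the GameState, notifies the HUD, unlocks, disables interaction and opens it, or plays an error sound if funds are short.
; Once unlocked, sphere overlap drives a timeline that swings both leaves open or reverses them closed, toggling their Camera collision response.
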(event `self.ReceiveBeginPlay`
  (set `self.Button` (`|FormatText` "INSERT {amount} MEMORIES TO UNLOCK" (`self.Cost`))))

(event `self.Interact`
  (bind _cost (`self.Cost`))
  (`parent.Interact`)
  (if (`self.locked`)
    (bind _asnew_game_state_gs (cast `/Game/Resources/Characters/Player/Blueprints/NewGameState_GS` (`GameplayStatics.GetGameState`)))
    (bind _scraps (`/Game/Resources/Characters/Player/Blueprints/NewGameState_GS.Scraps` _asnew_game_state_gs))
    (if (>= _scraps _cost)
      (set `/Game/Resources/Characters/Player/Blueprints/NewGameState_GS.Scraps` (- _scraps _cost) _asnew_game_state_gs)
      (bind _asnew_game_mode_gm (cast `/Game/Resources/Characters/Player/Blueprints/NewGameMode_GM` (`GameplayStatics.GetGameMode`)))
      (`/Game/Resources/Widgets/HUD_Widget.ScrapConsumed` (`/Game/Resources/Characters/Player/Blueprints/NewGameMode_GM.HUD_ref` _asnew_game_mode_gm))
      (set `self.locked` false)
      (`self.DoorOpen`)
      (set `self.CanInteract?` false)
      (set `self.Interactable` false)
      (else
        (`FMODBlueprintStatics.PlayEvent2D` "/Game/FMOD/Events/Sounds/UI/UI_Error.UI_Error")))))

(event `DoorOpen`
  (`PrimitiveComponent.SetCollisionResponseToChannel` (`self.Door`) "ECC_Camera" "ECR_Ignore")
  (`PrimitiveComponent.SetCollisionResponseToChannel` (`self.Door2`) "ECC_Camera" "ECR_Ignore")
  (bind (_direction _progress) (`Timeline|Door Open` :!label _label)
    (:`Update`
      (bind _returnvalue (`KismetMathLibrary.Lerp` 0.0 -90.0 _progress))
      (`SceneComponent.K2_SetRelativeRotation` (`self.Door`) (`KismetMathLibrary.MakeRotator` 0.0 _returnvalue) false false)
      (`SceneComponent.K2_SetRelativeRotation` (`self.Door2`) (`KismetMathLibrary.MakeRotator` 180.0 (* _returnvalue -1.0) 180.0) false false))))

(event `self.Sphere.OnComponentBeginOverlap`
  (params (OverlappedComponent :type "PrimitiveComponent Object Reference") (OtherActor :type "Actor Object Reference") (OtherComp :type "PrimitiveComponent Object Reference") (OtherBodyIndex :type Integer) (bFromSweep :type Boolean) (SweepResult :type "HitResult Structure (by ref)"))
  (if (not (`self.locked`))
    (cast `/Game/Resources/Characters/Player/Blueprints/BP_PlayerCharacter` OtherActor)
    (`self.DoorOpen`)))

(event `DoorClose`
  (`PrimitiveComponent.SetCollisionResponseToChannel` (`self.Door`) "ECC_Camera" "ECR_Block")
  (`PrimitiveComponent.SetCollisionResponseToChannel` (`self.Door2`) "ECC_Camera" "ECR_Block")
  (goto _label :!via `Reverse`))

(event `self.Sphere.OnComponentEndOverlap`
  (params (OverlappedComponent :type "PrimitiveComponent Object Reference") (OtherActor :type "Actor Object Reference") (OtherComp :type "PrimitiveComponent Object Reference") (OtherBodyIndex :type Integer))
  (cast `/Game/Resources/Characters/Player/Blueprints/BP_PlayerCharacter` OtherActor)
  (`self.DoorClose`))

(fn `UserConstructionScript`
  (`parent.UserConstructionScript`))