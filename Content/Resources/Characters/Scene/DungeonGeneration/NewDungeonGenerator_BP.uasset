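; Procedural dungeon generator that builds each chunk from the data table row for the GameState's current chunk.
; Seeded weighted rolls, shifted by current room type and battle/bridge counters, pick rooms until all specials are placed, then the end room.
; Generation caps near 32 rooms, rejecting layouts without an end; hub mode targets a hub end room instead.
; It also selects special or normal doors and teleports the player to PlayerStart on auto-start without start override.
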(event `self.ReceiveBeginPlay`
  (if (`self.Auto Start`)
    (`|ExecutionSequence` :!label _label
      (:`then_0`
        (bind _asnew_game_mode_gm (cast `/Game/Resources/Characters/Player/Blueprints/NewGameMode_GM` (`GameplayStatics.GetGameMode`)))
        (set `/Game/Resources/Characters/Player/Blueprints/NewGameMode_GM.LevelGen_ref` self _asnew_game_mode_gm))
      (:`then_1`
        (`self.Generate`)))))

(event `/Game/Resources/Characters/Interactables/interactable_interface.msg_interact`
  (goto _label))

(event `self.OnPostGeneration_BP`
  ;[0 0.1562 1] Teleport Player
  (if (and (not (`self.overwrite start`)) (`self.Auto Start`))
    (bind _outactors (`GameplayStatics.GetAllActorsOfClass` "/Script/Engine.PlayerStart"))
    (if (`KismetArrayLibrary.Array_IsNotEmpty` _outactors)
      (bind _asbp_player_character (cast `/Game/Resources/Characters/Player/Blueprints/BP_PlayerCharacter` (`GameplayStatics.GetPlayerPawn` 0)))
      (`self.K2_SetActorLocation` _asbp_player_character (`self.K2_GetActorLocation` (`|GetArrayItem` _outactors)) false true))))

(event `self.OnPreGeneration_BP`
  (set `self.RandomStream` (`KismetMathLibrary.MakeRandomStream` (`self.GetSeed`)))
  (set `self.Stepcount` 0)
  (bind _asnew_game_state_gs (cast `/Game/Resources/Characters/Player/Blueprints/NewGameState_GS` (`GameplayStatics.GetGameState`)))
  (bind _returnvalue (`|GetDataTableRow` "/Game/Resources/Characters/Scene/DungeonGeneration/ChunkData_DT.ChunkData_DT" (`KismetStringLibrary.Conv_StringToName` (`KismetStringLibrary.Conv_IntToString` (`/Game/Resources/Characters/Player/Blueprints/NewGameState_GS.CurrentChunk` _asnew_game_state_gs))))
    (:`then`
      (bind (_start _end _battle _special _secrets) (break `/Game/Resources/Characters/Scene/DungeonGeneration/ChunkData_Struct` _returnvalue))
      (set `self.CurrentChunkData` (select `bool` (`self.overwrite start`) :`false` _returnvalue :`true` (make `/Game/Resources/Characters/Scene/DungeonGeneration/ChunkData_Struct` (`self.StartRoom`) _end _battle _special _secrets)))
      (bind _output_get (set `self.SpecialRoomsLeft` _special))
      (`KismetSystemLibrary.PrintString` (`KismetStringLibrary.Conv_IntToString` (`KismetArrayLibrary.Array_Length` _output_get))))))

(event `self.OnRoomAdded_BP`
  (params (NewRoom :type "RoomData Object Reference"))
  (if (`self.SpawnHub`)
    (set `self.SpawnHubStepSucess` true)
    (else
      (`KismetArrayLibrary.Array_Add` (`self.AllSpawnedRooms`) NewRoom)
      (bind _asnew_room_data (cast `/Game/Resources/Characters/Scene/DungeonGeneration/NewRoomData` NewRoom))
      (bind _type (`/Game/Resources/Characters/Scene/DungeonGeneration/NewRoomData.Type` _asnew_room_data))
      (`KismetSystemLibrary.PrintString` (`KismetTextLibrary.Conv_TextToString` (`|FormatText` "WOW WE ACTUALLY {NAME}" (`|GetEnumeratorNameAsString` _type))))
      (switch `/Game/Resources/Characters/Scene/DungeonGeneration/Roomtype_Enum` _type
        (:`NewEnumerator0`
          (`/Engine/EditorBlueprintResources/StandardMacros.IncrementInt` (`self.Stepcount`)
            (:`  `
              (set `self.Bridgecount` 0))))
        (:`NewEnumerator1`
          (set `self.Stepcount` 0)
          (set `self.Bridgecount` 0)
          (bind _returnvalue (`KismetArrayLibrary.Array_RemoveItem` (`self.SpecialRoomsLeft`) _asnew_room_data))
          (if _returnvalue
            (`KismetSystemLibrary.PrintString` "OK I TOOK IT OUT")))
        (:`NewEnumerator3`
          (`/Engine/EditorBlueprintResources/StandardMacros.IncrementInt` (`self.Bridgecount`)))))))

(fn `CalculateSpawnrate`
  (params (CurrentRoom :type "RoomData Object Reference"))
  (returns (`Final Spawnrate` :type "Map of /Game/Resources/Characters/Scene/DungeonGeneration/Roomtype_Enum Enum to Float (double-precision)"))
  (locals (Spawnrate :type "Map of /Game/Resources/Characters/Scene/DungeonGeneration/Roomtype_Enum Enum to Float (double-precision)"))
  (`BlueprintMapLibrary.Map_Clear` (`local.Spawnrate`))
  (`/Engine/EditorBlueprintResources/StandardMacros.IsValid` CurrentRoom
    (:`Is Valid`
      (bind _asnew_room_data (cast `/Game/Resources/Characters/Scene/DungeonGeneration/NewRoomData` CurrentRoom))
      (switch `/Game/Resources/Characters/Scene/DungeonGeneration/Roomtype_Enum` (`/Game/Resources/Characters/Scene/DungeonGeneration/NewRoomData.Type` _asnew_room_data)
        (:`NewEnumerator0`
          (`BlueprintMapLibrary.Map_Add` (`local.Spawnrate`) "NewEnumerator0" (`KismetMathLibrary.MapRangeClamped` (`KismetMathLibrary.Conv_IntToDouble` (`self.Stepcount`)) 0.0 3.0 100.0))
          (`BlueprintMapLibrary.Map_Add` (`local.Spawnrate`) "NewEnumerator1" (`KismetMathLibrary.MapRangeClamped` (`KismetMathLibrary.Conv_IntToDouble` (`self.Stepcount`)) 0.0 3.0 0.0 100.0))
          (`BlueprintMapLibrary.Map_Add` (`local.Spawnrate`) "NewEnumerator3" 100.0))
        (:`NewEnumerator1`
          (`BlueprintMapLibrary.Map_Add` (`local.Spawnrate`) "NewEnumerator0" 100.0)
          (`BlueprintMapLibrary.Map_Add` (`local.Spawnrate`) "NewEnumerator1" 1.0)
          (`BlueprintMapLibrary.Map_Add` (`local.Spawnrate`) "NewEnumerator3" 80.0))
        (:`NewEnumerator3`
          (`BlueprintMapLibrary.Map_Add` (`local.Spawnrate`) "NewEnumerator0" 50.0)
          (`BlueprintMapLibrary.Map_Add` (`local.Spawnrate`) "NewEnumerator1" 50.0)
          (`BlueprintMapLibrary.Map_Add` (`local.Spawnrate`) "NewEnumerator3" (`KismetMathLibrary.MapRangeClamped` (`KismetMathLibrary.Conv_IntToDouble` (`self.Bridgecount`)) 0.0 5.0 25.0))))
      (`KismetSystemLibrary.PrintString` "Spawnrate Created")
      (return (`local.Spawnrate`)))
    (:`Is Not Valid`
      ;[1 0 0.7031] Default Spawn Battle
      (`KismetSystemLibrary.PrintString` "THIS SHOULD NEVER HAPPEN +++" true true (struct :`R` 1.0 :`B` 0.617487 :`A` 1.0))
      (return (`|MakeMap` "NewEnumerator0" 100.0 :!type "/Game/Resources/Characters/Scene/DungeonGeneration/Roomtype_Enum Enum")))))

(fn `ChooseDoor`
  (params (CurrentRoom :type "RoomData Object Reference") (NextRoom :type "RoomData Object Reference"))
  (returns (ReturnValue :type "Door Class Reference"))
  (bind (_start _end _battle _special) (break `/Game/Resources/Characters/Scene/DungeonGeneration/ChunkData_Struct` (`self.CurrentChunkData`)))
  (if (and (`KismetSystemLibrary.IsValid` CurrentRoom) (`KismetSystemLibrary.IsValid` NextRoom))
    (if (or (`KismetArrayLibrary.Array_Contains` _special CurrentRoom) (`KismetArrayLibrary.Array_Contains` _special NextRoom))
      (return "/Game/Resources/Characters/Scene/DungeonGeneration/SpecialTriggerDoor_BP_2.SpecialTriggerDoor_BP_2_C")
      (else
        ;[0 1 0.8828] TODO: If it's bridge both then don't spoawn
        (return "/Game/Resources/Characters/Scene/DungeonGeneration/NewTriggerDoor_BP.NewTriggerDoor_BP_C")))
    (else
      (return null))))

(fn `ChooseFirstRoomData`
  (returns (ReturnValue :type "RoomData Object Reference"))
  (return (`.Start_2_790A22D74A8F20F48CC21491D9CA8F08` (break `/Game/Resources/Characters/Scene/DungeonGeneration/ChunkData_Struct` (`self.CurrentChunkData`)))))

(fn `ChooseNextRoomData`
  (params (CurrentRoom :type "RoomData Object Reference"))
  (returns (ReturnValue :type "RoomData Object Reference"))
  (bind (_currentchunkdata_start _currentchunkdata_end) (break `/Game/Resources/Characters/Scene/DungeonGeneration/ChunkData_Struct` (`self.CurrentChunkData`)))
  (bind (_currentchunkdata_start_2 _currentchunkdata_end_2 _currentchunkdata_battle) (break `/Game/Resources/Characters/Scene/DungeonGeneration/ChunkData_Struct` (`self.CurrentChunkData`)))
  (bind (_currentchunkdata_start_3 _currentchunkdata_end_3) (break `/Game/Resources/Characters/Scene/DungeonGeneration/ChunkData_Struct` (`self.CurrentChunkData`)))
  (if (`self.HubSpawner`)
    (return "/Game/Resources/Maps/ProceduralLevels/Hub/R_HubEnd_Data1.R_HubEnd_Data1")
    (else
      ;[0 1 0.3672] Spawn an ExitRoom if we have reached the minimum number of room and we don't have an ExitRoom yet
      (if (and (<= (`KismetArrayLibrary.Array_Length` (`self.SpecialRoomsLeft`)) 0) (not (`self.HasAlreadyRoomData` _currentchunkdata_end)))
        (`KismetSystemLibrary.PrintString` "FIINISHED" true true (struct :`R` 0.053319 :`B` 1.0 :`A` 1.0))
        (return _currentchunkdata_end_3)
        (else
          (bind _final_spawnrate (`self.CalculateSpawnrate` CurrentRoom))
          (bind _array_element (`self.SelectRoom` _final_spawnrate))
          (switch `/Game/Resources/Characters/Scene/DungeonGeneration/Roomtype_Enum` _array_element
            (:`NewEnumerator0`
              ;[1 0 0.3984] Battle
              (bind _returnvalue (`self.GetRandomRoomData` _currentchunkdata_battle))
              (`KismetSystemLibrary.PrintString` "Add Battle" true true (struct :`R` 1.0 :`B` 0.036154 :`A` 1.0))
              (return _returnvalue))
            (:`NewEnumerator1`
              ;[0 0.7187 1] Special
              (bind _returnvalue_2 (`self.GetRandomRoomData` (`self.SpecialRoomsLeft`)))
              (`KismetSystemLibrary.PrintString` "Add Speical" true true (struct :`R` 1.0 :`G` 0.75565 :`A` 1.0))
              (return _returnvalue_2))
            (:`NewEnumerator2`
              (return "/Game/Resources/Maps/ProceduralLevels/R_Rec_Data.R_Rec_Data"))
            (:`NewEnumerator3`
              ;[1 0 0.09375] Bridge
              (bind _returnvalue_3 (`self.GetRandomRoomData` (`|MakeArray` "/Game/Resources/Maps/ProceduralLevels/R_Bridge_Data.R_Bridge_Data" "/Game/Resources/Maps/ProceduralLevels/R_Bridge2_Data.R_Bridge2_Data" :!type "RoomData Object Reference")))
              (`KismetSystemLibrary.PrintString` "Add BRIDGE" true true (struct :`R` 0.118126 :`G` 0.697917 :`A` 1.0))
              (return _returnvalue_3))))))))

(fn `ContinueToAddRoom`
  (returns (ReturnValue :type Boolean))
  (bind (_currentchunkdata_start _currentchunkdata_end) (break `/Game/Resources/Characters/Scene/DungeonGeneration/ChunkData_Struct` (`self.CurrentChunkData`)))
  (bind _returnvalue (not (`self.HasAlreadyRoomData` _currentchunkdata_end)))
  (if (`self.HubSpawner`)
    (return (not (`self.HasAlreadyRoomData` "/Game/Resources/Maps/ProceduralLevels/Hub/R_HubEnd_Data1.R_HubEnd_Data1")))
    (else
      (`KismetSystemLibrary.PrintString` (`KismetStringLibrary.Conv_BoolToString` _returnvalue) true true (struct :`R` 1.0 :`B` 0.899543 :`A` 1.0))
      (`KismetSystemLibrary.PrintString` "Conitnue -------------------" true true (struct :`R` 0.753803 :`G` 1.0 :`A` 1.0))
      (return (and _returnvalue (< (`self.GetNbRoom`) 32))))))

(fn `IsValidDungeon`
  (returns (ReturnValue :type Boolean))
  (bind (_currentchunkdata_start _currentchunkdata_end) (break `/Game/Resources/Characters/Scene/DungeonGeneration/ChunkData_Struct` (`self.CurrentChunkData`)))
  (if (or (`self.HubSpawner`) (`self.HasAlreadyRoomData` _currentchunkdata_end))
    (return true)
    (else
      (`KismetSystemLibrary.PrintString` "Bad Dungeon Restart!" true true (struct :`G` 1.0 :`B` 0.265653 :`A` 1.0))
      (`KismetSystemLibrary.PrintString` (`KismetStringLibrary.Conv_IntToString` (`self.GetSeed`)))
      (set `self.Stepcount` 0)
      (set `self.SpecialRoomsLeft` (`.Special_11_7F0DB8404D6F520AEFA614A33DD56062` (break `/Game/Resources/Characters/Scene/DungeonGeneration/ChunkData_Struct` (`self.CurrentChunkData`))))
      (return false))))

(fn `SelectRoom`
  (params (Rate :type "Map of /Game/Resources/Characters/Scene/DungeonGeneration/Roomtype_Enum Enum to Float (double-precision)"))
  (returns (`Array Element` :type "/Game/Resources/Characters/Scene/DungeonGeneration/Roomtype_Enum Enum"))
  (locals (TotalWeight :type "Float (double-precision)") (SelectedWeight :type "Float (double-precision)") (CurrentWeight :type "Float (double-precision)"))
  (`|ExecutionSequence`
    (:`then_0`
      (bind _keys (`BlueprintMapLibrary.Map_Keys` Rate))
      ;[1 0 0.1406] Get the total amount of weight you can have
      (for _array_element _keys
        (set `local.TotalWeight` (+ (`local.TotalWeight`) (`BlueprintMapLibrary.Map_Find` Rate _array_element)))))
    (:`then_1`
      ;[0 0.2969 1] Create a random range based on the max value
      (bind _output_get (set `local.SelectedWeight` (`KismetMathLibrary.RandomFloatInRangeFromStream` 0.0 (`local.TotalWeight`) (`self.RandomStream`))))
      (`KismetSystemLibrary.PrintString` (`KismetStringLibrary.Conv_DoubleToString` _output_get) true true (struct :`R` 0.893402 :`G` 1.0 :`A` 1.0)))
    (:`then_2`
      ;[1 0 0.7031] Calculate which item to drop
      (bind _keys_2 (`BlueprintMapLibrary.Map_Keys` Rate))
      (for _array_element_2 _keys_2
        (bind _output_get_2 (set `local.CurrentWeight` (+ (`BlueprintMapLibrary.Map_Find` Rate _array_element_2) (`local.CurrentWeight`))))
        (if (<= (`local.SelectedWeight`) _output_get_2)
          (`KismetSystemLibrary.PrintString` (`|GetEnumeratorNameAsString` _array_element_2) true true (struct :`R` 0.951201 :`G` 1.0 :`A` 1.0))
          (return _array_element_2)))
      (`KismetSystemLibrary.PrintString` "WTF MAN")
      (return "NewEnumerator0"))))

(fn `UserConstructionScript`)