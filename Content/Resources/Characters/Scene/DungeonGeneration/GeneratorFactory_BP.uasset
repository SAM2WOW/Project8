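; GeneratorFactory_BP is a placed factory actor that spawns a NewDungeonGenerator_BP at its own transform on BeginPlay.
; It passes its configured settings to the new generator, covering auto start, start room, hub spawner, start overwrite, player teleport and starter generator flag.
; It saves the spawned generator and forwards MsgInteract calls to it, acting as a proxy for interaction.
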(event `self.ReceiveBeginPlay`
  (bind _returnvalue (`|SpawnActorFromClass` "/Game/Resources/Characters/Scene/DungeonGeneration/NewDungeonGenerator_BP.NewDungeonGenerator_BP_C" (`self.GetTransform`) "Undefined" "OverrideRootScale" null (`self.Auto Start`) (`self.Start Room`) (`self.Hub Spawner`) (`self.Overwrite Start`) (`self.Teleport Player`) (`self.Starter Generator`) null))
  (set `self.SavedGenerator` _returnvalue))

(event `/Game/Resources/Characters/Interactables/interactable_interface.msg_interact`
  (`/Game/Resources/Characters/Interactables/interactable_interface.msg_interact` (`self.SavedGenerator`)))

(fn `UserConstructionScript`)