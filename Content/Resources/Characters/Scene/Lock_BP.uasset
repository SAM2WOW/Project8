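; Level lock actor that keeps its target objects locked until a set of enemies is destroyed.
; On BeginPlay it locks all LockedTargets via lock messages and binds to each ControlTarget's destroyed event, first gathering enemies from SpawnerTargets a tick later if any are set.
; Destroyed enemies leave the list; when it empties, a one-time three-second delay precedes unlocking.
; The death-dispatcher binding is disconnected and its handler is empty.
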(event `self.ReceiveBeginPlay`
  (bind _spawnertargets (`self.SpawnerTargets`))
  (if (`KismetArrayLibrary.Array_IsEmpty` _spawnertargets)
    (`self.Set All Lock State` true :!label _label)
    (for _array_element (`self.ControlTargets`)
      (add `self.OnDestroyed` _array_element (delegate `On Destroyed`)))
    (else
      (`KismetSystemLibrary.DelayUntilNextTick`)
      (for _array_element_2 _spawnertargets
        (`KismetArrayLibrary.Array_Add` (`self.ControlTargets`) (`/Game/Resources/Characters/Enemy/Spawner/SpawnerCable_BP.Enemy` _array_element_2))
        (goto _label)))))

(event `On Death`
  (params (Ref :type "/Game/Resources/Characters/Enemy/EnemyBase_BP Object Reference")))

(event `On Destroyed` :!signature `self.OnDestroyed`
  (params (DestroyedActor :type "Actor Object Reference"))
  (bind _controltargets (`self.ControlTargets`))
  (bind _asenemy_base_bp (cast `/Game/Resources/Characters/Enemy/EnemyBase_BP` DestroyedActor))
  (bind _returnvalue (`KismetArrayLibrary.Array_Find` _controltargets _asenemy_base_bp))
  (if (!= _returnvalue -1)
    (`KismetArrayLibrary.Array_Remove` _controltargets _returnvalue)
    (if (`KismetArrayLibrary.Array_IsEmpty` (`self.ControlTargets`))
      (`/Engine/EditorBlueprintResources/StandardMacros.DoOnce` false
        (:`Completed`
          (`KismetSystemLibrary.Delay` 3.0)
          (`self.Set All Lock State` false))))))

(event `Set All Lock State`
  (params (Lock :type Boolean))
  (for _array_element (`self.LockedTargets`)
    (if Lock
      (message `/Game/Resources/Characters/Interactables/interactable_interface.msg_lock` _array_element)
      (else
        (message `/Game/Resources/Characters/Interactables/interactable_interface.msg_unlock` _array_element)))))

(fn `UserConstructionScript`)