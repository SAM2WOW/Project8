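; Jelly cutting arm weapon that spins up on a light attack and carries attachable modules locked onto the player pawn.
; Tick ramps the pivot's yaw speed while attacking, then slows and reverses it back toward rest.
; Physics Control switches the arm's end mesh from simulated to kinematic during attacks, following an arrow target.
; Module projectiles start shortly after the spin and stop on release or after a retriggerable timeout.
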(event `self.ReceiveBeginPlay`
  ;[0 1 0.2734] Create a control
  (bind _returnvalue (`PhysicsControlComponent.MakeControl` :`self` (`self.PhysicsControl`) :`ChildMeshComponent` (`self.end`) :`ChildBoneName` "Bone_007_end" :`ControlData` (make `PhysicsControlData` 1.0)))
  (set `self.MainControlName` _returnvalue)
  (`PhysicsControlComponent.MakeNamedBodyModifier` (`self.PhysicsControl`) "Movement" (`self.end`) "None" "Simulated" "QueryAndPhysics" 0.0 true))

(event `self.ReceiveTick`
  (params (DeltaSeconds :type "Float (single-precision)"))
  (bind _pivot (`self.pivot`))
  (bind _arrow (`self.Arrow`))
  (bind _returnvalue (`SceneComponent.K2_GetComponentLocation` _arrow))
  (bind _returnvalue_2 (`SceneComponent.K2_GetComponentRotation` _arrow))
  (bind (_relativerotation_roll _relativerotation_pitch _relativerotation_yaw) (`KismetMathLibrary.BreakRotator` (`SceneComponent.RelativeRotation` _pivot)))
  (`PhysicsControlComponent.SetControlTargetPositionAndOrientation` (`self.PhysicsControl`) (`self.MainControlName`) _returnvalue _returnvalue_2 0.0 false false)
  (`PhysicsControlComponent.SetBodyModifierKinematicTarget` (`self.PhysicsControl`) "Movement" _returnvalue _returnvalue_2 false)
  (bind _output_get (set `self.rotateSpeed` (`KismetMathLibrary.FClamp` (+ (`self.rotateSpeed`) (`KismetMathLibrary.SelectFloat` 1.0 -1.0 (`self.rotating`))) (`KismetMathLibrary.SelectFloat` -4.0 0.0 (>= (`KismetMathLibrary.Abs` _relativerotation_yaw) 4.0)) 24.0)))
  (`SceneComponent.K2_AddRelativeRotation` _pivot (`KismetMathLibrary.MakeRotator` 0.0 0.0 _output_get) false false)
  (if (<= _output_get 5.0)
    _))

(event `self.AttachModule`
  (params (Module :type "/Game/Resources/Characters/Modules/ModuleBase_BP Object Reference"))
  (bind _attachpoint (`self.AttachPoint`))
  ;[0.05469 0 1] Modules
  (`self.K2_SetActorRelativeRotation` Module (struct :`Pitch` 90.0 :`Roll` 90.0) false false)
  (`/Game/Resources/Characters/Modules/ModuleManager_BPC.Attach Module` (`self.ModuleManager_BPC`) Module (`SceneComponent.K2_GetComponentLocation` _attachpoint) _attachpoint)
  (`/Game/Resources/Characters/Modules/ModuleManager_BPC.Update Locked Target` (`self.ModuleManager_BPC`) (`GameplayStatics.GetPlayerPawn` 0)))

(event `self.DetachModule`
  (params (Module :type "/Game/Resources/Characters/Modules/ModuleBase_BP Object Reference"))
  (bind _returnvalue (`KismetArrayLibrary.Array_Find` (`/Game/Resources/Characters/Modules/ModuleManager_BPC.Modules` (`self.ModuleManager_BPC`)) Module))
  ;[0.05469 0 1] Modules
  (if (!= _returnvalue -1)
    (bind _output_get (`/Game/Resources/Characters/Modules/ModuleManager_BPC.Remove Module` (`self.ModuleManager_BPC`) _returnvalue))
    (`self.K2_DestroyActor` _output_get)))

(event `Fire`
  (set `self.rotating` true)
  (`PhysicsControlComponent.SetBodyModifierMovementType` (`self.PhysicsControl`) "Movement" "Kinematic")
  (`KismetSystemLibrary.RetriggerableDelay` 1.5)
  (set `self.rotating` false)
  (`PhysicsControlComponent.SetBodyModifierMovementType` (`self.PhysicsControl`) "Movement" "Simulated")
  (`/Game/Resources/Characters/Modules/ModuleManager_BPC.LightProjectileStop` (`self.ModuleManager_BPC`)))

(event `self.LightStart`
  (`self.Fire`)
  (`KismetSystemLibrary.Delay` 0.3)
  (`/Game/Resources/Characters/Modules/ModuleManager_BPC.LightProjectileStart` (`self.ModuleManager_BPC`)))

(event `self.LightStop`
  (`/Game/Resources/Characters/Modules/ModuleManager_BPC.LightProjectileStop` (`self.ModuleManager_BPC`))
  (set `self.rotating` false)
  (`PhysicsControlComponent.SetBodyModifierMovementType` (`self.PhysicsControl`) "Movement" "Simulated"))

(fn `UserConstructionScript`
  (`parent.UserConstructionScript`))