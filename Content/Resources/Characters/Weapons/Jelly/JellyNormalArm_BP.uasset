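; Jelly character weapon arm that carries attachable modules and forwards deploy, light projectile and charged heavy attacks to ModuleManagerBPC.
; Tick feeds one of two arrow transforms, chosen by the Rotating flag, to Physics Control targets on the End mesh.
; Light fire switches that body from simulated to kinematic until stopped.
; Heavy charging shows a Niagara effect, and attack preparation sweeps custom depth along the segments.
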(event `self.ReceiveBeginPlay`
  (`parent.ReceiveBeginPlay`)
  ;[0 1 0.2734] Create a control
  (bind _returnvalue (`PhysicsControlComponent.MakeControl` :`self` (`self.PhysicsControl`) :`ChildMeshComponent` (`self.end`) :`ChildBoneName` "Bone_007_end" :`ControlData` (make `PhysicsControlData` 5.0 1.0 0.0 0.0 5.0)))
  (set `self.MainControlName` _returnvalue)
  (`PhysicsControlComponent.MakeNamedBodyModifier` (`self.PhysicsControl`) "Movement" (`self.end`) "None" "Simulated" "QueryAndPhysics" 0.0 true))

(event `self.ReceiveTick`
  (params (DeltaSeconds :type "Float (single-precision)"))
  (bind _returnvalue (select `bool` (`self.Rotating`) :`false` (`self.Arrow`) :`true` (`self.Arrow1`)))
  (bind _returnvalue_2 (`SceneComponent.K2_GetComponentLocation` _returnvalue))
  (bind _returnvalue_3 (`SceneComponent.K2_GetComponentRotation` _returnvalue))
  (`PhysicsControlComponent.SetControlTargetPositionAndOrientation` (`self.PhysicsControl`) (`self.MainControlName`) _returnvalue_2 _returnvalue_3 0.0 false false)
  (`PhysicsControlComponent.SetBodyModifierKinematicTarget` (`self.PhysicsControl`) "Movement" _returnvalue_2 _returnvalue_3 false))

(event `self.AttachModule`
  (params (Module :type "/Game/Resources/Characters/Modules/ModuleBase_BP Object Reference"))
  (bind _attachpoint (`self.AttachPoint`))
  ;[0.05469 0 1] Modules
  (`self.K2_SetActorRelativeRotation` Module (struct :`Pitch` 90.0 :`Roll` 90.0) false false)
  (`/Game/Resources/Characters/Modules/ModuleManager_BPC.Attach Module` (`self.ModuleManager_BPC`) Module (`SceneComponent.K2_GetComponentLocation` _attachpoint) _attachpoint)
  (`/Game/Resources/Characters/Modules/ModuleManager_BPC.Update Locked Target` (`self.ModuleManager_BPC`) (`GameplayStatics.GetPlayerPawn` 0)))

(event `self.DetachModule`
  (params (Module :type "/Game/Resources/Characters/Modules/ModuleBase_BP Object Reference"))
  (bind _returnvalue (`KismetArrayLibrary.Array_Find` (`/Game/Resources/Characters/Modules/ModuleManager_BPC.Modules` (`self.ModuleManager_BPC`)) Module))
  ;[0.05469 0 1] Modules
  (if (!= _returnvalue -1)
    (bind _output_get (`/Game/Resources/Characters/Modules/ModuleManager_BPC.Remove Module` (`self.ModuleManager_BPC`) _returnvalue))
    (`self.K2_DestroyActor` _output_get)))

(event `Fire`)

(event `self.LightStart`
  (`/Game/Resources/Characters/Modules/ModuleManager_BPC.LightProjectileStart` (`self.ModuleManager_BPC`))
  (set `self.rotating` true)
  (`PhysicsControlComponent.SetBodyModifierMovementType` (`self.PhysicsControl`) "Movement" "Kinematic"))

(event `self.LightStop`
  (`/Game/Resources/Characters/Modules/ModuleManager_BPC.LightProjectileStop` (`self.ModuleManager_BPC`))
  (`PhysicsControlComponent.SetBodyModifierMovementType` (`self.PhysicsControl`) "Movement" "Simulated")
  (`KismetSystemLibrary.RetriggerableDelay` 0.1)
  (set `self.rotating` false))

(event `self.PreparingAttack`
  (bind _array (`|MakeArray` (`self.root`) (`self.Cube2`) (`self.Cube3`) (`self.end`)))
  ;[0.1719 1 0] Preparing Attack Effeccts
  (bind _index (`/Game/Resources/Characters/Player/Blueprints/NewActorMacroLibrary.ForLoopWithDelay` 0 3 0.1)
    (:`Loop Body`
      (`PrimitiveComponent.SetRenderCustomDepth` (`|GetArrayItem` _array _index) true))
    (:`Completed`
      (bind _index_2 (`/Game/Resources/Characters/Player/Blueprints/NewActorMacroLibrary.ForLoopWithDelay` 0 3 0.1)
        (:`Loop Body`
          (`PrimitiveComponent.SetRenderCustomDepth` (`|GetArrayItem` _array _index_2) false))))))

(event `self.Deploy`
  (set `self.rotating` true)
  (`/Game/Resources/Characters/Modules/ModuleManager_BPC.Deploy` (`self.ModuleManager_BPC`))
  (`KismetSystemLibrary.RetriggerableDelay` 0.2 :!label _label)
  (set `self.rotating` false))

(event `self.HeavyStartCharge`
  (set `self.rotating` true)
  (bind _returnvalue (`NiagaraFunctionLibrary.SpawnSystemAttached` "/Game/Resources/VFX/Charging_NS_2.Charging_NS_2" (`self.end`) "None" (0.0 0.0 0.0) (struct) "KeepRelativeOffset")))

(event `self.HeavyStopCharge`
  (params (Charge :type "Float (double-precision)"))
  (`/Game/Resources/Characters/Modules/ModuleManager_BPC.HeavyAttack` (`self.ModuleManager_BPC`) Charge)
  (`ActorComponent.K2_DestroyComponent` (stale `self.HeavyStartCharge` _returnvalue))
  (goto _label))

(fn `UserConstructionScript`
  (`parent.UserConstructionScript`))