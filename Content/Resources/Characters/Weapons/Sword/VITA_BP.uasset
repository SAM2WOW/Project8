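; VITA is a floating sword weapon that follows its Host and performs light, charged heavy, projectile and deploy actions.
; Tick interpolates the actor toward a Mode-based target (idle slot, attack point, aim, edit, parry), while PhysicsControl drives SwordBody toward SwordTarget.
; Attacks pair timeline spins with immediate sphere-trace damage, knockback on heavy hits, and feedback.
; Attachable modules in ModuleManagerBPC receive attack and deploy calls; holding light attack starts projectile mode and charges a special.
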(event `self.AttachModule`
  (params (Module :type "/Game/Resources/Characters/Modules/ModuleBase_BP Object Reference"))
  (bind (_origin _boxextent) (`KismetSystemLibrary.GetComponentBounds` (`self.Box`)))
  ;[0.05469 0 1] Modules
  (`/Game/Resources/Characters/Modules/ModuleManager_BPC.Attach Module` (`self.ModuleManager_BPC`) Module (`KismetMathLibrary.RandomPointInBoundingBox` _origin (/ _boxextent 2)) (`self.swordBody`)))

(event `self.ReceiveBeginPlay`
  ;[0.125 1 0] P
  (`parent.ReceiveBeginPlay`)
  (`PhysicsControlComponent.MakeControl` :`self` (`self.PhysicsControl`) :`ChildMeshComponent` (`self.swordBody`) :`ControlData` (make `PhysicsControlData` 2.0 1.0 0.0 0.0 3.0))
  (`PhysicsControlComponent.MakeBodyModifier` (`self.PhysicsControl`) (`self.swordBody`) "None" "Simulated" "QueryAndPhysics" 0.0 true))

(event `self.DetachModule`
  (params (Module :type "/Game/Resources/Characters/Modules/ModuleBase_BP Object Reference"))
  (bind _returnvalue (`KismetArrayLibrary.Array_Find` (`/Game/Resources/Characters/Modules/ModuleManager_BPC.Modules` (`self.ModuleManager_BPC`)) Module))
  ;[0.05469 0 1] Modules
  (if (!= _returnvalue -1)
    (bind _output_get (`/Game/Resources/Characters/Modules/ModuleManager_BPC.Remove Module` (`self.ModuleManager_BPC`) _returnvalue))
    (`self.K2_DestroyActor` _output_get)))

(event `self.ReceiveTick`
  (params (DeltaSeconds :type "Float (single-precision)"))
  (bind _returnvalue (`GameplayStatics.GetWorldDeltaSeconds`))
  (bind (_returnvalue_location _returnvalue_rotation) (`KismetMathLibrary.BreakTransform` (`self.GetTransform`)))
  (bind _physicscontrol (`self.PhysicsControl`))
  (bind _mode (`self.Mode`))
  (bind _host (`self.Host`))
  (bind _speed (`self.Speed`))
  (bind _swordtarget (`self.swordTarget`))
  (bind _returnvalue_2 (`SceneComponent.K2_GetComponentLocation` _swordtarget))
  (bind _returnvalue_3 (`SceneComponent.K2_GetComponentRotation` _swordtarget))
  (bind _returnvalue_4 (`self.K2_GetActorLocation` _host))
  (bind _returnvalue_5 (`self.K2_GetActorRotation` _host))
  (bind _returnvalue_6 (`KismetMathLibrary.GetForwardVector` (`self.AimRotation`)))
  (bind _pitch (.pitch _returnvalue_5))
  (bind _yaw (.yaw _returnvalue_5))
  (bind _followcamera (`/Game/Resources/Characters/Player/Blueprints/BP_PlayerCharacter.FollowCamera` (cast `/Game/Resources/Characters/Player/Blueprints/BP_PlayerCharacter` (`GameplayStatics.GetPlayerCharacter` 0) :!pure true)))
  (bind _returnvalue_7 (+ (.roll _returnvalue_5) 90.0))
  (`parent.ReceiveTick` DeltaSeconds)
  (bind _locked_target (`self.Locked Target`)
    (:`then`
      (set `self.AimRotation` (`KismetMathLibrary.FindLookAtRotation` _returnvalue_4 (`self.K2_GetActorLocation` _locked_target))))
    (:`else`
      (set `self.AimRotation` _returnvalue_5)))
  (bind _slot (message `/Game/Resources/Characters/Weapons/Sword/VitaSlot_BPInter.Get Idle Slot` (`self.Host`)))
  (bind (_returnvalue_location_2 _returnvalue_rotation_2) (`KismetMathLibrary.BreakTransform` (`SceneComponent.K2_GetComponentToWorld` _slot)))
  (`self.K2_SetActorTransform` (`KismetMathLibrary.MakeTransform` (`KismetMathLibrary.VInterpTo` _returnvalue_location (select `/Game/Resources/Characters/Weapons/Sword/SwordModes_Enum` _mode :`NewEnumerator0` _returnvalue_location_2 :`NewEnumerator1` (`self.TargetLoc`) :`NewEnumerator2` (+ _returnvalue_4 (* _returnvalue_6 300.0)) :`NewEnumerator3` (+ (`SceneComponent.K2_GetComponentLocation` _followcamera) (* (`SceneComponent.GetForwardVector` _followcamera) 200.0) (`SceneComponent.GetRightVector` _followcamera)) :`NewEnumerator4` (+ _returnvalue_4 (* _returnvalue_6 100.0))) _returnvalue _speed) (`KismetMathLibrary.RLerp` _returnvalue_rotation (select `/Game/Resources/Characters/Weapons/Sword/SwordModes_Enum` _mode :`NewEnumerator0` _returnvalue_rotation_2 :`NewEnumerator1` (`self.TargetRot`) :`NewEnumerator2` (`KismetMathLibrary.MakeRotator` _returnvalue_7 (+ _pitch 90.0) _yaw) :`NewEnumerator3` (`SceneComponent.K2_GetComponentRotation` _followcamera) :`NewEnumerator4` (`KismetMathLibrary.MakeRotator` _returnvalue_7 _pitch _yaw)) (* _speed _returnvalue) true)))
  (`|ExecutionSequence`
    (:`then_0`
      (`PhysicsControlComponent.SetControlTargetPositionAndOrientation` _physicscontrol "0" _returnvalue_2 _returnvalue_3 0.0 true false)
      (`PhysicsControlComponent.SetBodyModifierKinematicTarget` _physicscontrol "Body_0" _returnvalue_2 _returnvalue_3 false))
    (:`then_1`
      ;[0 1 0.6484] Holding Charge
      (if (`self.Shooting`)
        (bind _output_get (set `self.HoldCharge` (`KismetMathLibrary.FMin` (+ (`self.HoldCharge`) (* (`GameplayStatics.GetWorldDeltaSeconds`) (`self.HoldChargeSpeed`))) 1.0)))
        (if (and (not (`self.HoldSpecial`)) (>= _output_get 1.0))
          (set `self.HoldSpecial` true))))))

(event `self.HeavyStartCharge`
  ;[1 0.6697 0] Heavy Attack
  (set `self.Mode` "NewEnumerator4")
  (set `self.Speed` 40.0))

(event `self.LightStart`
  (bind (_returnvalue_location _returnvalue_rotation) (`KismetMathLibrary.BreakTransform` (`self.GetTransform`)))
  (bind _targetloc (`self.TargetLoc`))
  (bind _locked_target (`self.Locked Target`))
  (bind _host (`self.Host`))
  (bind _returnvalue (`self.K2_GetActorLocation` _host))
  (bind _returnvalue_2 (`self.K2_GetActorLocation` _locked_target))
  (bind _returnvalue_3 (`self.K2_GetActorLocation` (`self.Host`)))
  (bind _returnvalue_4 (+ _returnvalue (* (`KismetMathLibrary.GetForwardVector` (`self.K2_GetActorRotation` _host)) 300.0)))
  ;[0.8607 1 0] Light Attack
  (set `self.LightAttackHold` true)
  (if (not (`self.Actioning`))
    (set `self.Actioning` true)
    (`KismetSystemLibrary.K2_ClearAndInvalidateTimerHandle` (`self.ReturnTimer`))
    (`|ExecutionSequence`
      (:`then_0`
        ;;[0.8516 1 0] Find Location and Rotation
        (`/Engine/EditorBlueprintResources/StandardMacros.IsValid` _locked_target
          (:`Is Valid`
            (set `self.TargetLoc` (+ (`KismetMathLibrary.SelectVector` (+ _returnvalue_3 (* (`KismetMathLibrary.GetForwardVector` (`KismetMathLibrary.FindLookAtRotation` _returnvalue_3 _returnvalue_2)) 300.0)) _returnvalue_2 (> (`KismetMathLibrary.Vector_Distance` _returnvalue_2 _returnvalue_3) 300.0)) (* (`KismetMathLibrary.RandomUnitVector`) 100.0)))
            (set `self.NewRot` (`KismetMathLibrary.RandomRotator` true)))
          (:`Is Not Valid`
            (bind (_outhit _returnvalue_5) (`KismetSystemLibrary.LineTraceSingle` _returnvalue _returnvalue_4 "TraceTypeQuery1"))
            (if _returnvalue_5
              (bind (_bblockinghit _binitialoverlap _time _distance _location _impactpoint _normal) (`GameplayStatics.BreakHitResult` _outhit))
              (bind _output_get (set `self.TargetLoc` _location))
              (bind _returnvalue_6 (`KismetMathLibrary.Conv_VectorToRotator` _normal))
              (set `self.NewRot` _returnvalue_6)
              (`GameplayStatics.SpawnDecalAtLocation` "/Game/Resources/Materials/Decal/slash_decal_Mat.slash_decal_Mat" (20.0 106.0 50.0) _output_get _returnvalue_6 10.0)
              (else
                (set `self.TargetLoc` _returnvalue_4)
                (set `self.NewRot` (`KismetMathLibrary.RandomRotator` true)))))))
      (:`then_1`
        ;;[0.5938 0 1] Animation
        (set `self.Mode` "NewEnumerator1")
        (set `self.TempTargetRot` (`self.TargetRot`))
        (set `self.TempTargetLoc` (`self.TargetLoc`))
        (bind (_direction _0) (`Timeline|Swinging` :!via `PlayFromStart`)
          (:`Update`
            (set `self.TargetRot` (`KismetMathLibrary.RLerp` (`self.TempTargetRot`) (`self.NewRot`) _0))
            (`SceneComponent.K2_SetRelativeRotation` (`self.swordTarget`) (`KismetMathLibrary.MakeRotator` 180.0 (`KismetMathLibrary.Lerp` 360.0 0.0 _0) 90.0) false true)
            (set `self.Speed` (`KismetMathLibrary.Lerp` 30.0 5.0 _0)))
          (:`Finished`
            (set `self.Actioning` false)
            (if (`self.LightAttackHold`)
              (`self.Shoot`)
              (else
                (bind _returnvalue_7 (`KismetSystemLibrary.K2_SetTimer` null "Finish Swing" (`self.ReturnTime`)))
                (set `self.ReturnTimer` _returnvalue_7))))))
      (:`then_2`
        ;;[0.8984 0 1] Actual Attack
        (bind _channel (`self.Get Trace Channel`))
        (bind (_outhits _returnvalue_8) (`KismetSystemLibrary.SphereTraceMulti` _targetloc _targetloc 150.0 _channel))
        (if _returnvalue_8
          (for _array_element _outhits
            (`GameplayStatics.ApplyDamage` (`.HitActor` (`GameplayStatics.BreakHitResult` _array_element)) 80.0 null self "/Script/Engine.DamageType")
            (`GameplayStatics.SpawnForceFeedbackAttached` "/Game/Resources/Characters/Weapons/Sword/Feedbacks/Light_Feed.Light_Feed" (`self.swordTarget`) "None" (0.0 0.0 0.0) (struct) "SnapToTarget" false false (`KismetMathLibrary.RandomFloatInRange` 0.8 1.0) 0.0 null)
            (bind _asnew_game_state_gs (cast `/Game/Resources/Characters/Player/Blueprints/NewGameState_GS` (`GameplayStatics.GetGameState`)))
            (`/Game/Resources/Characters/Player/Blueprints/NewGameState_GS.Enter Damange` _asnew_game_state_gs 0.3)
            (bind _asnew_game_mode_gm (cast `/Game/Resources/Characters/Player/Blueprints/NewGameMode_GM` (`GameplayStatics.GetGameMode`)))
            (`/Game/Resources/Widgets/HUD_Widget.Crosshair Hit Anim` (`/Game/Resources/Characters/Player/Blueprints/NewGameMode_GM.HUD_ref` _asnew_game_mode_gm)))))
      (:`then_3`
        ;;[0.6406 1 0] Call all Modules
        (`/Game/Resources/Characters/Modules/ModuleManager_BPC.LightAttack` (`self.ModuleManager_BPC`)))
      (:`then_4`
        ;;[1 0.75 0] Effects
        (`FMODBlueprintStatics.PlayEventAttached` "/Game/FMOD/Events/Sounds/Sword_Swing.Sword_Swing" (`self.swordTarget`) "None" (0.0 0.0 0.0) "SnapToTarget" true)
        (`|SpawnActorFromClass` "/Game/Resources/Characters/Destructables/FS_MasterField_Child.FS_MasterField_Child_C" (`KismetMathLibrary.MakeTransform` _returnvalue_location _returnvalue_rotation) "AlwaysSpawn" "OverrideRootScale" null null)
        (bind _asnew_game_mode_gm_2 (cast `/Game/Resources/Characters/Player/Blueprints/NewGameMode_GM` (`GameplayStatics.GetGameMode`)))
        (`/Game/Resources/Widgets/HUD_Widget.Attack Anim` (`/Game/Resources/Characters/Player/Blueprints/NewGameMode_GM.HUD_ref` _asnew_game_mode_gm_2))))))

(event `self.HeavyStopCharge`
  (params (Charge :type "Float (double-precision)"))
  (bind (_returnvalue_location _returnvalue_rotation) (`KismetMathLibrary.BreakTransform` (`self.GetTransform`)))
  (bind _host (`self.Host`))
  (bind _targetloc (`self.TargetLoc`))
  ;[1 0.6697 0] Heavy Attack
  (if (== Charge 0.0)
    (`self.Finish Swing`)
    (elif (not (`self.Actioning`))
      (set `self.Actioning` true)
      (`KismetSystemLibrary.K2_ClearAndInvalidateTimerHandle` (`self.ReturnTimer`))
      (set `self.TargetLoc` (`self.K2_GetActorLocation` (`self.Host`)))
      (set `self.TargetRot` (`self.K2_GetActorRotation` (`self.Host`)))
      (set `self.Mode` "NewEnumerator1")
      (`|ExecutionSequence`
        (:`then_0`
          (bind (_direction _0) (`Timeline|Timeline` :!via `PlayFromStart`)
            (:`Update`
              (`SceneComponent.K2_SetRelativeRotation` (`self.swordTarget`) (`KismetMathLibrary.MakeRotator` 180.0 (`KismetMathLibrary.Lerp` 720.0 0.0 _0) 90.0) false true)
              (set `self.Speed` (`KismetMathLibrary.Lerp` 30.0 5.0 _0))
              (set `self.TargetLoc` (+ (`self.K2_GetActorLocation` _host) (* (`KismetMathLibrary.GetForwardVector` (`KismetMathLibrary.ComposeRotators` (`self.K2_GetActorRotation` _host) (`KismetMathLibrary.RLerp` (struct :`Yaw` 600.0) (struct) _0))) 200.0))))
            (:`Finished`
              (set `self.Actioning` false)
              (bind _returnvalue (`KismetSystemLibrary.K2_SetTimer` null "Finish Swing" (`self.ReturnTime`)))
              (set `self.ReturnTimer` _returnvalue))))
        (:`then_1`
          (`/Game/Resources/Characters/Modules/ModuleManager_BPC.HeavyAttack` (`self.ModuleManager_BPC`) Charge))
        (:`then_2`
          (bind _channel (`self.Get Trace Channel`))
          (bind (_outhits _returnvalue_2) (`KismetSystemLibrary.SphereTraceMulti` _targetloc _targetloc 400.0 _channel))
          (if _returnvalue_2
            (for _array_element _outhits
              (`GameplayStatics.ApplyDamage` (`.HitActor` (`GameplayStatics.BreakHitResult` _array_element)) (`KismetMathLibrary.Lerp` 100.0 300.0 Charge) null self "/Game/Resources/Characters/Weapons/Sword/Heavy_DamageType.Heavy_DamageType_C")
              (`|ExecutionSequence`
                (:`then_0`
                  (`GameplayStatics.SpawnForceFeedbackAttached` "/Game/Resources/Characters/Weapons/Sword/Feedbacks/Light_Feed.Light_Feed" (`self.swordTarget`) "None" (0.0 0.0 0.0) (struct) "SnapToTarget" false false 1.0 0.0 null)
                  (bind _asnew_game_state_gs (cast `/Game/Resources/Characters/Player/Blueprints/NewGameState_GS` (`GameplayStatics.GetGameState`)))
                  (`/Game/Resources/Characters/Player/Blueprints/NewGameState_GS.Enter Damange` _asnew_game_state_gs 1.0)
                  (bind _asnew_game_mode_gm (cast `/Game/Resources/Characters/Player/Blueprints/NewGameMode_GM` (`GameplayStatics.GetGameMode`)))
                  (`/Game/Resources/Widgets/HUD_Widget.Crosshair Hit Anim` (`/Game/Resources/Characters/Player/Blueprints/NewGameMode_GM.HUD_ref` _asnew_game_mode_gm)))
                (:`then_1`
                  (message `/Game/Resources/Characters/Player/Blueprints/Knockback_BPInter.Apply Knockback` (`.HitActor` (`GameplayStatics.BreakHitResult` _array_element)) (`GameplayStatics.GetPlayerPawn` 0) (`KismetMathLibrary.Lerp` 500.0 3000.0 Charge) 200.0))))))
        (:`then_3`
          (`FMODBlueprintStatics.PlayEventAttached` "/Game/FMOD/Events/Sounds/Sword_Swing.Sword_Swing" (`self.swordTarget`) "None" (0.0 0.0 0.0) "SnapToTarget" true)
          (`|SpawnActorFromClass` "/Game/Resources/Characters/Destructables/FS_MasterField_Child.FS_MasterField_Child_C" (`KismetMathLibrary.MakeTransform` _returnvalue_location _returnvalue_rotation) "AlwaysSpawn" "OverrideRootScale" null null)
          (bind _asnew_game_mode_gm_2 (cast `/Game/Resources/Characters/Player/Blueprints/NewGameMode_GM` (`GameplayStatics.GetGameMode`)))
          (`/Game/Resources/Widgets/HUD_Widget.Attack Anim` (`/Game/Resources/Characters/Player/Blueprints/NewGameMode_GM.HUD_ref` _asnew_game_mode_gm_2)))))))

(event `Finish Swing`
  ;[1 0.7091 0] Finish Swing
  (set `self.Mode` "NewEnumerator0")
  (set `self.Speed` 5.0)
  (`PhysicsControlComponent.SetBodyModifierMovementType` (`self.PhysicsControl`) "Body_0" "Kinematic"))

(event `self.LightStop`
  ;[1 0.4309 0] Finished Projectile Attack
  (set `self.LightAttackHold` false)
  (if (`self.Shooting`)
    (set `self.Shooting` false)
    (for _array_element (`/Game/Resources/Characters/Modules/ModuleManager_BPC.Modules` (`self.ModuleManager_BPC`))
      (`/Game/Resources/Characters/Modules/ModuleBase_BP.LightProjectileStop` _array_element)
      (if (`self.HoldSpecial`)
        (`/Game/Resources/Characters/Modules/ModuleBase_BP.HeavyAttack` _array_element 1.0)))
    (set `self.HoldCharge` 0.0)
    (set `self.HoldSpecial` false)
    (bind _returnvalue (`KismetSystemLibrary.K2_SetTimer` null "Finish Swing" (`self.ReturnTime`)))
    (set `self.ReturnTimer` _returnvalue)
    (`PhysicsControlComponent.SetBodyModifierMovementType` (`self.PhysicsControl`) "Body_0" "Kinematic")))

(event `Shoot`
  ;[1 0.1588 0] Start Projectile Mode
  (set `self.Shooting` true)
  (`/Game/Resources/Characters/Modules/ModuleManager_BPC.LightProjectileStart` (`self.ModuleManager_BPC`))
  (set `self.Mode` "NewEnumerator2")
  (`PhysicsControlComponent.SetBodyModifierMovementType` (`self.PhysicsControl`) "Body_0" "Simulated"))

(event `Deploy`
  (bind _asbp_player_character (cast `/Game/Resources/Characters/Player/Blueprints/BP_PlayerCharacter` (`GameplayStatics.GetPlayerPawn` 0) :!pure true))
  (bind _returnvalue (`self.K2_GetActorRotation` _asbp_player_character))
  (bind _returnvalue_2 (+ (`self.K2_GetActorLocation` _asbp_player_character) (* (`KismetMathLibrary.GetForwardVector` _returnvalue) 100.0)))
  ;[0.2188 0 1] Deploy
  (if (not (`self.Actioning`))
    (set `self.Actioning` true)
    (`KismetSystemLibrary.K2_ClearAndInvalidateTimerHandle` (`self.ReturnTimer`))
    (set `self.Speed` 40.0)
    (set `self.TargetLoc` (+ _returnvalue_2 (0.0 0.0 100.0)))
    (set `self.TargetRot` _returnvalue)
    (set `self.Mode` "NewEnumerator1")
    (`KismetSystemLibrary.Delay` 0.3)
    (set `self.Speed` 20.0)
    (set `self.TargetLoc` (+ _returnvalue_2 (0.0 0.0 -50.0)))
    (`|ExecutionSequence`
      (:`then_0`
        (`KismetSystemLibrary.Delay` 0.1)
        (`/Game/Resources/Characters/Modules/ModuleManager_BPC.Deploy` (`self.ModuleManager_BPC`))
        (`GameplayStatics.SpawnForceFeedbackAttached` "/Game/Resources/Characters/Weapons/Sword/Feedbacks/Light_Feed.Light_Feed" (`self.swordTarget`) "None" (0.0 0.0 0.0) (struct) "SnapToTarget" false false 1.0 0.0 null))
      (:`then_1`
        (`KismetSystemLibrary.Delay` 0.3)
        (set `self.Mode` "NewEnumerator0")
        (set `self.Actioning` false)))))

(event `DeployInteract`
  (params (InteractTarget :type "Actor Object Reference"))
  (bind _returnvalue (`self.K2_GetActorLocation` InteractTarget))
  (if (`self.MovementLocked`)
    (set `self.MovementLocked` false)
    (set `self.Actioning` false)
    (set `self.Mode` "NewEnumerator0")
    (else
      (set `self.MovementLocked` true)
      (set `self.Actioning` true)
      (set `self.TargetLoc` (+ _returnvalue (0.0 0.0 300.0)))
      (set `self.TargetRot` (`self.K2_GetActorRotation` InteractTarget))
      (set `self.Mode` "NewEnumerator1")
      (set `self.Speed` 15.0)
      (`KismetSystemLibrary.Delay` 0.5)
      (set `self.TargetLoc` (+ _returnvalue (0.0 0.0 100.0)))
      (`KismetSystemLibrary.Delay` 0.2)
      (set `self.Actioning` false))))

(fn `UserConstructionScript`)