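; Module pickup collectable that registers its module with the game state when collected.
; It extends a parent collectable, calling the parent's OnCollect, then passing its Type to CollectModule on NewGameState_GS.
; BeginPlay, Tick and construction only call the parent.
; Disconnected leftover nodes would link a hint widget to the pickup and toggle visibility by player distance, overlap and collected state, but never run.
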(event `self.ReceiveBeginPlay`
  (`parent.ReceiveBeginPlay`))

(event `self.ReceiveTick`
  (params (DeltaSeconds :type "Float (single-precision)"))
  (`parent.ReceiveTick` DeltaSeconds))

(event `self.On Collect`
  (`parent.On Collect`)
  (bind _asnew_game_state_gs (cast `/Game/Resources/Characters/Player/Blueprints/NewGameState_GS` (`GameplayStatics.GetGameState`)))
  (`/Game/Resources/Characters/Player/Blueprints/NewGameState_GS.Collect Module` _asnew_game_state_gs (`self.Type`) 1 0 false))

(fn `UserConstructionScript`
  (`parent.UserConstructionScript`))