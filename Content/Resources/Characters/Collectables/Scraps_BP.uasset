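; Scrap collectable that reports its Amount to NewGameState_GS when collected, with its memory sphere scaled by that Amount.
; On Tick it seeks a nearby combinable scrap within MaxAmount, locks both, and lerps them together on a timeline.
; The survivor absorbs the amount, destroys the other and plays a scale bounce, while ReleaseMerge unlocks a claimed partner.
; Text renders show merge state every frame; bounce sound logic is disconnected.
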(event `Update Size`
  (bind _returnvalue (`KismetMathLibrary.MapRangeClamped` (`KismetMathLibrary.Conv_IntToDouble` (`self.Amount`)) 1.0 (`KismetMathLibrary.Conv_IntToDouble` (`self.MaxAmount`)) 0.7 2.0))
  ;[0.007812 0 1] Update Size
  (`SceneComponent.SetRelativeScale3D` (`self.MemorySphere_NS`) (`KismetMathLibrary.MakeVector` _returnvalue _returnvalue _returnvalue)))

(event `self.ReceiveTick`
  (params (DeltaSeconds :type "Float (single-precision)"))
  ;[1 0 0.04687] Combine Scraps
  (`parent.ReceiveTick` DeltaSeconds)
  (`|ExecutionSequence`
    (:`then_0`
      (if (and (< (`self.Amount`) (`self.MaxAmount`)) (`self.CanCombine?`))
        (for _array_element (`PrimitiveComponent.GetOverlappingActors` (`self.Sphere1`) "Scraps_BP_C")
          (bind _asscraps_bp (cast `/Game/Resources/Characters/Collectables/Scraps_BP` _array_element))
          (if (and (<= (`self.GetDistanceTo` _asscraps_bp self) 100.0) (< (+ (`/Game/Resources/Characters/Collectables/Scraps_BP.Amount` _asscraps_bp) (`self.Amount`)) (`self.MaxAmount`)) (not (`/Game/Resources/Characters/Collectables/CollectableBase_BP.Collected` _asscraps_bp)) (`/Game/Resources/Characters/Collectables/Scraps_BP.CanCombine?` _asscraps_bp))
            (set `/Game/Resources/Characters/Collectables/CollectableBase_BP.Collected` true _asscraps_bp)
            (set `self.Collected` true)
            (set `/Game/Resources/Characters/Collectables/Scraps_BP.CanCombine?` false _asscraps_bp)
            (set `self.MergeScrap` _asscraps_bp)
            (`PrimitiveComponent.SetCollisionEnabled` (`/Game/Resources/Characters/Collectables/CollectableBase_BP.Sphere1` _asscraps_bp) "NoCollision")
            (`|ExecutionSequence`
              (:`then_0`
                (break))
              (:`then_1`
                (set `self.CanCombine?` false)
                (set `self.TempLocation` (`self.K2_GetActorLocation`))
                (bind (_direction _collect) (`Timeline|Timeline`)
                  (:`Update`
                    (`self.K2_SetActorLocation` (`KismetMathLibrary.VLerp` (`self.TempLocation`) (`self.K2_GetActorLocation` (`self.MergeScrap`)) (/ _collect 2.0)))
                    (`self.K2_SetActorLocation` (`self.MergeScrap`) (`KismetMathLibrary.VLerp` (`self.K2_GetActorLocation` (`self.MergeScrap`)) (`self.TempLocation`) (/ _collect 2.0)) false false))
                  (:`Finished`
                    (bind _asscraps_bp_2 (cast `/Game/Resources/Characters/Collectables/Scraps_BP` (`self.MergeScrap`)))
                    (set `self.Amount` (+ (`/Game/Resources/Characters/Collectables/Scraps_BP.Amount` _asscraps_bp_2) (`self.Amount`)))
                    (`self.Update Size`)
                    (bind _asscraps_bp_3 (cast `/Game/Resources/Characters/Collectables/Scraps_BP` (`self.MergeScrap`)))
                    (`self.Release Merge` _asscraps_bp_3)
                    (`self.K2_DestroyActor` _asscraps_bp_3)
                    ;;[1 0 0.4453] Bounce Animation
                    (set `self.TempScale` (`SceneComponent.RelativeScale3D` (`self.MemorySphere_NS`)))
                    (bind (_direction_2 _collect_2) (`Timeline|Timeline_0` :!via `PlayFromStart`)
                      (:`Update`
                        (`SceneComponent.SetRelativeScale3D` (`self.MemorySphere_NS`) (* (`self.TempScale`) _collect_2)))
                      (:`Finished`
                        (set `self.Collected` false) ; Restore Collection State
                        (set `self.CanCombine?` true)))))))))))
    (:`then_1`
      (`TextRenderComponent.K2_SetText` (`self.TextRender1`) (`KismetTextLibrary.Conv_BoolToText` (`self.CanCombine?`)))
      (`TextRenderComponent.K2_SetText` (`self.TextRender`) (`KismetTextLibrary.Conv_BoolToText` (`self.Collected`))))))

(event `Release Merge`
  (bind _mergescrap (`self.MergeScrap`))
  ;[0 1 0.8828] Release
  (`/Engine/EditorBlueprintResources/StandardMacros.IsValid` _mergescrap
    (:`Is Valid`
      (bind _asscraps_bp (cast `/Game/Resources/Characters/Collectables/Scraps_BP` _mergescrap))
      (`PrimitiveComponent.SetCollisionEnabled` (`/Game/Resources/Characters/Collectables/CollectableBase_BP.Sphere1` _asscraps_bp) "QueryAndPhysics")
      (set `/Game/Resources/Characters/Collectables/CollectableBase_BP.Collected` false _asscraps_bp)
      (set `/Game/Resources/Characters/Collectables/Scraps_BP.CanCombine?` true _asscraps_bp))))

(event `self.On Collect`
  ;[1 0.9375 0] On Collect
  (set `self.CanCombine?` false)
  (`self.Release Merge`)
  (`parent.On Collect`)
  (bind _asnew_game_state_gs (cast `/Game/Resources/Characters/Player/Blueprints/NewGameState_GS` (`GameplayStatics.GetGameState`)))
  (`/Game/Resources/Characters/Player/Blueprints/NewGameState_GS.Collect Scrap` _asnew_game_state_gs (`self.Amount`)))

(event `self.ProjectileMovement.OnProjectileBounce`
  (params (ImpactResult :type "HitResult Structure (by ref)") (ImpactVelocity :type "Vector Structure (by ref)"))
  ;[1 0 0.1406] Bouncing Sounds
)

(fn `UserConstructionScript`
  (`parent.UserConstructionScript`)
  (`self.Update Size`))