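; Health pickup, derived from a parent collectable, that heals the player in proportion to its Amount when collected.
; On Tick it finds nearby pickups of its type that keep the total under MaxAmount and locks both from collection.
; A timeline pulls them together, then one absorbs the other's Amount, rescales its sphere effect and bounces.
; ReleaseMerge frees a locked partner, and collection is forced if the player still overlaps after merging.
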(event `Update Size`
  (bind _returnvalue (`KismetMathLibrary.MapRangeClamped` (`KismetMathLibrary.Conv_IntToDouble` (`self.Amount`)) 1.0 (`KismetMathLibrary.Conv_IntToDouble` (`self.MaxAmount`)) 0.7 2.0))
  ;[0.007812 0 1] Update Size
  (`SceneComponent.SetRelativeScale3D` (`self.MemorySphere_NS`) (`KismetMathLibrary.MakeVector` _returnvalue _returnvalue _returnvalue)))

(event `self.ReceiveTick`
  (params (DeltaSeconds :type "Float (single-precision)"))
  ;[1 0 0.04687] Combine Scraps
  (`parent.ReceiveTick` DeltaSeconds)
  (`|ExecutionSequence`
    (:`then_0`
      (if (and (< (`self.Amount`) (`self.MaxAmount`)) (`self.CanCombine?`))
        (for _array_element (`PrimitiveComponent.GetOverlappingActors` (`self.Sphere1`) "Health_BP_C")
          (bind _ashealth_bp (cast `/Game/Resources/Characters/Collectables/Health_BP` _array_element))
          (if (and (<= (`self.GetDistanceTo` _ashealth_bp self) 100.0) (< (+ (`/Game/Resources/Characters/Collectables/Health_BP.Amount` _ashealth_bp) (`self.Amount`)) (`self.MaxAmount`)) (not (`/Game/Resources/Characters/Collectables/CollectableBase_BP.Collected` _ashealth_bp)) (`/Game/Resources/Characters/Collectables/Health_BP.CanCombine?` _ashealth_bp))
            (set `/Game/Resources/Characters/Collectables/CollectableBase_BP.Collected` true _ashealth_bp)
            (set `self.Collected` true)
            (set `/Game/Resources/Characters/Collectables/Health_BP.CanCombine?` false _ashealth_bp)
            (set `self.MergeScrap` _ashealth_bp)
            (`PrimitiveComponent.SetCollisionEnabled` (`/Game/Resources/Characters/Collectables/CollectableBase_BP.Sphere1` _ashealth_bp) "NoCollision")
            (`|ExecutionSequence`
              (:`then_0`
                (break))
              (:`then_1`
                (set `self.CanCombine?` false)
                (set `self.TempLocation` (`self.K2_GetActorLocation`))
                (bind (_direction _collect) (`Timeline|Timeline`)
                  (:`Update`
                    (`self.K2_SetActorLocation` (`KismetMathLibrary.VLerp` (`self.TempLocation`) (`self.K2_GetActorLocation` (`self.MergeScrap`)) (/ _collect 2.0)))
                    (`self.K2_SetActorLocation` (`self.MergeScrap`) (`KismetMathLibrary.VLerp` (`self.K2_GetActorLocation` (`self.MergeScrap`)) (`self.TempLocation`) (/ _collect 2.0)) false false))
                  (:`Finished`
                    (bind _ashealth_bp_2 (cast `/Game/Resources/Characters/Collectables/Health_BP` (`self.MergeScrap`)))
                    (set `self.Amount` (+ (`/Game/Resources/Characters/Collectables/Health_BP.Amount` _ashealth_bp_2) (`self.Amount`)))
                    (`self.Update Size`)
                    (bind _ashealth_bp_3 (cast `/Game/Resources/Characters/Collectables/Health_BP` (`self.MergeScrap`)))
                    (`self.Release Merge` _ashealth_bp_3)
                    (`self.K2_DestroyActor` _ashealth_bp_3)
                    (`FMODBlueprintStatics.PlayEventAtLocation` null (`self.GetTransform`))
                    ;;[1 0 0.4453] Bounce Animation
                    (set `self.TempScale` (`SceneComponent.RelativeScale3D` (`self.MemorySphere_NS`)))
                    (bind (_direction_2 _collect_2) (`Timeline|Timeline_0` :!via `PlayFromStart`)
                      (:`Update`
                        (`SceneComponent.SetRelativeScale3D` (`self.MemorySphere_NS`) (* (`self.TempScale`) _collect_2)))
                      (:`Finished`
                        (set `self.Collected` false) ; Restore Collection State
                        (set `self.CanCombine?` true)
                        ;[0.5938 0 1] Force Collected when player is still in the collision sphere when it enabled
                        (if (`KismetArrayLibrary.Array_IsNotEmpty` (`PrimitiveComponent.GetOverlappingActors` (`self.Sphere1`) "/Game/Resources/Characters/Player/Blueprints/BP_PlayerCharacter.BP_PlayerCharacter_C"))
                          (`self.Force Collected`))))))))))))))

(event `Release Merge`
  (bind _mergescrap (`self.MergeScrap`))
  ;[0 1 0.8828] Release
  (`/Engine/EditorBlueprintResources/StandardMacros.IsValid` _mergescrap
    (:`Is Valid`
      (bind _ashealth_bp (cast `/Game/Resources/Characters/Collectables/Health_BP` _mergescrap))
      (`PrimitiveComponent.SetCollisionEnabled` (`/Game/Resources/Characters/Collectables/CollectableBase_BP.Sphere1` _ashealth_bp) "QueryAndPhysics")
      (set `/Game/Resources/Characters/Collectables/CollectableBase_BP.Collected` false _ashealth_bp)
      (set `/Game/Resources/Characters/Collectables/Health_BP.CanCombine?` true _ashealth_bp))))

(event `self.On Collect`
  ;[1 0.9375 0] On Collect
  (set `self.CanCombine?` false)
  (`self.Release Merge`)
  (`parent.On Collect`)
  (bind _asbp_player_character (cast `/Game/Resources/Characters/Player/Blueprints/BP_PlayerCharacter` (`GameplayStatics.GetPlayerPawn` 0)))
  (message `/Game/Resources/Characters/Player/Blueprints/ApplyingStat_BPInter.Apply Healing` _asbp_player_character (* (`KismetMathLibrary.Conv_IntToDouble` (`self.Amount`)) 20.0)))

(event `self.ProjectileMovement.OnProjectileBounce`
  (params (ImpactResult :type "HitResult Structure (by ref)") (ImpactVelocity :type "Vector Structure (by ref)"))
  ;[1 0 0.1406] Bouncing Sounds
)

(fn `UserConstructionScript`
  (`parent.UserConstructionScript`)
  (`self.Update Size`))