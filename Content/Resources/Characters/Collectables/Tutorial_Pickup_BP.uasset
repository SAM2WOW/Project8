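; Tutorial collectable pickup that registers a sword pickup and triggers a fake door when collected.
; It extends a parent collectable and deactivates its projectile movement on BeginPlay.
; On collect, it runs the parent logic, then calls SowrdPickup on NewGameMode_GM and FakeSpawn on the referenced fake door.
; The projectile bounce event is empty, leaving its scrap sound and debug print unconnected.
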(event `self.ReceiveBeginPlay`
  (`parent.ReceiveBeginPlay`)
  (`ActorComponent.Deactivate` (`self.ProjectileMovement`)))

(event `self.On Collect`
  (`parent.On Collect`)
  (bind _asnew_game_mode_gm (cast `/Game/Resources/Characters/Player/Blueprints/NewGameMode_GM` (`GameplayStatics.GetGameMode`)))
  (`/Game/Resources/Characters/Player/Blueprints/NewGameMode_GM.SowrdPickup` _asnew_game_mode_gm)
  (`/Game/Resources/Meshes/Environments/0_Univerisal/FakeDoor_BP.FakeSpawn` (`self.ref_fakedoor`)))

(event `self.ProjectileMovement.OnProjectileBounce`
  (params (ImpactResult :type "HitResult Structure (by ref)") (ImpactVelocity :type "Vector Structure (by ref)")))

(fn `UserConstructionScript`
  (`parent.UserConstructionScript`))