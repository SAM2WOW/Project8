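; SuperLogPickup_BP is a collectable pickup that unlocks every memory log entry at once.
; On collect, it runs the parent logic, then copies every row of MemoryLog_DT into the game state's LogEntries map, keyed by row name.
; It then posts a "SUPER LOG PICKUPED" console message with the Log_Added icon through the game mode's HUD reference.
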(event `self.On Collect`
  (`parent.On Collect`)
  (bind _outrownames (`DataTableFunctionLibrary.GetDataTableRowNames` "/Game/Resources/Characters/Interactables/MemoryLog_DT.MemoryLog_DT"))
  (for _array_element _outrownames
    (bind _returnvalue (`|GetDataTableRow` "/Game/Resources/Characters/Interactables/MemoryLog_DT.MemoryLog_DT" _array_element)
      (:`then`
        (bind _asnew_game_state_gs (cast `/Game/Resources/Characters/Player/Blueprints/NewGameState_GS` (`GameplayStatics.GetGameState`)))
        (`BlueprintMapLibrary.Map_Add` (`/Game/Resources/Characters/Player/Blueprints/NewGameState_GS.LogEntries` _asnew_game_state_gs) _array_element _returnvalue))))
  (bind _asnew_game_mode_gm (cast `/Game/Resources/Characters/Player/Blueprints/NewGameMode_GM` (`GameplayStatics.GetGameMode`)))
  (`/Game/Resources/Widgets/HUD_Widget.Add Console` (`/Game/Resources/Characters/Player/Blueprints/NewGameMode_GM.HUD_ref` _asnew_game_mode_gm) "SUPER LOG PICKUPED" "" 8.0 "/Game/Resources/Widgets/Textures/Console/Log_Added.Log_Added"))

(fn `UserConstructionScript`
  (`parent.UserConstructionScript`))