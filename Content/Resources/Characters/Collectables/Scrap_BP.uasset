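; Scrap collectable pickup that flies toward the player like a magnet and disappears on reaching them.
; Overlap of its Sphere1 component with BP_PlayerCharacter sets the Magnet flag, which is never cleared.
; While flagged, Tick uses VInterpTo to move the actor toward player pawn 0 without sweep, destroying it at close range.
; The Blueprint itself grants nothing to the player on pickup.
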(event `self.ReceiveTick`
  (params (DeltaSeconds :type "Float (single-precision)"))
  (if (`self.Magnet`)
    (`self.K2_SetActorLocation` (`KismetMathLibrary.VInterpTo` (`self.K2_GetActorLocation`) (`self.K2_GetActorLocation` (`GameplayStatics.GetPlayerPawn` 0)) DeltaSeconds 5.0))
    (if (< (`self.GetDistanceTo` (`GameplayStatics.GetPlayerPawn` 0) self) 50.0)
      (`self.K2_DestroyActor`))))

(event `self.Sphere1.OnComponentBeginOverlap`
  (params (OverlappedComponent :type "PrimitiveComponent Object Reference") (OtherActor :type "Actor Object Reference") (OtherComp :type "PrimitiveComponent Object Reference") (OtherBodyIndex :type Integer) (bFromSweep :type Boolean) (SweepResult :type "HitResult Structure (by ref)"))
  (cast `/Game/Resources/Characters/Player/Blueprints/BP_PlayerCharacter` OtherActor)
  (set `self.Magnet` true))

(fn `UserConstructionScript`)