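; Base collectable pickup that scatters in a random direction on spawn and is drawn into the player on contact.
; Projectile Movement supplies the launch, and overlapping Sphere1 with the player character starts the Collect timeline, which lerps the pickup toward the player pawn's live location.
; When the timeline finishes, OnCollect plays the Scrap audio event and the actor destroys itself.
; Older magnet and stop-on-impact logic remains disconnected.
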(event `self.ReceiveBeginPlay`
  (`ProjectileMovementComponent.SetVelocityInLocalSpace` (`self.ProjectileMovement`) (`KismetMathLibrary.RandomUnitVector`)))

(event `self.ReceiveTick`
  (params (DeltaSeconds :type "Float (single-precision)")))

(event `self.Sphere1.OnComponentBeginOverlap`
  (params (OverlappedComponent :type "PrimitiveComponent Object Reference") (OtherActor :type "Actor Object Reference") (OtherComp :type "PrimitiveComponent Object Reference") (OtherBodyIndex :type Integer) (bFromSweep :type Boolean) (SweepResult :type "HitResult Structure (by ref)"))
  (cast `/Game/Resources/Characters/Player/Blueprints/BP_PlayerCharacter` OtherActor)
  (set `self.TempLocation` (`self.K2_GetActorLocation`))
  (bind (_direction _collect) (`Timeline|Collect`)
    (:`Update`
      (`self.K2_SetActorLocation` (`KismetMathLibrary.VLerp` (`self.TempLocation`) (`self.K2_GetActorLocation` (`GameplayStatics.GetPlayerPawn` 0)) _collect)))
    (:`Finished`
      (`self.On Collect`)
      (`self.K2_DestroyActor`))))

(event `On Collect`
  (`FMODBlueprintStatics.PlayEventAtLocation` "/Game/FMOD/Events/Sounds/Scrap.Scrap" (`KismetMathLibrary.MakeTransform` (`self.K2_GetActorLocation`))))

(event `self.CoreSphere.OnComponentBeginOverlap`
  (params (OverlappedComponent :type "PrimitiveComponent Object Reference") (OtherActor :type "Actor Object Reference") (OtherComp :type "PrimitiveComponent Object Reference") (OtherBodyIndex :type Integer) (bFromSweep :type Boolean) (SweepResult :type "HitResult Structure (by ref)")))

(event `self.ProjectileMovement.OnProjectileStop`
  (params (ImpactResult :type "HitResult Structure (by ref)"))
  ;[1 0 0.9141] Stop Completeluy
)

(fn `UserConstructionScript`)