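; Collectable pickup that grants every module type in the game at once.
; On collect it runs the parent logic, then walks every row of ModuleInfo_DT and calls CollectModule on NewGameState_GS repeatedly, with the count driven by that row's Level1 value.
; A visibility check based on player distance, overlap and collected state is present but never runs.
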(event `self.On Collect`
  (`parent.On Collect`)
  (bind _outrownames (`DataTableFunctionLibrary.GetDataTableRowNames` "/Game/Resources/Characters/Modules/ModuleInfo_DT.ModuleInfo_DT"))
  (for _array_element _outrownames
    (bind _returnvalue (`|GetDataTableRow` "/Game/Resources/Characters/Modules/ModuleInfo_DT.ModuleInfo_DT" _array_element)
      (:`then`
        (for _ (range (+ (`.Level1_31_F549955C417A318510FC59B0C3338F54` (break `/Game/Resources/Characters/Modules/ModuleInfo_Struct` _returnvalue)) 1))
          (bind _asnew_game_state_gs (cast `/Game/Resources/Characters/Player/Blueprints/NewGameState_GS` (`GameplayStatics.GetGameState`)))
          (`/Game/Resources/Characters/Player/Blueprints/NewGameState_GS.Collect Module` _asnew_game_state_gs (make `/Game/Resources/Characters/Modules/ModuleInventory_Struct` _array_element null)))))))

(fn `UserConstructionScript`
  (`parent.UserConstructionScript`))