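; BasicEnemyAI_BP is a basic enemy that follows the player character once it comes within range.
; It caches player 0 on BeginPlay and compares their 2D distance to FollowRange every Tick.
; A DoOnce gates AIMoveTo toward the player so the move is not reissued every frame.
; The gate resets only when the move succeeds, so a failed move leaves it closed.
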(event `self.ReceiveBeginPlay`
  (set `self.Player Character Object` (`GameplayStatics.GetPlayerCharacter` 0)))

(event `self.ReceiveTick`
  (params (DeltaSeconds :type "Float (single-precision)"))
  ;[1 1 1] Check if player character is in range
  (if (<= (`KismetMathLibrary.Vector_Distance2D` (.location (`self.GetTransform` (`self.Player Character Object`))) (.location (`self.GetTransform` self))) (`self.Follow Range`))
    (`/Engine/EditorBlueprintResources/StandardMacros.DoOnce` false :!label _label
      (:`Completed`
        (`|AIMoveTo` self (0.0 0.0 0.0) (`self.Player Character Object`) 100.0 true
          (:`OnSuccess`
            (goto _label :!via `Reset`)))))))

(fn `UserConstructionScript`)