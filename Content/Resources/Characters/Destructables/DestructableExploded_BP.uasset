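; Exploded stand-in for a destructible: a Geometry Collection actor whose rest collection is set from RestCollectionIn at construction.
; On BeginPlay it plays a glass-break sound and, if Amount is positive, spawns that many Scraps_BP actors and makes debris ignore Pawns.
; Chaos collisions occasionally play impact audio with a debug box, and the first removal event triggers delayed self-destruction.
; Radial damage and other collision nodes are unconnected.
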(event `self.ReceiveBeginPlay`
  (bind _amount (`self.Amount`))
  (`|ExecutionSequence`
    (:`then_0`
      (if (> _amount 0)
        (for _ (range _amount)
          (`|SpawnActorFromClass` "/Game/Resources/Characters/Collectables/Scraps_BP.Scraps_BP_C" (`KismetMathLibrary.MakeTransform` (`self.K2_GetActorLocation`)) "AlwaysSpawn" "OverrideRootScale" null null))
        (`PrimitiveComponent.SetCollisionResponseToChannel` (`self.GeometryCollection`) "ECC_Pawn" "ECR_Ignore")))
    (:`then_1`
      (`FMODBlueprintStatics.PlayEventAtLocation` "/Game/FMOD/Events/Sounds/Collectables/Glass_Break.Glass_Break" (`self.GetTransform`)))))

(event `self.GeometryCollection.OnChaosBreakEvent`
  (params (BreakEvent :type "ChaosBreakEvent Structure (by ref)")))

(event `self.GeometryCollection.OnChaosRemovalEvent`
  (params (RemovalEvent :type "ChaosRemovalEvent Structure (by ref)"))
  (`/Engine/EditorBlueprintResources/StandardMacros.DoOnce` false
    (:`Completed`
      (`KismetSystemLibrary.Delay` 10.0)
      (`self.K2_DestroyActor`))))

(event `self.GeometryCollection.OnChaosPhysicsCollision`
  (params (CollisionInfo :type "ChaosPhysicsCollisionInfo Structure (by ref)"))
  (bind (_component _othercomponent _location _normal) (break `ChaosPhysicsCollisionInfo` CollisionInfo))
  (if (`KismetMathLibrary.RandomBoolWithWeight` 0.1)
    (`KismetSystemLibrary.DrawDebugBox` _location (10.0 10.0 10.0) (struct :`R` 1.0 :`G` 0.018288 :`B` 0.332501 :`A` 1.0) (struct) 5.0)
    (`FMODBlueprintStatics.PlayEventAtLocation` "/Game/FMOD/Events/Sounds/Collectables/Glass_Collision.Glass_Collision" (`KismetMathLibrary.MakeTransform` _location (`KismetMathLibrary.Conv_VectorToRotator` _normal)))))

(fn `UserConstructionScript`
  (`GeometryCollectionComponent.SetRestCollection` (`self.GeometryCollection`) (`self.Rest Collection In`)))