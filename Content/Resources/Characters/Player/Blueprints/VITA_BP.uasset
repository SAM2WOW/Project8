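; VITA is the player's floating sword companion, which registers itself on BP_PlayerCharacter and performs melee, ranged and deploy moves.
; Tick eases it toward either an action target or the player's SwordIdle point.
; LightSwing plays a timeline swing with sphere-trace damage, then shoots bullets at the locked target or forward while the attack input stays held, otherwise returning on a timer.
; Deploy scripts a short raise-and-drop move in front of the player.
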(event `self.ReceiveBeginPlay`
  (bind _asbp_player_character (cast `/Game/Resources/Characters/Player/Blueprints/BP_PlayerCharacter` (`GameplayStatics.GetPlayerPawn` 0)))
  (set `/Game/Resources/Characters/Player/Blueprints/BP_PlayerCharacter.Sword` self _asbp_player_character))

(event `self.ReceiveTick`
  (params (DeltaSeconds :type "Float (single-precision)"))
  (bind _returnvalue (`GameplayStatics.GetWorldDeltaSeconds`))
  (bind (_returnvalue_location _returnvalue_rotation) (`KismetMathLibrary.BreakTransform` (`self.GetTransform`)))
  (bind _target (`self.Target`))
  (bind _speed (`self.Speed`))
  (bind (_returnvalue_location_2 _returnvalue_rotation_2) (`KismetMathLibrary.BreakTransform` (`SceneComponent.K2_GetComponentToWorld` (`/Game/Resources/Characters/Player/Blueprints/BP_PlayerCharacter.Sword Idle ` (cast `/Game/Resources/Characters/Player/Blueprints/BP_PlayerCharacter` (`GameplayStatics.GetPlayerPawn` 0) :!pure true)))))
  (`self.K2_SetActorTransform` (`KismetMathLibrary.MakeTransform` (`KismetMathLibrary.VInterpTo` _returnvalue_location (`KismetMathLibrary.SelectVector` (`self.TargetLoc`) _returnvalue_location_2 _target) _returnvalue _speed) (`KismetMathLibrary.RInterpTo` _returnvalue_rotation (`KismetMathLibrary.SelectRotator` (`self.TargetRot`) _returnvalue_rotation_2 _target) _returnvalue _speed))))

(event `LightSwing`
  (params (Location :type "Vector Structure") (Rotation :type "Rotator Structure"))
  (bind _targetloc (`self.TargetLoc`))
  (if (not (`self.Actioning`))
    (set `self.Actioning` true)
    (`KismetSystemLibrary.K2_ClearAndInvalidateTimerHandle` (`self.ReturnTimer`))
    (set `self.TargetLoc` (+ Location (* (`KismetMathLibrary.RandomUnitVector`) 20.0)))
    (set `self.TargetRot` Rotation)
    (set `self.Target` true)
    (`|ExecutionSequence`
      (:`then_0`
        (bind (_direction _0) (`Timeline|Swinging` :!via `PlayFromStart`)
          (:`Update`
            (`SceneComponent.K2_SetRelativeRotation` (`self.sword`) (`KismetMathLibrary.MakeRotator` 180.0 (`KismetMathLibrary.Lerp` 320.0 0.0 _0) 180.0) false true)
            (`SceneComponent.K2_SetRelativeLocation` (`self.sword`) (`KismetMathLibrary.VLerp` (-200.0 0.0 0.0) (0.0 0.0 0.0) _0) false false)
            (set `self.Speed` (`KismetMathLibrary.Lerp` 40.0 5.0 _0)))
          (:`Finished`
            (set `self.Actioning` false)
            (if (`|GetInputActionValue`)
              (`self.Shoot`)
              (else
                (bind _returnvalue (`KismetSystemLibrary.K2_SetTimer` null "Finish Swing" (`self.ReturnTime`)))
                (set `self.ReturnTimer` _returnvalue))))))
      (:`then_1`
        (bind (_outhits _returnvalue_2) (`KismetSystemLibrary.SphereTraceMulti` :`Start` _targetloc :`End` _targetloc :`Radius` 150.0 :`TraceChannel` "TraceTypeQuery3" :`DrawDebugType` "ForOneFrame"))
        (if _returnvalue_2
          (for _array_element _outhits
            (`GameplayStatics.ApplyDamage` (`.HitActor` (`GameplayStatics.BreakHitResult` _array_element)) 200.0 null self "/Script/Engine.DamageType")))))))

(event `Finish Swing`
  (`self.Return`))

(event `EnhancedInput|/Game/Resources/Characters/Player/Input/Actions/IA_LightAttack`
  (params (ActionValue :type Boolean) (ElapsedSeconds :type "Float (double-precision)") (TriggeredSeconds :type "Float (double-precision)") (InputAction :type "InputAction Object Reference" :default "/Game/Resources/Characters/Player/Input/Actions/IA_LightAttack.IA_LightAttack"))
  (:`Completed`
    (if (`self.Shooting`)
      (set `self.Shooting` false)
      (`KismetSystemLibrary.K2_ClearAndInvalidateTimerHandle` (stale `Shoot` _returnvalue))
      (bind _returnvalue (`KismetSystemLibrary.K2_SetTimer` null "Finish Swing" (`self.ReturnTime`)))
      (set `self.ReturnTimer` _returnvalue))))

(event `Shoot`
  (set `self.Shooting` true)
  (bind _returnvalue (`KismetSystemLibrary.K2_SetTimerDelegate` (delegate `Fire`) 0.1 true))
  (`KismetSystemLibrary.PrintString` "FIRE!!!" true true (struct :`R` 1.0 :`B` 0.094325 :`A` 1.0)))

(event `Fire`
  (bind (_returnvalue_location _returnvalue_rotation) (`KismetMathLibrary.BreakTransform` (`self.GetTransform`)))
  (bind _asbp_player_character (cast `/Game/Resources/Characters/Player/Blueprints/BP_PlayerCharacter` (`GameplayStatics.GetPlayerPawn` 0) :!pure true))
  (bind _returnvalue (`self.K2_GetActorRotation` _asbp_player_character))
  (bind _lockedtarget (`/Game/Resources/Characters/Player/Blueprints/BP_PlayerCharacter.LockedTarget` (cast `/Game/Resources/Characters/Player/Blueprints/BP_PlayerCharacter` (`GameplayStatics.GetPlayerPawn` 0) :!pure true))
    (:`then`
      (`|SpawnActorFromClass` "/Game/Resources/Characters/Player/Blueprints/TempBullet_BP.TempBullet_BP_C" (`KismetMathLibrary.MakeTransform` _returnvalue_location (`KismetMathLibrary.FindLookAtRotation` (`self.K2_GetActorLocation` self) (`self.K2_GetActorLocation` _lockedtarget))) "AlwaysSpawn" "OverrideRootScale" null null))
    (:`else`
      (`|SpawnActorFromClass` "/Game/Resources/Characters/Player/Blueprints/TempBullet_BP.TempBullet_BP_C" (`KismetMathLibrary.MakeTransform` _returnvalue_location _returnvalue_rotation) "AlwaysSpawn" "OverrideRootScale" null null)))
  (set `self.TargetLoc` (+ (`self.K2_GetActorLocation` _asbp_player_character) (* (`KismetMathLibrary.GetForwardVector` _returnvalue) 300.0)))
  (set `self.TargetRot` (`KismetMathLibrary.MakeRotator` (+ (.roll _returnvalue) 90.0) (.pitch _returnvalue) (.yaw _returnvalue))))

(event `Return`
  ;[1 1 1] Return
  (set `self.Target` false))

(event `Deploy`
  (bind _asbp_player_character (cast `/Game/Resources/Characters/Player/Blueprints/BP_PlayerCharacter` (`GameplayStatics.GetPlayerPawn` 0) :!pure true))
  (bind _returnvalue (`self.K2_GetActorRotation` _asbp_player_character))
  (bind _returnvalue_2 (+ (`self.K2_GetActorLocation` _asbp_player_character) (* (`KismetMathLibrary.GetForwardVector` _returnvalue) 100.0)))
  ;[1 1 1] Deploy
  (if (not (`self.Actioning`))
    (set `self.Actioning` true)
    (`KismetSystemLibrary.K2_ClearAndInvalidateTimerHandle` (`self.ReturnTimer`))
    (set `self.Speed` 40.0)
    (set `self.TargetLoc` (+ _returnvalue_2 (0.0 0.0 100.0)))
    (set `self.TargetRot` (`KismetMathLibrary.ComposeRotators` _returnvalue (struct :`Yaw` 90.0)))
    (set `self.Target` true)
    (`KismetSystemLibrary.Delay` 0.3)
    (set `self.Speed` 20.0)
    (set `self.TargetLoc` (+ _returnvalue_2 (0.0 0.0 -50.0)))
    (`KismetSystemLibrary.Delay` 0.3)
    (set `self.Target` false)
    (set `self.Actioning` false)))

(fn `UserConstructionScript`)