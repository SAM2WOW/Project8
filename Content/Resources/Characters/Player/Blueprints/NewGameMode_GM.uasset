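; Game mode that owns the player HUD and handles game over, pausing, loading and returning to the main menu.
; BeginPlay creates the HUD; pausing opens a pause menu and switches input mode and cursor.
; Game over shows a console message, briefly slows time, reverses the HUD intro and reloads the level.
; Loading opens the map saved in slot p0; music startup and tutorial logic are disconnected.
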(event `self.ReceiveBeginPlay`
  (bind _returnvalue (`GameplayStatics.GetPlayerController` 0))
  (`|ExecutionSequence`
    (:`then_0`
      (`WidgetBlueprintLibrary.SetInputMode_GameOnly` _returnvalue)
      (set `PlayerController.bShowMouseCursor` false _returnvalue)
      (bind _returnvalue_2 (`|CreateWidget` "/Game/Resources/Widgets/HUD_Widget.HUD_Widget_C"))
      (bind _output_get (set `self.HUD_ref` _returnvalue_2))
      (`UserWidget.AddToViewport` _output_get 0))))

(event `Gameover`
  (bind _hud_ref (`self.HUD_ref`))
  (bind _hud_ref_2 (`self.HUD_ref`))
  (bind _intro (`/Game/Resources/Widgets/HUD_Widget.Intro` _hud_ref))
  ;[1 0.02344 0] Game Over
  (`FMODBlueprintStatics.EventInstanceStop` (`self.BGM_ref`) true)
  (`/Game/Resources/Widgets/HUD_Widget.GameoverHide` _hud_ref_2)
  (`/Game/Resources/Widgets/HUD_Widget.Add Console` _hud_ref_2 "Flesh Destroyed" "Reconnecting to SYSTEM 6" 3.0 "/Game/Resources/Widgets/Textures/Console/Error.Error")
  (`GameplayStatics.SetGlobalTimeDilation` 0.3)
  (`KismetSystemLibrary.Delay` 0.1)
  (`GameplayStatics.SetGlobalTimeDilation` 1.0)
  (`KismetSystemLibrary.Delay` 1.2)
  (`UserWidget.PlayAnimation` _hud_ref _intro 0.0 1 "Reverse" 1.0 false)
  (`KismetSystemLibrary.Delay` (+ (`WidgetAnimation.GetEndTime` _intro) 0.2))
  (bind _returnvalue (`GameplayStatics.GetCurrentLevelName` true))
  (`GameplayStatics.OpenLevel` (`KismetStringLibrary.Conv_StringToName` _returnvalue)))

(event `PauseGame`
  (params (bPaused :type Boolean))
  (bind _returnvalue (`GameplayStatics.GetPlayerController` 0))
  (if bPaused
    (`GameplayStatics.SetGamePaused` true)
    (bind _returnvalue_2 (`|CreateWidget` "/Game/Resources/Widgets/PauseMenu_Widget.PauseMenu_Widget_C"))
    (`UserWidget.AddToViewport` _returnvalue_2 0)
    (`WidgetBlueprintLibrary.SetInputMode_GameAndUIEx` _returnvalue _returnvalue_2)
    (set `PlayerController.bShowMouseCursor` true _returnvalue)
    (else
      (`GameplayStatics.SetGamePaused` false)
      (`WidgetBlueprintLibrary.SetInputMode_GameOnly` _returnvalue true)
      (set `PlayerController.bShowMouseCursor` false _returnvalue))))

(event `LoadSave`
  (`FMODBlueprintStatics.EventInstanceStop` (`self.BGM_ref`))
  (bind _returnvalue (`GameplayStatics.LoadGameFromSlot` "p0"))
  (bind _asnew_save_game (cast `/Game/Resources/Characters/Player/Blueprints/Save/NewSaveGame` _returnvalue))
  (`GameplayStatics.OpenLevel` (`KismetStringLibrary.Conv_StringToName` (`/Game/Resources/Characters/Player/Blueprints/Save/NewSaveGame.CurrentMap` _asnew_save_game))))

(event `ToMainMenu`
  (`FMODBlueprintStatics.EventInstanceStop` (`self.BGM_ref`))
  (`GameplayStatics.OpenLevel` "MainMenu"))

(fn `UserConstructionScript`)