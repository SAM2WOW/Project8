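; Game state for the player's persistent progress and shared combat state, restored from a save slot on BeginPlay.
; Tracks scraps, chunk, log entries, flags and a module inventory with crafting, slot-based installation and loadouts, updating the HUD.
; SaveGame writes everything plus player state, while SetFlag can autosave a single flag.
; Also drives timeline-based slow-motion and damage post effects, and derives combat modes each tick from the attacking enemy count.
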(event `self.ReceiveBeginPlay`
  ;[0 0.8359 1] RestoreSave
  (bind _returnvalue (`GameplayStatics.DoesSaveGameExist` (`self.SlotName`)))
  (if _returnvalue
    (bind _returnvalue_2 (`GameplayStatics.LoadGameFromSlot` (`self.SlotName`)))
    (bind _asnew_save_game (cast `/Game/Resources/Characters/Player/Blueprints/Save/NewSaveGame` _returnvalue_2))
    (set `self.Scraps` (`/Game/Resources/Characters/Player/Blueprints/Save/NewSaveGame.Scraps` _asnew_save_game))
    (bind _asnew_game_mode_gm (cast `/Game/Resources/Characters/Player/Blueprints/NewGameMode_GM` (`GameplayStatics.GetGameMode`)))
    (`/Game/Resources/Widgets/HUD_Widget.Scrap Collected` (`/Game/Resources/Characters/Player/Blueprints/NewGameMode_GM.HUD_ref` _asnew_game_mode_gm))
    (set `self.CurrentChunk` (`/Game/Resources/Characters/Player/Blueprints/Save/NewSaveGame.CurrentChunk` _asnew_save_game))
    (set `self.LogEntries` (`/Game/Resources/Characters/Player/Blueprints/Save/NewSaveGame.LogEntries` _asnew_save_game))
    (set `self.ModuleCollection` (`/Game/Resources/Characters/Player/Blueprints/Save/NewSaveGame.ModuleCollection` _asnew_save_game))
    (set `self.SavedLoadout` (`/Game/Resources/Characters/Player/Blueprints/Save/NewSaveGame.SavedLoadout` _asnew_save_game))
    (set `self.Flags` (`/Game/Resources/Characters/Player/Blueprints/Save/NewSaveGame.Flags` _asnew_save_game))
    (else
      (bind _asnew_game_mode_gm_2 (cast `/Game/Resources/Characters/Player/Blueprints/NewGameMode_GM` (`GameplayStatics.GetGameMode`)))
      (set `/Game/Resources/Characters/Player/Blueprints/NewGameMode_GM.No Sword Mode` true _asnew_game_mode_gm_2))))

(event `Collect Module`
  (params (Name :type Name) (Scrap :type Integer :default 1) (Avaliable :type Integer) (`Message?` :type Boolean))
  (bind _modulecollection (`self.ModuleCollection`))
  (bind _returnvalue (`KismetTextLibrary.TextToUpper` (`KismetTextLibrary.Conv_NameToText` Name)))
  (bind (_value _returnvalue_2) (`BlueprintMapLibrary.Map_Find` _modulecollection Name))
  ;[0.2891 1 0] Collect Module
  (if _returnvalue_2
    (`BlueprintMapLibrary.Map_Add` _modulecollection Name (make `/Game/Resources/Characters/Modules/ModuleCollection_Struct` (+ (break `/Game/Resources/Characters/Modules/ModuleCollection_Struct` _value) Scrap) (+ (`.Avaliable_10_EF681991451349B4AD0BC096DC322166` (break `/Game/Resources/Characters/Modules/ModuleCollection_Struct` _value)) Avaliable) (`.Installed_9_818FED464A6562A3282B64BCF64F96CD` (break `/Game/Resources/Characters/Modules/ModuleCollection_Struct` _value))))
    (if `Message?`
      (bind _asnew_game_mode_gm (cast `/Game/Resources/Characters/Player/Blueprints/NewGameMode_GM` (`GameplayStatics.GetGameMode`)))
      (bind _returnvalue_3 (`|GetDataTableRow` "/Game/Resources/Characters/Modules/ModuleInfo_DT.ModuleInfo_DT" Name)
        (:`then`
          (bind _can_update (`self.Check Crafting` "None"))
          (`/Game/Resources/Widgets/HUD_Widget.Add Console` (`/Game/Resources/Characters/Player/Blueprints/NewGameMode_GM.HUD_ref` _asnew_game_mode_gm) (`|FormatText` "<RichText.Emphasis>{name}</> Added" _returnvalue) (select `bool` _can_update :`true` "Crafting Avaliable" :!type "Text") 6.0 (`.Icon_25_16583C9B489E3D999070A78068EEEC6B` (break `/Game/Resources/Characters/Modules/ModuleInfo_Struct` _returnvalue_3))))))
    (else
      (`BlueprintMapLibrary.Map_Add` _modulecollection Name (make `/Game/Resources/Characters/Modules/ModuleCollection_Struct` Scrap Avaliable))
      (if `Message?`
        (bind _asnew_game_mode_gm_2 (cast `/Game/Resources/Characters/Player/Blueprints/NewGameMode_GM` (`GameplayStatics.GetGameMode`)))
        (bind _returnvalue_4 (`|GetDataTableRow` "/Game/Resources/Characters/Modules/ModuleInfo_DT.ModuleInfo_DT" Name)
          (:`then`
            (`/Game/Resources/Widgets/HUD_Widget.Add Console` (`/Game/Resources/Characters/Player/Blueprints/NewGameMode_GM.HUD_ref` _asnew_game_mode_gm_2) "<RichText.Emphasis>MODULE</> Discovered" (`|FormatText` "{name}" _returnvalue) 10.0 "/Game/Resources/Widgets/Textures/Console/Module_Added.Module_Added")))))))

(event `Collect Scrap`
  (params (Amount :type Integer :default 1))
  ;[0.2422 1 0] Collect Scrap
  (set `self.Scraps` (+ (`self.Scraps`) Amount))
  (bind _asbp_player_character (cast `/Game/Resources/Characters/Player/Blueprints/BP_PlayerCharacter` (`GameplayStatics.GetPlayerPawn` 0)))
  (`/Game/Resources/Characters/Player/Blueprints/BP_PlayerCharacter.Increase Deploy Charge` _asbp_player_character (`KismetMathLibrary.Conv_IntToDouble` (* Amount 4)))
  (bind _asnew_game_mode_gm (cast `/Game/Resources/Characters/Player/Blueprints/NewGameMode_GM` (`GameplayStatics.GetGameMode`)))
  (`/Game/Resources/Widgets/HUD_Widget.Scrap Collected` (`/Game/Resources/Characters/Player/Blueprints/NewGameMode_GM.HUD_ref` _asnew_game_mode_gm)))

(event `Set Sword Color`
  (params (Value :type "LinearColor Structure"))
  ;[0.9219 0 1] Set Sword Color
  (bind _output_get (set `self.SwordColor` Value))
  (bind _asbp_player_character (cast `/Game/Resources/Characters/Player/Blueprints/BP_PlayerCharacter` (`GameplayStatics.GetPlayerPawn` 0)))
  (bind _sword (`/Game/Resources/Characters/Player/Blueprints/BP_PlayerCharacter.Sword` _asbp_player_character))
  (`/Engine/EditorBlueprintResources/StandardMacros.IsValid` _sword
    (:`Is Valid`
      (`/Game/Resources/Characters/Weapons/Sword/VITA_BP.Update Sword Color` _sword _output_get))))

(event `Install Module`
  (params (Module :type "/Game/Resources/Characters/Modules/ModuleInventory_Struct Structure") (`Change Data?` :type Boolean :default true) (Position :type Integer) (Slot :type Integer))
  (bind _type (break `/Game/Resources/Characters/Modules/ModuleInventory_Struct` Module))
  (bind (_type_2 _ref) (break `/Game/Resources/Characters/Modules/ModuleInventory_Struct` Module))
  (bind _modulecollection (`self.ModuleCollection`))
  (bind _value (`BlueprintMapLibrary.Map_Find` _modulecollection _type))
  ;[0.2656 0 1] Attach Module
  (if `Change Data?`
    (bind _avaliable (`self.Check Inventory Module Avaliability` _type))
    (if _avaliable
      (`BlueprintMapLibrary.Map_Add` _modulecollection _type (make `/Game/Resources/Characters/Modules/ModuleCollection_Struct` (break `/Game/Resources/Characters/Modules/ModuleCollection_Struct` _value) (- (`.Avaliable_10_EF681991451349B4AD0BC096DC322166` (break `/Game/Resources/Characters/Modules/ModuleCollection_Struct` _value)) 1) (+ (`.Installed_9_818FED464A6562A3282B64BCF64F96CD` (break `/Game/Resources/Characters/Modules/ModuleCollection_Struct` _value)) 1)))
      (`KismetArrayLibrary.Array_Add` (`self.VitaInstalled`) (make `/Game/Resources/Characters/Modules/ModuleInventory_Struct` _type_2 _ref) :!label _label)
      (for _index (range Slot)
        (`KismetArrayLibrary.Array_Set` (`self.VitaSlots`) (+ _index Position) (make `/Game/Resources/Characters/Modules/ModuleInventory_Struct` _type_2 _ref)))
      (bind (_module_count _charge_count) (`self.CountModules`))
      (bind _asnew_game_mode_gm (cast `/Game/Resources/Characters/Player/Blueprints/NewGameMode_GM` (`GameplayStatics.GetGameMode`)))
      (`/Game/Resources/Widgets/HUD_Widget.Update Deploy Amount` (`/Game/Resources/Characters/Player/Blueprints/NewGameMode_GM.HUD_ref` _asnew_game_mode_gm) _charge_count)
      (else
        (`KismetSystemLibrary.PrintString` "Wait this is not in the Enough???" true true (struct :`R` 1.0 :`B` 0.184391 :`A` 1.0))))
    (else
      (goto _label))))

(event `Uninstall Module`
  (params (Module :type "/Game/Resources/Characters/Modules/ModuleInventory_Struct Structure"))
  (bind (_type _ref) (break `/Game/Resources/Characters/Modules/ModuleInventory_Struct` Module))
  (bind _type_2 (break `/Game/Resources/Characters/Modules/ModuleInventory_Struct` Module))
  (bind _vitainstalled (`self.VitaInstalled`))
  (bind _modulecollection (`self.ModuleCollection`))
  (bind _returnvalue (`KismetArrayLibrary.Array_Find` _vitainstalled Module))
  (bind _value (`BlueprintMapLibrary.Map_Find` _modulecollection _type_2))
  ;[1 0.02344 0] Detach Module
  (if (!= _returnvalue -1)
    (`KismetArrayLibrary.Array_Remove` _vitainstalled _returnvalue)
    (`|ExecutionSequence`
      (:`then_0`
        (`BlueprintMapLibrary.Map_Add` _modulecollection _type_2 (make `/Game/Resources/Characters/Modules/ModuleCollection_Struct` (break `/Game/Resources/Characters/Modules/ModuleCollection_Struct` _value) (+ (`.Avaliable_10_EF681991451349B4AD0BC096DC322166` (break `/Game/Resources/Characters/Modules/ModuleCollection_Struct` _value)) 1) (- (`.Installed_9_818FED464A6562A3282B64BCF64F96CD` (break `/Game/Resources/Characters/Modules/ModuleCollection_Struct` _value)) 1))))
      (:`then_1`
        (for _index (range (`/Game/Resources/Characters/Modules/ModuleBase_BP.Slot` _ref))
          (`KismetArrayLibrary.Array_Set` (`self.VitaSlots`) (+ _index (`/Game/Resources/Characters/Modules/ModuleBase_BP.Position` _ref)) (make `/Game/Resources/Characters/Modules/ModuleInventory_Struct` "None" null)))
        (bind (_module_count _charge_count) (`self.CountModules`))
        (bind _asnew_game_mode_gm (cast `/Game/Resources/Characters/Player/Blueprints/NewGameMode_GM` (`GameplayStatics.GetGameMode`)))
        (`/Game/Resources/Widgets/HUD_Widget.Update Deploy Amount` (`/Game/Resources/Characters/Player/Blueprints/NewGameMode_GM.HUD_ref` _asnew_game_mode_gm) _charge_count)))
    (else
      (`KismetSystemLibrary.PrintString` "ERROR TRYING TO REMOVE NONE"))))

(event `Mini Slowmo`
  (params (Level :type "Float (double-precision)"))
  (if (not (`self.Slowmo`))
    (`GameplayStatics.SetGlobalTimeDilation` 0.3)
    (set `self.Slowmo` true)
    (`KismetSystemLibrary.RetriggerableDelay` (`KismetMathLibrary.Lerp` 0.01 0.06 Level))
    (`GameplayStatics.SetGlobalTimeDilation` 1.0)
    (set `self.Slowmo` false)))

(event `Save Game`
  ;[0 0.5078 1] Save Data
  (bind _returnvalue (`GameplayStatics.DoesSaveGameExist` (`self.SlotName`)))
  (if _returnvalue
    (bind _returnvalue_2 (`GameplayStatics.LoadGameFromSlot` (`self.SlotName`)))
    (set `self.SaveData` _returnvalue_2)
    (else
      (bind _returnvalue_3 (`GameplayStatics.CreateSaveGameObject` "/Game/Resources/Characters/Player/Blueprints/Save/NewSaveGame.NewSaveGame_C"))
      (set `self.SaveData` _returnvalue_3)))
  (bind _asnew_save_game (cast `/Game/Resources/Characters/Player/Blueprints/Save/NewSaveGame` (`self.SaveData`)))
  (`|ExecutionSequence`
    (:`then_0`
      (bind _asbp_player_character (cast `/Game/Resources/Characters/Player/Blueprints/BP_PlayerCharacter` (`GameplayStatics.GetPlayerPawn` 0)))
      (set `/Game/Resources/Characters/Player/Blueprints/Save/NewSaveGame.PlayerTransform` (`self.GetTransform` _asbp_player_character) _asnew_save_game)
      (set `/Game/Resources/Characters/Player/Blueprints/Save/NewSaveGame.PlayerHealth` (`/Game/Resources/Characters/Player/Blueprints/BP_PlayerCharacter.Health` _asbp_player_character) _asnew_save_game)
      (set `/Game/Resources/Characters/Player/Blueprints/Save/NewSaveGame.PlayerCharge` (`/Game/Resources/Characters/Player/Blueprints/BP_PlayerCharacter.DeployCharge` _asbp_player_character) _asnew_save_game)
      (set `/Game/Resources/Characters/Player/Blueprints/Save/NewSaveGame.SwordColor` (`self.SwordColor`) _asnew_save_game)
      (set `/Game/Resources/Characters/Player/Blueprints/Save/NewSaveGame.CurrentChunk` (`self.CurrentChunk`) _asnew_save_game)
      (set `/Game/Resources/Characters/Player/Blueprints/Save/NewSaveGame.Flags` (`self.Flags`) _asnew_save_game))
    (:`then_1`
      (set `/Game/Resources/Characters/Player/Blueprints/Save/NewSaveGame.Scraps` (`self.Scraps`) _asnew_save_game)
      (set `/Game/Resources/Characters/Player/Blueprints/Save/NewSaveGame.ModuleCollection` (`self.ModuleCollection`) _asnew_save_game)
      (set `/Game/Resources/Characters/Player/Blueprints/Save/NewSaveGame.LogEntries` (`self.LogEntries`) _asnew_save_game)
      (set `/Game/Resources/Characters/Player/Blueprints/Save/NewSaveGame.SavedLoadout` (`self.SavedLoadout`) _asnew_save_game)
      (bind _moduleinstalled (`/Game/Resources/Characters/Player/Blueprints/Save/NewSaveGame.ModuleInstalled` _asnew_save_game))
      (`KismetArrayLibrary.Array_Clear` _moduleinstalled)
      (for _array_element (`self.VitaInstalled`)
        (`KismetArrayLibrary.Array_Add` _moduleinstalled (make `/Game/Resources/Characters/Modules/ModuleSave_Struct` (break `/Game/Resources/Characters/Modules/ModuleInventory_Struct` _array_element) (`/Game/Resources/Characters/Modules/ModuleBase_BP.Position` (`.Ref_13_681E062642B3B066754CCDAFCC922AF4` (break `/Game/Resources/Characters/Modules/ModuleInventory_Struct` _array_element)))))))
    (:`then_2`
      (bind _returnvalue_4 (`GameplayStatics.GetCurrentLevelName` true))
      (set `/Game/Resources/Characters/Player/Blueprints/Save/NewSaveGame.CurrentMap` _returnvalue_4 _asnew_save_game)
      (`GameplayStatics.SaveGameToSlot` _asnew_save_game (`self.SlotName`))
      (bind _asnew_game_mode_gm (cast `/Game/Resources/Characters/Player/Blueprints/NewGameMode_GM` (`GameplayStatics.GetGameMode`)))
      (`/Game/Resources/Widgets/HUD_Widget.Add Console` (`/Game/Resources/Characters/Player/Blueprints/NewGameMode_GM.HUD_ref` _asnew_game_mode_gm) "Game Saved" "" 8.0 "/Game/Resources/Widgets/Textures/Console/Saved.Saved"))
    (:`then_3`
      (`FMODBlueprintStatics.PlayEvent2D` "/Game/FMOD/Events/Sounds/UI/UI_Save.UI_Save"))))

(event `CancelSlowMo`
  ;[1 0 0.6562] Slowmo
  (bind (_direction _slow) (`Timeline|Timeline` :`NewTime` 0.5 :!via `PlayFromStart` :!label _label_2)
    (:`Update`
      (bind _returnvalue (`KismetMathLibrary.Lerp` 1.0 0.1 _slow))
      (`GameplayStatics.SetGlobalTimeDilation` _returnvalue)
      (`KismetSystemLibrary.PrintString` (`KismetStringLibrary.Conv_DoubleToString` _returnvalue)))
    (:`Finished`
      (set `self.Slowmo` false)
      (bind _asnew_game_mode_gm (cast `/Game/Resources/Characters/Player/Blueprints/NewGameMode_GM` (`GameplayStatics.GetGameMode`)))
      (set `/Game/Chameleon/Chameleon.Anamorphic Lens Flares` false (`/Game/Resources/Characters/Player/Blueprints/NewGameMode_GM.Post_ref` _asnew_game_mode_gm)))))

(event `Enter Slowmo`
  (params (Time :type "Float (double-precision)"))
  ;[1 0 0.6562] Slowmo
  (if (`self.Slowmo`)
    (`/Engine/EditorBlueprintResources/StandardMacros.DoOnce` false :!label _label_3
      (:`Completed`
        (`GameplayStatics.SetGlobalTimeDilation` 0.1 :!label _label_4)
        (`KismetSystemLibrary.RetriggerableDelay` Time)
        (goto _label_2 :!via `PlayFromStart`)))
    (else
      (`|ExecutionSequence`
        (:`then_0`
          (set `self.Slowmo` true)
          (goto _label_4))
        (:`then_1`
          (goto _label_3 :!via `Reset`))
        (:`then_2`
          (bind _asnew_game_mode_gm (cast `/Game/Resources/Characters/Player/Blueprints/NewGameMode_GM` (`GameplayStatics.GetGameMode`)))
          (set `/Game/Chameleon/Chameleon.Anamorphic Lens Flares` true (`/Game/Resources/Characters/Player/Blueprints/NewGameMode_GM.Post_ref` _asnew_game_mode_gm))
          (`self.Enter Damange` 0.5))))))

(event `Enter Damange`
  (params (Amount :type "Float (double-precision)"))
  ;[0.2656 1 0] Set Damange Effect
  (`self.Mini Slowmo` Amount)
  (bind _asnew_game_mode_gm (cast `/Game/Resources/Characters/Player/Blueprints/NewGameMode_GM` (`GameplayStatics.GetGameMode`)))
  (bind _post_ref (`/Game/Resources/Characters/Player/Blueprints/NewGameMode_GM.Post_ref` _asnew_game_mode_gm))
  (set `/Game/Chameleon/Chameleon.Speed Lines` true _post_ref)
  (bind (_direction _newtrack_0) (`Timeline|Damage` :!via `PlayFromStart`)
    (:`Update`
      (`/Game/Chameleon/Chameleon.Set Chromatic` _post_ref (`KismetMathLibrary.Lerp` 0.12 (`KismetMathLibrary.Lerp` 0.12 2.0 Amount) _newtrack_0))
      (`/Game/Chameleon/Chameleon.Set Ambience Intensity` _post_ref (`KismetMathLibrary.Lerp` 0.2 (`KismetMathLibrary.Lerp` 0.2 1.0 Amount) _newtrack_0))
      (`/Game/Chameleon/Chameleon.Set Ambience Color` _post_ref (`KismetMathLibrary.LinearColorLerp` (struct :`G` 0.351533 :`B` 1.0 :`A` 1.0) (`KismetMathLibrary.LinearColorLerp` (struct :`G` 0.351533 :`B` 1.0 :`A` 1.0) (struct :`R` 0.054146 :`G` 0.424743 :`B` 1.0 :`A` 1.0) Amount) _newtrack_0))
      (set `/Game/Chameleon/Chameleon.Speed Lines Intensity` (`KismetMathLibrary.Lerp` 0.0 (`KismetMathLibrary.Lerp` 0.0 0.04 Amount) _newtrack_0) _post_ref))
    (:`Finished`
      (set `/Game/Chameleon/Chameleon.Speed Lines` false _post_ref))))

(event `self.ReceiveTick`
  (params (DeltaSeconds :type "Float (single-precision)"))
  (bind _returnvalue (`BlueprintSetLibrary.Set_Length` (`self.EnemiesTryingToAttack`)))
  ;[1 0 0.3516] Check if combat
  (`|ExecutionSequence`
    (:`then_0`
      (bind _output_get (set `self.IsCombat?` (> _returnvalue 0)))
      (if _output_get
        (bind _asnew_game_mode_gm (cast `/Game/Resources/Characters/Player/Blueprints/NewGameMode_GM` (`GameplayStatics.GetGameMode`)))
        (`/Game/Resources/Widgets/HUD_Widget.DisableInteract` (`/Game/Resources/Characters/Player/Blueprints/NewGameMode_GM.HUD_ref` _asnew_game_mode_gm))
        (else
          (bind _asnew_game_mode_gm_2 (cast `/Game/Resources/Characters/Player/Blueprints/NewGameMode_GM` (`GameplayStatics.GetGameMode`)))
          (`/Game/Resources/Widgets/HUD_Widget.EnableInteract` (`/Game/Resources/Characters/Player/Blueprints/NewGameMode_GM.HUD_ref` _asnew_game_mode_gm_2)))))
    (:`then_1`
      (bind _asnew_game_mode_gm_3 (cast `/Game/Resources/Characters/Player/Blueprints/NewGameMode_GM` (`GameplayStatics.GetGameMode`)))
      (set `/Game/Resources/Characters/Player/Blueprints/NewGameMode_GM.CombatMode` (>= _returnvalue 2) _asnew_game_mode_gm_3))))

(fn `Apply Loadout`
  (params (Loadout :type "/Game/Resources/Characters/Modules/ModuleLoadout_Struct Structure"))
  (bind _asbp_player_character (cast `/Game/Resources/Characters/Player/Blueprints/BP_PlayerCharacter` (`GameplayStatics.GetPlayerPawn` 0)))
  (bind _sword (`/Game/Resources/Characters/Player/Blueprints/BP_PlayerCharacter.Sword` _asbp_player_character))
  (`/Engine/EditorBlueprintResources/StandardMacros.IsValid` _sword
    (:`Is Valid`
      (`/Game/Resources/Characters/Weapons/Sword/VITA_BP.Apply Loadout` _sword Loadout))))

(fn `Check Crafting`
  (params (Name :type Name))
  (returns (`Can Update` :type Boolean))
  (bind (_value _returnvalue) (`BlueprintMapLibrary.Map_Find` (`self.ModuleCollection`) Name))
  (bind _returnvalue_2 (`|GetDataTableRow` "/Game/Resources/Characters/Modules/ModuleInfo_DT.ModuleInfo_DT" Name)
    (:`then`
      (return (and _returnvalue (>= (break `/Game/Resources/Characters/Modules/ModuleCollection_Struct` _value) (`.Level1_31_F549955C417A318510FC59B0C3338F54` (break `/Game/Resources/Characters/Modules/ModuleInfo_Struct` _returnvalue_2))))))))

(fn `Check Inventory Module Avaliability`
  (params (Name :type Name))
  (returns (Avaliable :type Boolean))
  (bind (_value _returnvalue) (`BlueprintMapLibrary.Map_Find` (`self.ModuleCollection`) Name))
  (if _returnvalue
    (if (>= (`.Avaliable_10_EF681991451349B4AD0BC096DC322166` (break `/Game/Resources/Characters/Modules/ModuleCollection_Struct` _value)) 1)
      (return true)
      (else
        _)))
  (return false))

(fn `Check Slot`
  (params (Position :type Integer))
  (returns (Empty :type Boolean))
  (bind _vitaslots (`self.VitaSlots`))
  (bind (_output_type _output_ref) (break `/Game/Resources/Characters/Modules/ModuleInventory_Struct` (`|GetArrayItem` _vitaslots)))
  (if (`KismetArrayLibrary.Array_IsValidIndex` _vitaslots Position)
    (`/Engine/EditorBlueprintResources/StandardMacros.IsValid` _output_ref
      (:`Is Valid`
        (return false))
      (:`Is Not Valid`
        (return true)))
    (else
      (return false))))

(fn `Check Slots`
  (params (Position :type Integer) (Slot :type Integer))
  (returns (Empty :type Boolean))
  (bind _vitaslots (`self.VitaSlots`))
  ;[1 0 0.5625] Manual Center Check
  (if (and (< Position 5) (> (+ Position Slot) 5))
    (return false)
    (else
      (for _index (range Slot)
        (bind _returnvalue (+ _index Position))
        (if (`KismetArrayLibrary.Array_IsValidIndex` _vitaslots _returnvalue)
          (bind (_output_type _output_ref) (break `/Game/Resources/Characters/Modules/ModuleInventory_Struct` (`|GetArrayItem` _vitaslots _returnvalue)))
          (`/Engine/EditorBlueprintResources/StandardMacros.IsValid` _output_ref
            (:`Is Valid`
              (return false)))
          (else
            (return false))))
      (return true))))

(fn `CountModules`
  (returns (`Module Count` :type Integer) (`Charge Count` :type Integer))
  (locals (Count :type Integer) (ChargeCount :type Integer))
  (set `local.Count` 0)
  (set `local.ChargeCount` 0)
  (for _array_element (`self.VitaInstalled`)
    (bind _returnvalue (`|GetDataTableRow` "/Game/Resources/Characters/Modules/ModuleInfo_DT.ModuleInfo_DT" (break `/Game/Resources/Characters/Modules/ModuleInventory_Struct` _array_element))
      (:`then`
        (set `local.Count` (+ (`.Slot_21_1D7852C84A7ECB8AAF7305AE36820569` (break `/Game/Resources/Characters/Modules/ModuleInfo_Struct` _returnvalue)) (`local.Count`)))
        (if (`KismetSystemLibrary.IsValidClass` (`.Buildable_12_952B647D4466188B0B8913A0526CC98B` (break `/Game/Resources/Characters/Modules/ModuleInfo_Struct` _returnvalue)))
          (set `local.ChargeCount` (+ (`.Slot_21_1D7852C84A7ECB8AAF7305AE36820569` (break `/Game/Resources/Characters/Modules/ModuleInfo_Struct` _returnvalue)) (`local.ChargeCount`)))))))
  (bind _output_get (set `self.LastModuleCount` (`local.Count`)))
  (bind _output_get_2 (set `self.LastChargeCount` (`local.ChargeCount`)))
  (`KismetSystemLibrary.PrintString` (`KismetTextLibrary.Conv_TextToString` (`|FormatText` "CHARGE IS {num}" _output_get_2)))
  (return _output_get _output_get_2))

(fn `Craft Module`
  (params (`Module Name` :type Name))
  (returns (Done :type Boolean))
  (bind _value (`BlueprintMapLibrary.Map_Find` (`self.ModuleCollection`) (`local.Module Name`)))
  (if (`BlueprintMapLibrary.Map_Contains` (`self.ModuleCollection`) `Module Name`)
    (bind _returnvalue (`|GetDataTableRow` "/Game/Resources/Characters/Modules/ModuleInfo_DT.ModuleInfo_DT" (`local.Module Name`))
      (:`then`
        (if (>= (break `/Game/Resources/Characters/Modules/ModuleCollection_Struct` (`BlueprintMapLibrary.Map_Find` (`self.ModuleCollection`) `Module Name`)) (`.Level1_31_F549955C417A318510FC59B0C3338F54` (break `/Game/Resources/Characters/Modules/ModuleInfo_Struct` _returnvalue)))
          (`BlueprintMapLibrary.Map_Add` (`self.ModuleCollection`) (`local.Module Name`) (make `/Game/Resources/Characters/Modules/ModuleCollection_Struct` (- (break `/Game/Resources/Characters/Modules/ModuleCollection_Struct` _value) (`.Level1_31_F549955C417A318510FC59B0C3338F54` (break `/Game/Resources/Characters/Modules/ModuleInfo_Struct` _returnvalue))) (+ (`.Avaliable_10_EF681991451349B4AD0BC096DC322166` (break `/Game/Resources/Characters/Modules/ModuleCollection_Struct` _value)) 1) (`.Installed_9_818FED464A6562A3282B64BCF64F96CD` (break `/Game/Resources/Characters/Modules/ModuleCollection_Struct` _value))))
          (return true)
          (else
            (return false)))))
    (else
      (return false))))

(fn `Get Flag`
  (params (Key :type "Name (by ref)"))
  (returns (Value :type Boolean))
  (bind (_value _returnvalue) (`BlueprintMapLibrary.Map_Find` (`self.Flags`) Key))
  (if _returnvalue
    (return _value)
    (else
      (return false))))

(fn `Increase Chunk`
  (`/Engine/EditorBlueprintResources/StandardMacros.IncrementInt` (`self.CurrentChunk`)))

(fn `Load Loadout`
  (params (Index :type Integer))
  (`self.Apply Loadout` (`|GetArrayItem` (`self.SavedLoadout`) Index)))

(fn `Save Loadout`
  (params (Index :type Integer))
  (locals (Loadout :type "Array of /Game/Resources/Characters/Modules/ModuleSave_Struct Structure"))
  (`KismetArrayLibrary.Array_Clear` (`local.Loadout`))
  (for _array_element (`self.VitaInstalled`)
    (`KismetArrayLibrary.Array_Add` (`local.Loadout`) (make `/Game/Resources/Characters/Modules/ModuleSave_Struct` (break `/Game/Resources/Characters/Modules/ModuleInventory_Struct` _array_element) (`/Game/Resources/Characters/Modules/ModuleBase_BP.Position` (`.Ref_13_681E062642B3B066754CCDAFCC922AF4` (break `/Game/Resources/Characters/Modules/ModuleInventory_Struct` _array_element))))))
  (`KismetArrayLibrary.Array_Set` (`self.SavedLoadout`) Index (make `/Game/Resources/Characters/Modules/ModuleLoadout_Struct` (`local.Loadout`))))

(fn `Set Flag`
  (params (Key :type "Name (by ref)") (Value :type "Boolean (by ref)") (`Autosave?` :type Boolean))
  (`BlueprintMapLibrary.Map_Add` (`self.Flags`) Key Value)
  ;[1 0 0.4922] Auto Save only the change variable
  (if `Autosave?`
    (bind _returnvalue (`GameplayStatics.DoesSaveGameExist` (`self.SlotName`)))
    (if _returnvalue
      (bind _returnvalue_2 (`GameplayStatics.LoadGameFromSlot` (`self.SlotName`)))
      (bind _asnew_save_game (cast `/Game/Resources/Characters/Player/Blueprints/Save/NewSaveGame` _returnvalue_2))
      (`BlueprintMapLibrary.Map_Add` (`/Game/Resources/Characters/Player/Blueprints/Save/NewSaveGame.Flags` _asnew_save_game) Key Value)
      (`GameplayStatics.SaveGameToSlot` _asnew_save_game (`self.SlotName`)))))

(fn `UserConstructionScript`)