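; TempTutorial_BP is a temporary tutorial that shows a sequence of on-screen input hints to the player.
; Three seconds after BeginPlay, it sends the current List entry's text and button to the game mode's HUD, targeting the player's Sword.
; Deploy, heavy attack, light attack, dash and edit-mode inputs advance Index when their display name matches the entry's Action.
; Each advance clears the hint, then shows the next after a short delay until List ends.
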(event `self.ReceiveBeginPlay`
  (bind (_output_text _output_button) (break `/Game/Resources/Characters/Player/Blueprints/Tutorial_Struct` (`|GetArrayItem` (`self.List`) (`self.Index`))))
  (`KismetSystemLibrary.Delay` 3.0)
  (bind _asnew_game_mode_gm (cast `/Game/Resources/Characters/Player/Blueprints/NewGameMode_GM` (`GameplayStatics.GetGameMode`) :!label _label))
  (`/Game/Resources/Widgets/HUD_Widget.Set Interactable` (`/Game/Resources/Characters/Player/Blueprints/NewGameMode_GM.HUD_ref` _asnew_game_mode_gm) true (`KismetSystemLibrary.MakeLiteralText` _output_text) _output_button (`/Game/Resources/Characters/Player/Blueprints/BP_PlayerCharacter.Sword` (cast `/Game/Resources/Characters/Player/Blueprints/BP_PlayerCharacter` (`GameplayStatics.GetPlayerPawn` 0) :!pure true))))

(event `self.ReceiveTick`
  (params (DeltaSeconds :type "Float (single-precision)")))

(event `EnhancedInput|/Game/Resources/Characters/Player/Input/Actions/IA_Deploy`
  (params (ActionValue :type Boolean) (ElapsedSeconds :type "Float (double-precision)") (TriggeredSeconds :type "Float (double-precision)") (InputAction :type "InputAction Object Reference" :default "/Game/Resources/Characters/Player/Input/Actions/IA_Deploy.IA_Deploy"))
  (bind (_output_text _output_button _output_action) (break `/Game/Resources/Characters/Player/Blueprints/Tutorial_Struct` (`|GetArrayItem` (`self.List`) (`self.Index`))))
  (:`Completed`
    (if (`KismetStringLibrary.EqualEqual_StrStr` (`KismetSystemLibrary.GetDisplayName` InputAction) _output_action)
      (bind _result (`/Engine/EditorBlueprintResources/StandardMacros.IncrementInt` (`self.Index`) :!label _label_2)
        (:`  `
          (if (<= _result (`KismetArrayLibrary.Array_LastIndex` (`self.List`)))
            (bind _asnew_game_mode_gm (cast `/Game/Resources/Characters/Player/Blueprints/NewGameMode_GM` (`GameplayStatics.GetGameMode`)))
            (`/Game/Resources/Widgets/HUD_Widget.Set Interactable` (`/Game/Resources/Characters/Player/Blueprints/NewGameMode_GM.HUD_ref` _asnew_game_mode_gm) false "" "r" null)
            (`KismetSystemLibrary.Delay` 0.5)
            (goto _label)
            (else
              (bind _asnew_game_mode_gm_2 (cast `/Game/Resources/Characters/Player/Blueprints/NewGameMode_GM` (`GameplayStatics.GetGameMode`)))
              (`/Game/Resources/Widgets/HUD_Widget.Set Interactable` (`/Game/Resources/Characters/Player/Blueprints/NewGameMode_GM.HUD_ref` _asnew_game_mode_gm_2) false "" "r" null))))))))

(event `EnhancedInput|/Game/Resources/Characters/Player/Input/Actions/IA_HeavyAttack`
  (params (ActionValue :type Boolean) (ElapsedSeconds :type "Float (double-precision)") (TriggeredSeconds :type "Float (double-precision)") (InputAction :type "InputAction Object Reference" :default "/Game/Resources/Characters/Player/Input/Actions/IA_HeavyAttack.IA_HeavyAttack"))
  (bind (_output_text _output_button _output_action) (break `/Game/Resources/Characters/Player/Blueprints/Tutorial_Struct` (`|GetArrayItem` (`self.List`) (`self.Index`))))
  (:`Completed`
    (if (`KismetStringLibrary.EqualEqual_StrStr` (`KismetSystemLibrary.GetDisplayName` InputAction) _output_action)
      (goto _label_2))))

(event `EnhancedInput|/Game/Resources/Characters/Player/Input/Actions/IA_LightAttack`
  (params (ActionValue :type Boolean) (ElapsedSeconds :type "Float (double-precision)") (TriggeredSeconds :type "Float (double-precision)") (InputAction :type "InputAction Object Reference" :default "/Game/Resources/Characters/Player/Input/Actions/IA_LightAttack.IA_LightAttack"))
  (bind (_output_text _output_button _output_action) (break `/Game/Resources/Characters/Player/Blueprints/Tutorial_Struct` (`|GetArrayItem` (`self.List`) (`self.Index`))))
  (:`Completed`
    (if (`KismetStringLibrary.EqualEqual_StrStr` (`KismetSystemLibrary.GetDisplayName` InputAction) _output_action)
      (goto _label_2))))

(event `EnhancedInput|/Game/Resources/Characters/Player/Input/Actions/IA_Dashing`
  (params (ActionValue :type Boolean) (ElapsedSeconds :type "Float (double-precision)") (TriggeredSeconds :type "Float (double-precision)") (InputAction :type "InputAction Object Reference" :default "/Game/Resources/Characters/Player/Input/Actions/IA_Dashing.IA_Dashing"))
  (bind (_output_text _output_button _output_action) (break `/Game/Resources/Characters/Player/Blueprints/Tutorial_Struct` (`|GetArrayItem` (`self.List`) (`self.Index`))))
  (:`Completed`
    (if (`KismetStringLibrary.EqualEqual_StrStr` (`KismetSystemLibrary.GetDisplayName` InputAction) _output_action)
      (goto _label_2))))

(event `EnhancedInput|/Game/Resources/Characters/Player/Input/Actions/IA_EditMode`
  (params (ActionValue :type Boolean) (ElapsedSeconds :type "Float (double-precision)") (TriggeredSeconds :type "Float (double-precision)") (InputAction :type "InputAction Object Reference" :default "/Game/Resources/Characters/Player/Input/Actions/IA_EditMode.IA_EditMode"))
  (bind (_output_text _output_button _output_action) (break `/Game/Resources/Characters/Player/Blueprints/Tutorial_Struct` (`|GetArrayItem` (`self.List`) (`self.Index`))))
  (:`Completed`
    (if (`KismetStringLibrary.EqualEqual_StrStr` (`KismetSystemLibrary.GetDisplayName` InputAction) _output_action)
      (goto _label_2))))

(fn `UserConstructionScript`)