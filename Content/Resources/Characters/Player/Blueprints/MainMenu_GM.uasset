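; Main menu Game Mode that shows the menu and handles starting a new game or continuing a saved one.
; BeginPlay adds the menu widget, starts the FMOD menu music and switches to UI-only input with a visible cursor.
; Both game events stop the music: Continue opens the map stored in the save slot, while New Game deletes the slot and opens HubBackup.
; A disconnected save-creation chain never runs.
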(event `self.ReceiveBeginPlay`
  (bind _returnvalue (`GameplayStatics.GetPlayerController` 0))
  (`|ExecutionSequence`
    (:`then_0`
      (bind _returnvalue_2 (`|CreateWidget` "/Game/Resources/Widgets/MainMenu_Widget.MainMenu_Widget_C"))
      (bind _output_get (set `self.HUD_ref` _returnvalue_2))
      (`UserWidget.AddToViewport` _output_get 0))
    (:`then_1`
      (bind _returnvalue_3 (`FMODBlueprintStatics.PlayEvent2D` "/Game/FMOD/Events/BGM/Menu_BGM.Menu_BGM"))
      (set `self.BGM_ref` _returnvalue_3))
    (:`then_2`
      (`WidgetBlueprintLibrary.SetInputMode_UIOnlyEx` _returnvalue (`self.HUD_ref`))
      (set `PlayerController.bShowMouseCursor` true _returnvalue))))

(event `ContinueGame`
  (`FMODBlueprintStatics.EventInstanceStop` (`self.BGM_ref`))
  (bind _returnvalue (`GameplayStatics.LoadGameFromSlot` (`self.Slot Name`)))
  (bind _asnew_save_game (cast `/Game/Resources/Characters/Player/Blueprints/Save/NewSaveGame` _returnvalue))
  (`GameplayStatics.OpenLevel` (`KismetStringLibrary.Conv_StringToName` (`/Game/Resources/Characters/Player/Blueprints/Save/NewSaveGame.CurrentMap` _asnew_save_game))))

(event `NewGame`
  (`FMODBlueprintStatics.EventInstanceStop` (`self.BGM_ref`))
  (`GameplayStatics.DeleteGameInSlot` (`self.Slot Name`))
  (`GameplayStatics.OpenLevel` "HubBackup"))

(fn `UserConstructionScript`)