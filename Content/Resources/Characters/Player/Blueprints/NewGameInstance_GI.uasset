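; Game instance Blueprint that links the music and sound volume settings to FMOD audio buses.
; On Init it registers a float CVar setting for each, keeping any already registered value or defaulting to full volume.
; Change callbacks, also fired immediately on registration, set the volume of the BGM and Sounds buses, so saved or edited values apply directly to the mix.
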(event `self.ReceiveInit`
  (`SettingsManager.RegisterFloatCVarSettingWithCallback` "Game.Audio.Music" (`KismetMathLibrary.SelectFloat` (`ConsoleUtils.GetFloatCVar` "Game.Audio.Music") 1.0 (`ConsoleUtils.IsCVarRegistered` "Game.Audio.Music")) "FMOD Master Audio" (delegate `On Music Audio Changed`) true)
  (`SettingsManager.RegisterFloatCVarSettingWithCallback` "Game.Audio.Sound" (`KismetMathLibrary.SelectFloat` (`ConsoleUtils.GetFloatCVar` "Game.Audio.Sound") 1.0 (`ConsoleUtils.IsCVarRegistered` "Game.Audio.Sound")) "FMOD Master Audio" (delegate `On Sound Audio Changed`) true))

(event `On Music Audio Changed`
  (params (NewValue :type "Float (single-precision)"))
  (`FMODBlueprintStatics.BusSetVolume` "/Game/FMOD/Buses/BGM.BGM" NewValue))

(event `On Sound Audio Changed`
  (params (NewValue :type "Float (single-precision)"))
  (`FMODBlueprintStatics.BusSetVolume` "/Game/FMOD/Buses/Sounds.Sounds" NewValue))