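; MusicArea_BP is a box trigger volume that sets the game's current music for the area the player is in.
; When BP_PlayerCharacter enters the box, it writes its NewMusic value to CurrentMusic on NewGameMode_GM, and on exit it resets that to the first enum entry.
; A next-tick check on BeginPlay applies the music if the player already starts inside the box.
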(event `self.ReceiveBeginPlay`
  (`KismetSystemLibrary.DelayUntilNextTick`)
  (if (> (`KismetArrayLibrary.Array_Length` (`PrimitiveComponent.GetOverlappingActors` (`self.Box`) "/Game/Resources/Characters/Player/Blueprints/BP_PlayerCharacter.BP_PlayerCharacter_C")) 0)
    (bind _asnew_game_mode_gm (cast `/Game/Resources/Characters/Player/Blueprints/NewGameMode_GM` (`GameplayStatics.GetGameMode`) :!label _label))
    (set `/Game/Resources/Characters/Player/Blueprints/NewGameMode_GM.CurrentMusic` (`self.NewMusic`) _asnew_game_mode_gm)))

(event `self.Box.OnComponentBeginOverlap`
  (params (OverlappedComponent :type "PrimitiveComponent Object Reference") (OtherActor :type "Actor Object Reference") (OtherComp :type "PrimitiveComponent Object Reference") (OtherBodyIndex :type Integer) (bFromSweep :type Boolean) (SweepResult :type "HitResult Structure (by ref)"))
  (cast `/Game/Resources/Characters/Player/Blueprints/BP_PlayerCharacter` OtherActor)
  (goto _label))

(event `self.Box.OnComponentEndOverlap`
  (params (OverlappedComponent :type "PrimitiveComponent Object Reference") (OtherActor :type "Actor Object Reference") (OtherComp :type "PrimitiveComponent Object Reference") (OtherBodyIndex :type Integer))
  (cast `/Game/Resources/Characters/Player/Blueprints/BP_PlayerCharacter` OtherActor)
  (bind _asnew_game_mode_gm (cast `/Game/Resources/Characters/Player/Blueprints/NewGameMode_GM` (`GameplayStatics.GetGameMode`)))
  (set `/Game/Resources/Characters/Player/Blueprints/NewGameMode_GM.CurrentMusic` "NewEnumerator0" _asnew_game_mode_gm))

(fn `UserConstructionScript`)