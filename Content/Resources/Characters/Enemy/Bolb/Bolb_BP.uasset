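; Bolb enemy with a gravity-free physics body that follows a control target, two fins driven toward the body, and a two-layer potion-liquid look.
; Physics Control drives body and fins, while Tick eases liquid distortion toward CalculateKnetic, whose velocity-based math is left unconnected.
; Knockback zeroes the body control, applies an impulse that ignores Causer, then restores control multipliers through a timeline.
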(event `self.ReceiveBeginPlay`
  (bind _body (`self.Body`))
  (`|ExecutionSequence`
    (:`then_0`
      (bind _returnvalue (`PrimitiveComponent.CreateDynamicMaterialInstance` (`self.Outer`) 0 "/Game/PotionLiquidSim/PotionBottle/Materials/MI_TransparentPotionLiquid_Outer.MI_TransparentPotionLiquid_Outer" "None"))
      (bind _returnvalue_2 (`PrimitiveComponent.CreateDynamicMaterialInstance` (`self.Inner`) 0 "/Game/PotionLiquidSim/PotionBottle/Materials/MI_TransparentPotionLiquid_Inner.MI_TransparentPotionLiquid_Inner" "None"))
      (bind _output_get (set `self.Mat_liquid1` _returnvalue))
      (bind _output_get_2 (set `self.Mat Liquid 2` _returnvalue_2))
      (`MaterialInstanceDynamic.SetScalarParameterValue` _output_get_2 "Distortion Amount" 0.05)
      (`MaterialInstanceDynamic.SetScalarParameterValue` _output_get "Distortion Amount" 0.05)
      (`MaterialInstanceDynamic.SetScalarParameterValue` (`self.Mat_liquid1`) "Fill Amount" 0.55)
      (`MaterialInstanceDynamic.SetScalarParameterValue` (`self.Mat Liquid 2`) "Fill Amount" 0.55))
    (:`then_1`
      (bind _returnvalue_3 (`PhysicsControlComponent.MakeControl` :`self` (`self.PhysicsControl`) :`ChildMeshComponent` _body :`ControlData` (make `PhysicsControlData` 1.0 1.0 0.05 0.0 1.0 1.0 0.05)))
      (`PhysicsControlComponent.MakeBodyModifier` (`self.PhysicsControl`) _body "None" "Simulated" "QueryAndPhysics" 0.0 true)
      (`PhysicsControlComponent.MakeNamedControl` :`self` (`self.PhysicsControl`) :`Name` "FinL" :`ChildMeshComponent` (`self.FinR`) :`ControlData` (make `PhysicsControlData` 1.0 1.0 0.0 0.0 5.0))
      (`PhysicsControlComponent.MakeNamedControl` :`self` (`self.PhysicsControl`) :`Name` "FinR" :`ChildMeshComponent` (`self.FinL`) :`ControlData` (make `PhysicsControlData` 1.0 1.0 0.0 0.0 5.0)))))

(event `self.ReceiveTick`
  (params (DeltaSeconds :type "Float (single-precision)"))
  (bind _body (`self.Body`))
  (bind _physicscontrol (`self.PhysicsControl`))
  (bind _body_2 (`self.Body`))
  (bind _returnvalue (`SceneComponent.K2_GetComponentLocation` _body_2))
  (bind (_returnvalue_location _returnvalue_rotation) (`KismetMathLibrary.BreakTransform` (`SceneComponent.K2_GetComponentToWorld` (`self.control_target`))))
  (bind _returnvalue_2 (`SceneComponent.K2_GetComponentRotation` _body_2))
  (bind _output_get (set `self.Current_Distortion` (`KismetMathLibrary.FInterpTo` (`self.Current_Distortion`) (+ (`KismetMathLibrary.FClamp` (/ (`KismetMathLibrary.VSize` (`PrimitiveComponent.GetPhysicsAngularVelocityInRadians` _body "None")) 30.0)) (`KismetMathLibrary.FClamp` (/ (`KismetMathLibrary.VSize` (`SceneComponent.GetComponentVelocity` _body)) 1500.0) 0.01)) DeltaSeconds 0.8)))
  (`MaterialInstanceDynamic.SetScalarParameterValue` (`self.Mat_liquid1`) "Distortion Amount" _output_get)
  (`MaterialInstanceDynamic.SetScalarParameterValue` (`self.Mat Liquid 2`) "Distortion Amount" _output_get)
  (`PhysicsControlComponent.SetControlTargetPositionAndOrientation` _physicscontrol (stale `self.ReceiveBeginPlay` _returnvalue_3) _returnvalue_location _returnvalue_rotation 0.0 false false)
  (`PhysicsControlComponent.SetControlTargetPositionAndOrientation` _physicscontrol "FinL" _returnvalue _returnvalue_2 0.0 true false)
  (`PhysicsControlComponent.SetControlTargetPositionAndOrientation` (`self.PhysicsControl`) "FinR" _returnvalue _returnvalue_2 0.0 true false)
  (`PhysicsControlComponent.SetBodyModifierKinematicTarget` :`self` (`self.PhysicsControl`) :`Name` "Body_0" :`KinematicTargetPosition` _returnvalue_location))

(event `Knockback`
  (params (Causer :type "Actor Object Reference") (Force :type "Float (double-precision)") (Height :type "Float (double-precision)"))
  (bind (_returnvalue_x _returnvalue_y) (`KismetMathLibrary.BreakVector` (`KismetMathLibrary.GetForwardVector` (`KismetMathLibrary.FindLookAtRotation` (`self.K2_GetActorLocation`) (`self.K2_GetActorLocation`)))))
  ;[0.1484 1 0] Knockback Event
  (`PhysicsControlComponent.SetControlMultipliers` (`self.PhysicsControl`) (stale `self.ReceiveBeginPlay` _returnvalue_3) (make `PhysicsControlMultipliers` (0.0 0.0 0.0) (0.0 0.0 0.0) (1.0 1.0 1.0) 0.0) true)
  (`PrimitiveComponent.AddImpulse` (`self.Body`) (+ (* (`KismetMathLibrary.MakeVector` _returnvalue_x _returnvalue_y) Force) Height) "None" true)
  (bind (_direction _newtrack_0) (`Timeline|Timeline` :!via `PlayFromStart`)
    (:`Update`
      (bind _returnvalue (`KismetMathLibrary.Conv_DoubleToVector` _newtrack_0))
      (`PhysicsControlComponent.SetControlMultipliers` (`self.PhysicsControl`) (stale `self.ReceiveBeginPlay` _returnvalue_3) (make `PhysicsControlMultipliers` _returnvalue _returnvalue (1.0 1.0 1.0) _newtrack_0 _newtrack_0) true))))

(fn `UserConstructionScript`)