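; Fish enemy Blueprint, an enemy-base child that steers toward a point above the player every tick; Move adds input when within range.
; LightAttack shows a camera-facing telegraph burst with a sound, then after delays notifies the behavior tree it finished, as does CancelAttack.
; Parry tilts the target rotation, plays a damage-driven hit sound and knocks the fish upward.
; The Attack timeline's sphere-trace damage is wired, but the timeline is only ever stopped here.
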(event `self.ReceiveBeginPlay`
  (`parent.ReceiveBeginPlay`))

(event `self.ReceiveTick`
  (params (DeltaSeconds :type "Float (single-precision)"))
  (`parent.ReceiveTick` DeltaSeconds)
  (`self.AddMovementInput` (`KismetMathLibrary.GetForwardVector` (`KismetMathLibrary.FindLookAtRotation` (`self.K2_GetActorLocation`) (+ (`self.K2_GetActorLocation` (`GameplayStatics.GetPlayerPawn` 0)) (0.0 0.0 200.0)))) :!label _label))

(event `Move`
  (if (<= (`self.GetDistanceTo` (`GameplayStatics.GetPlayerPawn` 0) self) 3000.0)
    (goto _label)))

(event `self.LightAttack`
  (bind _returnvalue (+ (`self.K2_GetActorLocation`) (0.0 0.0 50.0)))
  (`parent.LightAttack`)
  (`NiagaraFunctionLibrary.SpawnSystemAtLocation` "/Game/Resources/VFX/Brust_NS.Brust_NS" _returnvalue (`KismetMathLibrary.FindLookAtRotation` _returnvalue (`PlayerCameraManager.GetCameraLocation` (`GameplayStatics.GetPlayerCameraManager` 0))))
  (`FMODBlueprintStatics.PlayEventAttached` "/Game/FMOD/Events/Sounds/Enemy/Enemy_Hint.Enemy_Hint" (`self.Mesh`) "None" (0.0 0.0 0.0) "SnapToTarget")
  ;[0.9688 1 0] Code for attacking that was in EnemyBase_BP
  (`KismetSystemLibrary.Delay` 0.6)
  (`KismetSystemLibrary.Delay` 2.0)
  ;;[1 0 0.5391] Used to notify behavior tree
  (`self.AttackFinishedDispatcher` :!label _label_2)
  (`KismetSystemLibrary.PrintString` "Finished Attacking" true true (struct :`R` 1.0 :`G` 0.963927 :`A` 1.0)))

(event `self.CancelAttack`
  (bind _returnvalue (`self.K2_GetActorLocation`))
  ;[0.9688 1 0] Code for attacking that was in EnemyBase_BP
  (`parent.CancelAttack`)
  (`|ExecutionSequence`
    (:`then_0`
      (`Timeline|Attack` :!via `Stop`
        (:`Finished`
          (goto _label_2))
        (:`Event`
          (`|ExecutionSequence`
            (:`then_0`
              (bind (_outhits _returnvalue_2) (`KismetSystemLibrary.SphereTraceMulti` _returnvalue _returnvalue 300.0 "TraceTypeQuery4"))
              (if _returnvalue_2
                (for _array_element _outhits
                  (`GameplayStatics.ApplyDamage` (`.HitActor` (`GameplayStatics.BreakHitResult` _array_element)) 100.0 (`self.GetController`) self "/Script/Engine.DamageType")
                  (break))))
            (:`then_1`
              (`FMODBlueprintStatics.PlayEventAttached` "/Game/FMOD/Events/Sounds/Enemy/Enemy_Attack.Enemy_Attack" (`self.Mesh`) "None" (0.0 0.0 0.0) "SnapToTarget"))))))
    (:`then_1`
      (goto _label_2))))

(event `/Game/Resources/Characters/Player/Blueprints/Parry_BPInter.Apply Parry`
  (params (Causer :type "Actor Object Reference") (Damage :type "Float (double-precision)"))
  (`KismetSystemLibrary.PrintString` "PARRY!!!!" true true (struct :`R` 1.0 :`G` 0.607333 :`B` 0.167448 :`A` 1.0))
  (set `self.TargetRotation` (struct :`Pitch` 60.0))
  (bind _returnvalue (`FMODBlueprintStatics.PlayEventAttached` "/Game/FMOD/Events/Sounds/Enemy/Enemy_Hit.Enemy_Hit" (`self.Mesh`) "None" (0.0 0.0 0.0) "SnapToTarget"))
  (`FMODAudioComponent.SetParameter` _returnvalue "Damage" Damage)
  (`self.Apply Knockback` Causer 0.0 200.0))

(fn `UserConstructionScript`
  (`parent.UserConstructionScript`))