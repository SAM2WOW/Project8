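; BundleSpawner_BP is an enemy spawner that carries a ring of SpawnerCable_BP actors and bursts on interaction.
; On BeginPlay it spawns the cables with random enemy labels and spaces their Cylinder1 components evenly in an elevated circle.
; Tick slowly yaws each cable.
; MsgInteract swaps the sphere for an exploded destructible, fires a radial impulse, then forwards the interaction to each cable through a delayed loop.
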(event EventBeginPlay
  (bind _returnvalue (Transformation|GetActorTransform))
  (for _index (range 0 (- (Variables|Default|GetAmount) 1))
    (bind _returnvalue_2 (Game|SpawnActorfromClass "/Game/Resources/Characters/Enemy/Spawner/SpawnerCable_BP.SpawnerCable_BP_C" (Math|Transform|MakeTransform (.location _returnvalue) (.rotation _returnvalue) "1.000000,1.000000,1.000000") "Undefined" 0 false (.OutItem (Utilities|Array|Random (Variables|Default|GetEnemyLabels))) false 0))
    (Transformation|SetWorldLocation (Variables|/Game/Resources/Characters/Enemy/Spawner/SpawnerCable_BP.SpawnerCable_BP_C|GetCylinder1 _returnvalue_2) (+ (Transformation|GetActorLocation) (Math|Vector|RotateVectorAroundAxis "320.000000,0.000000,1000.000000" (|((360/Total)*Index) (Math|Conversions|ToFloat(Integer) _index) (Math|Conversions|ToFloat(Integer) (Variables|Default|GetAmount))) (Math|Vector|VectorUp))) false false)
    (Utilities|Array|Add (Variables|Default|GetCables) _returnvalue_2)))

(event EventTick
  (params (DeltaSeconds :type Float%20%28single-precision%29))
  (for _array_element (Variables|Default|GetCables)
    (Transformation|AddActorLocalRotation _array_element (Math|Rotator|MakeRotator 0.0 0.0 (* DeltaSeconds 1e+01)) false false)))

(event EventMsgInteract
  (Rendering|SetVisibility (Variables|Default|GetSphere) false false)
  (Game|SpawnActorfromClass "/Game/Resources/Characters/Destructables/DestructableExploded_BP_Spawner.DestructableExploded_BP_Spawner_C" (Transformation|GetWorldTransform (Variables|Default|GetSphere)) "AlwaysSpawn" 0 0 0)
  (Components|Activation|SetActive (Variables|Default|GetRadialForce) true false)
  (Utilities|FlowControl|DelayUntilNextTick)
  (Class|RadialForceComponent|FireImpulse (Variables|Default|GetRadialForce))
  (bind _index (Utilities|ForLoopwithDelay 0 (- (Utilities|Array|Length (Variables|Default|GetCables)) 1) 0.2)
    (:Loop%20Body
      (Default|MsgInteract (Utilities|Array|Get(acopy) (Variables|Default|GetCables) _index)))
    (:Completed
      (Components|Activation|SetActive (Variables|Default|GetRadialForce) false false))))

(fn ConstructionScript)