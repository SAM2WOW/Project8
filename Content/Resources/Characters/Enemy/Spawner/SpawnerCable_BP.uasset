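; Enemy spawner that hangs a dormant, upside-down enemy from a cable until released.
; BeginPlay spawns it from EnemyLabel_DT by label, or randomly if flagged or not found, with AI unpossessed.
; Tick optionally sways the cable on an offset sine and pins the locked enemy to its Cube.
; MsgInteract, or player overlap when RangeStart is set, frees and possesses the enemy, plays an unplug sound and retracts the cable before destroying itself.
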(event `self.ReceiveBeginPlay`
  (bind _returnvalue (`self.GetTransform`))
  (bind _random (`self.Random`))
  (if _random
    (set `self.Random` true :!label _label)
    (bind _outrownames (`DataTableFunctionLibrary.GetDataTableRowNames` "/Game/Resources/Characters/Enemy/EnemyLabel_DT.EnemyLabel_DT"))
    (bind _returnvalue_2 (`|GetDataTableRow` "/Game/Resources/Characters/Enemy/EnemyLabel_DT.EnemyLabel_DT" (`KismetArrayLibrary.Array_Random` _outrownames))
      (:`then`
        _))
    (else
      (bind _returnvalue_3 (`|GetDataTableRow` "/Game/Resources/Characters/Enemy/EnemyLabel_DT.EnemyLabel_DT" (`self.EnemyLabel`))
        (:`then`
          _)
        (:`RowNotFound`
          (goto _label)))))
  (bind (_enemy _weapon _behavior) (break `/Game/Resources/Characters/Enemy/EnemyLabel_Struct` (select `bool` _random :`false` _returnvalue_3 :`true` _returnvalue_2)))
  (bind _returnvalue_4 (`|SpawnActorFromClass` _enemy (`KismetMathLibrary.MakeTransform` (.location _returnvalue) (`KismetMathLibrary.MakeRotator` 180.0 0.0 (.yaw (.rotation _returnvalue)))) "AlwaysSpawn" "OverrideRootScale" null 300.0 50.0 _behavior true _weapon (`self.EnemyLabel`) null))
  (bind _output_get (set `self.Enemy` _returnvalue_4))
  (`/Game/Resources/Characters/Enemy/EnemyBase_BP.ToggleBehaviorTree` _output_get)
  (`/Game/Resources/Characters/Enemy/EnemyBase_BP.PossessAI` _output_get false)
  (set `self.InitialOffset` (`KismetMathLibrary.RandomFloatInRange` 0.0 10.0)))

(event `/Game/Resources/Characters/Interactables/interactable_interface.msg_interact`
  (`|ExecutionSequence`
    (:`then_0`
      (bind (_direction _newtrack_0) (`Timeline|Timeline` :!via `PlayFromStart`)
        (:`Update`
          (`self.K2_AddActorLocalOffset` (`KismetMathLibrary.MakeVector` 0.0 0.0 (`KismetMathLibrary.Lerp` 0.0 1000.0 _newtrack_0))))
        (:`Finished`
          (`self.K2_DestroyActor`))))
    (:`then_1`
      (`KismetSystemLibrary.RetriggerableDelay` 0.2)
      (`self.K2_SetActorRotation` (`self.Enemy`) (`self.K2_GetActorRotation`) false)
      (set `self.Locked` false)
      (`/Game/Resources/Characters/Enemy/EnemyBase_BP.PossessAI` (`self.Enemy`) true)
      (`FMODBlueprintStatics.PlayEventAtLocation` "/Game/FMOD/Events/Sounds/Enemy/Enemy_Unplug.Enemy_Unplug" (`KismetMathLibrary.MakeTransform` (`SceneComponent.K2_GetComponentLocation` (`self.Cube`)))))))

(event `self.ReceiveTick`
  (params (DeltaSeconds :type "Float (single-precision)"))
  (bind _returnvalue (* (`KismetMathLibrary.Sin` (* (+ (`KismetSystemLibrary.GetGameTimeInSeconds`) (`self.InitialOffset`)) 1.0)) 60.0))
  (`|ExecutionSequence`
    (:`then_0`
      (if (`self.Moving`)
        (`SceneComponent.K2_SetRelativeLocation` (`self.Cylinder1`) (`KismetMathLibrary.MakeVector` _returnvalue 0.0 (+ _returnvalue 1000.0)) false false)))
    (:`then_1`
      (if (`self.Locked`)
        (`self.K2_SetActorLocation` (`self.Enemy`) (`SceneComponent.K2_GetComponentLocation` (`self.Cube`)) false false)))))

(event `self.Sphere.OnComponentBeginOverlap`
  (params (OverlappedComponent :type "PrimitiveComponent Object Reference") (OtherActor :type "Actor Object Reference") (OtherComp :type "PrimitiveComponent Object Reference") (OtherBodyIndex :type Integer) (bFromSweep :type Boolean) (SweepResult :type "HitResult Structure (by ref)"))
  (if (`self.Range Start`)
    (cast `/Game/Resources/Characters/Player/Blueprints/BP_PlayerCharacter` OtherActor)
    (`/Game/Resources/Characters/Interactables/interactable_interface.msg_interact`)))

(fn `UserConstructionScript`)