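; Enemy spawner actor that creates a JellyEnemy_BP at its Arrow component's location and rotation.
; It spawns on the interact message, or automatically on BeginPlay when AutoStart is set.
; Each spawn forwards the spawner's attack range, attack movement speed and initial weapons to the enemy, adjusting position if blocked but always spawning.
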(event `self.ReceiveBeginPlay`
  (if (`self.AutoStart`)
    (`self.msg_interact`)))

(event `self.msg_interact`
  (bind _arrow (`self.Arrow`))
  (`|SpawnActorFromClass` "/Game/Resources/Characters/Enemy/JellyEnemy_BP.JellyEnemy_BP_C" (`KismetMathLibrary.MakeTransform` (`SceneComponent.K2_GetComponentLocation` _arrow) (`SceneComponent.K2_GetComponentRotation` _arrow)) "AdjustIfPossibleButAlwaysSpawn" "OverrideRootScale" null (`self.Attack Range`) (`self.Attack Movement Speed`) false (`self.Initial Weapons`) null))

(fn `UserConstructionScript`)