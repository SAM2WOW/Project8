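; EnemySpawner_test_BP is a test enemy spawner that produces jelly enemies while the player overlaps it.
; Player overlap begin and end toggle a Spawning flag, which a looping timer started on BeginPlay checks every second.
; When the flag is set, it spawns a JellyEnemy_BP running the buildable-attacking melee behavior tree at a random horizontal offset around Sphere1, ignoring collision.
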(event `self.ReceiveBeginPlay`
  (`KismetSystemLibrary.K2_SetTimerDelegate` (delegate `Spawn`) 1.0 true))

(event `self.ReceiveActorBeginOverlap`
  (params (OtherActor :type "Actor Object Reference"))
  (cast `/Game/Resources/Characters/Player/Blueprints/BP_PlayerCharacter` OtherActor)
  (set `self.spawning` true))

(event `self.ReceiveActorEndOverlap`
  (params (OtherActor :type "Actor Object Reference"))
  (cast `/Game/Resources/Characters/Player/Blueprints/BP_PlayerCharacter` OtherActor)
  (set `self.spawning` false))

(event `Spawn`
  (if (`self.spawning`)
    (`AIBlueprintHelperLibrary.SpawnAIFromClass` "/Game/Resources/Characters/Enemy/JellyEnemy_BP.JellyEnemy_BP_C" "/Game/Resources/Characters/Enemy/BehaviorTrees/MeleeEnemyAttackBuildables_BT.MeleeEnemyAttackBuildables_BT" (+ (* (`KismetMathLibrary.RandomUnitVector`) (100.0 100.0 0.0)) (`SceneComponent.K2_GetComponentLocation` (`self.Sphere1`))) (struct) true null)))

(fn `UserConstructionScript`)