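; Flying fish enemy that homes in on the player and, at close range, fires timed WeaponManager attacks with a cooldown, using a weapon attached to its lower fin.
; A Physics Control makes the low-gravity body chase the capsule.
; Knockbacks and parries loosen that control, then a timeline restores it while pulling the actor to the body.
; Death disables AI, plays an emissive glow, then spawns debris and drops a module.
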(event `self.ReceiveBeginPlay`
  (bind _weaponslot (`self.weaponSlot`))
  (bind _body (`self.Body`))
  (bind (_output_weapon _output_modules) (break `/Game/Resources/Characters/Weapons/WeaponConfig_Struct` (`|GetArrayItem` (`self.InitialWeapons`))))
  (`parent.ReceiveBeginPlay`)
  (bind _returnvalue (`PhysicsControlComponent.MakeControl` :`self` (`self.PhysicsControl`) :`ChildMeshComponent` _body :`ControlData` (make `PhysicsControlData` 5.0 1.0 3.0 0.0 3.0)))
  (set `self.NewVar_0` _returnvalue)
  (`PhysicsControlComponent.MakeBodyModifier` (`self.PhysicsControl`) _body "None" "Simulated" "QueryAndPhysics" 0.2 false)
  ;[0 0.9062 1] Attach Weapons
  (bind _returnvalue_2 (`|SpawnActorFromClass` _output_weapon (`KismetMathLibrary.MakeTransform` (`SceneComponent.K2_GetComponentLocation` _weaponslot) (`SceneComponent.K2_GetComponentRotation` _weaponslot)) "Undefined" "OverrideRootScale" null _output_modules null))
  (`/Game/Resources/Characters/Weapons/WeaponManager_BPC.Add Weapon` (`self.WeaponManager_BPC`) _returnvalue_2)
  (`self.K2_AttachToComponent` _returnvalue_2 (`self.LowerFin`) "None" "KeepWorld" "KeepWorld" "KeepWorld" true)
  (`/Game/Resources/Characters/Weapons/WeaponManager_BPC.Update Locked Target` (`self.WeaponManager_BPC`) (`GameplayStatics.GetPlayerPawn` 0)))

(event `self.ReceiveAnyDamage`
  (params (Damage :type "Float (single-precision)") (DamageType :type "DamageType Object Reference") (InstigatedBy :type "Controller Object Reference") (DamageCauser :type "Actor Object Reference"))
  (bind _physicscontrol (`self.PhysicsControl`))
  (bind (_returnvalue_x _returnvalue_y) (`KismetMathLibrary.BreakVector` (`KismetMathLibrary.GetForwardVector` (`KismetMathLibrary.FindLookAtRotation` (`self.K2_GetActorLocation`) (`self.K2_GetActorLocation`)))))
  (`parent.ReceiveAnyDamage` Damage DamageType InstigatedBy DamageCauser)
  (`PhysicsControlComponent.SetControlMultipliers` _physicscontrol (`self.NewVar_0`) (make `PhysicsControlMultipliers` (0.1 0.1 0.1) (1.0 1.0 1.0) (1.0 1.0 1.0) 0.0) false)
  (`PrimitiveComponent.AddImpulse` (`self.Body`) (+ (* (`KismetMathLibrary.MakeVector` _returnvalue_x _returnvalue_y) (200.0 200.0 100.0)) (0.0 0.0 0.0)) "None" false)
  (`KismetSystemLibrary.RetriggerableDelay` 0.2)
  (if (not (`self.stunned`))
    (`PhysicsControlComponent.SetControlMultipliers` _physicscontrol (`self.NewVar_0`) (make `PhysicsControlMultipliers` (1.0 1.0 1.0)) false)))

(event `self.ReceiveTick`
  (params (DeltaSeconds :type "Float (single-precision)"))
  (bind _returnvalue (`GameplayStatics.GetPlayerPawn` 0))
  (bind _capsulecomponent (`self.CapsuleComponent`))
  (bind _returnvalue_2 (> (`self.GetDistanceTo` _returnvalue) 450.0))
  (`parent.ReceiveTick` DeltaSeconds)
  (`|ExecutionSequence`
    (:`then_0`
      (`PhysicsControlComponent.SetControlTargetPositionAndOrientation` (`self.PhysicsControl`) (`self.NewVar_0`) (`SceneComponent.K2_GetComponentLocation` _capsulecomponent) (`KismetMathLibrary.ComposeRotators` (`SceneComponent.K2_GetComponentRotation` _capsulecomponent) (struct :`Yaw` -90.0)) 0.0 false false)
      (`SceneComponent.K2_SetWorldLocation` (`self.Collider`) (`SceneComponent.K2_GetComponentLocation` (`self.Body`)) false false))
    (:`then_1`
      (if (not _returnvalue_2) :!label _label
        (`/Engine/EditorBlueprintResources/StandardMacros.DoOnce` false :!label _label_2
          (:`Completed`
            (`self.LightAttack`))))
      (`self.AddMovementInput` (`KismetMathLibrary.GetForwardVector` (`KismetMathLibrary.FindLookAtRotation` (`self.K2_GetActorLocation`) (+ (`self.K2_GetActorLocation` _returnvalue) (0.0 0.0 160.0)))) (`KismetMathLibrary.SelectFloat` 1.0 0.05 _returnvalue_2)))))

(event `Move`
  (if (<= (`self.GetDistanceTo` (`GameplayStatics.GetPlayerPawn` 0) self) 2000.0)
    (goto _label)))

(event `self.LightAttack`
  (bind _weaponmanager_bpc (`self.WeaponManager_BPC`))
  (`parent.LightAttack`)
  (`NiagaraFunctionLibrary.SpawnSystemAttached` "/Game/Resources/VFX/Shine_NS.Shine_NS" (`self.Body`) "None" (0.0 0.0 0.0) (struct) "SnapToTarget" true)
  (`FMODBlueprintStatics.PlayEventAttached` "/Game/FMOD/Events/Sounds/Enemy/Enemy_Hint.Enemy_Hint" (`self.Mesh`) "None" (0.0 0.0 0.0) "SnapToTarget")
  ;[0.9688 1 0] Code for attacking that was in EnemyBase_BP
  (`KismetSystemLibrary.Delay` 0.6)
  (`|ExecutionSequence`
    (:`then_0`
      (`/Game/Resources/Characters/Weapons/WeaponManager_BPC.LightStart` _weaponmanager_bpc (`/Game/Resources/Characters/Weapons/WeaponManager_BPC.Weapons` _weaponmanager_bpc))
      (`KismetSystemLibrary.K2_SetTimer` null "End Attack" (`KismetMathLibrary.RandomFloatInRange` 0.3 3.0)))
    (:`then_1`
      (`FMODBlueprintStatics.PlayEventAttached` "/Game/FMOD/Events/Sounds/Enemy/Enemy_Attack.Enemy_Attack" (`self.Mesh`) "None" (0.0 0.0 0.0) "SnapToTarget"))))

(event `End Attack`
  (bind _weaponmanager_bpc (`self.WeaponManager_BPC`))
  ;[0.9688 1 0] Code for attacking that was in EnemyBase_BP
  (`/Game/Resources/Characters/Weapons/WeaponManager_BPC.LightStop` _weaponmanager_bpc (`/Game/Resources/Characters/Weapons/WeaponManager_BPC.Weapons` _weaponmanager_bpc) :!label _label_3)
  ;;[1 0 0.5391] Used to notify behavior tree
  (`self.AttackFinishedDispatcher`)
  (`KismetSystemLibrary.PrintString` "Finished Attacking" false false (struct :`R` 1.0 :`G` 0.963927 :`A` 1.0))
  (`KismetSystemLibrary.RetriggerableDelay` 3.0)
  (goto _label_2 :!via `Reset`))

(event `self.CancelAttack`
  ;[0.9688 1 0] Code for attacking that was in EnemyBase_BP
  (`parent.CancelAttack`)
  (`|ExecutionSequence`
    (:`then_1`
      (goto _label_3))))

(event `self.Apply Knockback`
  (params (Causer :type "Actor Object Reference") (Force :type "Float (double-precision)") (Height :type "Float (double-precision)"))
  (bind _newvar_0 (`self.NewVar_0`))
  (bind _physicscontrol (`self.PhysicsControl`))
  (bind (_returnvalue_x _returnvalue_y) (`KismetMathLibrary.BreakVector` (`KismetMathLibrary.GetForwardVector` (`KismetMathLibrary.FindLookAtRotation` (`self.K2_GetActorLocation` Causer) (`self.K2_GetActorLocation`)))))
  ;[0.1484 1 0] Knockback Event
  (set `self.stunned` true)
  ;[0.1484 1 0] Knockback Event
  (`PhysicsControlComponent.SetControlMultipliers` (`self.PhysicsControl`) "None" (make `PhysicsControlMultipliers` (0.0 0.0 0.0) (1.0 1.0 1.0) (1.0 1.0 1.0) 0.0) true)
  (`PrimitiveComponent.AddImpulse` (`self.Body`) (+ (* (`KismetMathLibrary.MakeVector` _returnvalue_x _returnvalue_y) Force) (`KismetMathLibrary.MakeVector` 0.0 0.0 Height)) "None" true)
  (`|ExecutionSequence`
    (:`then_0`
      (bind (_direction _newtrack_0 _location_lerp) (`Timeline|Timeline` :`NewTime` (`KismetMathLibrary.MapRangeClamped` (/ Force 250.0) 0.0 1.0 0.9) :!via `SetNewTime` :!label _label_4)
        (:`Update`
          (`PhysicsControlComponent.SetControlMultipliers` _physicscontrol _newvar_0 (make `PhysicsControlMultipliers` (`KismetMathLibrary.Conv_DoubleToVector` _newtrack_0) (1.0 1.0 1.0) (1.0 1.0 1.0) _newtrack_0) true)
          (`self.K2_SetActorLocation` (`KismetMathLibrary.VLerp` (`self.K2_GetActorLocation`) (`SceneComponent.K2_GetComponentLocation` (`self.Body`)) _location_lerp)))
        (:`Finished`
          (set `self.stunned` false)
          (`PhysicsControlComponent.SetControlMultipliers` _physicscontrol _newvar_0 (make `PhysicsControlMultipliers` (1.0 1.0 1.0)) true))))
    (:`then_1`
      (goto _label_4))))

(event `/Game/Resources/Characters/Player/Blueprints/Parry_BPInter.Apply Parry`
  (params (Causer :type "Actor Object Reference") (Damage :type "Float (double-precision)"))
  (`KismetSystemLibrary.PrintString` "PARRY!!!!" true true (struct :`R` 1.0 :`G` 0.607333 :`B` 0.167448 :`A` 1.0))
  (set `self.TargetRotation` (struct :`Pitch` 60.0))
  (bind _returnvalue (`FMODBlueprintStatics.PlayEventAttached` "/Game/FMOD/Events/Sounds/Enemy/Enemy_Hit.Enemy_Hit" (`self.Mesh`) "None" (0.0 0.0 0.0) "SnapToTarget"))
  (`FMODAudioComponent.SetParameter` _returnvalue "Damage" Damage)
  (`self.Apply Knockback` Causer 20.0 200.0))

(event `self.OnDeath`
  (bind _weaponmanager_bpc (`self.WeaponManager_BPC`))
  ;[1 0.9844 0] On Death
  (`parent.OnDeath`)
  (`/Game/Resources/Characters/Weapons/WeaponManager_BPC.LightStop` _weaponmanager_bpc (`/Game/Resources/Characters/Weapons/WeaponManager_BPC.Weapons` _weaponmanager_bpc))
  (`|SpawnActorFromClass` "/Game/Resources/Characters/Destructables/DestructableExploded_BP_Core.DestructableExploded_BP_Core_C" (`SceneComponent.K2_GetComponentToWorld` (`self.Tank`)) "AlwaysSpawn" "OverrideRootScale" null 0 null)
  (`ActorComponent.K2_DestroyComponent` (`self.Tank`))
  (`ActorComponent.K2_DestroyComponent` (`self.MemorySphere_NS`))
  ;;[1 0.5859 0] Destroy AI Capability
  (`self.PossessAI` false)
  (`self.ToggleBehaviorTree`)
  (`PhysicsControlComponent.SetControlEnabled` (`self.PhysicsControl`) (`self.NewVar_0`) false)
  (`PrimitiveComponent.SetCollisionEnabled` (`self.Collider`) "NoCollision")
  (`SceneComponent.SetVisibility` (`self.Widget`) false false)
  (set `CharacterMovementComponent.GravityScale` 0.0 (`self.CharacterMovement`))
  (`self.Apply Knockback` self (`KismetMathLibrary.RandomFloatInRange` 100.0 300.0) (`KismetMathLibrary.RandomFloatInRange` 10.0 50.0))
  (`PrimitiveComponent.SetCollisionResponseToAllChannels` (`self.CapsuleComponent`) "ECR_Ignore")
  (`PrimitiveComponent.SetCollisionResponseToAllChannels` (`self.Body`) "ECR_Ignore")
  ;;[0 0.3672 1] Cool Transform Animation
  (bind _returnvalue (`PrimitiveComponent.CreateDynamicMaterialInstance` (`self.FishBody`) 0 "/Game/Resources/Materials/Common/Transform_Mat.Transform_Mat" "None"))
  (bind _output_get (set `self.Transform_Mat` _returnvalue))
  (`PrimitiveComponent.SetMaterial` (`self.FishBody`) 0 _output_get)
  (`PrimitiveComponent.SetMaterial` (`self.Tank`) 0 _output_get)
  (`PrimitiveComponent.SetMaterial` (`self.LowerFin`) 0 _output_get)
  (`PrimitiveComponent.SetMaterial` (`self.BackFin`) 0 _output_get)
  (`PrimitiveComponent.SetMaterial` (`self.UpperFin`) 0 _output_get)
  (`PrimitiveComponent.SetMaterial` (`self.FinshEye`) 0 _output_get)
  (bind (_direction _newtrack_0) (`Timeline|Timeline_0` :!via `PlayFromStart`)
    (:`Update`
      (`MaterialInstanceDynamic.SetScalarParameterValue` (`self.Transform_Mat`) "Emmisive" (`KismetMathLibrary.Lerp` 0.0 10.0 _newtrack_0)))
    (:`Finished`
      ;;[0.3828 1 0] Play Camera Shakes
      (`GameplayStatics.PlayWorldCameraShake` "/Game/Resources/Characters/Player/Blueprints/Camera/Big_CameraShake.Big_CameraShake_C" (`self.K2_GetActorLocation`) 500.0 3000.0)
      (`|SpawnActorFromClass` "/Game/Resources/Characters/Destructables/DestructableExploded_BP_Fish.DestructableExploded_BP_Fish_C" (`SceneComponent.K2_GetComponentToWorld` (`self.FishBody`)) "AlwaysSpawn" "OverrideRootScale" null 0 null)
      (`self.Drop Module`)
      (`self.K2_DestroyActor`))))

(fn `UserConstructionScript`
  (`parent.UserConstructionScript`))