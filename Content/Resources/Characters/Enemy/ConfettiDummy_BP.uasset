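; Confetti dummy enemy that carries jelly arm weapons and tilts its mesh with its movement direction.
; BeginPlay, marked as test setup, attaches two cosmetic-style dummy cutting arms and one managed normal arm, fits managed weapons with confetti modules and targets the player.
; LightAttack immediately reports finished to the behavior tree, as the real attack chain is disconnected.
; Parries play a hit sound and knock it upward.
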(event `self.ReceiveTick`
  (params (DeltaSeconds :type "Float (single-precision)"))
  (bind _returnvalue (`GameplayStatics.GetWorldDeltaSeconds`))
  (bind _mesh (`self.Mesh`))
  (bind (_relativerotation_roll _relativerotation_pitch) (`KismetMathLibrary.BreakRotator` (`SceneComponent.RelativeRotation` _mesh)))
  ;[0 0.6719 1] Walking Tilting
  (`parent.ReceiveTick` DeltaSeconds)
  (`SceneComponent.K2_SetRelativeRotation` _mesh (`KismetMathLibrary.MakeRotator` (`KismetMathLibrary.FInterpTo` _relativerotation_roll (* (`KismetAnimationLibrary.CalculateDirection` (`MovementComponent.Velocity` (`self.CharacterMovement`)) (`KismetMathLibrary.ComposeRotators` (`self.K2_GetActorRotation`) (struct :`Yaw` 90.0))) -0.2) _returnvalue 2.0) (`KismetMathLibrary.FInterpTo` _relativerotation_pitch (* (`KismetAnimationLibrary.CalculateDirection` (`MovementComponent.Velocity` (`self.CharacterMovement`)) (`self.K2_GetActorRotation`)) 0.2) _returnvalue 2.0) 270.0) false false))

(event `self.ReceiveBeginPlay`
  (bind (_returnvalue_location _returnvalue_rotation) (`KismetMathLibrary.BreakTransform` (`self.GetTransform`)))
  (bind (_returnvalue_location_2 _returnvalue_rotation_2) (`KismetMathLibrary.BreakTransform` (`self.GetTransform`)))
  (bind _returnvalue (`SceneComponent.K2_GetComponentLocation` (`self.Arrow2`)))
  ;[0 0.9062 1] Temp Test Attach Modules
  (`parent.ReceiveBeginPlay`)
  (for _index (range 2)
    (bind _returnvalue_2 (`|SpawnActorFromClass` "/Game/Resources/Characters/Weapons/Jelly/JellyCuttingArm_BP_Dummy.JellyCuttingArm_BP_Dummy_C" (`KismetMathLibrary.MakeTransform` _returnvalue (`KismetMathLibrary.ComposeRotators` _returnvalue_rotation_2 (`KismetMathLibrary.MakeRotator` 0.0 0.0 (`KismetMathLibrary.Conv_IntToDouble` (+ (* _index 180) 90))))) "Undefined" "OverrideRootScale" null null))
    (bind _asweapon_base_bp (cast `/Game/Resources/Characters/Weapons/WeaponBase_BP` _returnvalue_2))
    (`self.K2_AttachToActor` _asweapon_base_bp self "None" "KeepWorld" "KeepWorld" "KeepWorld" true))
  (bind _returnvalue_3 (`|SpawnActorFromClass` "/Game/Resources/Characters/Weapons/Jelly/JellyNormalArm_BP.JellyNormalArm_BP_C" (`KismetMathLibrary.MakeTransform` _returnvalue (struct :`Yaw` 180.0)) "Undefined" "OverrideRootScale" null null))
  (`|ExecutionSequence`
    (:`then_0`
      (bind _asweapon_base_bp_2 (cast `/Game/Resources/Characters/Weapons/WeaponBase_BP` _returnvalue_3))
      (`/Game/Resources/Characters/Weapons/WeaponManager_BPC.Add Weapon` (`self.WeaponManager_BPC`) _asweapon_base_bp_2)
      (`self.K2_AttachToActor` _asweapon_base_bp_2 self "None" "KeepWorld" "KeepWorld" "KeepWorld" true))
    (:`then_1`
      (for _array_element (`/Game/Resources/Characters/Weapons/WeaponManager_BPC.Weapons` (`self.WeaponManager_BPC`))
        (bind _returnvalue_4 (`|SpawnActorFromClass` "/Game/Resources/Characters/Modules/Turrets/ConfettiMod_BP.ConfettiMod_BP_C" (`KismetMathLibrary.MakeTransform` _returnvalue_location _returnvalue_rotation) "Undefined" "OverrideRootScale" null null))
        (bind _asmodule_base_bp (cast `/Game/Resources/Characters/Modules/ModuleBase_BP` _returnvalue_4))
        (`/Game/Resources/Characters/Weapons/WeaponManager_BPC.AttachModule` (`self.WeaponManager_BPC`) _array_element _asmodule_base_bp))
      (`/Game/Resources/Characters/Weapons/WeaponManager_BPC.Update Locked Target` (`self.WeaponManager_BPC`) (`GameplayStatics.GetPlayerPawn` 0)))))

(event `self.LightAttack`
  (`self.AttackFinishedDispatcher`))

(event `End Attack`
  ;[0.9688 1 0] Code for attacking that was in EnemyBase_BP
  (`/Game/Resources/Characters/Weapons/WeaponManager_BPC.LightStop` (`self.WeaponManager_BPC`) (`self.NewArray`) :!label _label)
  ;;[1 0 0.5391] Used to notify behavior tree
  (`self.AttackFinishedDispatcher`)
  (`KismetSystemLibrary.PrintString` "Finished Attacking" true true (struct :`R` 1.0 :`G` 0.963927 :`A` 1.0)))

(event `self.CancelAttack`
  ;[0.9688 1 0] Code for attacking that was in EnemyBase_BP
  (`parent.CancelAttack`)
  (`KismetSystemLibrary.K2_ClearAndInvalidateTimerHandle` (`self.AttackLoopTimer`))
  (goto _label))

(event `/Game/Resources/Characters/Player/Blueprints/Parry_BPInter.Apply Parry`
  (params (Causer :type "Actor Object Reference") (Damage :type "Float (double-precision)"))
  (`KismetSystemLibrary.PrintString` "PARRY!!!!" true true (struct :`R` 1.0 :`G` 0.607333 :`B` 0.167448 :`A` 1.0))
  (set `self.TargetRotation` (struct :`Pitch` 60.0))
  (bind _returnvalue (`FMODBlueprintStatics.PlayEventAttached` "/Game/FMOD/Events/Sounds/Enemy/Enemy_Hit.Enemy_Hit" (`self.Mesh`) "None" (0.0 0.0 0.0) "SnapToTarget"))
  (`FMODAudioComponent.SetParameter` _returnvalue "Damage" Damage)
  (`self.Apply Knockback` Causer 0.0 200.0))

(fn `Get Idle Slot`
  (returns (Slot :type "SceneComponent Object Reference"))
  (return (`self.Slot`)))

(fn `UserConstructionScript`
  (`parent.UserConstructionScript`))