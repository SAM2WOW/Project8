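; Squid enemy that tilts with movement and attacks the player using a ring of spawned modular weapons.
; A Physics Control keeps the Squid body on ControlTarget until damage releases it and knocks it away.
; Attacks telegraph, fire all weapons for a random duration, notify the behavior tree, and draw AttackRange from a random module's data.
; Parries interrupt attacks; death plays an emissive glow, then spawns debris and drops a module.
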(event `self.ReceiveTick`
  (params (DeltaSeconds :type "Float (single-precision)"))
  (bind _returnvalue (`GameplayStatics.GetWorldDeltaSeconds`))
  (bind _mesh (`self.Mesh`))
  (bind (_returnvalue_location _returnvalue_rotation) (`KismetMathLibrary.BreakTransform` (`SceneComponent.K2_GetComponentToWorld` (`self.controlTarget`))))
  (bind (_relativerotation_roll _relativerotation_pitch) (`KismetMathLibrary.BreakRotator` (`SceneComponent.RelativeRotation` _mesh)))
  ;[0 0.6719 1] Walking Tilting
  (`parent.ReceiveTick` DeltaSeconds)
  (`SceneComponent.K2_SetRelativeRotation` _mesh (`KismetMathLibrary.MakeRotator` (`KismetMathLibrary.FInterpTo` _relativerotation_roll (* (`KismetAnimationLibrary.CalculateDirection` (`MovementComponent.Velocity` (`self.CharacterMovement`)) (`KismetMathLibrary.ComposeRotators` (`self.K2_GetActorRotation`) (struct :`Yaw` 90.0))) -0.5) _returnvalue 2.0) (`KismetMathLibrary.FInterpTo` _relativerotation_pitch (* (`KismetAnimationLibrary.CalculateDirection` (`MovementComponent.Velocity` (`self.CharacterMovement`)) (`self.K2_GetActorRotation`)) 0.5) _returnvalue 2.0) 270.0) false false)
  (`PhysicsControlComponent.SetControlTargetPositionAndOrientation` (`self.PhysicsControl`) (stale `self.ReceiveBeginPlay` _returnvalue_3) _returnvalue_location _returnvalue_rotation 0.0 true false))

(event `self.ReceiveAnyDamage`
  (params (Damage :type "Float (single-precision)") (DamageType :type "DamageType Object Reference") (InstigatedBy :type "Controller Object Reference") (DamageCauser :type "Actor Object Reference"))
  (bind _squid (`self.squid`))
  (bind (_returnvalue_x _returnvalue_y) (`KismetMathLibrary.BreakVector` (`KismetMathLibrary.GetForwardVector` (`KismetMathLibrary.FindLookAtRotation` (`self.K2_GetActorLocation` DamageCauser) (`self.K2_GetActorLocation`)))))
  (`PhysicsControlComponent.SetControlMultipliers` (`self.PhysicsControl`) (stale `self.ReceiveBeginPlay` _returnvalue_3) (make `PhysicsControlMultipliers` (1.0 1.0 1.0)) false)
  (`parent.ReceiveAnyDamage` Damage DamageType InstigatedBy DamageCauser)
  (`/Engine/EditorBlueprintResources/StandardMacros.IsValid` _squid
    (:`Is Valid`
      (`PrimitiveComponent.AddImpulse` _squid (+ (* (`KismetMathLibrary.MakeVector` _returnvalue_x _returnvalue_y) (20000.0 20000.0 10000.0)) (0.0 0.0 0.0)) "None" false))))

(event `self.ReceiveBeginPlay`
  (bind _returnvalue (`self.GetTransform`))
  (bind _initialweapons (`self.InitialWeapons`))
  ;[0 0.9062 1] Attach Weapons
  (`parent.ReceiveBeginPlay`)
  (for (_array_element _array_index) _initialweapons
    (bind _returnvalue_2 (`|SpawnActorFromClass` (break `/Game/Resources/Characters/Weapons/WeaponConfig_Struct` _array_element) (`KismetMathLibrary.MakeTransform` (`SceneComponent.K2_GetComponentLocation` (`self.weaponSlot`)) (`KismetMathLibrary.MakeRotator` (.roll (.rotation _returnvalue)) (.pitch (.rotation _returnvalue)) (+ (`KismetMathLibrary.Conv_IntToDouble` (* _array_index (/ 360 (`KismetArrayLibrary.Array_Length` _initialweapons)))) (.yaw (.rotation _returnvalue))))) "Undefined" "OverrideRootScale" null (`.Modules_7_722CB5DD464C73B8CC52358F6C998AF4` (break `/Game/Resources/Characters/Weapons/WeaponConfig_Struct` _array_element)) null))
    (`/Game/Resources/Characters/Weapons/WeaponManager_BPC.Add Weapon` (`self.WeaponManager_BPC`) _returnvalue_2)
    (`self.K2_AttachToComponent` _returnvalue_2 (`self.squid`) "None" "KeepWorld" "KeepWorld" "KeepWorld" true))
  (`/Game/Resources/Characters/Weapons/WeaponManager_BPC.Update Locked Target` (`self.WeaponManager_BPC`) (`GameplayStatics.GetPlayerPawn` 0))
  (bind _returnvalue_3 (`PhysicsControlComponent.MakeControl` :`self` (`self.PhysicsControl`) :`ChildMeshComponent` (`self.squid`) :`ControlData` (make `PhysicsControlData` 5.0)))
  (`PhysicsControlComponent.MakeBodyModifier` (`self.PhysicsControl`) null "None" "Simulated" "QueryAndPhysics" 0.2 false)
  ;[1 0 0.04688] Randomly Update Attack Range
  (bind _returnvalue_4 (`|GetDataTableRow` "/Game/Resources/Characters/Modules/ModuleInfo_DT.ModuleInfo_DT" (`/Game/Resources/Characters/Modules/ModuleBase_BP.Type` (`KismetArrayLibrary.Array_Random` (`/Game/Resources/Characters/Modules/ModuleManager_BPC.Modules` (`/Game/Resources/Characters/Weapons/WeaponBase_BP.ModuleManager_BPC` (`KismetArrayLibrary.Array_Random` (`/Game/Resources/Characters/Weapons/WeaponManager_BPC.Weapons` (`self.WeaponManager_BPC`))))))) :!label _label)
    (:`then`
      (`BlackboardComponent.SetValueAsFloat` (`AIBlueprintHelperLibrary.GetBlackboard` null) "AttackRange" (`.Distance_38_5471E5C54575821453EEA4AA64479627` (break `/Game/Resources/Characters/Modules/ModuleInfo_Struct` _returnvalue_4))))))

(event `Update Attack Range`
  ;[1 0 0.04688] Randomly Update Attack Range
  (goto _label))

(event `self.LightAttack`
  (bind _weaponmanager_bpc (`self.WeaponManager_BPC`))
  (bind _weaponmanager_bpc_2 (`self.WeaponManager_BPC`))
  (`parent.LightAttack`)
  (`NiagaraFunctionLibrary.SpawnSystemAttached` "/Game/Resources/VFX/Shine_NS.Shine_NS" (`self.Sphere`) "None" (0.0 0.0 0.0) (struct) "KeepRelativeOffset" true)
  (`FMODBlueprintStatics.PlayEventAttached` "/Game/FMOD/Events/Sounds/Enemy/Enemy_Hint.Enemy_Hint" (`self.Mesh`) "None" (0.0 0.0 0.0) "SnapToTarget")
  (`/Game/Resources/Characters/Weapons/WeaponManager_BPC.PreparingAttack` _weaponmanager_bpc_2 (`/Game/Resources/Characters/Weapons/WeaponManager_BPC.Weapons` _weaponmanager_bpc_2))
  ;[0.9688 1 0] Code for attacking that was in EnemyBase_BP
  (`KismetSystemLibrary.Delay` 0.6)
  (`FMODBlueprintStatics.PlayEventAttached` "/Game/FMOD/Events/Sounds/Enemy/Enemy_Attack.Enemy_Attack" (`self.Mesh`) "None" (0.0 0.0 0.0) "SnapToTarget")
  (`/Game/Resources/Characters/Weapons/WeaponManager_BPC.LightStart` _weaponmanager_bpc (`/Game/Resources/Characters/Weapons/WeaponManager_BPC.Weapons` _weaponmanager_bpc))
  (`self.Update Attack Range`)
  (bind _returnvalue (`KismetSystemLibrary.K2_SetTimer` null "End Attack" (`KismetMathLibrary.RandomFloatInRange` 0.3 3.0)))
  (set `self.AttackLoopTimer` _returnvalue))

(event `End Attack`
  (bind _weaponmanager_bpc (`self.WeaponManager_BPC`))
  ;[0.9688 1 0] Code for attacking that was in EnemyBase_BP
  (`/Game/Resources/Characters/Weapons/WeaponManager_BPC.LightStop` _weaponmanager_bpc (`/Game/Resources/Characters/Weapons/WeaponManager_BPC.Weapons` _weaponmanager_bpc) :!label _label_2)
  ;;[1 0 0.5391] Used to notify behavior tree
  (`self.AttackFinishedDispatcher`)
  (`KismetSystemLibrary.PrintString` "Finished Attacking" true true (struct :`R` 1.0 :`G` 0.963927 :`A` 1.0)))

(event `self.CancelAttack`
  ;[0.9688 1 0] Code for attacking that was in EnemyBase_BP
  (`parent.CancelAttack`)
  (`KismetSystemLibrary.K2_ClearAndInvalidateTimerHandle` (`self.AttackLoopTimer`))
  (goto _label_2))

(event `/Game/Resources/Characters/Player/Blueprints/Parry_BPInter.Apply Parry`
  (params (Causer :type "Actor Object Reference") (Damage :type "Float (double-precision)"))
  (`KismetSystemLibrary.PrintString` "PARRY!!!!" true true (struct :`R` 1.0 :`G` 0.607333 :`B` 0.167448 :`A` 1.0))
  (set `self.TargetRotation` (struct :`Pitch` 60.0))
  (bind _returnvalue (`FMODBlueprintStatics.PlayEventAttached` "/Game/FMOD/Events/Sounds/Enemy/Enemy_Hit.Enemy_Hit" (`self.Mesh`) "None" (0.0 0.0 0.0) "SnapToTarget"))
  (`FMODAudioComponent.SetParameter` _returnvalue "Damage" Damage)
  (`self.Apply Knockback` Causer 0.0 200.0)
  (`self.End Attack`))

(event `self.OnDeath`
  (bind _weaponmanager_bpc (`self.WeaponManager_BPC`))
  ;[1 0.9844 0] On Death
  (`parent.OnDeath`)
  (`/Game/Resources/Characters/Weapons/WeaponManager_BPC.LightStop` _weaponmanager_bpc (`/Game/Resources/Characters/Weapons/WeaponManager_BPC.Weapons` _weaponmanager_bpc))
  (`|SpawnActorFromClass` "/Game/Resources/Characters/Destructables/DestructableExploded_BP_Core.DestructableExploded_BP_Core_C" (`SceneComponent.K2_GetComponentToWorld` (`self.Sphere`)) "AlwaysSpawn" "OverrideRootScale" null 0 null)
  (`ActorComponent.K2_DestroyComponent` (`self.Sphere`))
  (`ActorComponent.K2_DestroyComponent` (`self.MemorySphere_NS`))
  ;;[1 0.5859 0] Destroy AI Capability
  (`self.PossessAI` false)
  (`self.ToggleBehaviorTree`)
  (`SceneComponent.SetVisibility` (`self.Widget`) false false)
  (set `CharacterMovementComponent.GravityScale` 0.0 (`self.CharacterMovement`))
  (`self.Apply Knockback` self (`KismetMathLibrary.RandomFloatInRange` 100.0 300.0) (`KismetMathLibrary.RandomFloatInRange` 10.0 50.0))
  (`PrimitiveComponent.SetCollisionResponseToAllChannels` (`self.CapsuleComponent`) "ECR_Ignore")
  ;;[0 0.3672 1] Cool Transform Animation
  (bind _returnvalue (`PrimitiveComponent.CreateDynamicMaterialInstance` (`self.squid`) 0 "/Game/Resources/Materials/Common/Transform_Mat.Transform_Mat" "None"))
  (bind _output_get (set `self.Transform_Mat` _returnvalue))
  (`PrimitiveComponent.SetMaterial` (`self.squid`) 0 _output_get)
  (bind (_direction _newtrack_0) (`Timeline|Timeline_0` :!via `PlayFromStart`)
    (:`Update`
      (`MaterialInstanceDynamic.SetScalarParameterValue` (`self.Transform_Mat`) "Emmisive" (`KismetMathLibrary.Lerp` 0.0 10.0 _newtrack_0)))
    (:`Finished`
      ;;[0.3828 1 0] Play Camera Shakes
      (`GameplayStatics.PlayWorldCameraShake` "/Game/Resources/Characters/Player/Blueprints/Camera/Big_CameraShake.Big_CameraShake_C" (`self.K2_GetActorLocation`) 500.0 3000.0)
      (`|SpawnActorFromClass` "/Game/Resources/Characters/Destructables/DestructableExploded_BP_Squid.DestructableExploded_BP_Squid_C" (`SceneComponent.K2_GetComponentToWorld` (`self.squid`)) "AlwaysSpawn" "OverrideRootScale" null 0 null)
      (`self.Drop Module`)
      (`self.K2_DestroyActor`))))

(event `self.ReceiveDestroyed`
  (bind _mesh (`self.Mesh`))
  (`parent.ReceiveDestroyed`)
  (`KismetSystemLibrary.PrintString` "Spawn Funny")
  (bind _returnvalue (`|SpawnActorFromClass` "/Script/Engine.SkeletalMeshActor" (`SceneComponent.K2_GetComponentToWorld` _mesh) "AlwaysSpawn" "OverrideRootScale" null null))
  (`SkeletalMeshComponent.SetSkeletalMeshAsset` (`SkeletalMeshActor.SkeletalMeshComponent` _returnvalue) (`SkeletalMeshComponent.SkeletalMeshAsset` _mesh))
  (`PrimitiveComponent.SetSimulatePhysics` (`SkeletalMeshActor.SkeletalMeshComponent` _returnvalue) true))

(event `self.ReceivePossessed`
  (params (NewController :type "Controller Object Reference"))
  (bind _sphere (`self.Sphere`))
  (`SceneComponent.SetVisibility` _sphere true false)
  (`SceneComponent.SetVisibility` (`self.MemorySphere_NS`) true false)
  (`NiagaraFunctionLibrary.SpawnSystemAttached` "/Game/Resources/VFX/Shine_NS.Shine_NS" _sphere "None" (0.0 0.0 0.0) (struct) "KeepRelativeOffset" true))

(event `self.ReceiveUnpossessed`
  (params (OldController :type "Controller Object Reference"))
  (`SceneComponent.SetVisibility` (`self.Sphere`) false false)
  (`SceneComponent.SetVisibility` (`self.MemorySphere_NS`) false false))

(fn `UserConstructionScript`
  (`parent.UserConstructionScript`))