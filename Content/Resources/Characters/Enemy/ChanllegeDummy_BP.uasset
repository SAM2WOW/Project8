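; Challenge dummy enemy that takes damage, reacts to hits and explodes on death, extending parent character logic.
; Damage lowers health and drives a timed healthbar, hit audio and VFX, with heavy hits also cancelling attacks and shaking the camera.
; Knockback uses a timeline to offset a sphere component instead of moving the actor.
; Death spawns destructible explosions in two delayed stages, then destroys the actor and unregisters its healthbar from the GameState.
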(event `self.ReceiveBeginPlay`
  (`parent.ReceiveBeginPlay`)
  (set `self.Origin` (`self.K2_GetActorLocation`)))

(event `self.ReceiveTick`
  (params (DeltaSeconds :type "Float (single-precision)"))
  (`parent.ReceiveTick` DeltaSeconds))

(event `self.ReceiveAnyDamage`
  (params (Damage :type "Float (single-precision)") (DamageType :type "DamageType Object Reference") (InstigatedBy :type "Controller Object Reference") (DamageCauser :type "Actor Object Reference"))
  (bind _widget (`self.Widget`))
  (bind _returnvalue (== (`GameplayStatics.GetObjectClass` DamageType) "/Game/Resources/Characters/Weapons/Sword/Heavy_DamageType.Heavy_DamageType_C"))
  (set `self.DamageStack` (+ (`self.DamageStack`) Damage))
  (bind _output_get (set `self.Health` (`KismetMathLibrary.FMax` (- (`self.Health`) Damage))))
  (`|ExecutionSequence`
    (:`then_0`
      ;[0.875 1 0] Hide Enemy Healthbar After a while
      (`SceneComponent.SetVisibility` _widget true false)
      (`KismetSystemLibrary.RetriggerableDelay` 5.0)
      (`/Game/Resources/Widgets/EnemyHealth_Widget.Hide` (`self.HealthWidget`))
      (`KismetSystemLibrary.RetriggerableDelay` 0.3)
      (`SceneComponent.SetVisibility` _widget false false))
    (:`then_1`
      ;[0.125 0 1] On Receive Heavy Attack
      (if _returnvalue
        (`self.CancelAttack`)
        (`GameplayStatics.PlayWorldCameraShake` "/Game/Resources/Characters/Player/Blueprints/Camera/Small_CameraShake.Small_CameraShake_C" (`self.K2_GetActorLocation`) 200.0 2000.0)))
    (:`then_2`
      (bind _returnvalue_2 (`FMODBlueprintStatics.PlayEventAttached` "/Game/FMOD/Events/Sounds/Enemy/Enemy_Hit.Enemy_Hit" (`self.Mesh`) "None" (0.0 0.0 0.0) "SnapToTarget"))
      (`FMODAudioComponent.SetParameter` _returnvalue_2 "Damage" (`KismetMathLibrary.FClamp` Damage 0.0 100.0))
      (`/Game/Resources/Widgets/EnemyHealth_Widget.Received Damage` (`self.HealthWidget`) _returnvalue)
      (`NiagaraFunctionLibrary.SpawnSystemAtLocation` "/Game/Resources/VFX/ParryHit_NS.ParryHit_NS" (`SceneComponent.K2_GetComponentLocation` (`self.Mesh`))))
    (:`then_3`
      (`KismetSystemLibrary.RetriggerableDelay` 1.0)
      (set `self.DamageStack` 0.0))
    (:`then_4`
      (if (<= _output_get 0.0)
        (`self.OnDeath`)
        ;[1 0 0.375] After Dying
        (`|ExecutionSequence`
          (:`then_2`
            ;;[0 1 0.8594] Remove Tracked Widgets
            (bind _asnew_game_state_gs (cast `/Game/Resources/Characters/Player/Blueprints/NewGameState_GS` (`GameplayStatics.GetGameState`)))
            (`KismetArrayLibrary.Array_RemoveItem` (`/Game/Resources/Characters/Player/Blueprints/NewGameState_GS.HealthBars` _asnew_game_state_gs) (`self.HealthWidget`))))))))

(event `/Game/Resources/Characters/Player/Blueprints/ApplyingStat_BPInter.Apply Knockback`
  (params (Causer :type "Actor Object Reference") (Force :type "Float (double-precision)") (Height :type "Float (double-precision)"))
  (bind (_returnvalue_x _returnvalue_y) (`KismetMathLibrary.BreakVector` (`KismetMathLibrary.GetForwardVector` (`KismetMathLibrary.FindLookAtRotation` (`self.K2_GetActorLocation` Causer) (`self.K2_GetActorLocation`)))))
  ;[0.1484 1 0] Knockback Event
  (bind _output_get (set `self.Velocity` (+ (* (`KismetMathLibrary.MakeVector` _returnvalue_x _returnvalue_y) Force) (`KismetMathLibrary.MakeVector` 0.0 0.0 Height))))
  (bind (_direction _newtrack_0) (`Timeline|Timeline` :!via `PlayFromStart`)
    (:`Update`
      (bind (_x _y) (`KismetMathLibrary.BreakVector3f` _output_get))
      (`SceneComponent.K2_SetRelativeLocation` (`self.Sphere1`) (`KismetMathLibrary.MakeVector` (`KismetMathLibrary.Lerp` 0.0 (`KismetMathLibrary.FClamp` _x -40.0 40.0) _newtrack_0) (`KismetMathLibrary.Lerp` 0.0 (`KismetMathLibrary.FClamp` _y -40.0 40.0) _newtrack_0) -80.0) false false))))

(event `self.OnDeath`
  (`parent.OnDeath`)
  (`SceneComponent.SetVisibility` (`self.Widget`) false false)
  (set `CharacterMovementComponent.GravityScale` 0.0 (`self.CharacterMovement`))
  (`PrimitiveComponent.SetCollisionResponseToAllChannels` (`self.CapsuleComponent`) "ECR_Ignore")
  (`ActorComponent.K2_DestroyComponent` (`self.Sphere1`))
  (`ActorComponent.K2_DestroyComponent` (`self.MemorySphere_NS`))
  (`|SpawnActorFromClass` "/Game/Resources/Characters/Destructables/DestructableExploded_BP_Core.DestructableExploded_BP_Core_C" (`SceneComponent.K2_GetComponentToWorld` (`self.Sphere1`)) "Undefined" "OverrideRootScale" null 0 null)
  (`PrimitiveComponent.SetMaterial` (`self.Sphere2`) 0 "/Game/Resources/Materials/Common/Transform_Mat.Transform_Mat")
  (`KismetSystemLibrary.Delay` 0.5)
  ;[0.3828 1 0] Play Camera Shakes
  (`GameplayStatics.PlayWorldCameraShake` "/Game/Resources/Characters/Player/Blueprints/Camera/Big_CameraShake.Big_CameraShake_C" (`self.K2_GetActorLocation`) 500.0 3000.0)
  (`|SpawnActorFromClass` "/Game/Resources/Characters/Destructables/DestructableExploded_BP_Core.DestructableExploded_BP_Core_C" (`SceneComponent.K2_GetComponentToWorld` (`self.Sphere`)) "AlwaysSpawn" "OverrideRootScale" null (`KismetMathLibrary.RandomInteger` 4) null)
  (`self.K2_DestroyActor`))

(fn `UserConstructionScript`
  (`parent.UserConstructionScript`))