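; Jelly Cutter enemy that attacks the player with two opposed cutting arms, each fitted with a cutter module through WeaponManagerBPC.
; Light attacks telegraph with a burst effect and sound, then run all weapons for a randomly chosen duration before notifying the behavior tree.
; A parry knocks it upward and cancels the attack, and death spawns a destructible geometry collection.
; Tick tilts the mesh according to movement direction.
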(event `self.ReceiveTick`
  (params (DeltaSeconds :type "Float (single-precision)"))
  (bind _returnvalue (`GameplayStatics.GetWorldDeltaSeconds`))
  (bind _mesh (`self.Mesh`))
  (bind (_relativerotation_roll _relativerotation_pitch) (`KismetMathLibrary.BreakRotator` (`SceneComponent.RelativeRotation` _mesh)))
  ;[0 0.6719 1] Walking Tilting
  (`parent.ReceiveTick` DeltaSeconds)
  (`SceneComponent.K2_SetRelativeRotation` _mesh (`KismetMathLibrary.MakeRotator` (`KismetMathLibrary.FInterpTo` _relativerotation_roll (* (`KismetAnimationLibrary.CalculateDirection` (`MovementComponent.Velocity` (`self.CharacterMovement`)) (`KismetMathLibrary.ComposeRotators` (`self.K2_GetActorRotation`) (struct :`Yaw` 90.0))) -0.2) _returnvalue 2.0) (`KismetMathLibrary.FInterpTo` _relativerotation_pitch (* (`KismetAnimationLibrary.CalculateDirection` (`MovementComponent.Velocity` (`self.CharacterMovement`)) (`self.K2_GetActorRotation`)) 0.2) _returnvalue 2.0) 270.0) false false))

(event `self.ReceiveBeginPlay`
  (bind (_returnvalue_location _returnvalue_rotation) (`KismetMathLibrary.BreakTransform` (`self.GetTransform`)))
  (bind (_returnvalue_location_2 _returnvalue_rotation_2) (`KismetMathLibrary.BreakTransform` (`self.GetTransform`)))
  ;[0 0.9062 1] Temp Test Attach Modules
  (`parent.ReceiveBeginPlay`)
  (for _index (range 2)
    (bind _returnvalue (`|SpawnActorFromClass` (select `int` (`KismetMathLibrary.RandomInteger` 2) :`0` "/Game/Resources/Characters/Weapons/Jelly/JellyCuttingArm_BP.JellyCuttingArm_BP_C" :`1` "/Game/Resources/Characters/Weapons/Jelly/JellyCuttingArm_BP.JellyCuttingArm_BP_C" :!type "Actor Class Reference") (`KismetMathLibrary.MakeTransform` (`SceneComponent.K2_GetComponentLocation` (`self.Arrow2`)) (`KismetMathLibrary.ComposeRotators` _returnvalue_rotation_2 (`KismetMathLibrary.MakeRotator` 0.0 0.0 (`KismetMathLibrary.Conv_IntToDouble` (+ (* _index 180) 90))))) "Undefined" "OverrideRootScale" null null))
    (bind _asweapon_base_bp (cast `/Game/Resources/Characters/Weapons/WeaponBase_BP` _returnvalue))
    (`/Game/Resources/Characters/Weapons/WeaponManager_BPC.Add Weapon` (`self.WeaponManager_BPC`) _asweapon_base_bp)
    (`self.K2_AttachToActor` _asweapon_base_bp self "None" "KeepWorld" "KeepWorld" "KeepWorld" true))
  (for _array_element (`/Game/Resources/Characters/Weapons/WeaponManager_BPC.Weapons` (`self.WeaponManager_BPC`))
    (bind _returnvalue_2 (`|SpawnActorFromClass` "/Game/Resources/Characters/Modules/Cutter/CutterMod_BP.CutterMod_BP_C" (`KismetMathLibrary.MakeTransform` _returnvalue_location _returnvalue_rotation) "Undefined" "OverrideRootScale" null null))
    (bind _asmodule_base_bp (cast `/Game/Resources/Characters/Modules/ModuleBase_BP` _returnvalue_2))
    (`/Game/Resources/Characters/Weapons/WeaponManager_BPC.AttachModule` (`self.WeaponManager_BPC`) _array_element _asmodule_base_bp))
  (`/Game/Resources/Characters/Weapons/WeaponManager_BPC.Update Locked Target` (`self.WeaponManager_BPC`) (`GameplayStatics.GetPlayerPawn` 0)))

(event `self.LightAttack`
  (bind _returnvalue (+ (`self.K2_GetActorLocation`) (0.0 0.0 50.0)))
  (bind _weapons (`/Game/Resources/Characters/Weapons/WeaponManager_BPC.Weapons` (`self.WeaponManager_BPC`)))
  (`parent.LightAttack`)
  (`NiagaraFunctionLibrary.SpawnSystemAtLocation` "/Game/Resources/VFX/Brust_NS.Brust_NS" _returnvalue (`KismetMathLibrary.FindLookAtRotation` _returnvalue (`PlayerCameraManager.GetCameraLocation` (`GameplayStatics.GetPlayerCameraManager` 0))))
  (`FMODBlueprintStatics.PlayEventAttached` "/Game/FMOD/Events/Sounds/Enemy/Enemy_Hint.Enemy_Hint" (`self.Mesh`) "None" (0.0 0.0 0.0) "SnapToTarget")
  ;[0.9688 1 0] Code for attacking that was in EnemyBase_BP
  (`KismetSystemLibrary.Delay` 0.6)
  (`KismetArrayLibrary.Array_Clear` (`self.NewArray`))
  (for _index (range (+ (`KismetArrayLibrary.Array_Length` _weapons) 1))
    (`KismetArrayLibrary.Array_Add` (`self.NewArray`) (`|GetArrayItem` _weapons _index)))
  (`FMODBlueprintStatics.PlayEventAttached` "/Game/FMOD/Events/Sounds/Enemy/Enemy_Attack.Enemy_Attack" (`self.Mesh`) "None" (0.0 0.0 0.0) "SnapToTarget")
  (switch `int` (`KismetMathLibrary.RandomInteger` 3)
    (:`Default`
      (`/Game/Resources/Characters/Weapons/WeaponManager_BPC.LightStart` (`self.WeaponManager_BPC`) (`self.NewArray`) :!label _label)
      (bind _returnvalue_2 (`KismetSystemLibrary.K2_SetTimer` null "End Attack" 1.0))
      (set `self.AttackLoopTimer` _returnvalue_2))
    (:`0`
      (goto _label))
    (:`1`
      (`/Game/Resources/Characters/Weapons/WeaponManager_BPC.LightStart` (`self.WeaponManager_BPC`) (`self.NewArray`))
      (bind _returnvalue_3 (`KismetSystemLibrary.K2_SetTimer` null "End Attack" 0.7))
      (set `self.AttackLoopTimer` _returnvalue_3))
    (:`2`
      (`/Game/Resources/Characters/Weapons/WeaponManager_BPC.LightStart` (`self.WeaponManager_BPC`) (`self.NewArray`))
      (bind _returnvalue_4 (`KismetSystemLibrary.K2_SetTimer` null "End Attack" 3.0))
      (set `self.AttackLoopTimer` _returnvalue_4))))

(event `End Attack`
  ;[0.9688 1 0] Code for attacking that was in EnemyBase_BP
  (`/Game/Resources/Characters/Weapons/WeaponManager_BPC.LightStop` (`self.WeaponManager_BPC`) (`self.NewArray`) :!label _label_2)
  ;;[1 0 0.5391] Used to notify behavior tree
  (`self.AttackFinishedDispatcher`)
  (`KismetSystemLibrary.PrintString` "Finished Attacking" true true (struct :`R` 1.0 :`G` 0.963927 :`A` 1.0)))

(event `self.CancelAttack`
  ;[0.9688 1 0] Code for attacking that was in EnemyBase_BP
  (`parent.CancelAttack`)
  (`KismetSystemLibrary.K2_ClearAndInvalidateTimerHandle` (`self.AttackLoopTimer`))
  (goto _label_2))

(event `/Game/Resources/Characters/Player/Blueprints/Parry_BPInter.Apply Parry`
  (params (Causer :type "Actor Object Reference") (Damage :type "Float (double-precision)"))
  (`KismetSystemLibrary.PrintString` "==================================PARRY!!!!" true true (struct :`R` 1.0 :`G` 0.607333 :`B` 0.167448 :`A` 1.0))
  (set `self.TargetRotation` (struct :`Pitch` 60.0))
  (bind _returnvalue (`FMODBlueprintStatics.PlayEventAttached` "/Game/FMOD/Events/Sounds/Enemy/Enemy_Hit.Enemy_Hit" (`self.Mesh`) "None" (0.0 0.0 0.0) "SnapToTarget"))
  (`FMODAudioComponent.SetParameter` _returnvalue "Damage" Damage)
  (`self.Apply Knockback` Causer 0.0 200.0)
  (`self.CancelAttack`))

(event `self.On Death`
  (`|SpawnActorFromClass` "/Game/Resources/Characters/Destructables/DestructableExploded_BP.DestructableExploded_BP_C" (`SceneComponent.K2_GetComponentToWorld` (`self.Sphere`)) "AlwaysSpawn" "OverrideRootScale" null 4 null "/Game/Resources/Characters/Destructables/GeometryCollections/Sphere2_GeometryCollection.Sphere2_GeometryCollection")
  (`FMODBlueprintStatics.PlayEventAtLocation` "/Game/FMOD/Events/Sounds/Collectables/Glass_Hit.Glass_Hit" (`self.GetTransform`))
  (`ActorComponent.K2_DestroyComponent` (`self.Sphere`))
  (`ActorComponent.K2_DestroyComponent` (`self.MemorySphere_NS`)))

(fn `Get Idle Slot`
  (returns (Slot :type "SceneComponent Object Reference"))
  (return (`self.Slot`)))

(fn `UserConstructionScript`
  (`parent.UserConstructionScript`))