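; Damage dummy enemy that springs back to its spawn point and refills its health whenever it reaches zero.
; Each hit adds to a camera-facing damage total that clears after one second without hits.
; Hits also drive the health widget, sound and Niagara effect, while heavy damage cancels attacks and shakes the camera.
; Death logic for loot drops and game-state cleanup is present but disconnected.
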(event `self.ReceiveBeginPlay`
  (`parent.ReceiveBeginPlay`)
  (set `self.Origin` (`self.K2_GetActorLocation`)))

(event `self.ReceiveTick`
  (params (DeltaSeconds :type "Float (single-precision)"))
  (bind _textrender (`self.TextRender`))
  (`parent.ReceiveTick` DeltaSeconds)
  (`self.K2_SetActorLocation` (`KismetMathLibrary.VInterpTo` (`self.K2_GetActorLocation`) (`self.Origin`) DeltaSeconds 20.0))
  (`SceneComponent.K2_SetWorldRotation` _textrender (`KismetMathLibrary.FindLookAtRotation` (`SceneComponent.K2_GetComponentLocation` _textrender) (`PlayerCameraManager.GetCameraLocation` (`GameplayStatics.GetPlayerCameraManager` 0))) false false))

(event `self.ReceiveAnyDamage`
  (params (Damage :type "Float (single-precision)") (DamageType :type "DamageType Object Reference") (InstigatedBy :type "Controller Object Reference") (DamageCauser :type "Actor Object Reference"))
  (bind _widget (`self.Widget`))
  (bind _returnvalue (== (`GameplayStatics.GetObjectClass` DamageType) "/Game/Resources/Characters/Weapons/Sword/Heavy_DamageType.Heavy_DamageType_C"))
  (set `self.DamageStack` (+ (`self.DamageStack`) Damage))
  (`TextRenderComponent.K2_SetText` (`self.TextRender`) (`KismetTextLibrary.Conv_DoubleToText` (`self.DamageStack`) "HalfToEven"))
  (bind _output_get (set `self.Health` (`KismetMathLibrary.FMax` (- (`self.Health`) Damage))))
  (`|ExecutionSequence`
    (:`then_0`
      ;[0.875 1 0] Hide Enemy Healthbar After a while
      (`SceneComponent.SetVisibility` _widget true false)
      (`KismetSystemLibrary.RetriggerableDelay` 5.0)
      (`/Game/Resources/Widgets/EnemyHealth_Widget.Hide` (`self.HealthWidget`))
      (`KismetSystemLibrary.RetriggerableDelay` 0.3)
      (`SceneComponent.SetVisibility` _widget false false))
    (:`then_1`
      ;[0.125 0 1] On Receive Heavy Attack
      (if _returnvalue
        (`self.CancelAttack`)
        (`GameplayStatics.PlayWorldCameraShake` "/Game/Resources/Characters/Player/Blueprints/Camera/Small_CameraShake.Small_CameraShake_C" (`self.K2_GetActorLocation`) 200.0 2000.0)))
    (:`then_2`
      (bind _returnvalue_2 (`FMODBlueprintStatics.PlayEventAttached` "/Game/FMOD/Events/Sounds/Enemy/Enemy_Hit.Enemy_Hit" (`self.Mesh`) "None" (0.0 0.0 0.0) "SnapToTarget"))
      (`FMODAudioComponent.SetParameter` _returnvalue_2 "Damage" (`KismetMathLibrary.FClamp` Damage 0.0 100.0))
      (`/Game/Resources/Widgets/EnemyHealth_Widget.Received Damage` (`self.HealthWidget`) _returnvalue)
      (`NiagaraFunctionLibrary.SpawnSystemAtLocation` "/Game/Resources/VFX/ParryHit_NS.ParryHit_NS" (`SceneComponent.K2_GetComponentLocation` (`self.Mesh`))))
    (:`then_3`
      (`KismetSystemLibrary.RetriggerableDelay` 1.0)
      (set `self.DamageStack` 0.0)
      (`TextRenderComponent.K2_SetText` (`self.TextRender`) "0"))
    (:`then_4`
      (if (<= _output_get 0.0)
        (set `self.Health` (`self.Max Health`))))))

(fn `UserConstructionScript`
  (`parent.UserConstructionScript`))