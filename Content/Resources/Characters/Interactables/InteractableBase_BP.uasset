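; Base Blueprint for interactable objects, providing proximity hints, player registration and overridable interaction events.
; A world widget shows while the object is interactable and the player is nearby but outside the Sphere, checked on Tick.
; Sphere overlaps add or remove it on BP_PlayerCharacter with hint, button and image, then fire empty ActorEnter/ActorLeave hooks.
; Pressed and Interact, also triggered by MsgInteract, update the HUD's pressed state through NewGameMode_GM when CanInteract allows.
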(event `self.ReceiveTick`
  (params (DeltaSeconds :type "Float (single-precision)"))
  (bind _returnvalue (`GameplayStatics.GetPlayerPawn` 0))
  (`SceneComponent.SetVisibility` (`self.Widget`) (and true (<= (`self.GetHorizontalDistanceTo` _returnvalue) 1000.0) (`self.Interactable`) (not (`PrimitiveComponent.IsOverlappingActor` (`self.Sphere`) _returnvalue))) false))

(event `self.Sphere.OnComponentBeginOverlap`
  (params (OverlappedComponent :type "PrimitiveComponent Object Reference") (OtherActor :type "Actor Object Reference") (OtherComp :type "PrimitiveComponent Object Reference") (OtherBodyIndex :type Integer) (bFromSweep :type Boolean) (SweepResult :type "HitResult Structure (by ref)"))
  (if (`self.Interactable`)
    (bind _asbp_player_character (cast `/Game/Resources/Characters/Player/Blueprints/BP_PlayerCharacter` OtherActor))
    (`/Game/Resources/Characters/Player/Blueprints/BP_PlayerCharacter.Add Interactable` _asbp_player_character self (`self.Hint`) (`self.Button`) (`self.Image`))
    (`self.ActorEnter`)))

(event `self.Sphere.OnComponentEndOverlap`
  (params (OverlappedComponent :type "PrimitiveComponent Object Reference") (OtherActor :type "Actor Object Reference") (OtherComp :type "PrimitiveComponent Object Reference") (OtherBodyIndex :type Integer))
  (if (`self.Interactable`)
    (bind _asbp_player_character (cast `/Game/Resources/Characters/Player/Blueprints/BP_PlayerCharacter` OtherActor))
    (`/Game/Resources/Characters/Player/Blueprints/BP_PlayerCharacter.Remove Interactable` _asbp_player_character self)
    (`self.ActorLeave`)))

(event `Interact`
  ;[0.8281 0 1] Interact
  (if (`self.CanInteract?`)
    (bind _asnew_game_mode_gm (cast `/Game/Resources/Characters/Player/Blueprints/NewGameMode_GM` (`GameplayStatics.GetGameMode`)))
    (`/Game/Resources/Widgets/HUD_Widget.MessagePressed` (`/Game/Resources/Characters/Player/Blueprints/NewGameMode_GM.HUD_ref` _asnew_game_mode_gm) false)))

(event `Pressed`
  (if (`self.CanInteract?`)
    (bind _asnew_game_mode_gm (cast `/Game/Resources/Characters/Player/Blueprints/NewGameMode_GM` (`GameplayStatics.GetGameMode`)))
    (`/Game/Resources/Widgets/HUD_Widget.MessagePressed` (`/Game/Resources/Characters/Player/Blueprints/NewGameMode_GM.HUD_ref` _asnew_game_mode_gm) true)))

(event `ActorEnter`
  ;[1 0.4219 0] Enter Leave
)

(event `ActorLeave`
  ;[1 0.4219 0] Enter Leave
)

(event `/Game/Resources/Characters/Interactables/interactable_interface.msg_interact`
  (`self.Interact`))

(fn `UserConstructionScript`)