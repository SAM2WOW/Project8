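; Colorstation_BP is an interactable workbench where the player recolors their sword.
; Interacting enters menu mode, deploys the sword to the station, opens a ColorEdit widget and blends the camera to the station.
; A timeline grows and raises a cone, reversed on TurnOff, while idle Niagara effects switch off and back on.
; The sword's color-update event drives the glow color, and Tick slowly spins the sword target.
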(event `On Color Changed`
  (params (`New Color` :type "LinearColor Structure"))
  (`FXSystemComponent.SetColorParameter` (`self.ColorGlow_NS`) "InputColor" `New Color`))

(event `self.Interact`
  (bind _cone (`self.Cone`))
  (`parent.Interact`)
  (bind _asbp_player_character (cast `/Game/Resources/Characters/Player/Blueprints/BP_PlayerCharacter` (`GameplayStatics.GetPlayerCharacter` 0)))
  (`/Game/Resources/Characters/Player/Blueprints/BP_PlayerCharacter.MenuMode` _asbp_player_character true)
  (bind _sword (`/Game/Resources/Characters/Player/Blueprints/BP_PlayerCharacter.Sword` _asbp_player_character))
  (`/Game/Resources/Characters/Weapons/Sword/VITA_BP.DeployInteract` _sword self)
  (add `/Game/Resources/Characters/Weapons/Sword/VITA_BP.ColorUpdated` _sword (delegate `On Color Changed`))
  (bind _returnvalue (`|CreateWidget` "/Game/Resources/Widgets/ColorEdit_Widget.ColorEdit_Widget_C" (`GameplayStatics.GetPlayerController` 0)))
  (`UserWidget.AddToViewport` _returnvalue 0)
  (set `/Game/Resources/Widgets/ColorEdit_Widget.ColorStation_ref` self _returnvalue)
  (`NiagaraFunctionLibrary.SpawnSystemAttached` "/Game/Resources/VFX/Shine_NS.Shine_NS" (`self.Pickup_big_NS1`) "None" (0.0 0.0 0.0) (struct) "SnapToTarget")
  (`PlayerController.SetViewTargetWithBlend` (`GameplayStatics.GetPlayerController` 0) self 1.0 "VTBlend_EaseInOut" 3.0 true)
  (`FMODBlueprintStatics.PlayEvent2D` "/Game/FMOD/Events/Sounds/UI/UI_Workbench.UI_Workbench")
  (`ActorComponent.SetActive` (`self.Charging_NS_2`) false false)
  (`ActorComponent.SetActive` (`self.Pickup_big_NS1`) false false)
  (bind (_direction _newtrack_0) (`Timeline|Timeline` :!via `PlayFromStart` :!label _label)
    (:`Update`
      (bind _returnvalue_2 (`KismetMathLibrary.Lerp` 0.1 2.02521 _newtrack_0))
      (`SceneComponent.SetRelativeScale3D` _cone (`KismetMathLibrary.MakeVector` _returnvalue_2 _returnvalue_2 (`KismetMathLibrary.Lerp` 0.1 2.89522 _newtrack_0)))
      (`SceneComponent.K2_SetRelativeLocation` _cone (`KismetMathLibrary.MakeVector` 0.0 0.0 (`KismetMathLibrary.Lerp` -100.0 27.991792 _newtrack_0)) false false))))

(event `Turn Off`
  (`PlayerController.SetViewTargetWithBlend` (`GameplayStatics.GetPlayerController` 0) (`GameplayStatics.GetPlayerPawn` 0) 0.5 "VTBlend_EaseInOut" 3.0 true)
  (`ActorComponent.SetActive` (`self.Charging_NS_2`) true false)
  (`ActorComponent.SetActive` (`self.Pickup_big_NS1`) true false)
  (goto _label :!via `ReverseFromEnd`))

(event `self.ReceiveTick`
  (params (DeltaSeconds :type "Float (single-precision)"))
  (`parent.ReceiveTick` DeltaSeconds)
  (`SceneComponent.K2_AddLocalRotation` (`self.SwordTarget`) (struct :`Roll` 0.4) false false))

(fn `UserConstructionScript`
  (`parent.UserConstructionScript`))