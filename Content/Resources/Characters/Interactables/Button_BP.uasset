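; Interactable button that, on Interact, runs the parent behavior and relays an interact message to every connected target.
; Each press spawns a Shine Niagara effect attached to the memory sphere effect.
; Single-use buttons then destroy their sphere, effect and light, disable interaction and flatten the base to zero height with a timeline.
; Disconnected leftover graphs hold a rest, heal and save toggle and an older move-then-destroy animation.
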(event `self.Interact`
  (`parent.Interact`)
  (for _array_element (`self.Connected_target`)
    (message `/Game/Resources/Characters/Interactables/interactable_interface.msg_interact` _array_element))
  (`NiagaraFunctionLibrary.SpawnSystemAttached` "/Game/Resources/VFX/Shine_NS.Shine_NS" (`self.MemorySphere_NS`) "None" (0.0 0.0 0.0) (struct) "SnapToTarget")
  (if (`self.single use`)
    (`ActorComponent.K2_DestroyComponent` (`self.Sphere1`))
    (`ActorComponent.K2_DestroyComponent` (`self.MemorySphere_NS`))
    (`ActorComponent.K2_DestroyComponent` (`self.PointLight`))
    (set `self.Interactable` false)
    (bind (_direction _newtrack_0) (`Timeline|Timeline_0` :!via `PlayFromStart`)
      (:`Update`
        (`SceneComponent.SetRelativeScale3D` (`self.ButtonBase`) (`KismetMathLibrary.MakeVector` 0.344758 0.344758 (`KismetMathLibrary.Lerp` 0.424453 0.0 _newtrack_0)))))))

(fn `UserConstructionScript`
  (`parent.UserConstructionScript`))