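; TestButton_BP is a test interactable that spawns a Donut actor when interacted with.
; Its Interact event calls the parent implementation, prints "Hello", then spawns the Donut at a random horizontal offset of up to 100 units around its Sphere component.
; A loop forwarding Interact to ConnectedTarget actors and a second spawn node are left disconnected, so neither runs.
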(event `self.Interact`
  (`parent.Interact`)
  (`KismetSystemLibrary.PrintString` "Hello")
  (`|SpawnActorFromClass` "/Game/Resources/Characters/Interactables/Donut.Donut_C" (`KismetMathLibrary.Conv_VectorToTransform` (+ (* (`KismetMathLibrary.RandomUnitVector`) (100.0 100.0 0.0)) (`SceneComponent.K2_GetComponentLocation` (`self.Sphere`)))) "Undefined" "OverrideRootScale" null null))

(fn `UserConstructionScript`
  (`parent.UserConstructionScript`))