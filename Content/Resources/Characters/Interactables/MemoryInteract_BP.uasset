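; Collectible memory log interactable that loads its entry from the MemoryLog_DT data table by LogName and uses the title as its hint.
; Interacting shows the log text on the HUD.
; When the actor leaves, it disables sphere collision, and a timeline flies the cylinder to the player.
; It then plays a sound event, adds the log uniquely to game state, posts a HUD console notice and destroys itself.
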(event `self.ReceiveBeginPlay`
  (`parent.ReceiveBeginPlay`)
  (bind _returnvalue (`|GetDataTableRow` "/Game/Resources/Characters/Interactables/MemoryLog_DT.MemoryLog_DT" (`self.Log Name`))
    (:`then`
      (bind _output_get (set `self.Log` _returnvalue))
      (set `self.Hint` (`.Title_5_F1BD3547426FA6B7705BE295F91BBB1A` (break `/Game/Resources/Characters/Interactables/MemoryLog_Struct` _output_get))))))

(event `self.Interact`
  (bind (_log_title _log_text) (break `/Game/Resources/Characters/Interactables/MemoryLog_Struct` (`self.Log`)))
  (`parent.Interact`)
  (bind _asnew_game_mode_gm (cast `/Game/Resources/Characters/Player/Blueprints/NewGameMode_GM` (`GameplayStatics.GetGameMode`)))
  (`/Game/Resources/Widgets/HUD_Widget.Expand Message` (`/Game/Resources/Characters/Player/Blueprints/NewGameMode_GM.HUD_ref` _asnew_game_mode_gm) _log_text))

(event `self.ActorLeave`
  (`parent.ActorLeave`)
  (`PrimitiveComponent.SetCollisionEnabled` (`self.Sphere`) "NoCollision")
  (set `self.TempLocation` (`self.K2_GetActorLocation`))
  (bind (_direction _collect) (`Timeline|Timeline`)
    (:`Update`
      (`SceneComponent.K2_SetWorldLocation` (`self.Cylinder`) (`KismetMathLibrary.VLerp` (`self.TempLocation`) (`self.K2_GetActorLocation` (`GameplayStatics.GetPlayerPawn` 0)) _collect) false false))
    (:`Finished`
      (`self.On Collect`)
      (`self.K2_DestroyActor`))))

(event `On Collect`
  (bind _log_title (break `/Game/Resources/Characters/Interactables/MemoryLog_Struct` (`self.Log`)))
  (`FMODBlueprintStatics.PlayEventAtLocation` "/Game/FMOD/Events/Sounds/Scrap.Scrap" (`KismetMathLibrary.MakeTransform` (`self.K2_GetActorLocation`)))
  (bind _asnew_game_state_gs (cast `/Game/Resources/Characters/Player/Blueprints/NewGameState_GS` (`GameplayStatics.GetGameState`)))
  (`KismetArrayLibrary.Array_AddUnique` (`/Game/Resources/Characters/Player/Blueprints/NewGameState_GS.LogEntries` _asnew_game_state_gs) (`self.Log`))
  (bind _asnew_game_mode_gm (cast `/Game/Resources/Characters/Player/Blueprints/NewGameMode_GM` (`GameplayStatics.GetGameMode`)))
  (`/Game/Resources/Widgets/HUD_Widget.Add Console` (`/Game/Resources/Characters/Player/Blueprints/NewGameMode_GM.HUD_ref` _asnew_game_mode_gm) (`|FormatText` "<RichText.Emphasis>LOG FILE</> Added") _log_title 8.0 "/Game/Resources/Widgets/Textures/BuildableIcon.BuildableIcon"))

(fn `UserConstructionScript`
  (`parent.UserConstructionScript`))