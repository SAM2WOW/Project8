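; Interactable checkpoint where the player rests and the game saves.
; A FlipFlop on Interact alternates between resting the player with a full health refill and unresting them, and both branches run the save.
; The save loads or creates a NewSaveGame, copies player state, game-state scraps and modules, and the current map, writes it to the slot, then posts a HUD console notice.
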(event `self.Interact`
  (`parent.Interact`)
  (`/Engine/EditorBlueprintResources/StandardMacros.FlipFlop`
    (:`A`
      (bind _asbp_player_character (cast `/Game/Resources/Characters/Player/Blueprints/BP_PlayerCharacter` (`GameplayStatics.GetPlayerCharacter` 0)))
      (`/Game/Resources/Characters/Player/Blueprints/BP_PlayerCharacter.Rest` _asbp_player_character)
      (set `/Game/Resources/Characters/Player/Blueprints/BP_PlayerCharacter.Health` (`/Game/Resources/Characters/Player/Blueprints/BP_PlayerCharacter.MaxHealth` _asbp_player_character) _asbp_player_character))
    (:`B`
      (bind _asbp_player_character_2 (cast `/Game/Resources/Characters/Player/Blueprints/BP_PlayerCharacter` (`GameplayStatics.GetPlayerCharacter` 0)))
      (`/Game/Resources/Characters/Player/Blueprints/BP_PlayerCharacter.Unrest` _asbp_player_character_2)))
  (`|ExecutionSequence`
    (:`then_0`
      ;[0 0.5078 1] Save Data
      (bind _returnvalue (`GameplayStatics.DoesSaveGameExist` (`self.SlotName`)))
      (if _returnvalue
        (bind _returnvalue_2 (`GameplayStatics.LoadGameFromSlot` (`self.SlotName`)))
        (set `self.SaveData` _returnvalue_2)
        (else
          (bind _returnvalue_3 (`GameplayStatics.CreateSaveGameObject` "/Game/Resources/Characters/Player/Blueprints/Save/NewSaveGame.NewSaveGame_C"))
          (set `self.SaveData` _returnvalue_3)))
      (bind _asnew_save_game (cast `/Game/Resources/Characters/Player/Blueprints/Save/NewSaveGame` (`self.SaveData`)))
      (`|ExecutionSequence`
        (:`then_0`
          (bind _asbp_player_character_3 (cast `/Game/Resources/Characters/Player/Blueprints/BP_PlayerCharacter` (`GameplayStatics.GetPlayerPawn` 0)))
          (set `/Game/Resources/Characters/Player/Blueprints/Save/NewSaveGame.PlayerTransform` (`self.GetTransform` _asbp_player_character_3) _asnew_save_game)
          (set `/Game/Resources/Characters/Player/Blueprints/Save/NewSaveGame.PlayerHealth` (`/Game/Resources/Characters/Player/Blueprints/BP_PlayerCharacter.Health` _asbp_player_character_3) _asnew_save_game)
          (set `/Game/Resources/Characters/Player/Blueprints/Save/NewSaveGame.PlayerCharge` (`/Game/Resources/Characters/Player/Blueprints/BP_PlayerCharacter.DeployCharge` _asbp_player_character_3) _asnew_save_game))
        (:`then_1`
          (bind _asnew_game_state_gs (cast `/Game/Resources/Characters/Player/Blueprints/NewGameState_GS` (`GameplayStatics.GetGameState`)))
          (set `/Game/Resources/Characters/Player/Blueprints/Save/NewSaveGame.Scraps` (`/Game/Resources/Characters/Player/Blueprints/NewGameState_GS.Scraps` _asnew_game_state_gs) _asnew_save_game)
          (set `/Game/Resources/Characters/Player/Blueprints/Save/NewSaveGame.ModuleInstalled` (`/Game/Resources/Characters/Player/Blueprints/NewGameState_GS.Installed` _asnew_game_state_gs) _asnew_save_game)
          (set `/Game/Resources/Characters/Player/Blueprints/Save/NewSaveGame.ModuleInventory` (`/Game/Resources/Characters/Player/Blueprints/NewGameState_GS.Inventory` _asnew_game_state_gs) _asnew_save_game))
        (:`then_2`
          (bind _returnvalue_4 (`GameplayStatics.GetCurrentLevelName` true))
          (set `/Game/Resources/Characters/Player/Blueprints/Save/NewSaveGame.CurrentMap` _returnvalue_4 _asnew_save_game)
          (`GameplayStatics.SaveGameToSlot` _asnew_save_game (`self.SlotName`))
          (bind _asnew_game_mode_gm (cast `/Game/Resources/Characters/Player/Blueprints/NewGameMode_GM` (`GameplayStatics.GetGameMode`)))
          (`/Game/Resources/Widgets/HUD_Widget.Add Console` (`/Game/Resources/Characters/Player/Blueprints/NewGameMode_GM.HUD_ref` _asnew_game_mode_gm) "Game Saved" 8.0 null))))))

(fn `UserConstructionScript`
  (`parent.UserConstructionScript`))