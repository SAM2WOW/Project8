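; GenericLog_BP is an interactable log pickup that adds a memory log entry to the game state.
; On BeginPlay it loads its MemoryLog_DT row by LogName, then destroys itself if already logged or spawns a pickup effect.
; Interact expands the log text on the HUD.
; Leaving collects it only if the player has a valid Sword, recording the entry with sound, console notice and rumble, then destroying the actor.
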(event `self.ReceiveBeginPlay`
  (bind (_returnvalue_location _returnvalue_rotation) (`KismetMathLibrary.BreakTransform` (`self.GetTransform`)))
  (`parent.ReceiveBeginPlay`)
  (bind _returnvalue (`|GetDataTableRow` "/Game/Resources/Characters/Interactables/MemoryLog_DT.MemoryLog_DT" (`self.Log Name`))
    (:`then`
      (bind _output_get (set `self.Log` _returnvalue))
      (bind _asnew_game_state_gs (cast `/Game/Resources/Characters/Player/Blueprints/NewGameState_GS` (`GameplayStatics.GetGameState`)))
      (if (== (`KismetArrayLibrary.Array_Find` (`/Game/Resources/Characters/Player/Blueprints/NewGameState_GS.LogEntries` _asnew_game_state_gs) _output_get) -1)
        (bind (_title _text _texture) (break `/Game/Resources/Characters/Interactables/MemoryLog_Struct` _output_get))
        (set `self.Hint` _title)
        (set `self.Image` _texture)
        (bind _returnvalue_2 (`NiagaraFunctionLibrary.SpawnSystemAtLocation` "/Game/Resources/VFX/Pickup_NS.Pickup_NS" (- _returnvalue_location (0.0 0.0 20.0)) _returnvalue_rotation))
        (set `self.System` _returnvalue_2)
        (else
          (`self.K2_DestroyActor`))))))

(event `self.Interact`
  (bind (_log_title _log_text) (break `/Game/Resources/Characters/Interactables/MemoryLog_Struct` (`self.Log`)))
  (if (`self.CanInteract?`)
    (`parent.Interact`)
    (bind _asnew_game_mode_gm (cast `/Game/Resources/Characters/Player/Blueprints/NewGameMode_GM` (`GameplayStatics.GetGameMode`)))
    (`/Game/Resources/Widgets/HUD_Widget.Expand Message` (`/Game/Resources/Characters/Player/Blueprints/NewGameMode_GM.HUD_ref` _asnew_game_mode_gm) _log_text)))

(event `self.ActorLeave`
  (if (`self.CanCollect?`)
    (`parent.ActorLeave`)
    (bind _asbp_player_character (cast `/Game/Resources/Characters/Player/Blueprints/BP_PlayerCharacter` (`GameplayStatics.GetPlayerPawn` 0)))
    (`/Engine/EditorBlueprintResources/StandardMacros.IsValid` (`/Game/Resources/Characters/Player/Blueprints/BP_PlayerCharacter.Sword` _asbp_player_character)
      (:`Is Valid`
        (`self.On Collect`)
        (`self.K2_DestroyActor`)))))

(event `On Collect`
  (bind _log_title (break `/Game/Resources/Characters/Interactables/MemoryLog_Struct` (`self.Log`)))
  (set `self.Interactable` false)
  (`FMODBlueprintStatics.PlayEventAtLocation` "/Game/FMOD/Events/Sounds/Scrap.Scrap" (`KismetMathLibrary.MakeTransform` (`self.K2_GetActorLocation`)))
  (bind _asnew_game_state_gs (cast `/Game/Resources/Characters/Player/Blueprints/NewGameState_GS` (`GameplayStatics.GetGameState`)))
  (`KismetArrayLibrary.Array_AddUnique` (`/Game/Resources/Characters/Player/Blueprints/NewGameState_GS.LogEntries` _asnew_game_state_gs) (`self.Log`))
  (bind _asnew_game_mode_gm (cast `/Game/Resources/Characters/Player/Blueprints/NewGameMode_GM` (`GameplayStatics.GetGameMode`)))
  (`/Game/Resources/Widgets/HUD_Widget.Add Console` (`/Game/Resources/Characters/Player/Blueprints/NewGameMode_GM.HUD_ref` _asnew_game_mode_gm) (`self.CollectedText`) (select `bool` (`self.ShowTitle?`) :`true` _log_title) 8.0 "/Game/Resources/Widgets/Textures/Console/Log_Added.Log_Added")
  (`GameplayStatics.SpawnForceFeedbackAttached` "/Game/Resources/Characters/Weapons/Sword/Feedbacks/Collect_Feed.Collect_Feed" null "None" (0.0 0.0 0.0) (struct) "SnapToTarget" false false (`KismetMathLibrary.RandomFloatInRange` 0.2 0.9) 0.0 null))

(fn `UserConstructionScript`
  (`parent.UserConstructionScript`))