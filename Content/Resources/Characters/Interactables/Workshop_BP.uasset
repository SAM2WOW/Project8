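; Interactable workshop that puts the player into edit mode for customizing their sword.
; On Interact it deploys the player's Sword with itself as context, enables EditMode, blends the camera to the Sword and plays a shine effect and workbench sound.
; Tick slowly spins a sample module.
; A FlipFlop toggle that would exit edit mode is disconnected, so this Blueprint only handles entering it.
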(event `self.Interact`
  (`parent.Interact`)
  (bind _asbp_player_character (cast `/Game/Resources/Characters/Player/Blueprints/BP_PlayerCharacter` (`GameplayStatics.GetPlayerCharacter` 0)))
  (bind _sword (`/Game/Resources/Characters/Player/Blueprints/BP_PlayerCharacter.Sword` _asbp_player_character))
  (`/Game/Resources/Characters/Weapons/Sword/VITA_BP.DeployInteract` _sword self)
  (`/Game/Resources/Characters/Player/Blueprints/BP_PlayerCharacter.EditMode` _asbp_player_character true)
  (`PlayerController.SetViewTargetWithBlend` (`GameplayStatics.GetPlayerController` 0) _sword 1.0 "VTBlend_EaseInOut" 3.0 true)
  (`NiagaraFunctionLibrary.SpawnSystemAttached` "/Game/Resources/VFX/Shine_NS.Shine_NS" (`self.Pickup_big_NS1`) "None" (0.0 0.0 0.0) (struct) "SnapToTarget")
  (`FMODBlueprintStatics.PlayEvent2D` "/Game/FMOD/Events/Sounds/UI/UI_Workbench.UI_Workbench"))

(event `self.ReceiveTick`
  (params (DeltaSeconds :type "Float (single-precision)"))
  (`parent.ReceiveTick` DeltaSeconds)
  (`SceneComponent.K2_AddWorldRotation` (`self.SampleModule1`) (`KismetMathLibrary.MakeRotator` 0.0 0.0 (* DeltaSeconds 30.0)) false false))

(fn `UserConstructionScript`
  (`parent.UserConstructionScript`))