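; AreaTrigger_BP is an interactable trigger volume that activates linked targets when the player character enters its sphere.
; While Active, a player overlap calls Interact, which sends MsgInteractMessage to every ConnectedTarget entry and clears Active if SingleUse is set.
; An incoming MsgInteract also runs Interact, without checking Active.
; End overlap only casts to the player and has no further effect.
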(event `self.Sphere.OnComponentBeginOverlap`
  (params (OverlappedComponent :type "PrimitiveComponent Object Reference") (OtherActor :type "Actor Object Reference") (OtherComp :type "PrimitiveComponent Object Reference") (OtherBodyIndex :type Integer) (bFromSweep :type Boolean) (SweepResult :type "HitResult Structure (by ref)"))
  (if (`self.Active`)
    (cast `/Game/Resources/Characters/Player/Blueprints/BP_PlayerCharacter` OtherActor)
    (`self.Interact`)))

(event `self.Sphere.OnComponentEndOverlap`
  (params (OverlappedComponent :type "PrimitiveComponent Object Reference") (OtherActor :type "Actor Object Reference") (OtherComp :type "PrimitiveComponent Object Reference") (OtherBodyIndex :type Integer))
  (if (`self.Active`)
    (cast `/Game/Resources/Characters/Player/Blueprints/BP_PlayerCharacter` OtherActor)))

(event `Interact`
  (for _array_element (`self.Connected Target`)
    (message `/Game/Resources/Characters/Interactables/interactable_interface.msg_interact` _array_element))
  (if (`self.single use`)
    (set `self.Active` false)))

(event `/Game/Resources/Characters/Interactables/interactable_interface.msg_interact`
  (`self.Interact`))

(fn `UserConstructionScript`)