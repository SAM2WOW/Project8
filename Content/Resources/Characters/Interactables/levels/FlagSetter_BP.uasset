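; FlagSetter_BP is an interactable that records progress by setting a keyed flag in the game state.
; Interact, also triggered by MsgInteract, sets the Key flag to true on NewGameState_GS with autosave enabled.
; When IncreceLevel is enabled, it also increases the chunk and marks the level as changed in that game state.
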(event `Interact`
  (`|ExecutionSequence`
    (:`then_0`
      (bind _asnew_game_state_gs (cast `/Game/Resources/Characters/Player/Blueprints/NewGameState_GS` (`GameplayStatics.GetGameState`)))
      (`/Game/Resources/Characters/Player/Blueprints/NewGameState_GS.Set Flag` _asnew_game_state_gs (`self.Key`) true true)
      (if (`self.Increce Level`)
        (`/Game/Resources/Characters/Player/Blueprints/NewGameState_GS.Increase Chunk` _asnew_game_state_gs)
        (bind _asnew_game_state_gs_2 (cast `/Game/Resources/Characters/Player/Blueprints/NewGameState_GS` (`GameplayStatics.GetGameState`)))
        (set `/Game/Resources/Characters/Player/Blueprints/NewGameState_GS.LevelChanged` true _asnew_game_state_gs_2)))))

(event `/Game/Resources/Characters/Interactables/interactable_interface.msg_interact`
  (`self.Interact`))

(fn `UserConstructionScript`)