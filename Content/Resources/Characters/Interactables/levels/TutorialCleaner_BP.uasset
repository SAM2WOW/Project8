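; Interactable level actor that, despite its tutorial-cleaner name, restores mid-level state when play begins.
; If the game state flags RestoreMidLevelChunk, BeginPlay clears the flag, enables TeleportPlayer on GeneraterBP and sends an interact message to every connected target.
; Its own interact event is empty, and the save-game teleport check and ClearTutorial call are unwired leftovers.
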(event `self.ReceiveBeginPlay`
  (bind _asnew_game_state_gs (cast `/Game/Resources/Characters/Player/Blueprints/NewGameState_GS` (`GameplayStatics.GetGameState`)))
  (if (`/Game/Resources/Characters/Player/Blueprints/NewGameState_GS.RestoreMidLevelChunk` _asnew_game_state_gs)
    (set `/Game/Resources/Characters/Player/Blueprints/NewGameState_GS.RestoreMidLevelChunk` false _asnew_game_state_gs)
    (set `/Game/Resources/Characters/Scene/DungeonGeneration/NewDungeonGenerator_BP.teleportPlayer` true (`self.GeneraterBP`))
    (for _array_element (`self.Connected Target`)
      (message `/Game/Resources/Characters/Interactables/interactable_interface.msg_interact` _array_element))))

(event `/Game/Resources/Characters/Interactables/interactable_interface.msg_interact`)

(fn `UserConstructionScript`)