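; LevelRestore is a level interactable actor that restores mid-level progress when flagged by the game state.
; One tick after BeginPlay it consumes NewGameState_GS's RestoreMidLevelChunk flag, sets TeleportPlayer on the saved generator and prints that generator's location.
; It then sends MsgInteractMessage to every ConnectedTarget.
; An unwired save-slot check and tutorial-clearing call remain, and MsgInteract is empty.
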(event `self.ReceiveBeginPlay`
  (bind _savedgenerator (`/Game/Resources/Characters/Scene/DungeonGeneration/GeneratorFactory_BP.SavedGenerator` (`self.GeneraterBP`)))
  (`KismetSystemLibrary.DelayUntilNextTick`)
  (bind _asnew_game_state_gs (cast `/Game/Resources/Characters/Player/Blueprints/NewGameState_GS` (`GameplayStatics.GetGameState`)))
  (if (`/Game/Resources/Characters/Player/Blueprints/NewGameState_GS.RestoreMidLevelChunk` _asnew_game_state_gs)
    (set `/Game/Resources/Characters/Player/Blueprints/NewGameState_GS.RestoreMidLevelChunk` false _asnew_game_state_gs)
    (set `/Game/Resources/Characters/Scene/DungeonGeneration/NewDungeonGenerator_BP.teleportPlayer` true _savedgenerator)
    (`KismetSystemLibrary.PrintString` (`KismetStringLibrary.Conv_VectorToString` (`self.K2_GetActorLocation` _savedgenerator)) true true (struct :`R` 1.0 :`G` 0.928552 :`A` 1.0) 10.0)
    (for _array_element (`self.Connected Target`)
      (message `/Game/Resources/Characters/Interactables/interactable_interface.msg_interact` _array_element))))

(event `/Game/Resources/Characters/Interactables/interactable_interface.msg_interact`)

(fn `UserConstructionScript`)