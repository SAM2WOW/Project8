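; Destructible button that works as a damage-activated switch, reporting an "Enemy" tag and a trace channel.
; Each hit lowers Health and plays a glass sound; at zero it spawns DestructableExploded_BP with slow-mo, camera shake and Niagara effect.
; It then sends InteractMessage to every target actor and destroys itself.
; The construction script sets the Geometry Collection's rest collection, while its break events are empty and older scrap-spawning logic is disconnected.
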(event `self.ReceiveAnyDamage`
  (params (Damage :type "Float (single-precision)") (DamageType :type "DamageType Object Reference") (InstigatedBy :type "Controller Object Reference") (DamageCauser :type "Actor Object Reference"))
  (bind _returnvalue (`self.K2_GetActorLocation`))
  (bind _output_get (set `self.Health` (- (`self.Health`) Damage)))
  (`|ExecutionSequence`
    (:`then_0`
      (`FMODBlueprintStatics.PlayEventAtLocation` "/Game/FMOD/Events/Sounds/Collectables/Glass_Hit.Glass_Hit" (`self.GetTransform`)))
    (:`then_1`
      (if (<= _output_get 0.0)
        (`/Engine/EditorBlueprintResources/StandardMacros.DoOnce` false
          (:`Completed`
            (`|SpawnActorFromClass` "/Game/Resources/Characters/Destructables/DestructableExploded_BP.DestructableExploded_BP_C" (`self.GetTransform`) "AlwaysSpawn" "OverrideRootScale" null (`self.Amount`) null)
            (bind _asnew_game_state_gs (cast `/Game/Resources/Characters/Player/Blueprints/NewGameState_GS` (`GameplayStatics.GetGameState`)))
            (`/Game/Resources/Characters/Player/Blueprints/NewGameState_GS.Mini Slowmo` _asnew_game_state_gs 1.0)
            (`GameplayStatics.PlayWorldCameraShake` "/Game/Resources/Characters/Player/Blueprints/Camera/Small_CameraShake.Small_CameraShake_C" _returnvalue 200.0 2000.0)
            (`NiagaraFunctionLibrary.SpawnSystemAtLocation` "/Game/Resources/VFX/ParryHit_NS.ParryHit_NS" _returnvalue)
            (for _array_element (`self.Targetactors`)
              (message `/Game/Resources/Characters/Interactables/interactable_interface.msg_interact` _array_element))
            (`self.K2_DestroyActor`)))))))

(event `self.GeometryCollection.OnChaosBreakEvent`
  (params (BreakEvent :type "ChaosBreakEvent Structure (by ref)")))

(event `self.GeometryCollection.OnComponentSleep`
  (params (SleepingComponent :type "PrimitiveComponent Object Reference") (BoneName :type Name)))

(event `self.GeometryCollection.NotifyGeometryCollectionPhysicsStateChange`
  (params (FracturedComponent :type "GeometryCollectionComponent Object Reference")))

(fn `Get Tag`
  (returns (Tag :type Name))
  (return "Enemy"))

(fn `Get Trace Channel`
  (returns (Channel :type "ETraceTypeQuery Enum"))
  (return "TraceTypeQuery4"))

(fn `UserConstructionScript`
  (`GeometryCollectionComponent.SetRestCollection` (`self.GeometryCollection`) (`self.Rest Collection In`)))