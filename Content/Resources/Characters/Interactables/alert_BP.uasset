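; Interactable alert device that, when used, emits repeated noise for AI hearing at its own location.
; If not already Activated, Interact starts a looping timer and clears it after a delay; otherwise it clears the timer immediately.
; Each timer tick reports a loud noise event and spawns a black hole Niagara effect.
; Unconnected leftover logic covers linked-target triggering and a rest/save toggle.
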(event `self.Interact`
  (`parent.Interact`)
  (if (not (`self.activated`))
    (bind _returnvalue (`KismetSystemLibrary.K2_SetTimerDelegate` (delegate `Fire`) 1.0 true))
    (set `self.NewVar_0` _returnvalue)
    (`KismetSystemLibrary.Delay` 10.0))
  (`KismetSystemLibrary.K2_ClearAndInvalidateTimerHandle` (`self.NewVar_0`)))

(event `self.ReceiveTick`
  (params (DeltaSeconds :type "Float (single-precision)")))

(event `Fire`
  (bind _returnvalue (`self.K2_GetActorLocation`))
  (`AISense_Hearing.ReportNoiseEvent` _returnvalue 100.0 self)
  (`NiagaraFunctionLibrary.SpawnSystemAtLocation` "/Game/Resources/VFX/BlackHole_NS.BlackHole_NS" _returnvalue))

(fn `UserConstructionScript`
  (`parent.UserConstructionScript`))