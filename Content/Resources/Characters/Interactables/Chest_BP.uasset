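; Interactable loot chest that opens with a short cinematic and drops module pickups, or plays an error sound while locked.
; Locked state sets its effect and material on BeginPlay.
; Opening blends the camera, suspends input and HUD, plays a cast montage and ramps a dynamic material's emissive via Timeline.
; It then shakes the camera, spawns debris and pickups from Container plus one random data-table module, restores control and destroys itself.
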(event `self.ReceiveBeginPlay`
  (`ActorComponent.SetActive` (`self.Charging_NS_2`) (not (`self.Locked`)) false)
  (`PrimitiveComponent.SetMaterial` (`self.TheBox`) 3 (select `bool` (`self.Locked`) :`false` "/Game/Resources/Materials/Common/CheapEmmisive_Mat.CheapEmmisive_Mat" :`true` "/Game/Resources/Materials/Common/Simple_Mat_Dark.Simple_Mat_Dark" :!type "MaterialInterface Object Reference")))

(event `self.Interact`
  (bind _thebox (`self.TheBox`))
  (`parent.Interact`)
  (if (`self.Locked`)
    (`FMODBlueprintStatics.PlayEvent2D` "/Game/FMOD/Events/Sounds/UI/UI_Error.UI_Error")
    (else
      (set `self.Interactable` false)
      (`/Engine/EditorBlueprintResources/StandardMacros.DoOnce` false
        (:`Completed`
          (`FMODBlueprintStatics.PlayEvent2D` "/Game/FMOD/Events/Sounds/UI/UI_Awesome.UI_Awesome")
          ;[0 0.3437 1] Sequence
          (`self.DisableInput` (`GameplayStatics.GetPlayerPawn` 0) (`GameplayStatics.GetPlayerController` 0))
          (`PlayerController.SetViewTargetWithBlend` (`GameplayStatics.GetPlayerController` 0) self 0.5 "VTBlend_EaseInOut" 3.0 false)
          (bind _asnew_game_mode_gm (cast `/Game/Resources/Characters/Player/Blueprints/NewGameMode_GM` (`GameplayStatics.GetGameMode`)))
          (`Widget.SetRenderOpacity` (`/Game/Resources/Characters/Player/Blueprints/NewGameMode_GM.HUD_ref` _asnew_game_mode_gm) 0.0)
          (bind _asbp_player_character (cast `/Game/Resources/Characters/Player/Blueprints/BP_PlayerCharacter` (`GameplayStatics.GetPlayerCharacter` 0)))
          (`|PlayMontage` (`Character.Mesh` _asbp_player_character) "/Game/Resources/Animations/NewSelf/Standing_2H_Cast_Spell_01_Montage.Standing_2H_Cast_Spell_01_Montage"
            (:`then`
              (`ActorComponent.SetActive` (`self.Charging_NS_2`) false false)
              ;[0 0.3672 1] Cool Transform Animation
              (`FMODBlueprintStatics.PlayEventAtLocation` "/Game/FMOD/Events/Sounds/Others/Explode_Charging.Explode_Charging" (`self.GetTransform`))
              (bind _returnvalue (`PrimitiveComponent.CreateDynamicMaterialInstance` (`self.TheBox`) 0 "/Game/Resources/Materials/Common/Transform_Mat.Transform_Mat" "None"))
              (bind _output_get (set `self.Transform_Mat` _returnvalue))
              (`PrimitiveComponent.SetMaterial` _thebox 0 _output_get)
              (`PrimitiveComponent.SetMaterial` _thebox 1 _output_get)
              (`PrimitiveComponent.SetMaterial` _thebox 2 _output_get)
              (`PrimitiveComponent.SetMaterial` _thebox 3 _output_get)
              (bind (_direction _newtrack_0) (`Timeline|Timeline` :!via `PlayFromStart`)
                (:`Update`
                  (`MaterialInstanceDynamic.SetScalarParameterValue` (`self.Transform_Mat`) "Emmisive" (`KismetMathLibrary.Lerp` 0.0 10.0 _newtrack_0)))
                (:`Finished`
                  ;;[0.3828 1 0] Play Camera Shakes
                  (`GameplayStatics.PlayWorldCameraShake` "/Game/Resources/Characters/Player/Blueprints/Camera/Big_CameraShake.Big_CameraShake_C" (`self.K2_GetActorLocation`) 500.0 3000.0)
                  (`|SpawnActorFromClass` "/Game/Resources/Characters/Destructables/DestructableExploded_BP_Chest.DestructableExploded_BP_Chest_C" (`self.GetTransform`) "AlwaysSpawn" "OverrideRootScale" null 20 null)
                  (if true
                    (bind _outrownames (`DataTableFunctionLibrary.GetDataTableRowNames` "/Game/Resources/Characters/Modules/ModuleDescriptions_DT.ModuleDescriptions_DT"))
                    (`KismetArrayLibrary.Array_Add` (`self.Container`) (`KismetArrayLibrary.Array_Random` _outrownames)))
                  (for _array_element (`self.Container`)
                    (bind _returnvalue_2 (`|GetDataTableRow` "/Game/Resources/Characters/Modules/ModuleInfo_DT.ModuleInfo_DT" _array_element)
                      (:`then`
                        (`|SpawnActorFromClass` "/Game/Resources/Characters/Collectables/ModulePickup_BP.ModulePickup_BP_C" (`self.GetTransform`) "AdjustIfPossibleButAlwaysSpawn" "OverrideRootScale" null _array_element (`.Level1_31_F549955C417A318510FC59B0C3338F54` (break `/Game/Resources/Characters/Modules/ModuleInfo_Struct` _returnvalue_2)) 0 null))))
                  (`ActorComponent.K2_DestroyComponent` (`self.TheBox`))
                  (`ActorComponent.K2_DestroyComponent` (`self.squid`))
                  ;[0.7344 0 1] Sequene Ends
                  (`PlayerController.SetViewTargetWithBlend` (`GameplayStatics.GetPlayerController` 0) (`GameplayStatics.GetPlayerPawn` 0) 1.0 "VTBlend_EaseInOut" 3.0 false)
                  (`self.EnableInput` (`GameplayStatics.GetPlayerPawn` 0) (`GameplayStatics.GetPlayerController` 0))
                  (bind _asnew_game_mode_gm_2 (cast `/Game/Resources/Characters/Player/Blueprints/NewGameMode_GM` (`GameplayStatics.GetGameMode`)))
                  (`Widget.SetRenderOpacity` (`/Game/Resources/Characters/Player/Blueprints/NewGameMode_GM.HUD_ref` _asnew_game_mode_gm_2) 1.0)
                  (`KismetSystemLibrary.Delay` 1.5)
                  (`self.K2_DestroyActor`))))))))))

(fn `UserConstructionScript`
  (`parent.UserConstructionScript`))