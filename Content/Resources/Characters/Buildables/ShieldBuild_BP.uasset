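; ShieldBuild_BP is a buildable shield that expands a sphere and repels actors from other tags.
; On activation, a timeline scales Sphere1 up uniformly from zero to full size.
; When an actor overlaps the sphere, it prints that actor's name and compares tag messages.
; Actors with a differing, non-None tag receive a BounceMessage along the shield's forward vector.
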(event `self.OnActivated`
  (`parent.OnActivated`)
  (bind (_direction _newtrack_0) (`Timeline|Timeline` :!via `PlayFromStart`)
    (:`Update`
      (bind _returnvalue (`KismetMathLibrary.Lerp` 0.0 25.0 _newtrack_0))
      (`SceneComponent.SetRelativeScale3D` (`self.Sphere1`) (`KismetMathLibrary.MakeVector` _returnvalue _returnvalue _returnvalue)))))

(event `self.Sphere1.OnComponentBeginOverlap`
  (params (OverlappedComponent :type "PrimitiveComponent Object Reference") (OtherActor :type "Actor Object Reference") (OtherComp :type "PrimitiveComponent Object Reference") (OtherBodyIndex :type Integer) (bFromSweep :type Boolean) (SweepResult :type "HitResult Structure (by ref)"))
  (`KismetSystemLibrary.PrintString` (`KismetSystemLibrary.GetDisplayName` OtherActor) true true (struct :`G` 0.259517 :`B` 1.0 :`A` 1.0))
  (bind _tag (message `/Game/Resources/Characters/Modules/DamageOwner_BPInter.Get Tag` self))
  (bind _tag_2 (message `/Game/Resources/Characters/Modules/DamageOwner_BPInter.Get Tag` OtherActor))
  (if (and (!= _tag_2 "None") (!= _tag_2 _tag))
    (message `/Game/Resources/Characters/Modules/Turrets/Bullet_BPInter.Bounce` OtherActor (`KismetMathLibrary.GetForwardVector` (`self.K2_GetActorRotation`)))))

(fn `UserConstructionScript`
  (`parent.UserConstructionScript`))