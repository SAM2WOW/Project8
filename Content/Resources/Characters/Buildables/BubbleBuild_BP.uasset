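; BubbleBuild_BP is a buildable that, once activated, repeatedly sprays bubble projectiles in random directions.
; A looping timer triggers short staggered bursts of BubbleBullet_BP spawns from the StaticBubbleLayer component, passing itself as host along with its passives and base damage.
; Each shot replays the Shoot timeline to squash that layer's Z scale.
; An unconnected sphere-trace branch for aimed shots never runs.
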(event `self.OnActivated`
  (`parent.OnActivated`)
  (`KismetSystemLibrary.K2_SetTimerDelegate` (delegate `FireBubble`) 0.6 true)
  (`self.FireBubble`))

(event `FireBubble`
  (if (`self.Activated`)
    (`/Game/Resources/Characters/Player/Blueprints/NewActorMacroLibrary.ForLoopWithDelay` 0 2 0.1
      (:`Loop Body`
        (`self.Fire`)))))

(event `Fire`
  (bind (_returnvalue_roll _returnvalue_pitch _returnvalue_yaw) (`KismetMathLibrary.BreakRotator` (`KismetMathLibrary.RandomRotator` true)))
  (`|SpawnActorFromClass` "/Game/Resources/Characters/Modules/Bubble/BubbleBullet_BP.BubbleBullet_BP_C" (`KismetMathLibrary.MakeTransform` (`SceneComponent.K2_GetComponentLocation` (`self.StaticBubbleLayer`)) (`KismetMathLibrary.MakeRotator` _returnvalue_roll _returnvalue_pitch _returnvalue_yaw)) "AlwaysSpawn" "OverrideRootScale" null self (`self.Passive`) 40.0 null)
  (bind (_direction _x) (`Timeline|Shoot` :!via `PlayFromStart`)
    (:`Update`
      (`SceneComponent.SetRelativeScale3D` (`self.StaticBubbleLayer`) (`KismetMathLibrary.MakeVector` 1.0 1.0 (`KismetMathLibrary.Lerp` 2.0 0.1 _x))))))

(fn `UserConstructionScript`
  (`parent.UserConstructionScript`))