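; Goose buildable that explodes when destroyed, damaging and knocking back whatever is caught in the blast.
; On Destroyed it plays a honk audio event, spawns a scaled-up Niagara explosion, then sphere-traces around itself on the channel returned by GetTraceChannel.
; Each hit actor receives damage and an ApplyKnockback message, after which the parent's Destroyed logic runs.
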(event `self.ReceiveDestroyed`
  (bind _returnvalue (`self.K2_GetActorLocation`))
  (`FMODBlueprintStatics.PlayEventAtLocation` "/Game/FMOD/Events/Sounds/Module/Honk.Honk" (`self.GetTransform`))
  (`NiagaraFunctionLibrary.SpawnSystemAtLocation` "/Game/Resources/VFX/Bomlistic_NS.Bomlistic_NS" (`self.K2_GetActorLocation`) (struct) (6.0 6.0 6.0))
  (bind _channel (`/Game/Resources/Characters/Modules/DamageOwner_BPInter.Get Trace Channel`))
  (bind (_outhits _returnvalue_2) (`KismetSystemLibrary.SphereTraceMulti` _returnvalue _returnvalue 300.0 _channel))
  (if _returnvalue_2
    (for _array_element _outhits
      (`GameplayStatics.ApplyDamage` (`.HitActor` (`GameplayStatics.BreakHitResult` _array_element)) 300.0 null self "/Script/Engine.DamageType")
      (message `/Game/Resources/Characters/Player/Blueprints/ApplyingStat_BPInter.Apply Knockback` (`.HitActor` (`GameplayStatics.BreakHitResult` _array_element)) self 400.0 200.0)))
  (`parent.ReceiveDestroyed`))

(fn `UserConstructionScript`
  (`parent.UserConstructionScript`))