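; CutterBuild_BP is a spinning cutter buildable that damages actors within a small radius and knocks characters away while activated.
; A looping timer runs a sphere trace on the parent's channel, applying damage and launching hit characters outward with slight lift.
; Hits speed up the RotatingMovement spin until a retriggerable delay slows it, and drive the "Hit" parameter of an attached looping sound event.
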(event `self.ReceiveBeginPlay`
  (`parent.ReceiveBeginPlay`)
  (`KismetSystemLibrary.K2_SetTimer` null "Fire" 0.1 true)
  (bind _returnvalue (`FMODBlueprintStatics.PlayEventAttached` "/Game/FMOD/Events/Sounds/Module/Cutter_Fire.Cutter_Fire" (`self.Sphere_0`) "None" (0.0 0.0 0.0) "SnapToTarget" true true false))
  (set `self.SoundEvent` _returnvalue)
  (`ActorComponent.SetComponentTickEnabled` (`self.RotatingMovement`) true))

(event `Fire`
  (bind _returnvalue (`self.K2_GetActorLocation`))
  (bind _soundevent (`self.SoundEvent`))
  (if (`self.Activated`)
    (`|ExecutionSequence`
      (:`then_0`
        (bind _channel (message `/Game/Resources/Characters/Modules/ModuleOwner_BPInter.Get Trace Channel` (`self.Parent`)))
        (bind (_outhits _returnvalue_2) (`KismetSystemLibrary.SphereTraceMulti` _returnvalue _returnvalue 120.0 _channel))
        (if _returnvalue_2
          (set `RotatingMovementComponent.RotationRate` (struct :`Yaw` 1000.0) (`self.RotatingMovement`))
          (`|ExecutionSequence`
            (:`then_0`
              (`FMODAudioComponent.SetParameter` _soundevent "Hit" 0.5)
              (for _array_element _outhits
                (`GameplayStatics.ApplyDamage` (`.HitActor` (`GameplayStatics.BreakHitResult` _array_element)) 10.0 null (`self.Parent`) "/Script/Engine.DamageType")
                (bind _ascharacter (cast `Character` (`.HitActor` (`GameplayStatics.BreakHitResult` _array_element))))
                (bind (_returnvalue_x _returnvalue_y) (`KismetMathLibrary.BreakVector` (`KismetMathLibrary.GetForwardVector` (`KismetMathLibrary.FindLookAtRotation` (`self.K2_GetActorLocation`) (`self.K2_GetActorLocation` _ascharacter)))))
                (`Character.LaunchCharacter` _ascharacter (+ (* (`KismetMathLibrary.MakeVector` _returnvalue_x _returnvalue_y) 1000.0) (0.0 0.0 50.0)) false false)))
            (:`then_1`
              (`KismetSystemLibrary.RetriggerableDelay` 0.2)
              (set `RotatingMovementComponent.RotationRate` (struct :`Yaw` 300.0) (`self.RotatingMovement`))))
          (else
            (`FMODAudioComponent.SetParameter` _soundevent "Hit" 0.0)))))))

(fn `UserConstructionScript`
  (`parent.UserConstructionScript`))