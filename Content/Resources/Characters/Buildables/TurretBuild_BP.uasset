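; TurretBuild_BP is a buildable turret that automatically shoots at actors around it while activated.
; A looping timer calls Fire, which sphere-traces around the turret on the channel returned by GetTraceChannel.
; On a hit, it spawns a BulletBase_BP at the Cylinder, rotated toward the hit actor, passing itself as host along with the target and passives.
; The Shoot timeline animates the Cylinder's Z scale as firing feedback.
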(event `self.ReceiveBeginPlay`
  (`parent.ReceiveBeginPlay`)
  (`KismetSystemLibrary.K2_SetTimer` null "Fire" 0.2 true))

(event `Fire`
  (bind _returnvalue (`self.K2_GetActorLocation`))
  (bind _returnvalue_2 (`SceneComponent.K2_GetComponentLocation` (`self.Cylinder`)))
  (if (`self.Activated`)
    (bind _channel (`/Game/Resources/Characters/Modules/ModuleOwner_BPInter.Get Trace Channel`))
    (bind (_outhit _returnvalue_3) (`KismetSystemLibrary.SphereTraceSingle` :`Start` _returnvalue :`End` _returnvalue :`Radius` 1000.0 :`TraceChannel` _channel :`DrawDebugType` "ForDuration"))
    (if _returnvalue_3
      (bind (_bblockinghit _binitialoverlap _time _distance _location _impactpoint _normal _impactnormal _physmat _hitactor) (`GameplayStatics.BreakHitResult` _outhit))
      (`|SpawnActorFromClass` "/Game/Resources/Characters/Modules/Turrets/BulletBase_BP.BulletBase_BP_C" (`KismetMathLibrary.MakeTransform` _returnvalue_2 (`KismetMathLibrary.FindLookAtRotation` _returnvalue_2 (`self.K2_GetActorLocation` _hitactor))) "AlwaysSpawn" "OverrideRootScale" null (`self.Passive`) 10.0 self _hitactor null)
      (bind (_direction _x) (`Timeline|Shoot` :!via `PlayFromStart`)
        (:`Update`
          (`SceneComponent.SetRelativeScale3D` (`self.Cylinder`) (`KismetMathLibrary.MakeVector` 0.477184 0.477184 (`KismetMathLibrary.Lerp` 0.8 0.2 _x))))))))

(fn `UserConstructionScript`
  (`parent.UserConstructionScript`))