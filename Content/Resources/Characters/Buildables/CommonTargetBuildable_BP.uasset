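; Base-named buildable Blueprint for a deployable that auto-attacks a target using an attached weapon module.
; On activation it attaches the child-actor module to its body housing through the module manager, starts a looping fire timer and searches once for a target.
; The search sphere-traces within range, checks line of sight and passes the locked target to the module manager.
; The code rotating the housing toward the target is disconnected and never runs.
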(event `self.OnActivated`
  (`parent.OnActivated`)
  (`/Game/Resources/Characters/Modules/ModuleManager_BPC.Attach Module` (`self.ModuleManager_BPC`) (cast `/Game/Resources/Characters/Modules/ModuleBase_BP` (`ChildActorComponent.ChildActor` (`self.ModuleChildBP`)) :!pure true) (`SceneComponent.K2_GetComponentLocation` (`self.ModuleChildBP`)) (`self.DeployableBody1_Housing`))
  (`KismetSystemLibrary.K2_SetTimer` null "Fire" (`self.AttackInterval`) true)
  (`self.Find Target`))

(event `Find Target`
  (bind _returnvalue (`self.K2_GetActorLocation`))
  (if (`self.Activated`)
    (bind _channel (`/Game/Resources/Characters/Modules/DamageOwner_BPInter.Get Trace Channel`))
    (bind (_outhit _returnvalue_2) (`KismetSystemLibrary.SphereTraceSingle` _returnvalue _returnvalue (`self.TargetDistance`) _channel))
    (if _returnvalue_2
      (bind (_bblockinghit _binitialoverlap _time _distance _location _impactpoint _normal _impactnormal _physmat _hitactor) (`GameplayStatics.BreakHitResult` _outhit))
      (bind (_outhit_2 _returnvalue_3) (`KismetSystemLibrary.LineTraceSingle` _returnvalue _location "TraceTypeQuery1"))
      (if (not _returnvalue_3)
        (bind _output_get (set `self.LockedTarget` _hitactor))
        (`/Game/Resources/Characters/Modules/ModuleManager_BPC.Update Locked Target` (`self.ModuleManager_BPC`) _output_get)))))

(event `Fire`
  (`/Game/Resources/Characters/Modules/ModuleManager_BPC.LightAttack` (`self.ModuleManager_BPC`)))

(event `self.ReceiveTick`
  (params (DeltaSeconds :type "Float (single-precision)"))
  (`parent.ReceiveTick` DeltaSeconds))

(fn `UserConstructionScript`
  (`parent.UserConstructionScript`))