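; TurretBuild_BP is a buildable turret that automatically shoots at targets within a fixed radius.
; On activation, a looping timer calls Fire, which sphere-traces around the turret on the channel from GetTraceChannel while it stays active.
; A hit spawns a CommonBullet_BP aimed from the Arrow at the hit actor, passing the turret as host along with its passives.
; The Rotator then snaps its yaw to the target, and the Shoot timeline squashes its Z scale as firing feedback.
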(event `self.OnActivated`
  (`parent.OnActivated`)
  (`KismetSystemLibrary.K2_SetTimer` null "Fire" 0.2 true)
  (`self.Fire`))

(event `Fire`
  (bind _returnvalue (`self.K2_GetActorLocation`))
  (bind _returnvalue_2 (`SceneComponent.K2_GetComponentLocation` (`self.Arrow`)))
  (if (`self.Activated`)
    (bind _channel (`/Game/Resources/Characters/Modules/DamageOwner_BPInter.Get Trace Channel`))
    (bind (_outhit _returnvalue_3) (`KismetSystemLibrary.SphereTraceSingle` _returnvalue _returnvalue 1000.0 _channel))
    (if _returnvalue_3
      (bind (_bblockinghit _binitialoverlap _time _distance _location _impactpoint _normal _impactnormal _physmat _hitactor) (`GameplayStatics.BreakHitResult` _outhit))
      (`|SpawnActorFromClass` "/Game/Resources/Characters/Modules/Turrets/CommonBullet_BP.CommonBullet_BP_C" (`KismetMathLibrary.MakeTransform` _returnvalue_2 (`KismetMathLibrary.FindLookAtRotation` _returnvalue_2 (`self.K2_GetActorLocation` _hitactor))) "AlwaysSpawn" "OverrideRootScale" null self (`self.Passive`) 10.0 null)
      (bind (_returnvalue_roll _returnvalue_pitch _returnvalue_yaw) (`KismetMathLibrary.BreakRotator` (`KismetMathLibrary.FindLookAtRotation` (`self.K2_GetActorLocation`) (`self.K2_GetActorLocation` _hitactor))))
      (`SceneComponent.K2_SetWorldRotation` (`self.Rotator`) (`KismetMathLibrary.MakeRotator` 0.0 0.0 _returnvalue_yaw) false false)
      (bind (_direction _x) (`Timeline|Shoot` :!via `PlayFromStart`)
        (:`Update`
          (`SceneComponent.SetRelativeScale3D` (`self.Rotator`) (`KismetMathLibrary.MakeVector` 3.085534 3.085534 (`KismetMathLibrary.Lerp` 3.085534 2.394606 _x))))))))

(fn `UserConstructionScript`
  (`parent.UserConstructionScript`))