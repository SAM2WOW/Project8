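; Base Blueprint for buildable actors, which inherit their team tag and trace channel from a Parent, decay over time and drop scraps when destroyed.
; On BeginPlay it sets sphere collision for that channel, animates to its target location via a timeline, and registers a team-typed health bar with the game state.
; Tick drains health, AnyDamage subtracts hits from causers lacking its tag, and zero health destroys the actor.
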(event `self.ReceiveBeginPlay`
  (bind (_targetlocation_x _targetlocation_y _targetlocation_z) (`KismetMathLibrary.BreakVector` (`self.TargetLocation`)))
  (bind (_templocation_x _templocation_y _templocation_z) (`KismetMathLibrary.BreakVector` (`self.TempLocation`)))
  (`|ExecutionSequence`
    (:`then_0`
      (set `self.Tags` (`Actor.Tags` (`self.Parent`)))
      (set `self.TempLocation` (`self.K2_GetActorLocation`))
      (set `self.Health` (`self.MaxHealth`))
      (bind _channel (message `/Game/Resources/Characters/Modules/ModuleOwner_BPInter.Get Trace Channel` (`self.Parent`))) ; This is a stupid way of doing this
      (bind _output_get (set `self.Trace Channel` _channel))
      (`PrimitiveComponent.SetCollisionResponseToChannel` (`self.Sphere`) (select `ETraceTypeQuery` _output_get :`TraceTypeQuery1` "ECC_WorldStatic" :`TraceTypeQuery2` "ECC_WorldStatic" :`TraceTypeQuery3` "ECC_GameTraceChannel2" :`TraceTypeQuery4` "ECC_GameTraceChannel1" :!type "ECollisionChannel Enum") "ECR_Block"))
    (:`then_1`
      (bind (_direction _xy _z) (`Timeline|Spawn` :!via `PlayFromStart`)
        (:`Update`
          (`self.K2_SetActorLocation` (`KismetMathLibrary.MakeVector` (`KismetMathLibrary.Lerp` _templocation_x _targetlocation_x _xy) (`KismetMathLibrary.Lerp` _templocation_y _targetlocation_y _xy) (`KismetMathLibrary.Lerp` _templocation_z _targetlocation_z _z))))
        (:`Finished`
          (set `self.Activated` true))))
    (:`then_2`
      ;[0.9453 1 0] Connect the Health Widget
      (bind _asenemy_health_widget (cast `/Game/Resources/Widgets/EnemyHealth_Widget` (`WidgetComponent.GetWidget` (`self.Widget`))))
      (bind _output_get_2 (set `self.HealthWidget` _asenemy_health_widget))
      (set `/Game/Resources/Widgets/EnemyHealth_Widget.MaxHealth` (`self.MaxHealth`) _output_get_2)
      (bind _channel_2 (`self.Get Trace Channel`)) ; This is a stupid way of doing this
      (set `/Game/Resources/Widgets/EnemyHealth_Widget.Type` (select `ETraceTypeQuery` _channel_2 :`TraceTypeQuery1` "NewEnumerator0" :`TraceTypeQuery2` "NewEnumerator0" :`TraceTypeQuery3` "NewEnumerator2" :`TraceTypeQuery4` "NewEnumerator1" :!type "/Game/Resources/Widgets/Healthbar_Enum Enum") _asenemy_health_widget)
      ;;[0 1 0.8594] Funky Health Bar
      (bind _asnew_game_state_gs (cast `/Game/Resources/Characters/Player/Blueprints/NewGameState_GS` (`GameplayStatics.GetGameState`)))
      (`KismetArrayLibrary.Array_Add` (`/Game/Resources/Characters/Player/Blueprints/NewGameState_GS.HealthBars` _asnew_game_state_gs) (`self.HealthWidget`)))))

(event `self.ReceiveTick`
  (params (DeltaSeconds :type "Float (single-precision)"))
  (set `self.Health` (- (`self.Health`) (* DeltaSeconds (`self.DyingSpeed`))))
  ;[0.2656 0 1] Update Health Bar
  (set `/Game/Resources/Widgets/EnemyHealth_Widget.Health` (`self.Health`) (`self.HealthWidget`))
  (if (<= (stale `self.ReceiveAnyDamage` _output_get) 0.0) :!label _label
    (`self.K2_DestroyActor`)))

(event `self.ReceiveAnyDamage`
  (params (Damage :type "Float (single-precision)") (DamageType :type "DamageType Object Reference") (InstigatedBy :type "Controller Object Reference") (DamageCauser :type "Actor Object Reference"))
  (`KismetSystemLibrary.PrintString` (`KismetTextLibrary.Conv_TextToString` (`|FormatText` (`KismetSystemLibrary.GetDisplayName` self) "{self} got HIT by {name}! -{damge}" (`KismetSystemLibrary.GetDisplayName` DamageCauser) Damage)) true true (struct :`R` 1.0 :`B` 0.181067 :`A` 1.0))
  (bind _tag (`self.Get Tag`))
  (if (not (`self.ActorHasTag` DamageCauser _tag))
    (bind _output_get (set `self.Health` (- (`self.Health`) Damage)))
    (`/Game/Resources/Widgets/EnemyHealth_Widget.Received Damage` (`self.HealthWidget`))
    (goto _label)))

(event `self.ReceiveDestroyed`
  (for _ (range 2)
    (`|SpawnActorFromClass` "/Game/Resources/Characters/Collectables/Scraps_BP.Scraps_BP_C" (`KismetMathLibrary.MakeTransform` (`self.K2_GetActorLocation`)) "AlwaysSpawn" "OverrideRootScale" null null)))

(fn `Get Tag`
  (returns (Tag :type Name))
  (return (`|GetArrayItem` (`self.Tags`))))

(fn `Get Trace Channel`
  (returns (Channel :type "ETraceTypeQuery Enum"))
  (return (`self.Trace Channel`)))

(fn `UserConstructionScript`)