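; DroneBuild_BP is a one-shot buildable that releases three homing-target drones when something enters its range.
; While activated, a looping timer sphere-traces around it on the parent-supplied channel as a timeline bobs Cylinder1.
; On a hit it deactivates and spawns ModDrone_BP actors at random offsets, passing each the hit actor and a lifetime.
; The Shoot timeline then squashes its meshes and destroys the actor.
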(event `self.ReceiveBeginPlay`
  (`parent.ReceiveBeginPlay`)
  (`KismetSystemLibrary.K2_SetTimer` null "Fire" 1.0 true)
  (bind (_direction _newtrack_0) (`Timeline|Timeline` :!label _label)
    (:`Update`
      (`SceneComponent.K2_AddLocalOffset` (`self.Cylinder1`) (`KismetMathLibrary.MakeVector` 0.0 0.0 (`KismetMathLibrary.Lerp` -1.0 1.0 _newtrack_0)) false false))))

(event `Fire`
  (bind _returnvalue (`self.K2_GetActorLocation`))
  (bind _returnvalue_2 (`SceneComponent.K2_GetComponentLocation` (`self.Cylinder`)))
  (bind _returnvalue_3 (+ (* (`KismetMathLibrary.RandomUnitVector`) (100.0 100.0 0.0)) _returnvalue_2))
  (if (`self.Activated`)
    (bind _channel (message `/Game/Resources/Characters/Modules/DamageOwner_BPInter.Get Trace Channel` (`self.Parent`)))
    (bind (_outhit _returnvalue_4) (`KismetSystemLibrary.SphereTraceSingle` _returnvalue _returnvalue 1000.0 _channel))
    (if _returnvalue_4
      (set `self.dead` true)
      (set `self.Activated` false)
      (`|ExecutionSequence`
        (:`then_0`
          (goto _label :!via `Stop`))
        (:`then_1`
          (bind (_bblockinghit _binitialoverlap _time _distance _location _impactpoint _normal _impactnormal _physmat _hitactor) (`GameplayStatics.BreakHitResult` _outhit))
          (bind _returnvalue_5 (`KismetMathLibrary.FindLookAtRotation` _returnvalue_2 (`self.K2_GetActorLocation` _hitactor)))
          (bind _returnvalue_6 (`|SpawnActorFromClass` "/Game/Resources/Characters/Modules/Drone/ModDrone_BP.ModDrone_BP_C" (`KismetMathLibrary.MakeTransform` _returnvalue_3 _returnvalue_5) "AlwaysSpawn" "OverrideRootScale" null null (struct) null))
          (set `/Game/Resources/Characters/Modules/Drone/ModDrone_BP.target` _hitactor _returnvalue_6)
          (set `/Game/Resources/Characters/Modules/Drone/ModDrone_BP.life` 15.0 _returnvalue_6)
          (bind _returnvalue_7 (`|SpawnActorFromClass` "/Game/Resources/Characters/Modules/Drone/ModDrone_BP.ModDrone_BP_C" (`KismetMathLibrary.MakeTransform` _returnvalue_3 _returnvalue_5) "AlwaysSpawn" "OverrideRootScale" null null (struct) null))
          (set `/Game/Resources/Characters/Modules/Drone/ModDrone_BP.target` _hitactor _returnvalue_7)
          (set `/Game/Resources/Characters/Modules/Drone/ModDrone_BP.life` 15.0 _returnvalue_7)
          (bind _returnvalue_8 (`|SpawnActorFromClass` "/Game/Resources/Characters/Modules/Drone/ModDrone_BP.ModDrone_BP_C" (`KismetMathLibrary.MakeTransform` _returnvalue_3 _returnvalue_5) "AlwaysSpawn" "OverrideRootScale" null null (struct) null))
          (set `/Game/Resources/Characters/Modules/Drone/ModDrone_BP.target` _hitactor _returnvalue_8)
          (set `/Game/Resources/Characters/Modules/Drone/ModDrone_BP.life` 15.0 _returnvalue_8)
          (bind (_direction _x) (`Timeline|Shoot`)
            (:`Update`
              (bind _returnvalue_9 (`KismetMathLibrary.Lerp` 0.6 0.2 _x))
              (`SceneComponent.SetRelativeScale3D` (`self.Cylinder1`) (`KismetMathLibrary.MakeVector` 0.477184 0.477184 _returnvalue_9))
              (`SceneComponent.SetRelativeScale3D` (`self.base`) (`KismetMathLibrary.MakeVector` 0.477184 0.477184 _returnvalue_9)))
            (:`Finished`
              (`self.K2_DestroyActor`))))))))

(fn `UserConstructionScript`
  (`parent.UserConstructionScript`))