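; Confetti cannon buildable that acts as a one-shot proximity trap.
; Once activated, a per-tick sphere trace on the channel from GetTraceChannel triggers it a single time, marking it dead and stretching its cylinder via the Shoot timeline.
; Fire then spawns confetti Niagara and sound, applies damage and knockback to hits from a wider multi-sphere trace (debug drawing left on), and the actor destroys itself shortly after.
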(event `self.ReceiveBeginPlay`
  (`parent.ReceiveBeginPlay`))

(event `self.ReceiveTick`
  (params (DeltaSeconds :type "Float (single-precision)"))
  (bind _returnvalue (`self.K2_GetActorLocation`))
  (`parent.ReceiveTick` DeltaSeconds)
  (if (and (`self.Activated`) (not (`self.dead`)))
    (bind _channel (`/Game/Resources/Characters/Modules/DamageOwner_BPInter.Get Trace Channel`))
    (bind (_outhit _returnvalue_2) (`KismetSystemLibrary.SphereTraceSingle` _returnvalue _returnvalue 150.0 _channel))
    (if _returnvalue_2
      (`/Engine/EditorBlueprintResources/StandardMacros.DoOnce` false
        (:`Completed`
          (set `self.dead` true)
          (bind (_direction _x) (`Timeline|Shoot` :!via `PlayFromStart`)
            (:`Update`
              (`SceneComponent.SetRelativeScale3D` (`self.Cylinder2`) (`KismetMathLibrary.MakeVector` 0.353112 0.353112 (`KismetMathLibrary.Lerp` 0.353112 0.8 _x))))
            (:`Finished`
              (`self.Fire`)
              (`KismetSystemLibrary.Delay` 0.1)
              (`self.K2_DestroyActor`))))))))

(event `self.ReceiveDestroyed`
  (`parent.ReceiveDestroyed`))

(event `Fire`
  (bind _returnvalue (`self.K2_GetActorLocation`))
  (`NiagaraFunctionLibrary.SpawnSystemAtLocation` "/Game/Resources/VFX/TestParticle/Confetti_NS.Confetti_NS" (+ (`self.K2_GetActorLocation`) (0.0 0.0 50.0)) (struct :`Pitch` 90.0))
  (`FMODBlueprintStatics.PlayEventAtLocation` "/Game/FMOD/Events/Sounds/Module/Confetti_Fire.Confetti_Fire" (`self.GetTransform`))
  (bind _channel (`/Game/Resources/Characters/Modules/DamageOwner_BPInter.Get Trace Channel`))
  (bind (_outhits _returnvalue_2) (`KismetSystemLibrary.SphereTraceMulti` :`Start` _returnvalue :`End` _returnvalue :`Radius` 300.0 :`TraceChannel` _channel :`DrawDebugType` "ForDuration"))
  (if _returnvalue_2
    (for _array_element _outhits
      (`GameplayStatics.ApplyDamage` (`.HitActor` (`GameplayStatics.BreakHitResult` _array_element)) 500.0 null self "/Script/Engine.DamageType")
      (message `/Game/Resources/Characters/Player/Blueprints/ApplyingStat_BPInter.Apply Knockback` (`.HitActor` (`GameplayStatics.BreakHitResult` _array_element)) self 1500.0 600.0))))

(fn `UserConstructionScript`
  (`parent.UserConstructionScript`))