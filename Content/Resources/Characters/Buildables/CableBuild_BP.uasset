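; CableBuild_BP is a buildable actor that drops health when it is destroyed.
; On Destroyed it runs the parent logic, plays the Healing event at its location, then spawns a random handful of Health_BP actors there, each with a random yaw and a small random Amount.
; BeginPlay, overlap and Tick are disabled stubs, and the construction script only calls the parent.
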(event `self.ReceiveDestroyed`
  (bind (_returnvalue_roll _returnvalue_pitch _returnvalue_yaw) (`KismetMathLibrary.BreakRotator` (`KismetMathLibrary.RandomRotator` false)))
  (`parent.ReceiveDestroyed`)
  (`FMODBlueprintStatics.PlayEventAtLocation` "/Game/FMOD/Events/Sounds/Player/Healing.Healing" (`KismetMathLibrary.MakeTransform` (`self.K2_GetActorLocation`)))
  (for _ (range (+ (`KismetMathLibrary.RandomIntegerInRange` 5 8) 1))
    (`|SpawnActorFromClass` "/Game/Resources/Characters/Collectables/Health_BP.Health_BP_C" (`KismetMathLibrary.MakeTransform` (`self.K2_GetActorLocation`) (`KismetMathLibrary.MakeRotator` 0.0 0.0 _returnvalue_yaw)) "Undefined" "OverrideRootScale" null (`KismetMathLibrary.RandomInteger` 5) null)))

(fn `UserConstructionScript`
  (`parent.UserConstructionScript`))