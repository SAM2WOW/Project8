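; Legacy zone buildable that pulses on a looping timer, damaging actors around it and knocking them straight up.
; Each pulse raises Charge toward a cap, scaling the sphere trace radius, damage, launch height and Sphere2 visual, while a timeline animates Sphere1.
; A retriggerable delay resets Charge and hides Sphere2, but it outlasts the timer interval, so it completes only if pulsing stops.
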(event `self.ReceiveBeginPlay`
  (`parent.ReceiveBeginPlay`)
  (`KismetSystemLibrary.K2_SetTimer` null "Fire" 0.5 true))

(event `Fire`
  (bind _returnvalue (`self.K2_GetActorLocation`))
  (`SceneComponent.SetVisibility` (`self.Sphere2`) true false)
  (bind _output_get (set `self.Charge` (`KismetMathLibrary.FMin` (+ (`self.Charge`) 0.1) 1.0)))
  (`SceneComponent.SetRelativeScale3D` (`self.Sphere2`) (`KismetMathLibrary.VLerp` (2.0 2.0 2.0) (8.0 8.0 8.0) _output_get))
  (`|ExecutionSequence`
    (:`then_0`
      (bind _channel (`/Game/Resources/Characters/Modules/DamageOwner_BPInter.Get Trace Channel`))
      (bind (_outhits _returnvalue_2) (`KismetSystemLibrary.SphereTraceMulti` _returnvalue _returnvalue (`KismetMathLibrary.Lerp` 150.0 300.0 (`self.Charge`)) _channel))
      (if _returnvalue_2
        (for _array_element _outhits
          (`GameplayStatics.ApplyDamage` (`.HitActor` (`GameplayStatics.BreakHitResult` _array_element)) (`KismetMathLibrary.Lerp` 10.0 60.0 (`self.Charge`)) null self "/Script/Engine.DamageType")
          (message `/Game/Resources/Characters/Player/Blueprints/ApplyingStat_BPInter.Apply Knockback` (`.HitActor` (`GameplayStatics.BreakHitResult` _array_element)) self 0.0 (`KismetMathLibrary.Lerp` 100.0 400.0 (`self.Charge`))))))
    (:`then_1`
      (`KismetSystemLibrary.RetriggerableDelay` 0.7)
      (`SceneComponent.SetVisibility` (`self.Sphere2`) false false)
      (set `self.Charge` 0.0)
      (`SceneComponent.SetRelativeScale3D` (`self.Sphere2`) (3.0 3.0 3.0)))
    (:`then_2`
      (bind (_direction _x) (`Timeline|Timeline` :!via `PlayFromStart`)
        (:`Update`
          (bind _returnvalue_3 (`KismetMathLibrary.Lerp` 0.5 0.25 _x))
          (`SceneComponent.SetRelativeScale3D` (`self.Sphere1`) (`KismetMathLibrary.MakeVector` _returnvalue_3 _returnvalue_3 _returnvalue_3)))))))

(fn `UserConstructionScript`
  (`parent.UserConstructionScript`))