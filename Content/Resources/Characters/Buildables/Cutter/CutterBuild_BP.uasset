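; Cutter buildable Blueprint that travels steadily along its local X axis, damaging and knocking back what it touches.
; A fast looping timer runs Fire, which, while activated, sphere-traces around Sphere0 and applies damage and a knockback message to each hit.
; An attached looping-style sound event gets its Hit parameter set from the trace result.
; Targeting, rotation and scaling logic is left disconnected, and Navigate is empty.
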(event `self.ReceiveBeginPlay`
  (`parent.ReceiveBeginPlay`)
  (`KismetSystemLibrary.K2_SetTimer` null "Fire" 0.05 true)
  (bind _returnvalue (`FMODBlueprintStatics.PlayEventAttached` "/Game/FMOD/Events/Sounds/Module/Cutter_Fire.Cutter_Fire" (`self.Sphere_0`) "None" (0.0 0.0 0.0) "SnapToTarget" true true false))
  (set `self.SoundEvent` _returnvalue))

(event `Fire`
  (bind _soundevent (`self.SoundEvent`))
  (bind _returnvalue (`SceneComponent.K2_GetComponentLocation` (`self.Sphere_0`)))
  (if (`self.Activated`)
    (`|ExecutionSequence`
      (:`then_0`
        (bind _channel (`/Game/Resources/Characters/Modules/DamageOwner_BPInter.Get Trace Channel`))
        (bind (_outhits _returnvalue_2) (`KismetSystemLibrary.SphereTraceMulti` _returnvalue _returnvalue 150.0 _channel))
        (if _returnvalue_2
          (`FMODAudioComponent.SetParameter` _soundevent "Hit" 0.5)
          (for _array_element _outhits
            (`GameplayStatics.ApplyDamage` (`.HitActor` (`GameplayStatics.BreakHitResult` _array_element)) 5.0 null self "/Script/Engine.DamageType")
            (message `/Game/Resources/Characters/Player/Blueprints/ApplyingStat_BPInter.Apply Knockback` (`.HitActor` (`GameplayStatics.BreakHitResult` _array_element)) self 1000.0 50.0))
          (else
            (`FMODAudioComponent.SetParameter` _soundevent "Hit" 0.0)))))))

(event `self.ReceiveTick`
  (params (DeltaSeconds :type "Float (single-precision)"))
  (`parent.ReceiveTick` DeltaSeconds)
  (`self.K2_AddActorLocalOffset` (`KismetMathLibrary.MakeVector` (* DeltaSeconds 200.0))))

(event `Navigate`)

(fn `UserConstructionScript`
  (`parent.UserConstructionScript`))