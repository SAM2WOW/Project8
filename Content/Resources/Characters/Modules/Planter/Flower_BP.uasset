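; Flower actor in the Planter character module that pops up at a random size when it begins play.
; BeginPlay plays the Planter_Fire audio event at its location and gives the plane one of three flower material instances at random.
; A timeline's Explode curve then scales the whole actor uniformly from zero to a random target scale.
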(event `self.ReceiveBeginPlay`
  (`FMODBlueprintStatics.PlayEventAtLocation` "/Game/FMOD/Events/Sounds/Module/Planter_Fire.Planter_Fire" (`self.GetTransform`))
  (`PrimitiveComponent.SetMaterial` (`self.Plane`) 0 (select `int` (`KismetMathLibrary.RandomInteger` 3) :`0` "/Game/Resources/Characters/Modules/Planter/Flower_Mat_Inst.Flower_Mat_Inst" :`1` "/Game/Resources/Characters/Modules/Planter/Flower_Mat_Inst1.Flower_Mat_Inst1" :`2` "/Game/Resources/Characters/Modules/Planter/Flower_Mat_Inst2.Flower_Mat_Inst2" :!type "MaterialInterface Object Reference"))
  (set `self.TargetScale` (`KismetMathLibrary.RandomFloatInRange` 0.2 1.5))
  (bind (_direction _explode) (`Timeline|Timeline` :!via `PlayFromStart`)
    (:`Update`
      (bind _returnvalue (`KismetMathLibrary.Lerp` 0.0 (`self.TargetScale`) _explode))
      (`self.SetActorScale3D` (`KismetMathLibrary.MakeVector` _returnvalue _returnvalue _returnvalue)))))

(fn `UserConstructionScript`)