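; Mushroom_BP is a healing pickup from the Planter character module that restores health to an actor that touches it.
; On spawn it plays the Planter_Fire audio event at its location and grows from zero to full scale through a timeline-driven lerp.
; Each tick it yaws to face the player camera.
; Capsule overlap sends a healing message through the ApplyingStat_BPInter interface, then destroys the mushroom.
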(event `self.ReceiveBeginPlay`
  (`FMODBlueprintStatics.PlayEventAtLocation` "/Game/FMOD/Events/Sounds/Module/Planter_Fire.Planter_Fire" (`self.GetTransform`))
  (set `self.TargetScale` 1.0)
  (bind (_direction _explode) (`Timeline|Timeline` :!via `PlayFromStart`)
    (:`Update`
      (bind _returnvalue (`KismetMathLibrary.Lerp` 0.0 (`self.TargetScale`) _explode))
      (`self.SetActorScale3D` (`KismetMathLibrary.MakeVector` _returnvalue _returnvalue _returnvalue)))))

(event `self.ReceiveTick`
  (params (DeltaSeconds :type "Float (single-precision)"))
  (bind (_returnvalue_roll _returnvalue_pitch _returnvalue_yaw) (`KismetMathLibrary.BreakRotator` (`KismetMathLibrary.FindLookAtRotation` (`self.K2_GetActorLocation`) (`PlayerCameraManager.GetCameraLocation` (`GameplayStatics.GetPlayerCameraManager` 0)))))
  (`self.K2_SetActorRotation` (`KismetMathLibrary.MakeRotator` 0.0 0.0 _returnvalue_yaw)))

(event `self.Capsule.OnComponentBeginOverlap`
  (params (OverlappedComponent :type "PrimitiveComponent Object Reference") (OtherActor :type "Actor Object Reference") (OtherComp :type "PrimitiveComponent Object Reference") (OtherBodyIndex :type Integer) (bFromSweep :type Boolean) (SweepResult :type "HitResult Structure (by ref)"))
  (if (`KismetSystemLibrary.DoesImplementInterface` OtherActor "/Game/Resources/Characters/Player/Blueprints/ApplyingStat_BPInter.ApplyingStat_BPInter_C")
    (message `/Game/Resources/Characters/Player/Blueprints/ApplyingStat_BPInter.Apply Healing` OtherActor 100.0)
    (`self.K2_DestroyActor`)))

(fn `UserConstructionScript`)