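; Planter character module that plants flowers, or occasionally mushrooms, on the surface beneath it when its attacks fire.
; Light attack fires once, light projectile repeats Fire on a looping timer, and heavy attack fires a rapid burst that lasts longer at high charge.
; Each Fire traces downward, spawns a randomly rotated plant at the hit, and uses a timeline-driven cube to animate the spline mesh's end toward that point.
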(event `self.LightAttack`
  (`self.Fire`))

(event `self.LightProjectileStart`
  (bind _returnvalue (`KismetSystemLibrary.K2_SetTimer` null "Fire" 0.2 true)))

(event `self.LightProjectileStop`
  (`KismetSystemLibrary.K2_ClearAndInvalidateTimerHandle` (stale `self.LightProjectileStart` _returnvalue)))

(event `self.HeavyAttack`
  (params (Charge :type "Float (double-precision)"))
  (`parent.HeavyAttack` Charge)
  (bind _returnvalue (`KismetSystemLibrary.K2_SetTimer` null "Fire" 0.03 true))
  (`KismetSystemLibrary.Delay` (`KismetMathLibrary.SelectFloat` 0.3 0.15 (>= Charge 0.7)))
  (`KismetSystemLibrary.K2_ClearAndInvalidateTimerHandle` _returnvalue))

(event `self.ReceiveBeginPlay`
  (set `self.HitLocation` (`self.K2_GetActorLocation`)))

(event `Fire`
  (bind _returnvalue (`self.K2_GetActorLocation`))
  (bind _splinemesh (`self.SplineMesh`))
  (bind (_outhit _returnvalue_2) (`KismetSystemLibrary.LineTraceSingle` _returnvalue (+ _returnvalue (* (`KismetMathLibrary.Vector_Down`) 500.0)) "TraceTypeQuery1"))
  (if _returnvalue_2
    (`|ExecutionSequence`
      (:`then_0`
        (bind (_bblockinghit _binitialoverlap _time _distance _location _impactpoint) (`GameplayStatics.BreakHitResult` _outhit))
        (`SceneComponent.K2_SetWorldLocation` (`self.Cube`) _impactpoint false false)
        (set `self.HitLocation` _impactpoint)
        (bind (_direction _explode) (`Timeline|Timeline` :!via `PlayFromStart`)
          (:`Update`
            (`SceneComponent.K2_SetWorldLocation` (`self.Cube`) (`KismetMathLibrary.VLerp` (+ (* (`SceneComponent.GetForwardVector` _splinemesh) 80.0) (`SceneComponent.K2_GetComponentLocation` _splinemesh)) (`self.HitLocation`) _explode) false false)
            (`SplineMeshComponent.SetEndPosition` (`self.SplineMesh`) (`SceneComponent.RelativeLocation` (`self.Cube`)) true))))
      (:`then_1`
        (`|SpawnActorFromClass` (select `bool` (`KismetMathLibrary.RandomBoolWithWeight` 0.9) :`false` "/Game/Resources/Characters/Modules/Planter/Mushroom_BP.Mushroom_BP_C" :`true` "/Game/Resources/Characters/Modules/Planter/Flower_BP.Flower_BP_C" :!type "Actor Class Reference") (`KismetMathLibrary.MakeTransform` _impactpoint (`KismetMathLibrary.MakeRotator` 0.0 0.0 (`KismetMathLibrary.RandomFloatInRange` 0.0 359.0))) "Undefined" "OverrideRootScale" null null)))))

(event `self.ReceiveTick`
  (params (DeltaSeconds :type "Float (single-precision)"))
  (`parent.ReceiveTick` DeltaSeconds))

(fn `UserConstructionScript`
  (`parent.UserConstructionScript`))