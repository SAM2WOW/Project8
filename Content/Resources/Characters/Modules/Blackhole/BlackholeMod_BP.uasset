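; Black hole character module that pulls nearby actors toward itself on attack.
; Light and heavy attacks call Fire, which light projectile mode repeats on a looping timer until stopped.
; Fire triggers a radial impulse, Niagara effect and animation, then sphere-traces on the host's channel and sends hit actors negative-force knockback.
; Tick holds continuous radial force at zero, and the Grab flag is set but never read here.
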(event `self.On Installed`
  (`SkeletalMeshComponent.PlayAnimation` (`self.SK_DarkHoleGenerator`) "/Game/Resources/Characters/Modules/Blackhole/SK_DarkHoleGenerator_Anim_DarkHoleSK_DarkHole_StartUp.SK_DarkHoleGenerator_Anim_DarkHoleSK_DarkHole_StartUp" false :!label _label))

(event `self.On Uninstalled`
  (goto _label))

(event `self.LightAttack`
  (`self.Fire`))

(event `self.LightProjectileStart`
  (set `self.Grab` true)
  (bind _returnvalue (`KismetSystemLibrary.K2_SetTimer` null "Fire" 0.33 true)))

(event `self.LightProjectileStop`
  (set `self.Grab` false)
  (`KismetSystemLibrary.K2_ClearAndInvalidateTimerHandle` (stale `self.LightProjectileStart` _returnvalue)))

(event `Fire`
  (bind _returnvalue (`self.K2_GetActorLocation`))
  (`RadialForceComponent.FireImpulse` (`self.RadialForce`))
  (`NiagaraFunctionLibrary.SpawnSystemAtLocation` "/Game/Resources/VFX/BlackHole_NS.BlackHole_NS" (`self.K2_GetActorLocation`) (`self.K2_GetActorRotation`))
  (`SkeletalMeshComponent.PlayAnimation` (`self.SK_DarkHoleGenerator`) "/Game/Resources/Characters/Modules/Blackhole/SK_DarkHoleGenerator_Anim_DarkHoleSK_DarkHole_Fire.SK_DarkHoleGenerator_Anim_DarkHoleSK_DarkHole_Fire" false)
  (bind _channel (message `/Game/Resources/Characters/Modules/DamageOwner_BPInter.Get Trace Channel` (`self.Host`)))
  (bind (_outhits _returnvalue_2) (`KismetSystemLibrary.SphereTraceMulti` _returnvalue _returnvalue 500.0 _channel))
  (if _returnvalue_2
    (for _array_element _outhits
      (message `/Game/Resources/Characters/Player/Blueprints/ApplyingStat_BPInter.Apply Knockback` (`.HitActor` (`GameplayStatics.BreakHitResult` _array_element)) self -600.0 20.0))))

(event `self.HeavyAttack`
  (params (Charge :type "Float (double-precision)"))
  (`parent.HeavyAttack` Charge)
  (`self.Fire`))

(event `self.ReceiveTick`
  (params (DeltaSeconds :type "Float (single-precision)"))
  (`parent.ReceiveTick` DeltaSeconds)
  (set `RadialForceComponent.ForceStrength` (`KismetMathLibrary.SelectFloat` -2000.0) (`self.RadialForce`)))

(fn `UserConstructionScript`
  (`parent.UserConstructionScript`))