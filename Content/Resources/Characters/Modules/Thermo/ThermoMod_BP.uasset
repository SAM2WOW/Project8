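; Thermo character module that adds a passive on-hit area damage effect, labeled as fire damage in its debug print.
; CalculatePassive registers the module in the passive struct's function list and increments the stack count for its type.
; AmmoHit applies fixed radial damage with falloff around the module's own location, using the generic DamageType and Host as causer.
; The stack count only appears in the debug print and does not scale damage.
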(event `/Game/Resources/Characters/Modules/Passive_BPInter.Ammo Hit`
  (params (Actor :type "Actor Object Reference"))
  (bind (_currentpassive_type _currentpassive_speedscale _currentpassive_dmgscale _currentpassive_firerate _currentpassive_passivefunctions _currentpassive_passivecount) (break `/Game/Resources/Characters/Modules/ModulePassive_Struct` (`/Game/Resources/Characters/Modules/ModuleManager_BPC.CurrentPassive` (`self.Manager`))))
  (`KismetSystemLibrary.PrintString` (`KismetTextLibrary.Conv_TextToString` (`|FormatText` "Apply Fire Damage x {num}" (`BlueprintMapLibrary.Map_Find` _currentpassive_passivecount (`self.Type`)))) true true (struct :`R` 1.0 :`G` 0.04161 :`B` 0.640486 :`A` 1.0))
  (`GameplayStatics.ApplyRadialDamageWithFalloff` :`BaseDamage` 50.0 :`Origin` (`self.K2_GetActorLocation`) :`DamageInnerRadius` 50.0 :`DamageOuterRadius` 100.0 :`DamageFalloff` 0.5 :`DamageTypeClass` "/Script/Engine.DamageType" :`DamageCauser` (`self.Host`) :`InstigatedByController` null))

(fn `Calculate Passive`
  (params (`Old Passive` :type "/Game/Resources/Characters/Modules/ModulePassive_Struct Structure"))
  (returns (Passive :type "/Game/Resources/Characters/Modules/ModulePassive_Struct Structure"))
  (bind (_type _speedscale _dmgscale _firerate _passivefunctions _passivecount) (break `/Game/Resources/Characters/Modules/ModulePassive_Struct` `Old Passive`))
  (bind (_value _returnvalue) (`BlueprintMapLibrary.Map_Find` _passivecount (`self.Type`)))
  (`KismetArrayLibrary.Array_Add` _passivefunctions self)
  (if _returnvalue
    (`BlueprintMapLibrary.Map_Add` _passivecount (`self.Type`) (+ _value 1))
    (else
      (`BlueprintMapLibrary.Map_Add` _passivecount (`self.Type`) 1)))
  (return (make `/Game/Resources/Characters/Modules/ModulePassive_Struct` _type _speedscale _dmgscale _firerate _passivefunctions _passivecount)))

(fn `UserConstructionScript`
  (`parent.UserConstructionScript`))