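; Energy ball character module Blueprint that provides a heavy attack and a deployable buildable.
; Heavy attack calls the parent, repeats Fire on a fast timer for a short burst that lasts longer at high charge, then damages sphere-trace hits around the module.
; Deploy spawns the buildable from the module data table row, passing a random reachable point near the host as its target.
; Light attack events are empty, and the passive calculation returns its input unchanged.
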(event `HeavyAttack`
  (params (Charge :type "Float (double-precision)"))
  (bind _returnvalue (`self.K2_GetActorLocation`))
  (`parent.HeavyAttack` Charge)
  (bind _returnvalue_2 (`KismetSystemLibrary.K2_SetTimer` null "Fire" 0.03 true))
  (`KismetSystemLibrary.Delay` (`KismetMathLibrary.SelectFloat` 0.3 0.15 (>= Charge 0.7)))
  (`KismetSystemLibrary.K2_ClearAndInvalidateTimerHandle` _returnvalue_2)
  (bind _outhits (`KismetSystemLibrary.SphereTraceMulti` _returnvalue _returnvalue 300.0 "TraceTypeQuery3"))
  (for _array_element _outhits
    (`GameplayStatics.ApplyDamage` (`.HitActor` (`GameplayStatics.BreakHitResult` _array_element)) 100.0 null (`self.Host`) "/Script/Engine.DamageType")))

(event `LightAttack`
  ;[0 1 0.6719] // Attacks
)

(event `LightProjectileStart`
  ;[0 1 0.6719] // Attacks
)

(event `LightProjectileStop`
  ;[0 1 0.6719] // Attacks
)

(event `Deploy`
  (bind _returnvalue_location (`KismetMathLibrary.BreakTransform` (`self.GetTransform`)))
  (bind _host (`self.Host`))
  (bind (_returnvalue_roll _returnvalue_pitch _returnvalue_yaw) (`KismetMathLibrary.BreakRotator` (`self.K2_GetActorRotation` _host)))
  ;[0 1 0.6719] // Attacks
  (bind _returnvalue (`|GetDataTableRow` "/Game/Resources/Characters/Modules/ModuleInfo_DT.ModuleInfo_DT" (`self.Type`))
    (:`then`
      (if (`KismetSystemLibrary.IsValidClass` (`.Buildable_12_952B647D4466188B0B8913A0526CC98B` (break `/Game/Resources/Characters/Modules/ModuleInfo_Struct` _returnvalue)))
        (`|SpawnActorFromClass` (`.Buildable_12_952B647D4466188B0B8913A0526CC98B` (break `/Game/Resources/Characters/Modules/ModuleInfo_Struct` _returnvalue)) (`KismetMathLibrary.MakeTransform` _returnvalue_location (`KismetMathLibrary.MakeRotator` 0.0 0.0 _returnvalue_yaw)) "AdjustIfPossibleButAlwaysSpawn" "OverrideRootScale" null (`self.Host`) (`.BuildableHealth_28_23B734B641FBF7FD67ADF0AFDE5ACAD4` (break `/Game/Resources/Characters/Modules/ModuleInfo_Struct` _returnvalue)) (`NavigationSystemV1.K2_GetRandomReachablePointInRadius` (`self.K2_GetActorLocation` _host) 500.0 null null) (`self.Passive`) null)))))

(fn `Calculate Passive`
  (params (`Old Passive` :type "/Game/Resources/Characters/Modules/ModulePassive_Struct Structure"))
  (returns (Passive :type "/Game/Resources/Characters/Modules/ModulePassive_Struct Structure"))
  (return `Old Passive`))

(fn `UserConstructionScript`)