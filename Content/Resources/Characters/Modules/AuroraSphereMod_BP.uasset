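; Aurora Sphere weapon module that fires bullets at the locked target, or along its own facing when none is locked.
; Light attacks fire once or loop on a timer scaled by the passive fire rate; heavy attacks run a brief rapid burst with enlarged flashes, longer at high charge.
; Each shot passes host, passives and damage to the spawned bullet, stretches the cylinder briefly and rumbles the controller for player hosts.
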(event `self.LightAttack`
  (`parent.LightAttack`)
  (`self.Fire`))

(event `self.LightProjectileStop`
  (`parent.LightProjectileStop`)
  (`KismetSystemLibrary.K2_ClearAndInvalidateTimerHandle` (stale `self.LightProjectileStart` _returnvalue)))

(event `self.LightProjectileStart`
  (bind (_currentpassive_type _currentpassive_speedscale _currentpassive_dmgscale _currentpassive_firerate) (break `/Game/Resources/Characters/Modules/ModulePassive_Struct` (`/Game/Resources/Characters/Modules/ModuleManager_BPC.CurrentPassive` (`self.Manager`))))
  (`parent.LightProjectileStart`)
  (bind _returnvalue (`KismetSystemLibrary.K2_SetTimer` null "Fire" (* (`self.BaseFireRate`) _currentpassive_firerate) true))
  (`self.Fire`)
  (`KismetSystemLibrary.PrintString` "FIRE!!!" true true (struct :`R` 1.0 :`B` 0.094325 :`A` 1.0)))

(event `self.HeavyAttack`
  (params (Charge :type "Float (double-precision)"))
  (`parent.HeavyAttack` Charge)
  (set `self.ScaleParticle` (10.0 10.0 10.0))
  (`NiagaraFunctionLibrary.SpawnSystemAtLocation` "/Game/VFX_Pack/Niagara/NS_OverdriveHint.NS_OverdriveHint" (`SceneComponent.K2_GetComponentLocation` (`self.Cylinder`)))
  (bind _returnvalue (`KismetSystemLibrary.K2_SetTimer` null "Fire" 0.03 true))
  (`KismetSystemLibrary.Delay` (`KismetMathLibrary.SelectFloat` 0.3 0.15 (>= Charge 0.7)))
  (`KismetSystemLibrary.K2_ClearAndInvalidateTimerHandle` _returnvalue)
  (set `self.ScaleParticle` (1.0 1.0 1.0)))

(event `Fire`
  (bind (_returnvalue_location _returnvalue_rotation) (`KismetMathLibrary.BreakTransform` (`self.GetTransform`)))
  (bind _basedmg (`self.BaseDmg`))
  (bind _locked_target (`self.Locked Target`)
    (:`then`
      (`self.Spawn Bullet` _returnvalue_location (`KismetMathLibrary.FindLookAtRotation` (`self.K2_GetActorLocation` self) (`self.K2_GetActorLocation` _locked_target)) (1.0 1.0 1.0) _basedmg))
    (:`else`
      (`self.Spawn Bullet` _returnvalue_location _returnvalue_rotation (1.0 1.0 1.0) _basedmg)))
  (`SceneComponent.SetRelativeScale3D` (`self.Cylinder`) (0.201568 0.201568 0.60321))
  (`|ExecutionSequence`
    (:`then_0`
      (bind _tag (message `/Game/Resources/Characters/Modules/DamageOwner_BPInter.Get Tag` (`self.Host`)))
      (if (== _tag "Player")
        (`GameplayStatics.SpawnForceFeedbackAttached` "/Game/Resources/Characters/Weapons/Sword/Feedbacks/Fire_Feed.Fire_Feed" (`self.Cube`) "None" (0.0 0.0 0.0) (struct) "SnapToTarget" false false (`KismetMathLibrary.RandomFloatInRange` 0.5 1.0) 0.0 null)))
    (:`then_1`
      (`KismetSystemLibrary.RetriggerableDelay` 0.2)
      (`SceneComponent.SetRelativeScale3D` (`self.Cylinder`) (0.201568 0.201568 0.201568)))))

(event `self.Deploy`
  (`parent.Deploy`))

(fn `Spawn Bullet`
  (params (Location :type "Vector Structure") (Rotation :type "Rotator Structure") (Scale :type "Vector Structure") (BaseDmg :type "Float (double-precision)"))
  (`|SpawnActorFromClass` (`self.BulletClass`) (`KismetMathLibrary.MakeTransform` Location Rotation Scale) "AlwaysSpawn" "OverrideRootScale" null (`self.Host`) (`/Game/Resources/Characters/Modules/ModuleManager_BPC.CurrentPassive` (`self.Manager`)) BaseDmg null)
  (`NiagaraFunctionLibrary.SpawnSystemAtLocation` "/Game/VFX_Pack/Niagara/NS_test_Flash_16.NS_test_Flash_16" Location Rotation (`self.ScaleParticle`)))

(fn `UserConstructionScript`
  (`parent.UserConstructionScript`))