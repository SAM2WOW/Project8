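; BulletShield_BP is a moving projectile shield that deflects overlapping actors tagged differently from its host.
; On BeginPlay, the Spawn timeline scales the Cube from small to a thin, wide panel.
; Cube overlaps compare tag messages from Host and the other actor, sending BounceMessage with the shield's forward vector when a valid tag differs.
; When projectile movement stops, it spawns an impact effect and calls Kill.
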(event `self.ReceiveBeginPlay`
  (`parent.ReceiveBeginPlay`)
  (bind (_direction _track) (`Timeline|Spawn` :!via `PlayFromStart`)
    (:`Update`
      (`SceneComponent.SetRelativeScale3D` (`self.Cube`) (`KismetMathLibrary.VLerp` (0.1 0.1 0.1) (0.085 2.0 2.0) _track)))))

(event `self.Cube.OnComponentBeginOverlap`
  (params (OverlappedComponent :type "PrimitiveComponent Object Reference") (OtherActor :type "Actor Object Reference") (OtherComp :type "PrimitiveComponent Object Reference") (OtherBodyIndex :type Integer) (bFromSweep :type Boolean) (SweepResult :type "HitResult Structure (by ref)"))
  (bind _tag (message `/Game/Resources/Characters/Modules/DamageOwner_BPInter.Get Tag` (`self.Host`)))
  (bind _tag_2 (message `/Game/Resources/Characters/Modules/DamageOwner_BPInter.Get Tag` OtherActor))
  (if (and (!= _tag_2 "None") (!= _tag_2 _tag))
    (message `/Game/Resources/Characters/Modules/Turrets/Bullet_BPInter.Bounce` OtherActor (`KismetMathLibrary.GetForwardVector` (`self.K2_GetActorRotation`)))))

(event `self.ProjectileMovement.OnProjectileStop`
  (params (ImpactResult :type "HitResult Structure (by ref)"))
  (`NiagaraFunctionLibrary.SpawnSystemAtLocation` "/Game/VFX_Pack/Niagara/NS_Shoot_impact.NS_Shoot_impact" (`self.K2_GetActorLocation`) (`self.K2_GetActorRotation`))
  (`self.Kill`)
  (`KismetSystemLibrary.PrintString` "SHIELD IDED"))

(fn `UserConstructionScript`
  (`parent.UserConstructionScript`))