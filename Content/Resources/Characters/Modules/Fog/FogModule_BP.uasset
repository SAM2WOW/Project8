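; Character fog module that emits a fog burst as a light or heavy attack.
; Each shot spawns a Niagara fog system at the ejector, plays a fire sound event and restarts a timeline that stretches the ejector mesh along Z.
; A looping timer repeats shots during light projectile fire, while heavy attacks spawn a larger burst.
; The stretch animation also plays on begin play, install and uninstall.
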(event `self.LightAttack`
  (`self.Fire`))

(event `self.LightProjectileStart`
  (bind _returnvalue (`KismetSystemLibrary.K2_SetTimer` null "Fire" 0.3 true)))

(event `self.LightProjectileStop`
  (`KismetSystemLibrary.K2_ClearAndInvalidateTimerHandle` (stale `self.LightProjectileStart` _returnvalue)))

(event `self.ReceiveBeginPlay`
  (`parent.ReceiveBeginPlay`)
  (bind (_direction _explode) (`Timeline|Timeline` :!via `PlayFromStart` :!label _label)
    (:`Update`
      (`SceneComponent.SetRelativeScale3D` (`self.ConfettiEjector`) (`KismetMathLibrary.MakeVector` 1.0 1.0 (`KismetMathLibrary.Lerp` 1.0 3.0 _explode))))))

(event `Fire`
  (bind _confettiejector (`self.ConfettiEjector`))
  (`NiagaraFunctionLibrary.SpawnSystemAtLocation` "/Game/Resources/VFX/Fog_NS.Fog_NS" (`SceneComponent.K2_GetComponentLocation` _confettiejector) (`SceneComponent.K2_GetComponentRotation` _confettiejector))
  (`FMODBlueprintStatics.PlayEventAtLocation` "/Game/FMOD/Events/Sounds/Module/Fog_Fire.Fog_Fire" (`self.GetTransform`) :!label _label_2)
  (goto _label :!via `PlayFromStart`))

(event `self.On Installed`
  (goto _label :!via `PlayFromStart`))

(event `self.On Uninstalled`
  (goto _label :!via `PlayFromStart`))

(event `self.HeavyAttack`
  (params (Charge :type "Float (double-precision)"))
  (bind _confettiejector (`self.ConfettiEjector`))
  (`parent.HeavyAttack` Charge)
  (`NiagaraFunctionLibrary.SpawnSystemAtLocation` "/Game/Resources/VFX/Fog_NS.Fog_NS" (`SceneComponent.K2_GetComponentLocation` _confettiejector) (`SceneComponent.K2_GetComponentRotation` _confettiejector) (2.0 2.0 2.0))
  (goto _label_2))

(fn `UserConstructionScript`
  (`parent.UserConstructionScript`))