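; Shield module for a character that raises a shield while light-projectile input is active and fires a shield projectile on heavy attack.
; Tick interpolates the Cube's scale between collapsed and expanded, while the skeletal mesh plays open and close animations.
; Cube overlaps with differently tagged actors send them a bounce along the Arrow's forward vector.
; Heavy attack spawns BulletShield_BP scaled by charge, aimed at the locked target or along the host's rotation.
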(event `self.On Installed`
  (`SkeletalMeshComponent.PlayAnimation` (`self.SK_ShieldModule3`) "/Game/Resources/Characters/Modules/Shield/SK_ShieldModule3_Anim.SK_ShieldModule3_Anim" false))

(event `self.On Uninstalled`
  (`SkeletalMeshComponent.PlayAnimation` (`self.SK_ShieldModule3`) "/Game/Resources/Characters/Modules/Shield/SK_ShieldModule3_AnimClose.SK_ShieldModule3_AnimClose" false))

(event `self.ReceiveTick`
  (params (DeltaSeconds :type "Float (single-precision)"))
  (bind _cube (`self.Cube`))
  (`parent.ReceiveTick` DeltaSeconds)
  (`SceneComponent.SetRelativeScale3D` _cube (`KismetMathLibrary.VInterpTo` (`SceneComponent.RelativeScale3D` _cube) (`KismetMathLibrary.SelectVector` (1.5 0.15 1.5) (0.01 0.01 0.01) (`self.Expand`)) DeltaSeconds 20.0)))

(event `self.LightProjectileStart`
  (`parent.LightProjectileStart`)
  (set `self.Expand` true)
  (`SkeletalMeshComponent.PlayAnimation` (`self.SK_ShieldModule3`) "/Game/Resources/Characters/Modules/Shield/SK_ShieldModule3_Anim.SK_ShieldModule3_Anim" false))

(event `self.LightProjectileStop`
  (`parent.LightProjectileStop`)
  (set `self.Expand` false)
  (`SkeletalMeshComponent.PlayAnimation` (`self.SK_ShieldModule3`) "/Game/Resources/Characters/Modules/Shield/SK_ShieldModule3_AnimClose.SK_ShieldModule3_AnimClose" false))

(event `self.HeavyAttack`
  (params (Charge :type "Float (double-precision)"))
  (bind _returnvalue (* Charge 2.0))
  (bind _host (`self.Host`))
  (bind _passive (`self.Passive`))
  (bind _returnvalue_2 (`KismetMathLibrary.MakeVector` _returnvalue _returnvalue _returnvalue))
  (bind _returnvalue_3 (`self.K2_GetActorLocation` self))
  (`parent.HeavyAttack` Charge)
  (bind _locked_target (`self.Locked Target`)
    (:`then`
      (`|SpawnActorFromClass` "/Game/Resources/Characters/Modules/Shield/BulletShield_BP.BulletShield_BP_C" (`KismetMathLibrary.MakeTransform` _returnvalue_3 (`KismetMathLibrary.FindLookAtRotation` _returnvalue_3 (`self.K2_GetActorLocation` _locked_target)) _returnvalue_2) "AlwaysSpawn" "OverrideRootScale" null _host _passive 10.0 null))
    (:`else`
      (`|SpawnActorFromClass` "/Game/Resources/Characters/Modules/Shield/BulletShield_BP.BulletShield_BP_C" (`KismetMathLibrary.MakeTransform` _returnvalue_3 (`self.K2_GetActorRotation` (`self.Host`)) _returnvalue_2) "AlwaysSpawn" "OverrideRootScale" null _host _passive 10.0 null))))

(event `self.Cube.OnComponentBeginOverlap`
  (params (OverlappedComponent :type "PrimitiveComponent Object Reference") (OtherActor :type "Actor Object Reference") (OtherComp :type "PrimitiveComponent Object Reference") (OtherBodyIndex :type Integer) (bFromSweep :type Boolean) (SweepResult :type "HitResult Structure (by ref)"))
  (bind _tag (message `/Game/Resources/Characters/Modules/DamageOwner_BPInter.Get Tag` (`self.Host`)))
  (bind _tag_2 (message `/Game/Resources/Characters/Modules/DamageOwner_BPInter.Get Tag` OtherActor))
  (if (and (!= _tag_2 "None") (!= _tag_2 _tag))
    (`KismetSystemLibrary.PrintString` "SHIELD" true true (struct :`G` 0.229899 :`B` 1.0 :`A` 1.0))
    (message `/Game/Resources/Characters/Modules/Turrets/Bullet_BPInter.Bounce` OtherActor (`SceneComponent.GetForwardVector` (`self.Arrow`)))))

(fn `UserConstructionScript`
  (`parent.UserConstructionScript`))