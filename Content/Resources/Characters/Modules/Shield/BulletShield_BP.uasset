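; BulletShield_BP is a projectile shield that grows into a flat panel on spawn through a scale timeline.
; When its cube overlaps an actor with a tag different from its host's, it sends that actor a bounce message along the shield's forward vector.
; When projectile movement stops, it plays a Niagara burst and glass-break sound, then kills itself.
; An alternative destructible-shield spawn is left disconnected.
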(event `self.ReceiveBeginPlay`
  (`parent.ReceiveBeginPlay`)
  (bind (_direction _track) (`Timeline|Spawn` :!via `PlayFromStart`)
    (:`Update`
      (`SceneComponent.SetRelativeScale3D` (`self.Cube`) (`KismetMathLibrary.VLerp` (0.1 0.1 0.1) (1.0 0.1 1.0) _track)))))

(event `self.Cube.OnComponentBeginOverlap`
  (params (OverlappedComponent :type "PrimitiveComponent Object Reference") (OtherActor :type "Actor Object Reference") (OtherComp :type "PrimitiveComponent Object Reference") (OtherBodyIndex :type Integer) (bFromSweep :type Boolean) (SweepResult :type "HitResult Structure (by ref)"))
  (bind _tag (message `/Game/Resources/Characters/Modules/DamageOwner_BPInter.Get Tag` (`self.Host`)))
  (bind _tag_2 (message `/Game/Resources/Characters/Modules/DamageOwner_BPInter.Get Tag` OtherActor))
  (if (and (!= _tag_2 "None") (!= _tag_2 _tag))
    (message `/Game/Resources/Characters/Modules/Turrets/Bullet_BPInter.Bounce` OtherActor (`KismetMathLibrary.GetForwardVector` (`self.K2_GetActorRotation`)))))

(event `self.ProjectileMovement.OnProjectileStop`
  (params (ImpactResult :type "HitResult Structure (by ref)"))
  (`NiagaraFunctionLibrary.SpawnSystemAtLocation` "/Game/Resources/VFX/Bomlistic_NS.Bomlistic_NS" (`self.K2_GetActorLocation`) (`self.K2_GetActorRotation`))
  (`FMODBlueprintStatics.PlayEventAtLocation` "/Game/FMOD/Events/Sounds/Collectables/Glass_Break.Glass_Break" (`self.GetTransform`))
  (`self.Kill`)
  (`KismetSystemLibrary.PrintString` "SHIELD IDED"))

(fn `UserConstructionScript`
  (`parent.UserConstructionScript`))