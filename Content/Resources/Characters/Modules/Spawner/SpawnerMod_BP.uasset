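; SpawnerMod_BP is a spawner module that holds a dormant enemy until it is deployed.
; On BeginPlay it looks up EnemyLabel in a data table and spawns that enemy flipped upside down with its listed behavior tree and weapon, starting deactivated.
; While Locked, Tick pins the enemy to the Squid component's location.
; Deploy rights its rotation, unlocks it, enables AI possession and plays an unplug sound.
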(event `self.ReceiveBeginPlay`
  (bind _returnvalue (`self.GetTransform`))
  (`parent.ReceiveBeginPlay`)
  (bind _returnvalue_2 (`|GetDataTableRow` "/Game/Resources/Characters/Enemy/EnemyLabel_DT.EnemyLabel_DT" (`self.EnemyLabel`))
    (:`then`
      (bind (_enemy _weapon _behavior) (break `/Game/Resources/Characters/Enemy/EnemyLabel_Struct` _returnvalue_2))
      (bind _returnvalue_3 (`|SpawnActorFromClass` _enemy (`KismetMathLibrary.MakeTransform` (.location _returnvalue) (`KismetMathLibrary.MakeRotator` 180.0 0.0 (.yaw (.rotation _returnvalue)))) "AlwaysSpawn" "OverrideRootScale" null 300.0 50.0 _behavior true _weapon (`self.EnemyLabel`) null))
      (bind _output_get (set `self.Enemy` _returnvalue_3))
      (`/Game/Resources/Characters/Enemy/EnemyBase_BP.ToggleBehaviorTree` _output_get)
      (`/Game/Resources/Characters/Enemy/EnemyBase_BP.PossessAI` _output_get false))))

(event `self.ReceiveTick`
  (params (DeltaSeconds :type "Float (single-precision)"))
  (`parent.ReceiveTick` DeltaSeconds)
  (if (`self.Locked`)
    (`self.K2_SetActorLocation` (`self.Enemy`) (`SceneComponent.K2_GetComponentLocation` (`self.squid`)) false false)))

(event `self.Deploy`
  (if (`self.Locked`)
    (`self.K2_SetActorRotation` :`self` (`self.Enemy`))
    (set `self.Locked` false)
    (`/Game/Resources/Characters/Enemy/EnemyBase_BP.PossessAI` (`self.Enemy`) true)
    (`FMODBlueprintStatics.PlayEventAtLocation` "/Game/FMOD/Events/Sounds/Enemy/Enemy_Unplug.Enemy_Unplug" (`KismetMathLibrary.MakeTransform` (`SceneComponent.K2_GetComponentLocation` (`self.squid`))))))

(fn `UserConstructionScript`
  (`parent.UserConstructionScript`))