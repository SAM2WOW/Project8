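; CommonBullet_BP is a turret projectile that plays a firing sound event on spawn and damages actors it overlaps.
; Box overlaps apply damage, credited to Host, only when the other actor's tag message is set and differs from its own.
; Projectile stops attach a random, short-lived bullet decal to the hit surface.
; Both hit paths notify every Passives function via AmmoHitMessage, spawn impact Niagara effects and kill the bullet.
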(event `self.ReceiveBeginPlay`
  (`parent.ReceiveBeginPlay`)
  (`FMODBlueprintStatics.PlayEventAtLocation` "/Game/FMOD/Events/Sounds/Module/Turret_Fire.Turret_Fire" (`KismetMathLibrary.MakeTransform` (`self.K2_GetActorLocation`))))

(event `self.Box.OnComponentBeginOverlap`
  (params (OverlappedComponent :type "PrimitiveComponent Object Reference") (OtherActor :type "Actor Object Reference") (OtherComp :type "PrimitiveComponent Object Reference") (OtherBodyIndex :type Integer) (bFromSweep :type Boolean) (SweepResult :type "HitResult Structure (by ref)"))
  (bind (_passives_type _passives_speedscale _passives_dmgscale _passives_firerate _passives_passivefunctions) (break `/Game/Resources/Characters/Modules/ModulePassive_Struct` (`self.Passives`)))
  (bind _tag (message `/Game/Resources/Characters/Modules/DamageOwner_BPInter.Get Tag` self))
  (`KismetSystemLibrary.PrintString` (`KismetSystemLibrary.GetDisplayName` OtherActor) true true (struct :`R` 0.367304 :`B` 1.0 :`A` 1.0))
  (bind _tag_2 (message `/Game/Resources/Characters/Modules/DamageOwner_BPInter.Get Tag` OtherActor))
  (`KismetSystemLibrary.PrintString` (`KismetStringLibrary.Conv_NameToString` _tag_2) true true (struct :`R` 1.0 :`G` 0.294848 :`A` 1.0))
  (bind _returnvalue (and (!= _tag_2 "None") (!= _tag_2 _tag)))
  (`KismetSystemLibrary.PrintString` (`KismetStringLibrary.Conv_BoolToString` _returnvalue) true true (struct :`R` 1.0 :`G` 0.895769 :`A` 1.0))
  (if _returnvalue
    (`GameplayStatics.ApplyDamage` OtherActor (`self.BaseDmg`) null (`self.Host`) "/Script/Engine.DamageType")
    (for _array_element _passives_passivefunctions :!label _label
      (message `/Game/Resources/Characters/Modules/Passive_BPInter.Ammo Hit` _array_element null))
    (`NiagaraFunctionLibrary.SpawnSystemAtLocation` "/Game/VFX_Pack/Niagara/NS_Shoot_impact.NS_Shoot_impact" (`self.K2_GetActorLocation`) (`self.K2_GetActorRotation`))
    (`self.Kill`)))

(event `self.ProjectileMovement.OnProjectileStop`
  (params (ImpactResult :type "HitResult Structure (by ref)"))
  (`KismetSystemLibrary.PrintString` (`KismetSystemLibrary.GetDisplayName` ImpactResult_HitActor) true true (struct :`R` 1.0 :`G` 0.09272 :`A` 1.0))
  (bind _returnvalue (`GameplayStatics.SpawnDecalAttached` (select `int` (`KismetMathLibrary.RandomInteger` 6) :`0` "/Game/Resources/Materials/Decal/bullet_decal_Mat_Inst3.bullet_decal_Mat_Inst3" :`1` "/Game/Resources/Materials/Decal/bullet_decal_Mat_Inst1.bullet_decal_Mat_Inst1" :`2` "/Game/Resources/Materials/Decal/bullet_decal_Mat_Inst2.bullet_decal_Mat_Inst2" :`3` "/Game/Resources/Materials/Decal/bullet_decal_Mat_Inst4.bullet_decal_Mat_Inst4" :`4` "/Game/Resources/Materials/Decal/bullet_decal_Mat_Inst5.bullet_decal_Mat_Inst5" :`5` "/Game/Resources/Materials/Decal/bullet_decal_Mat_Inst6.bullet_decal_Mat_Inst6" :!type "MaterialInterface Object Reference") (30.0 30.0 30.0) ImpactResult_HitComponent "None" ImpactResult_Location (`KismetMathLibrary.Conv_VectorToRotator` ImpactResult_Normal) "KeepWorldPosition" 5.0))
  (goto _label))

(fn `Get Tag`
  (returns (Tag :type Name))
  (return (`|GetArrayItem` (`self.Tags`))))

(fn `Get Trace Channel`
  (returns (Channel :type "ETraceTypeQuery Enum"))
  (return "TraceTypeQuery1"))

(fn `UserConstructionScript`)