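; ShieldMod_BP is a turret module Blueprint that implements a chargeable heavy attack.
; HeavyAttack spawns a bullet at the actor's own location and rotation, scaling it from normal to double size by the Charge value.
; BeginPlay, overlap and Tick are disabled stubs, and the construction script only calls its parent.
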(event `/Game/Resources/Characters/Modules/ModuleBase_BP.HeavyAttack`
  (params (Charge :type "Float (double-precision)"))
  (bind (_returnvalue_location _returnvalue_rotation) (`KismetMathLibrary.BreakTransform` (`self.GetTransform`)))
  (`self.Spawn Bullet` _returnvalue_location _returnvalue_rotation (`KismetMathLibrary.VLerp` (1.0 1.0 1.0) (2.0 2.0 2.0) Charge)))

(fn `UserConstructionScript`
  (`parent.UserConstructionScript`))