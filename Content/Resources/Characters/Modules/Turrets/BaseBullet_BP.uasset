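; BaseBullet_BP is a turret projectile that tags itself from its Host and kills itself after a base timeout.
; BeginPlay and Kill forward ammo begin and destroy messages to the functions in its Passives list.
; Kill also spawns an FS_MasterField_Child at the bullet's transform before destroying it.
; Bounce reflects velocity off a given normal and plays a blocked sound event, while passive speed scaling is present but unconnected.
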(event `self.ReceiveBeginPlay`
  (bind (_passives_type _passives_speedscale _passives_dmgscale _passives_firerate _passives_passivefunctions) (break `/Game/Resources/Characters/Modules/ModulePassive_Struct` (`self.Passives`)))
  (bind _tag (message `/Game/Resources/Characters/Modules/DamageOwner_BPInter.Get Tag` (`self.Host`)))
  (`KismetArrayLibrary.Array_Add` (`self.Tags`) _tag)
  ;[0 1 0.3672] Projectile Timeout
  (`KismetSystemLibrary.Delay` (`self.BaseTimeout`))
  (`self.Kill`)
  (for _array_element _passives_passivefunctions
    (message `/Game/Resources/Characters/Modules/Passive_BPInter.Ammo Begin` _array_element)))

(event `Kill`
  (bind (_passives_type _passives_speedscale _passives_dmgscale _passives_firerate _passives_passivefunctions) (break `/Game/Resources/Characters/Modules/ModulePassive_Struct` (`self.Passives`)))
  (for _array_element _passives_passivefunctions
    (message `/Game/Resources/Characters/Modules/Passive_BPInter.Ammo Destroy` _array_element))
  (`|SpawnActorFromClass` "/Game/Resources/Characters/Destructables/FS_MasterField_Child.FS_MasterField_Child_C" (`self.GetTransform`) "AlwaysSpawn" "OverrideRootScale" null null)
  (`self.K2_DestroyActor`))

(event `/Game/Resources/Characters/Modules/Turrets/Bullet_BPInter.Bounce`
  (params (Normal :type "Vector Structure"))
  (bind (_returnvalue_location _returnvalue_rotation) (`KismetMathLibrary.BreakTransform` (`self.GetTransform`)))
  (bind _projectilemovement (`self.ProjectileMovement`))
  (set `MovementComponent.Velocity` (`KismetMathLibrary.GetReflectionVector` (`MovementComponent.Velocity` _projectilemovement) Normal) _projectilemovement)
  (`FMODBlueprintStatics.PlayEventAtLocation` "/Game/FMOD/Events/Sounds/Module/Bullet_Blocked.Bullet_Blocked" (`KismetMathLibrary.MakeTransform` _returnvalue_location _returnvalue_rotation)))

(fn `UserConstructionScript`)