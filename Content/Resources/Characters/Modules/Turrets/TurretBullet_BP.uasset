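; Turret bullet projectile that flies at a passive-scaled speed, plays fire sound and muzzle effects on spawn, and expires after a timeout.
; Overlapping an actor of the target's class applies passive-scaled damage and destroys the bullet.
; A projectile stop also destroys it, without dealing damage.
; Passive functions receive begin, hit and destroy messages, letting turret modifiers hook into the bullet's lifecycle.
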(event `self.ReceiveBeginPlay`
  (bind (_passives_type _passives_speedscale _passives_dmgscale _passives_firerate _passives_passivefunctions) (break `/Game/Resources/Characters/Modules/ModulePassive_Struct` (`self.Passives`)))
  (for _array_element _passives_passivefunctions
    (message `/Game/Resources/Characters/Modules/Passive_BPInter.Ammo Begin` _array_element))
  (set `ProjectileMovementComponent.MaxSpeed` (* _passives_speedscale 5000.0) (`self.ProjectileMovement`))
  (`FMODBlueprintStatics.PlayEventAtLocation` "/Game/FMOD/Events/Sounds/Turret_Fire.Turret_Fire" (`KismetMathLibrary.MakeTransform` (`self.K2_GetActorLocation`)))
  (`NiagaraFunctionLibrary.SpawnSystemAtLocation` "/Game/VFX_Pack/Niagara/NS_Shoot_bullet.NS_Shoot_bullet" (`self.K2_GetActorLocation`) (`self.K2_GetActorRotation`))
  ;[0 1 0.3672] Projectile Timeout
  (`KismetSystemLibrary.Delay` 5.0)
  (`self.Kill`))

(event `self.Sphere1.OnComponentBeginOverlap`
  (params (OverlappedComponent :type "PrimitiveComponent Object Reference") (OtherActor :type "Actor Object Reference") (OtherComp :type "PrimitiveComponent Object Reference") (OtherBodyIndex :type Integer) (bFromSweep :type Boolean) (SweepResult :type "HitResult Structure (by ref)"))
  (bind (_passives_type _passives_speedscale _passives_dmgscale) (break `/Game/Resources/Characters/Modules/ModulePassive_Struct` (`self.Passives`)))
  (bind (_passives_type_2 _passives_speedscale_2 _passives_dmgscale_2 _passives_firerate _passives_passivefunctions) (break `/Game/Resources/Characters/Modules/ModulePassive_Struct` (`self.Passives`)))
  (if (== (`GameplayStatics.GetObjectClass` OtherActor) (`GameplayStatics.GetObjectClass` (`self.Target`)))
    (`GameplayStatics.ApplyDamage` OtherActor (* _passives_dmgscale (`self.BaseDmg`)) null self "/Script/Engine.DamageType")
    (for _array_element _passives_passivefunctions :!label _label
      (message `/Game/Resources/Characters/Modules/Passive_BPInter.Ammo Hit` _array_element OtherActor))
    (`self.Kill`)))

(event `self.ProjectileMovement.OnProjectileStop`
  (params (ImpactResult :type "HitResult Structure (by ref)"))
  (goto _label))

(event `Kill`
  (bind (_passives_type _passives_speedscale _passives_dmgscale _passives_firerate _passives_passivefunctions) (break `/Game/Resources/Characters/Modules/ModulePassive_Struct` (`self.Passives`)))
  (for _array_element _passives_passivefunctions
    (message `/Game/Resources/Characters/Modules/Passive_BPInter.Ammo Destroy` _array_element))
  (`self.K2_DestroyActor`))

(fn `UserConstructionScript`)