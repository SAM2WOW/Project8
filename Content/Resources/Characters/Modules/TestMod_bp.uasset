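; Test character module that acts as a turret-style weapon, extending parent light attack and projectile events to fire TurretBullet_BP.
; On BeginPlay, a PhysicsControl component creates a control and gravity-free body modifier for the Cylinder mesh, targeted once at Cylinder1's transform.
; Light attack fires once, while projectile start runs a looping fire timer until stop.
; Shots aim at LockedTarget or follow player pawn rotation, briefly stretching the Cylinder as feedback.
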(event `self.ReceiveBeginPlay`
  (bind _physicscontrol (`self.PhysicsControl`))
  (bind (_returnvalue_location _returnvalue_rotation) (`KismetMathLibrary.BreakTransform` (`SceneComponent.K2_GetComponentToWorld` (`self.Cylinder1`))))
  (`PhysicsControlComponent.MakeControl` :`self` (`self.PhysicsControl`) :`ChildMeshComponent` (`self.Cylinder`) :`ControlData` (make `PhysicsControlData` 1.0 1.0 0.0 0.0 2.0))
  (`PhysicsControlComponent.MakeBodyModifier` (`self.PhysicsControl`) (`self.Cylinder`) "None" "Simulated" "QueryAndPhysics" 0.0 true)
  (`PhysicsControlComponent.SetControlTargetPositionAndOrientation` (`self.PhysicsControl`) "0" _returnvalue_location _returnvalue_rotation 0.0 true false)
  (`PhysicsControlComponent.SetControlMultipliers` _physicscontrol "0" (make `PhysicsControlMultipliers` (1.0 1.0 1.0)) true)
  (`PhysicsControlComponent.SetBodyModifierKinematicTarget` _physicscontrol "Body_0" _returnvalue_location _returnvalue_rotation false))

(event `self.LightAttack`
  (`parent.LightAttack`)
  (`self.Fire`))

(event `self.LightProjectileStop`
  (`parent.LightProjectileStop`)
  (`KismetSystemLibrary.K2_ClearAndInvalidateTimerHandle` (stale `self.LightProjectileStart` _returnvalue)))

(event `self.LightProjectileStart`
  (`parent.LightProjectileStart`)
  (bind _returnvalue (`KismetSystemLibrary.K2_SetTimerDelegate` (delegate `Fire`) 0.1 true))
  (`KismetSystemLibrary.PrintString` "FIRE!!!" true true (struct :`R` 1.0 :`B` 0.094325 :`A` 1.0)))

(event `Fire`
  (bind _returnvalue_location (`KismetMathLibrary.BreakTransform` (`self.GetTransform`)))
  (bind _locked_target (`self.Locked Target`)
    (:`then`
      (`|SpawnActorFromClass` "/Game/Resources/Characters/Modules/Turrets/TurretBullet_BP.TurretBullet_BP_C" (`KismetMathLibrary.MakeTransform` _returnvalue_location (`KismetMathLibrary.FindLookAtRotation` (`self.K2_GetActorLocation` self) (`self.K2_GetActorLocation` _locked_target))) "AlwaysSpawn" "OverrideRootScale" null (struct) 10.0 null null null))
    (:`else`
      (`|SpawnActorFromClass` "/Game/Resources/Characters/Modules/Turrets/TurretBullet_BP.TurretBullet_BP_C" (`KismetMathLibrary.MakeTransform` _returnvalue_location (`self.K2_GetActorRotation` (`GameplayStatics.GetPlayerPawn` 0))) "AlwaysSpawn" "OverrideRootScale" null (struct) 10.0 null null null)))
  (`SceneComponent.SetRelativeScale3D` (`self.Cylinder`) (0.201568 0.201568 0.60321))
  (`KismetSystemLibrary.RetriggerableDelay` 0.2)
  (`SceneComponent.SetRelativeScale3D` (`self.Cylinder`) (0.201568 0.201568 0.201568)))

(fn `UserConstructionScript`
  (`parent.UserConstructionScript`))