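; CableMod_BP is a character module that drains life from a locked target through a visible cable.
; Each tick it moves one sphere to the player and another to LockedTarget, showing the cable only while the target is valid.
; LightProjectileStart runs a looping timer that damages the target on the Host's behalf and heals the player by the damage applied.
; LightProjectileStop clears that timer.
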(event `self.ReceiveTick`
  (params (DeltaSeconds :type "Float (single-precision)"))
  (bind _cable (`self.Cable`))
  (`parent.ReceiveTick` DeltaSeconds)
  (`|ExecutionSequence`
    (:`then_0`
      (`SceneComponent.K2_SetWorldLocation` (`self.Sphere1`) (`self.K2_GetActorLocation` (`GameplayStatics.GetPlayerPawn` 0)) false false))
    (:`then_1`
      (bind _locked_target (`self.Locked Target`)
        (:`then`
          (`SceneComponent.SetVisibility` _cable true false)
          (`SceneComponent.K2_SetWorldLocation` (`self.Sphere`) (`self.K2_GetActorLocation` _locked_target) false false))
        (:`else`
          (`SceneComponent.SetVisibility` _cable false false))))))

(event `self.LightProjectileStart`
  (bind _returnvalue (`KismetSystemLibrary.K2_SetTimer` null "Fire" 0.1 true)))

(event `self.LightProjectileStop`
  (`KismetSystemLibrary.K2_ClearAndInvalidateTimerHandle` (stale `self.LightProjectileStart` _returnvalue)))

(event `Fire`
  (bind _locked_target (`self.Locked Target`)
    (:`then`
      (bind _returnvalue (`GameplayStatics.ApplyDamage` _locked_target 10.0 null (`self.Host`) "/Script/Engine.DamageType"))
      (bind _asbp_player_character (cast `/Game/Resources/Characters/Player/Blueprints/BP_PlayerCharacter` (`GameplayStatics.GetPlayerPawn` 0)))
      (`/Game/Resources/Characters/Player/Blueprints/BP_PlayerCharacter.Heal` _asbp_player_character _returnvalue))
    (:`else`)))

(fn `UserConstructionScript`
  (`parent.UserConstructionScript`))