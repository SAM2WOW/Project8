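; LockMod_BP is a child weapon module that disables a locked enemy while its light projectile is active.
; On light projectile start, it caches a valid LockedTarget, calls PossessAI(false) on that enemy and stops its weapons' light fire through the WeaponManager component.
; On stop, it calls PossessAI(true) on the cached enemy.
; Older tick-toggling logic for weapons and modules remains disconnected.
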(event `self.LightProjectileStart`
  (bind _locked_target (`self.Locked Target`))
  (`parent.LightProjectileStart`)
  (`/Engine/EditorBlueprintResources/StandardMacros.IsValid` _locked_target
    (:`Is Valid`
      (bind _output_get (set `self.Current Locked` _locked_target))
      (bind _asenemy_base_bp (cast `/Game/Resources/Characters/Enemy/EnemyBase_BP` _output_get))
      (`/Game/Resources/Characters/Enemy/EnemyBase_BP.PossessAI` _asenemy_base_bp false)
      (bind _weaponmanager_bpc (`/Game/Resources/Characters/Enemy/EnemyBase_BP.WeaponManager_BPC` _asenemy_base_bp))
      (`/Game/Resources/Characters/Weapons/WeaponManager_BPC.LightStop` _weaponmanager_bpc (`/Game/Resources/Characters/Weapons/WeaponManager_BPC.Weapons` _weaponmanager_bpc)))))

(event `self.LightProjectileStop`
  (`parent.LightProjectileStop`)
  (bind _asenemy_base_bp (cast `/Game/Resources/Characters/Enemy/EnemyBase_BP` (`self.Current Locked`)))
  (`/Game/Resources/Characters/Enemy/EnemyBase_BP.PossessAI` _asenemy_base_bp true))

(fn `UserConstructionScript`
  (`parent.UserConstructionScript`))