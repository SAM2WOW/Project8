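; Flashlight-style character module that turns its light attack input into an on/off switch for a spotlight.
; Each tick the spotlight smoothly rotates toward the locked target, or eases back to zero relative rotation when there is none.
; Light attack flip-flops the spotlight's visibility and plays a light switch sound at the module's location.
; Heavy attack and projectile events only defer to the parent class.
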(event `self.ReceiveTick`
  (params (DeltaSeconds :type "Float (single-precision)"))
  (bind _locked_target (`self.Locked Target`))
  (bind _spotlight (`self.SpotLight`))
  (`parent.ReceiveTick` DeltaSeconds)
  (`/Engine/EditorBlueprintResources/StandardMacros.IsValid` _locked_target
    (:`Is Valid`
      (`SceneComponent.K2_SetWorldRotation` _spotlight (`KismetMathLibrary.RInterpTo` (`SceneComponent.K2_GetComponentRotation` _spotlight) (`KismetMathLibrary.FindLookAtRotation` (`self.K2_GetActorLocation`) (`self.K2_GetActorLocation` _locked_target)) (`GameplayStatics.GetWorldDeltaSeconds`) 30.0) false false))
    (:`Is Not Valid`
      (`SceneComponent.K2_SetRelativeRotation` _spotlight (`KismetMathLibrary.RInterpTo` (`SceneComponent.RelativeRotation` _spotlight) (struct) (`GameplayStatics.GetWorldDeltaSeconds`) 30.0) false false))))

(event `self.LightAttack`
  (`parent.LightAttack`)
  (bind _isa (`/Engine/EditorBlueprintResources/StandardMacros.FlipFlop`)
    (:`A`
      _)
    (:`B`
      _))
  (`SceneComponent.SetVisibility` (`self.SpotLight`) _isa true)
  (`FMODBlueprintStatics.PlayEventAtLocation` "/Game/FMOD/Events/Sounds/Scene/Lightswitch.Lightswitch" (`self.GetTransform`)))

(event `self.HeavyAttack`
  (params (Charge :type "Float (double-precision)"))
  (`parent.HeavyAttack` Charge))

(event `self.LightProjectileStop`
  (`parent.LightProjectileStop`))

(event `self.LightProjectileStart`
  (`parent.LightProjectileStart`))

(fn `UserConstructionScript`
  (`parent.UserConstructionScript`))