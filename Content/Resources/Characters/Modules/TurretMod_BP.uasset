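; Turret character module that fires TurretBullet projectiles toward the locked target, or along the player pawn's facing when none is locked.
; Light input fires single shots or a looping timer stream; heavy attack runs a faster, enlarged-flash burst, longer at high charge.
; Each shot takes damage and speed from the Manager's passives, with muzzle flash, cylinder stretch and force feedback.
; Deploy spawns a TurretBuild actor targeting a random reachable nearby point.
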(event `self.LightAttack`
  (`parent.LightAttack`)
  (`self.Fire`))

(event `self.LightProjectileStop`
  (`parent.LightProjectileStop`)
  (`KismetSystemLibrary.K2_ClearAndInvalidateTimerHandle` (stale `self.LightProjectileStart` _returnvalue)))

(event `self.LightProjectileStart`
  (`parent.LightProjectileStart`)
  (bind _returnvalue (`KismetSystemLibrary.K2_SetTimerDelegate` (delegate `Fire`) 0.1 true))
  (`KismetSystemLibrary.PrintString` "FIRE!!!" true true (struct :`R` 1.0 :`B` 0.094325 :`A` 1.0)))

(event `self.HeavyAttack`
  (params (Charge :type "Float (double-precision)"))
  (`parent.HeavyAttack` Charge)
  (set `self.ScaleParticle` (10.0 10.0 10.0))
  (`NiagaraFunctionLibrary.SpawnSystemAtLocation` "/Game/VFX_Pack/Niagara/NS_OverdriveHint.NS_OverdriveHint" (`SceneComponent.K2_GetComponentLocation` (`self.Cylinder`)))
  (bind _returnvalue (`KismetSystemLibrary.K2_SetTimerDelegate` (delegate `Fire`) 0.03 true))
  (`KismetSystemLibrary.Delay` (`KismetMathLibrary.SelectFloat` 0.3 0.15 (>= Charge 0.7)))
  (`KismetSystemLibrary.K2_ClearAndInvalidateTimerHandle` _returnvalue)
  (set `self.ScaleParticle` (1.0 1.0 1.0)))

(event `Fire`
  (bind _returnvalue_location (`KismetMathLibrary.BreakTransform` (`self.GetTransform`)))
  (bind _scaleparticle (`self.ScaleParticle`))
  (bind _returnvalue (`self.K2_GetActorRotation` (`GameplayStatics.GetPlayerPawn` 0)))
  (bind _final_passive (`/Game/Resources/Characters/Modules/ModuleManager_BPC.Calc Passive` (`self.Manager`)))
  (`KismetSystemLibrary.PrintString` (`KismetStringLibrary.Conv_DoubleToString` (`.SpeedScale_13_A35F54134F7977324BDAD1A6AC268A2D` (break `/Game/Resources/Characters/Modules/ModulePassive_Struct` _final_passive))))
  (bind _locked_target (`self.Locked Target`)
    (:`then`
      (bind _returnvalue_2 (`KismetMathLibrary.FindLookAtRotation` (`self.K2_GetActorLocation` self) (`self.K2_GetActorLocation` _locked_target)))
      (`|SpawnActorFromClass` "/Game/Resources/Characters/Modules/TurretBullet_BP.TurretBullet_BP_C" (`KismetMathLibrary.MakeTransform` _returnvalue_location _returnvalue_2) "AlwaysSpawn" "OverrideRootScale" null (`.DmgScale_12_3E213CCD4A207058D69696A9166E8642` (break `/Game/Resources/Characters/Modules/ModulePassive_Struct` _final_passive)) (`.SpeedScale_13_A35F54134F7977324BDAD1A6AC268A2D` (break `/Game/Resources/Characters/Modules/ModulePassive_Struct` _final_passive)) null)
      (`NiagaraFunctionLibrary.SpawnSystemAtLocation` "/Game/VFX_Pack/Niagara/NS_test_Flash_16.NS_test_Flash_16" _returnvalue_location _returnvalue_2 _scaleparticle))
    (:`else`
      (`|SpawnActorFromClass` "/Game/Resources/Characters/Modules/TurretBullet_BP.TurretBullet_BP_C" (`KismetMathLibrary.MakeTransform` _returnvalue_location _returnvalue) "AlwaysSpawn" "OverrideRootScale" null (`.DmgScale_12_3E213CCD4A207058D69696A9166E8642` (break `/Game/Resources/Characters/Modules/ModulePassive_Struct` _final_passive)) (`.SpeedScale_13_A35F54134F7977324BDAD1A6AC268A2D` (break `/Game/Resources/Characters/Modules/ModulePassive_Struct` _final_passive)) null)
      (`NiagaraFunctionLibrary.SpawnSystemAtLocation` "/Game/VFX_Pack/Niagara/NS_test_Flash_16.NS_test_Flash_16" _returnvalue_location _returnvalue _scaleparticle)))
  (`SceneComponent.SetRelativeScale3D` (`self.Cylinder`) (0.201568 0.201568 0.60321))
  (`GameplayStatics.SpawnForceFeedbackAttached` "/Game/Resources/Characters/Sword/Fire_Feed.Fire_Feed" (`self.Cube`) "None" (0.0 0.0 0.0) (struct) "SnapToTarget" false false 1.0 0.0 null)
  (`KismetSystemLibrary.RetriggerableDelay` 0.2)
  (`SceneComponent.SetRelativeScale3D` (`self.Cylinder`) (0.201568 0.201568 0.201568)))

(event `self.Deploy`
  (bind _returnvalue_location (`KismetMathLibrary.BreakTransform` (`self.GetTransform`)))
  (`parent.Deploy`)
  (`|SpawnActorFromClass` "/Game/Resources/Characters/Buildables/TurretBuild_BP.TurretBuild_BP_C" (`KismetMathLibrary.MakeTransform` _returnvalue_location) "Undefined" "OverrideRootScale" null (`NavigationSystemV1.K2_GetRandomReachablePointInRadius` (`self.K2_GetActorLocation`) 500.0 null null) null))

(fn `UserConstructionScript`
  (`parent.UserConstructionScript`))