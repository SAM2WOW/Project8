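; Shield character module that gives its host a light-attack deflecting shield and a charged shield projectile.
; Light projectile start and stop grow and shrink the Cube, whose overlap bounces tagged actors along the Arrow's forward vector when their tag differs from the host's.
; Heavy attack spawns a BulletShield_BP scaled by charge, facing the locked target or otherwise using the host's rotation, and passes it the host and passives.
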(event `self.LightAttack`)

(event `self.LightProjectileStart`
  (`parent.LightProjectileStart`)
  (`SceneComponent.SetRelativeScale3D` (`self.Cube`) (0.102376 2.0 2.0)))

(event `self.LightProjectileStop`
  (`parent.LightProjectileStop`)
  (`SceneComponent.SetRelativeScale3D` (`self.Cube`) (0.102376 0.102376 0.102376)))

(event `self.HeavyAttack`
  (params (Charge :type "Float (double-precision)"))
  (bind _returnvalue (* Charge 2.0))
  (bind _host (`self.Host`))
  (bind _passive (`self.Passive`))
  (bind _returnvalue_2 (`KismetMathLibrary.MakeVector` _returnvalue _returnvalue _returnvalue))
  (bind _returnvalue_3 (`self.K2_GetActorLocation` self))
  (`parent.HeavyAttack` Charge)
  (bind _locked_target (`self.Locked Target`)
    (:`then`
      (`|SpawnActorFromClass` "/Game/Resources/Characters/Modules/BulletShield_BP.BulletShield_BP_C" (`KismetMathLibrary.MakeTransform` _returnvalue_3 (`KismetMathLibrary.FindLookAtRotation` _returnvalue_3 (`self.K2_GetActorLocation` _locked_target)) _returnvalue_2) "AlwaysSpawn" "OverrideRootScale" null _host _passive 10.0 null))
    (:`else`
      (`|SpawnActorFromClass` "/Game/Resources/Characters/Modules/BulletShield_BP.BulletShield_BP_C" (`KismetMathLibrary.MakeTransform` _returnvalue_3 (`self.K2_GetActorRotation` (`self.Host`)) _returnvalue_2) "AlwaysSpawn" "OverrideRootScale" null _host _passive 10.0 null))))

(event `self.Deploy`
  (`parent.Deploy`))

(event `self.Cube.OnComponentBeginOverlap`
  (params (OverlappedComponent :type "PrimitiveComponent Object Reference") (OtherActor :type "Actor Object Reference") (OtherComp :type "PrimitiveComponent Object Reference") (OtherBodyIndex :type Integer) (bFromSweep :type Boolean) (SweepResult :type "HitResult Structure (by ref)"))
  (bind _tag (message `/Game/Resources/Characters/Modules/DamageOwner_BPInter.Get Tag` (`self.Host`)))
  (bind _tag_2 (message `/Game/Resources/Characters/Modules/DamageOwner_BPInter.Get Tag` OtherActor))
  (if (and (!= _tag_2 "None") (!= _tag_2 _tag))
    (message `/Game/Resources/Characters/Modules/Turrets/Bullet_BPInter.Bounce` OtherActor (`SceneComponent.GetForwardVector` (`self.Arrow`)))))

(fn `UserConstructionScript`
  (`parent.UserConstructionScript`))