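; EnergyMod_BP is a character module that overrides the parent's attack and deploy events with confetti effects.
; Light and heavy attacks call Fire for Niagara confetti and sound; light projectile mode repeats it on a timer scaled by the manager's passive fire rate.
; Heavy attacks enlarge the confetti and add an upward burst at high charge.
; Deploy spawns ConfettiBuild_BP targeting a random reachable nearby point when a sphere trace finds world-static geometry.
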(event `self.LightAttack`
  (`parent.LightAttack`)
  (`KismetSystemLibrary.Delay` 0.1)
  (`self.Fire`))

(event `self.LightProjectileStop`
  (`parent.LightProjectileStop`)
  (`KismetSystemLibrary.K2_ClearAndInvalidateTimerHandle` (stale `self.LightProjectileStart` _returnvalue)))

(event `self.LightProjectileStart`
  (bind (_currentpassive_type _currentpassive_speedscale _currentpassive_dmgscale _currentpassive_firerate) (break `/Game/Resources/Characters/Modules/ModulePassive_Struct` (`/Game/Resources/Characters/Modules/ModuleManager_BPC.CurrentPassive` (`self.Manager`))))
  (`parent.LightProjectileStart`)
  (bind _returnvalue (`KismetSystemLibrary.K2_SetTimer` null "Fire" (* (`self.BaseFireRate`) _currentpassive_firerate) true))
  (`self.Fire`))

(event `self.HeavyAttack`
  (params (Charge :type "Float (double-precision)"))
  (bind _returnvalue (`SceneComponent.K2_GetComponentLocation` (`self.Arrow`)))
  (`parent.HeavyAttack` Charge)
  (set `self.ScaleParticle` (10.0 10.0 10.0))
  (`NiagaraFunctionLibrary.SpawnSystemAtLocation` "/Game/VFX_Pack/Niagara/NS_OverdriveHint.NS_OverdriveHint" (`SceneComponent.K2_GetComponentLocation` (`self.Cylinder`)))
  (`self.Fire`)
  (if (>= Charge 0.7)
    (`NiagaraFunctionLibrary.SpawnSystemAtLocation` "/Game/Resources/VFX/TestParticle/Confetti_NS.Confetti_NS" _returnvalue (`KismetMathLibrary.FindLookAtRotation` _returnvalue (+ _returnvalue (0.0 0.0 1000.0))) (`self.ScaleParticle`)))
  (`KismetSystemLibrary.Delay` 0.2)
  (set `self.ScaleParticle` (1.0 1.0 1.0)))

(event `Fire`
  (bind _arrow (`self.Arrow`))
  (`NiagaraFunctionLibrary.SpawnSystemAtLocation` "/Game/Resources/VFX/TestParticle/Confetti_NS.Confetti_NS" (`SceneComponent.K2_GetComponentLocation` _arrow) (`SceneComponent.K2_GetComponentRotation` _arrow) (`self.ScaleParticle`))
  (`FMODBlueprintStatics.PlayEventAtLocation` "/Game/FMOD/Events/Sounds/Module/Confetti_Fire.Confetti_Fire" (`self.GetTransform`)))

(event `self.Deploy`
  (bind _returnvalue_location (`KismetMathLibrary.BreakTransform` (`self.GetTransform`)))
  (bind _returnvalue (`self.K2_GetActorLocation`))
  (`parent.Deploy`)
  (bind (_outhit _returnvalue_2) (`KismetSystemLibrary.SphereTraceSingleForObjects` _returnvalue _returnvalue 1000.0 (`|MakeArray` "ObjectTypeQuery1" :!type "EObjectTypeQuery Enum")))
  (if _returnvalue_2
    (`|SpawnActorFromClass` "/Game/Resources/Characters/Buildables/ConfettiBuild_BP.ConfettiBuild_BP_C" (`KismetMathLibrary.MakeTransform` _returnvalue_location) "Undefined" "OverrideRootScale" null null 200.0 (`NavigationSystemV1.K2_GetRandomReachablePointInRadius` _returnvalue 500.0 null null) (struct) null)))

(fn `UserConstructionScript`
  (`parent.UserConstructionScript`))