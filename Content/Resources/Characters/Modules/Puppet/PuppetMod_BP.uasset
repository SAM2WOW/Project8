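; PuppetMod_BP is a puppet character module that maps light attack inputs to launch and pull states.
; Light attack and projectile start call Launch to set Firing, while projectile stop calls Pull to clear it.
; Heavy attack and Tick only call their parent versions.
; Unconnected movement logic would push the actor toward LockedTarget, or forward without one, while Firing, but it never runs.
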(event `self.LightAttack`
  (`self.Launch` :!label _label))

(event `self.LightProjectileStart`
  (goto _label))

(event `self.LightProjectileStop`
  (`self.Pull`))

(event `Launch`
  (set `self.Firing` true))

(event `Pull`
  (set `self.Firing` false))

(event `self.HeavyAttack`
  (params (Charge :type "Float (double-precision)"))
  (`parent.HeavyAttack` Charge))

(event `self.ReceiveTick`
  (params (DeltaSeconds :type "Float (single-precision)"))
  (`parent.ReceiveTick` DeltaSeconds))

(fn `UserConstructionScript`
  (`parent.UserConstructionScript`))