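; Hook projectile for the Puppet character that fires on spawn and yanks a target it hits.
; It copies the Host's team tag, then ignores overlapped actors whose tag is None or matches its own.
; A valid hit applies damage and negative-force knockback through message calls, then destroys the hook.
; Cancel only halts movement; Tick eases the hook to its spawn location only while Firing is false.
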(event `self.ReceiveBeginPlay`
  (set `self.InitialLocation` (`self.K2_GetActorLocation`))
  (bind _tag (message `/Game/Resources/Characters/Modules/DamageOwner_BPInter.Get Tag` (`self.Host`)))
  (`KismetArrayLibrary.Array_Add` (`self.Tags`) _tag)
  (`self.Fire`))

(event `Fire`
  (set `ProjectileMovementComponent.bSimulationEnabled` true (`self.ProjectileMovement`))
  (`KismetSystemLibrary.PrintString` "Hello")
  (set `self.Firing` true))

(event `Cancel`
  (`ProjectileMovementComponent.StopSimulating` (`self.ProjectileMovement`) (`GameplayStatics.MakeHitResult` false)))

(event `self.Sphere.OnComponentBeginOverlap`
  (params (OverlappedComponent :type "PrimitiveComponent Object Reference") (OtherActor :type "Actor Object Reference") (OtherComp :type "PrimitiveComponent Object Reference") (OtherBodyIndex :type Integer) (bFromSweep :type Boolean) (SweepResult :type "HitResult Structure (by ref)"))
  (bind _host (`self.Host`))
  (bind _tag (message `/Game/Resources/Characters/Modules/DamageOwner_BPInter.Get Tag` self))
  (bind _tag_2 (message `/Game/Resources/Characters/Modules/DamageOwner_BPInter.Get Tag` OtherActor))
  (if (and (!= _tag_2 "None") (!= _tag_2 _tag))
    (`ProjectileMovementComponent.StopSimulating` (`self.ProjectileMovement`) (`GameplayStatics.MakeHitResult` true true 0.0 0.0 (0.0 0.0 0.0) (0.0 0.0 0.0) (0.0 0.0 1.0) (0.0 0.0 1.0) null OtherActor))
    (message `/Game/Resources/Characters/Player/Blueprints/ApplyingStat_BPInter.Apply Knockback` OtherActor _host -1000.0 200.0)
    (`GameplayStatics.ApplyDamage` OtherActor 20.0 null _host "/Script/Engine.DamageType")
    (set `self.Firing` false)
    (`self.K2_DestroyActor`)))

(event `self.ReceiveTick`
  (params (DeltaSeconds :type "Float (single-precision)"))
  (if (not (`self.Firing`))
    (`self.K2_SetActorLocation` (`KismetMathLibrary.VInterpTo` (`self.K2_GetActorLocation`) (`self.InitialLocation`) DeltaSeconds 40.0))))

(fn `Get Tag`
  (returns (Tag :type Name))
  (return (`|GetArrayItem` (`self.Tags`))))

(fn `Get Trace Channel`
  (returns (Channel :type "ETraceTypeQuery Enum"))
  (return "TraceTypeQuery1"))

(fn `UserConstructionScript`)