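; Goose weapon module Blueprint that layers honking audio and goose animations onto the light and heavy attacks inherited from its parent.
; Light attacks, and heavy attacks at nearly full charge, play the Honk event at the actor's location with the firing animation.
; Installing and uninstalling both play the start-up animation.
; Spawn Bullet creates the projectile with host, current passive and base damage, plus a Niagara flash effect.
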(event `self.LightAttack`
  (bind (_returnvalue_location _returnvalue_rotation) (`KismetMathLibrary.BreakTransform` (`self.GetTransform`)))
  (`parent.LightAttack`)
  (`FMODBlueprintStatics.PlayEventAtLocation` "/Game/FMOD/Events/Sounds/Module/Honk.Honk" (`KismetMathLibrary.MakeTransform` _returnvalue_location _returnvalue_rotation) :!label _label)
  (`SkeletalMeshComponent.PlayAnimation` (`self.SK_GooseModule`) "/Game/Resources/Characters/Modules/Goose/SK_GooseModule_Anim_GooseSkeleton_GooseFiring.SK_GooseModule_Anim_GooseSkeleton_GooseFiring" false))

(event `self.LightProjectileStart`
  (`parent.LightProjectileStart`))

(event `self.LightProjectileStop`
  (`parent.LightProjectileStop`))

(event `self.HeavyAttack`
  (params (Charge :type "Float (double-precision)"))
  (`parent.HeavyAttack` Charge)
  ;[1 0.5391 0] See if this is a (somewhat) fully charged attack
  (if (>= Charge 0.9)
    (goto _label)))

(event `self.On Installed`
  (`SkeletalMeshComponent.PlayAnimation` (`self.SK_GooseModule`) "/Game/Resources/Characters/Modules/Goose/SK_GooseModule_Anim_GooseSkeleton_GooseStartUp.SK_GooseModule_Anim_GooseSkeleton_GooseStartUp" false :!label _label_2))

(event `self.On Uninstalled`
  (goto _label_2))

(fn `Spawn Bullet`
  (params (Location :type "Vector Structure") (Rotation :type "Rotator Structure") (Scale :type "Vector Structure") (BaseDmg :type "Float (double-precision)"))
  (`|SpawnActorFromClass` (`self.BulletClass`) (`KismetMathLibrary.MakeTransform` Location Rotation Scale) "AlwaysSpawn" "OverrideRootScale" null (`self.Host`) (`/Game/Resources/Characters/Modules/ModuleManager_BPC.CurrentPassive` (`self.Manager`)) BaseDmg null)
  (`NiagaraFunctionLibrary.SpawnSystemAtLocation` "/Game/VFX_Pack/Niagara/NS_test_Flash_16.NS_test_Flash_16" Location Rotation (`self.ScaleParticle`)))

(fn `UserConstructionScript`
  (`parent.UserConstructionScript`))