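; Drone weapon module that fires bullets at the locked target, or along the player's facing without one.
; A Physics Control body tracks an anchor component, switching from kinematic to simulated during attacks so anchor kicks read as springy recoil.
; Light attacks fire once or on a looping timer; heavy attacks add a timed burst of short-lived drones, longer at high charge.
; Deploy spawns a DroneBuild_BP with a random nearby reachable destination.
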(event `self.ReceiveBeginPlay`
  (`PhysicsControlComponent.MakeControl` :`self` (`self.PhysicsControl`) :`ChildMeshComponent` (`self.Cylinder`) :`ControlData` (make `PhysicsControlData` 1.0 1.0 0.0 0.0 2.0))
  (`PhysicsControlComponent.MakeBodyModifier` (`self.PhysicsControl`) (`self.Cylinder`) "None" "Kinematic" "QueryAndPhysics" 0.0 true))

(event `self.LightAttack`
  (`parent.LightAttack`)
  (`self.Fire`)
  (`PhysicsControlComponent.SetBodyModifierMovementType` (`self.PhysicsControl`) "Body_0" "Simulated")
  (`SceneComponent.K2_AddWorldOffset` (`self.Cylinder1`) (+ (* (`KismetMathLibrary.RandomUnitVector`) (400.0 200.0 400.0)) (0.0 0.0 100.0)) false false)
  (bind _returnvalue (`KismetSystemLibrary.K2_SetTimerDelegate` (delegate `CustomEvent`) 0.5))
  (set `self.ResetTimer` _returnvalue))

(event `CustomEvent`
  (`PhysicsControlComponent.SetBodyModifierMovementType` (`self.PhysicsControl`) "Body_0" "Kinematic"))

(event `self.LightProjectileStop`
  (`parent.LightProjectileStop`)
  (`KismetSystemLibrary.K2_ClearAndInvalidateTimerHandle` (stale `self.LightProjectileStart` _returnvalue))
  (`KismetSystemLibrary.K2_SetTimerDelegate` (delegate `CustomEvent`) 0.3))

(event `self.LightProjectileStart`
  (`parent.LightProjectileStart`)
  (bind _returnvalue (`KismetSystemLibrary.K2_SetTimerDelegate` (delegate `Fire`) 0.1 true))
  (`KismetSystemLibrary.PrintString` "FIRE!!!" true true (struct :`R` 1.0 :`B` 0.094325 :`A` 1.0))
  (`KismetSystemLibrary.K2_PauseTimerHandle` (`self.ResetTimer`))
  (`PhysicsControlComponent.SetBodyModifierMovementType` (`self.PhysicsControl`) "Body_0" "Simulated"))

(event `self.HeavyAttack`
  (params (Charge :type "Float (double-precision)"))
  (`parent.HeavyAttack` Charge)
  (`self.LightAttack`)
  (`KismetSystemLibrary.Delay` 0.1)
  (bind _returnvalue (`KismetSystemLibrary.K2_SetTimerDelegate` (delegate `SpawnDrone`) 0.05 true))
  (`KismetSystemLibrary.Delay` (`KismetMathLibrary.SelectFloat` 0.16 0.09 (>= Charge 0.7)))
  (`KismetSystemLibrary.K2_ClearAndInvalidateTimerHandle` _returnvalue))

(event `Fire`
  (bind _locked_target (`self.Locked Target`))
  (bind _host (`self.Host`))
  (bind _returnvalue (`self.K2_GetActorRotation` (`GameplayStatics.GetPlayerPawn` 0)))
  (bind _returnvalue_2 (`SceneComponent.K2_GetComponentLocation` (`self.Cylinder`)))
  (bind _currentpassive (`/Game/Resources/Characters/Modules/ModuleManager_BPC.CurrentPassive` (`self.Manager`)))
  (bind _locked_target_2 (`self.Locked Target`)
    (:`then`
      (bind _returnvalue_3 (`KismetMathLibrary.FindLookAtRotation` _returnvalue_2 (`self.K2_GetActorLocation` _locked_target_2)))
      (`|SpawnActorFromClass` "/Game/Resources/Characters/Modules/Turrets/BulletBase_BP.BulletBase_BP_C" (`KismetMathLibrary.MakeTransform` _returnvalue_2 _returnvalue_3) "AlwaysSpawn" "OverrideRootScale" null _currentpassive 10.0 _host _locked_target null)
      (`NiagaraFunctionLibrary.SpawnSystemAttached` "/Game/VFX_Pack/Niagara/NS_test_Flash_16.NS_test_Flash_16" null "None" _returnvalue_2 _returnvalue_3 "KeepRelativeOffset"))
    (:`else`
      (`|SpawnActorFromClass` "/Game/Resources/Characters/Modules/Turrets/BulletBase_BP.BulletBase_BP_C" (`KismetMathLibrary.MakeTransform` _returnvalue_2 _returnvalue) "AlwaysSpawn" "OverrideRootScale" null _currentpassive 10.0 _host _locked_target null)
      (`NiagaraFunctionLibrary.SpawnSystemAttached` "/Game/VFX_Pack/Niagara/NS_test_Flash_16.NS_test_Flash_16" null "None" _returnvalue_2 _returnvalue "KeepRelativeOffset")))
  (`SceneComponent.SetRelativeScale3D` (`self.Cylinder`) (0.201568 0.201568 0.201568))
  (`GameplayStatics.SpawnForceFeedbackAttached` "/Game/Resources/Characters/Weapons/Sword/Fire_Feed.Fire_Feed" (`self.Cube`) "None" (0.0 0.0 0.0) (struct) "SnapToTarget" false false 1.0 0.0 null)
  (`SceneComponent.K2_SetRelativeLocation` (`self.Cylinder1`) (0.0 -300.0 300.0) false true)
  (`KismetSystemLibrary.RetriggerableDelay` 0.2)
  (`SceneComponent.SetRelativeScale3D` (`self.Cylinder`) (0.201568 0.201568 0.201568))
  (`SceneComponent.K2_SetRelativeLocation` (`self.Cylinder1`) (0.0 0.0 0.0) false true))

(event `self.ReceiveTick`
  (params (DeltaSeconds :type "Float (single-precision)"))
  (bind (_returnvalue_location _returnvalue_rotation) (`KismetMathLibrary.BreakTransform` (`SceneComponent.K2_GetComponentToWorld` (`self.Cylinder1`))))
  (`PhysicsControlComponent.SetControlTargetPositionAndOrientation` (`self.PhysicsControl`) "0" _returnvalue_location _returnvalue_rotation 0.0 true false)
  (`PhysicsControlComponent.SetBodyModifierKinematicTarget` (`self.PhysicsControl`) "Body_0" _returnvalue_location _returnvalue_rotation false))

(event `SpawnDrone`
  (bind _returnvalue (`|SpawnActorFromClass` "/Game/Resources/Characters/Modules/Drone/ModDrone_BP.ModDrone_BP_C" (`KismetMathLibrary.MakeTransform` (+ (* (`KismetMathLibrary.RandomUnitVector`) (100.0 100.0 0.0)) (`SceneComponent.K2_GetComponentLocation` (`self.Cylinder`))) (struct)) "AlwaysSpawn" "OverrideRootScale" null null))
  (set `/Game/Resources/Characters/Modules/Drone/ModDrone_BP.target` (`self.Locked Target`) _returnvalue)
  (set `/Game/Resources/Characters/Modules/Drone/ModDrone_BP.life` 3.0 _returnvalue))

(event `self.Deploy`
  (bind _returnvalue_location (`KismetMathLibrary.BreakTransform` (`self.GetTransform`)))
  (`parent.Deploy`)
  (`|SpawnActorFromClass` "/Game/Resources/Characters/Buildables/DroneBuild_BP.DroneBuild_BP_C" (`KismetMathLibrary.MakeTransform` _returnvalue_location) "Undefined" "OverrideRootScale" null null 200.0 (`NavigationSystemV1.K2_GetRandomReachablePointInRadius` (`self.K2_GetActorLocation`) 500.0 null null) (struct) null))

(fn `UserConstructionScript`
  (`parent.UserConstructionScript`))