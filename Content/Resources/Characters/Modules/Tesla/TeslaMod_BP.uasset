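; Tesla character module that deals area damage around itself on light, held and heavy attacks, using confetti VFX and sound.
; Fire sphere-traces for targets to damage and briefly pulses the sphere mesh, repeating on a timer scaled by the passive fire rate while held.
; A nearly full heavy charge spawns TeslaChain_BP instead.
; Deploy spawns ConfettiBuild_BP targeting a random reachable point; SpawnBullet is defined but not called here.
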(event `Fire`
  (bind _returnvalue (`self.K2_GetActorLocation`))
  (bind _arrow (`self.Arrow`))
  ;[0.9219 0 1] VFX & Sound
  ;;[0 1 0.2266] Adding Particles
  (`NiagaraFunctionLibrary.SpawnSystemAtLocation` "/Game/Resources/VFX/TestParticle/Confetti_NS.Confetti_NS" (`SceneComponent.K2_GetComponentLocation` _arrow) (`SceneComponent.K2_GetComponentRotation` _arrow))
  ;;[0 1 0.9297] Animation/procedural effect
  (`SceneComponent.SetRelativeScale3D` (`self.Sphere`) (1.0 1.0 1.0))
  ;;[0.4541 0.6188 1] FMOD Sound Event
  (`FMODBlueprintStatics.PlayEventAtLocation` "/Game/FMOD/Events/Sounds/Module/Confetti_Fire.Confetti_Fire" (`self.GetTransform`))
  (bind _outhits (`KismetSystemLibrary.SphereTraceMulti` _returnvalue _returnvalue 300.0 "TraceTypeQuery3"))
  (for _array_element _outhits
    (`GameplayStatics.ApplyDamage` (`.HitActor` (`GameplayStatics.BreakHitResult` _array_element)) 100.0 null (`self.Host`) "/Script/Engine.DamageType"))
  (`KismetSystemLibrary.Delay` 0.2)
  (`SceneComponent.SetRelativeScale3D` (`self.Sphere`) (0.5 0.5 0.5)))

(event `self.LightAttack`
  (`parent.LightAttack`)
  (`self.Fire`))

(event `self.LightProjectileStart`
  (bind (_currentpassive_type _currentpassive_speedscale _currentpassive_dmgscale _currentpassive_firerate) (break `/Game/Resources/Characters/Modules/ModulePassive_Struct` (`/Game/Resources/Characters/Modules/ModuleManager_BPC.CurrentPassive` (`self.Manager`))))
  (`parent.LightProjectileStart`)
  (bind _returnvalue (`KismetSystemLibrary.K2_SetTimer` null "Fire" (* (`self.BaseFireRate`) _currentpassive_firerate) true))
  (`self.Fire`))

(event `self.LightProjectileStop`
  (`parent.LightProjectileStop`)
  (`KismetSystemLibrary.K2_ClearAndInvalidateTimerHandle` (stale `self.LightProjectileStart` _returnvalue)))

(event `self.HeavyAttack`
  (params (Charge :type "Float (double-precision)"))
  (`parent.HeavyAttack` Charge)
  ;[1 0.5391 0] See if this is a (somewhat) fully charged attack
  (if (>= Charge 0.9)
    (`|SpawnActorFromClass` "/Game/Resources/Characters/Modules/Tesla/TeslaChain_BP.TeslaChain_BP_C" (`self.GetTransform`) "Undefined" "OverrideRootScale" null null)
    (else
      (`self.Fire`))))

(event `self.Deploy`
  (bind _returnvalue_location (`KismetMathLibrary.BreakTransform` (`self.GetTransform`)))
  (bind _returnvalue (`self.K2_GetActorLocation`))
  (`parent.Deploy`)
  ;[0 0.08594 1] Just use it if you want to spawn buildable at random sphere range
  (bind (_outhit _returnvalue_2) (`KismetSystemLibrary.SphereTraceSingleForObjects` _returnvalue _returnvalue 1000.0 (`|MakeArray` "ObjectTypeQuery1" :!type "EObjectTypeQuery Enum")))
  (if _returnvalue_2
    ;[0.8516 1 0] You just need to cahnge the "Class" here
    (`|SpawnActorFromClass` "/Game/Resources/Characters/Buildables/ConfettiBuild_BP.ConfettiBuild_BP_C" (`KismetMathLibrary.MakeTransform` _returnvalue_location) "Undefined" "OverrideRootScale" null null 200.0 (`NavigationSystemV1.K2_GetRandomReachablePointInRadius` _returnvalue 500.0 null null) (struct) true null)))

(fn `Spawn Bullet`
  (params (Location :type "Vector Structure") (Rotation :type "Rotator Structure") (Scale :type "Vector Structure") (BaseDmg :type "Float (double-precision)"))
  (`|SpawnActorFromClass` (`self.BulletClass`) (`KismetMathLibrary.MakeTransform` Location Rotation Scale) "AlwaysSpawn" "OverrideRootScale" null (`self.Host`) (`/Game/Resources/Characters/Modules/ModuleManager_BPC.CurrentPassive` (`self.Manager`)) BaseDmg null)
  (`NiagaraFunctionLibrary.SpawnSystemAtLocation` "/Game/VFX_Pack/Niagara/NS_test_Flash_16.NS_test_Flash_16" Location Rotation (`self.ScaleParticle`)))

(fn `UserConstructionScript`
  (`parent.UserConstructionScript`))