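; Zone character module that deals area damage and upward knockback in a sphere around itself.
; Light attacks, a looping projectile timer and heavy attacks all call Fire, which builds Charge; heavy attacks double it and briefly raise its cap.
; Tick eases the sphere's scale with Charge, and its bounds set the delayed, debug-drawn trace radius.
; A retriggerable delay hides the sphere and resets Charge once firing pauses.
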(event `self.LightAttack`
  (`parent.LightAttack`)
  (if (<= (`self.Cooldown`) 0.0)
    (set `self.Cooldown` 0.4)
    (`self.Fire`)))

(event `self.LightProjectileStop`
  (`parent.LightProjectileStop`)
  (`KismetSystemLibrary.K2_ClearAndInvalidateTimerHandle` (stale `self.LightProjectileStart` _returnvalue)))

(event `self.LightProjectileStart`
  (`parent.LightProjectileStart`)
  (bind _returnvalue (`KismetSystemLibrary.K2_SetTimer` null "Fire" (`self.BaseFireRate`) true))
  (`self.Fire`))

(event `self.HeavyAttack`
  (params (Charge :type "Float (double-precision)"))
  (`parent.HeavyAttack` Charge)
  (set `self.Charge` (* Charge 2.0))
  (set `self.MaxCharge` 2.0)
  (`self.Fire`)
  (set `self.MaxCharge` 1.0))

(event `Fire`
  (bind _returnvalue (`self.K2_GetActorLocation`))
  (`SceneComponent.SetVisibility` (`self.Sphere`) true false)
  (set `self.Charge` (`KismetMathLibrary.FMin` (+ (`self.Charge`) 0.1) (`self.MaxCharge`)))
  (`|ExecutionSequence`
    (:`then_0`
      (`KismetSystemLibrary.Delay` 0.1)
      (bind _channel (message `/Game/Resources/Characters/Modules/DamageOwner_BPInter.Get Trace Channel` (`self.Host`)))
      (bind (_outhits _returnvalue_2) (`KismetSystemLibrary.SphereTraceMulti` :`Start` _returnvalue :`End` _returnvalue :`Radius` (`.SphereRadius` (`KismetSystemLibrary.GetComponentBounds` (`self.Sphere`))) :`TraceChannel` _channel :`DrawDebugType` "ForDuration"))
      (if _returnvalue_2
        (for _array_element _outhits
          (`GameplayStatics.ApplyDamage` (`.HitActor` (`GameplayStatics.BreakHitResult` _array_element)) (`KismetMathLibrary.Lerp` 10.0 60.0 (`self.Charge`)) null (`self.Host`) "/Script/Engine.DamageType")
          (message `/Game/Resources/Characters/Player/Blueprints/Knockback_BPInter.Apply Knockback` (`.HitActor` (`GameplayStatics.BreakHitResult` _array_element)) self 0.0 (`KismetMathLibrary.Lerp` 100.0 400.0 (`self.Charge`))))))
    (:`then_1`
      (`KismetSystemLibrary.RetriggerableDelay` 0.7)
      (`SceneComponent.SetVisibility` (`self.Sphere`) false false)
      (set `self.Charge` 0.0)
      (`SceneComponent.SetRelativeScale3D` (`self.Sphere`) (3.0 3.0 3.0)))))

(event `self.ReceiveTick`
  (params (DeltaSeconds :type "Float (single-precision)"))
  (bind _sphere (`self.Sphere`))
  (`parent.ReceiveTick` DeltaSeconds)
  (`SceneComponent.SetRelativeScale3D` _sphere (`KismetMathLibrary.VInterpTo` (`SceneComponent.RelativeScale3D` _sphere) (`KismetMathLibrary.VLerp` (2.0 2.0 2.0) (8.0 8.0 8.0) (`self.Charge`)) DeltaSeconds 20.0)))

(fn `UserConstructionScript`
  (`parent.UserConstructionScript`))