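; Cutter character module, a spinning melee weapon that damages and knocks back characters, with light, held and charged heavy attacks.
; Each attack triggers Fire, which briefly enlarges and spins the Sphere, sphere-traces for hits and sets the sound's Hit parameter.
; Heavy attacks use a timeline to extend the arm by charge with a wider radius.
; Deploy spawns CutterBuild_BP targeting a random reachable point when world-static geometry is nearby.
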(event `self.ReceiveBeginPlay`
  (`parent.ReceiveBeginPlay`)
  (bind _returnvalue (`FMODBlueprintStatics.PlayEventAttached` "/Game/FMOD/Events/Sounds/Module/Cutter_Fire.Cutter_Fire" (`self.Sphere`) "None" (0.0 0.0 0.0) "SnapToTarget" true false false))
  (set `self.SoundEvent` _returnvalue))

(event `self.LightAttack`
  (`parent.LightAttack`)
  (`FMODAudioComponent.Play` (`self.SoundEvent`))
  (`KismetSystemLibrary.Delay` 0.1)
  (`self.Fire`)
  (`FMODAudioComponent.Stop` (`self.SoundEvent`)))

(event `self.LightProjectileStart`
  (`parent.LightProjectileStart`)
  (`FMODAudioComponent.Play` (`self.SoundEvent`))
  (bind _returnvalue (`KismetSystemLibrary.K2_SetTimer` null "Fire" 0.1 true)))

(event `self.LightProjectileStop`
  (`parent.LightProjectileStop`)
  (`FMODAudioComponent.Stop` (`self.SoundEvent`))
  (`KismetSystemLibrary.K2_ClearAndInvalidateTimerHandle` (stale `self.LightProjectileStart` _returnvalue)))

(event `Fire`
  (bind _returnvalue (`self.K2_GetActorLocation`))
  (bind _host (`self.Host`))
  (bind _soundevent (`self.SoundEvent`))
  (`ActorComponent.SetComponentTickEnabled` (`self.RotatingMovement`) true)
  (`SceneComponent.SetRelativeScale3D` (`self.Sphere`) (0.3 0.3 0.3))
  (`|ExecutionSequence`
    (:`then_0`
      (bind (_outhits _returnvalue_2) (`KismetSystemLibrary.SphereTraceMulti` _returnvalue _returnvalue (`self.Radius`) "TraceTypeQuery3"))
      (if _returnvalue_2
        (`FMODAudioComponent.SetParameter` _soundevent "Hit" 1.0)
        (for _array_element _outhits
          (`GameplayStatics.ApplyDamage` (`.HitActor` (`GameplayStatics.BreakHitResult` _array_element)) 10.0 null _host "/Script/Engine.DamageType")
          (bind _ascharacter (cast `Character` (`.HitActor` (`GameplayStatics.BreakHitResult` _array_element))))
          (bind (_returnvalue_x _returnvalue_y) (`KismetMathLibrary.BreakVector` (`KismetMathLibrary.GetForwardVector` (`KismetMathLibrary.FindLookAtRotation` (`self.K2_GetActorLocation` _host) (`self.K2_GetActorLocation` _ascharacter)))))
          (`Character.LaunchCharacter` _ascharacter (+ (* (`KismetMathLibrary.MakeVector` _returnvalue_x _returnvalue_y) 1000.0) (0.0 0.0 80.0)) false false))
        (else
          (`FMODAudioComponent.SetParameter` _soundevent "Hit" 0.0))))
    (:`then_1`
      (`KismetSystemLibrary.RetriggerableDelay` 0.2)
      (`SceneComponent.SetRelativeScale3D` (`self.Sphere`) (0.144561 0.144561 0.144561))
      (`ActorComponent.SetComponentTickEnabled` (`self.RotatingMovement`) false))))

(event `self.HeavyAttack`
  (params (Charge :type "Float (double-precision)"))
  (bind _arm (`self.Arm`))
  (`parent.HeavyAttack` Charge)
  (`FMODAudioComponent.Play` (`self.SoundEvent`))
  (set `self.Radius` 180.0)
  (bind (_direction _newtrack_0) (`Timeline|Heavy` :!via `PlayFromStart`)
    (:`Update`
      (bind _returnvalue (`KismetMathLibrary.Lerp` 0.0 (`KismetMathLibrary.Lerp` 0.0 200.0 Charge) _newtrack_0))
      (`SceneComponent.K2_SetRelativeLocation` (`self.Sphere`) (`KismetMathLibrary.MakeVector` _returnvalue) false false)
      (`SceneComponent.SetRelativeScale3D` _arm (`KismetMathLibrary.MakeVector` _newtrack_0 0.271916 0.271916))
      (`SceneComponent.K2_SetRelativeLocation` _arm (`KismetMathLibrary.MakeVector` (/ _returnvalue 2.0)) false false))
    (:`Finished`
      (set `self.Radius` 80.0)
      (`FMODAudioComponent.Stop` (`self.SoundEvent`)))
    (:`Trigger`
      (`self.Fire`))))

(event `self.Deploy`
  (bind _returnvalue_location (`KismetMathLibrary.BreakTransform` (`self.GetTransform`)))
  (bind _returnvalue (`self.K2_GetActorLocation`))
  (`parent.Deploy`)
  (bind (_outhit _returnvalue_2) (`KismetSystemLibrary.SphereTraceSingleForObjects` _returnvalue _returnvalue 600.0 (`|MakeArray` "ObjectTypeQuery1" :!type "EObjectTypeQuery Enum")))
  (if _returnvalue_2
    (`|SpawnActorFromClass` "/Game/Resources/Characters/Buildables/CutterBuild_BP.CutterBuild_BP_C" (`KismetMathLibrary.MakeTransform` _returnvalue_location) "Undefined" "OverrideRootScale" null (`NavigationSystemV1.K2_GetRandomReachablePointInRadius` _returnvalue 300.0 null null) null)))

(fn `UserConstructionScript`
  (`parent.UserConstructionScript`))