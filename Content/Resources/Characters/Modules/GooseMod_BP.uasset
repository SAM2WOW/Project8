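; GooseMod_BP is a character attack module, a child Blueprint that adds goose honks on top of its parent's behavior.
; Light attacks always play the Honk event at the actor's location, while heavy attacks honk only when nearly fully charged.
; SpawnBullet spawns the bullet with host, current passive and base damage, plus a muzzle-flash-style particle system at the same spot.
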(event `self.LightAttack`
  (`parent.LightAttack`)
  (`FMODBlueprintStatics.PlayEventAtLocation` "/Game/FMOD/Events/Sounds/Module/Honk.Honk" (`self.GetTransform`)))

(event `self.LightProjectileStart`
  (`parent.LightProjectileStart`))

(event `self.LightProjectileStop`
  (`parent.LightProjectileStop`))

(event `self.HeavyAttack`
  (params (Charge :type "Float (double-precision)"))
  (`parent.HeavyAttack` Charge)
  ;[1 0.5391 0] See if this is a (somewhat) fully charged attack
  (if (>= Charge 0.9)
    (`FMODBlueprintStatics.PlayEventAtLocation` "/Game/FMOD/Events/Sounds/Module/Honk.Honk" (`self.GetTransform`))))

(event `self.Deploy`
  (`parent.Deploy`))

(fn `Spawn Bullet`
  (params (Location :type "Vector Structure") (Rotation :type "Rotator Structure") (Scale :type "Vector Structure") (BaseDmg :type "Float (double-precision)"))
  (`|SpawnActorFromClass` (`self.BulletClass`) (`KismetMathLibrary.MakeTransform` Location Rotation Scale) "AlwaysSpawn" "OverrideRootScale" null (`self.Host`) (`/Game/Resources/Characters/Modules/ModuleManager_BPC.CurrentPassive` (`self.Manager`)) BaseDmg null)
  (`NiagaraFunctionLibrary.SpawnSystemAtLocation` "/Game/VFX_Pack/Niagara/NS_test_Flash_16.NS_test_Flash_16" Location Rotation (`self.ScaleParticle`)))

(fn `UserConstructionScript`
  (`parent.UserConstructionScript`))