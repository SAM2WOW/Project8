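; Temporary flying drone module that shoots at nearby actors and self-destructs after a randomized lifetime, with a Niagara effect at spawn and death.
; A looping timer, gated by Activated, sphere-traces around the body, fires bullets at the hit actor and adopts it as Target if none is valid.
; Tick moves a reference point toward a height above Target, and Physics Control steers the gravity-free body to it.
; Older pursuit logic remains unconnected.
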(event `self.ReceiveBeginPlay`
  (bind _body (`self.Body`))
  (`NiagaraFunctionLibrary.SpawnSystemAtLocation` "/Game/VFX_Pack/Niagara/NS_Bolb.NS_Bolb" (`SceneComponent.K2_GetComponentLocation` (`self.Body`)))
  (`PhysicsControlComponent.MakeControl` :`self` (`self.PhysicsControl`) :`ChildMeshComponent` _body :`ControlData` (make `PhysicsControlData` 1.0 1.0 0.0 0.0 2.0))
  (`PhysicsControlComponent.MakeBodyModifier` (`self.PhysicsControl`) _body "None" "Simulated" "QueryAndPhysics" 0.0 true)
  (`KismetSystemLibrary.DelayUntilNextTick`)
  (`KismetSystemLibrary.K2_SetTimer` null "Fire" 0.3 true)
  (set `self.z_offset` (`KismetMathLibrary.RandomFloatInRange` 150.0 300.0))
  (`KismetSystemLibrary.Delay` (+ (`self.life`) (`KismetMathLibrary.RandomFloatInRange` 1.0 2.0)))
  (`NiagaraFunctionLibrary.SpawnSystemAtLocation` "/Game/VFX_Pack/Niagara/NS_Bolb.NS_Bolb" (`SceneComponent.K2_GetComponentLocation` (`self.Body`)))
  (`self.K2_DestroyActor`))

(event `Fire`
  (bind _returnvalue (`SceneComponent.K2_GetComponentLocation` (`self.Body`)))
  (bind _returnvalue_2 (`SceneComponent.K2_GetComponentLocation` (`self.Body`)))
  (if (`self.Activated`)
    (bind (_outhit _returnvalue_3) (`KismetSystemLibrary.SphereTraceSingle` _returnvalue_2 _returnvalue_2 800.0 "TraceTypeQuery3"))
    (if _returnvalue_3
      (bind (_bblockinghit _binitialoverlap _time _distance _location _impactpoint _normal _impactnormal _physmat _hitactor) (`GameplayStatics.BreakHitResult` _outhit))
      (`|SpawnActorFromClass` "/Game/Resources/Characters/Modules/Turrets/BulletBase_BP.BulletBase_BP_C" (`KismetMathLibrary.MakeTransform` _returnvalue (`KismetMathLibrary.FindLookAtRotation` _returnvalue (`self.K2_GetActorLocation` _hitactor))) "AlwaysSpawn" "OverrideRootScale" null (struct) 10.0 null null null)
      (if (not (`KismetSystemLibrary.IsValid` (`self.target`)))
        (set `self.target` _hitactor)))))

(event `self.ReceiveTick`
  (params (DeltaSeconds :type "Float (single-precision)"))
  (bind _ref (`self.ref`))
  (bind _returnvalue (`self.K2_GetActorLocation` (`self.target`)))
  (bind _returnvalue_location (`KismetMathLibrary.BreakTransform` (`SceneComponent.K2_GetComponentToWorld` (`self.ref`))))
  (bind (_x _y _z) (`KismetMathLibrary.BreakVector3f` _returnvalue))
  (bind _returnvalue_2 (* (`SceneComponent.K2_GetComponentLocation` _ref) (1.0 1.0 0.0)))
  (`|ExecutionSequence`
    (:`then_0`
      (if (`KismetSystemLibrary.IsValid` (`self.target`))
        (if (>= (`KismetMathLibrary.Vector_Distance` _returnvalue _returnvalue_2) 300.0)
          (`SceneComponent.K2_SetWorldLocation` _ref (+ (`KismetMathLibrary.VLerp` _returnvalue_2 (`KismetMathLibrary.MakeVector` _x _y) 0.1) (`KismetMathLibrary.MakeVector` 0.0 0.0 (+ _z (`self.z_offset`)))) false false)
          (else
            (`SceneComponent.K2_SetWorldLocation` (`self.ref`) (`SceneComponent.K2_GetComponentLocation` (`self.Body`)) false false)))))
    (:`then_1`
      (`PhysicsControlComponent.SetControlTargetPositionAndOrientation` (`self.PhysicsControl`) "0" _returnvalue_location (struct :`Roll` 90.0) 0.0 true false)
      (`PhysicsControlComponent.SetBodyModifierKinematicTarget` (`self.PhysicsControl`) "Body_0" _returnvalue_location (struct :`Roll` 90.0) false))))

(fn `UserConstructionScript`)