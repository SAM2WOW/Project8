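; Confetti character module that answers light, projectile and heavy attacks with confetti bursts; no damage logic appears here.
; Fire spawns Niagara confetti and sound, then plays a timeline stretching the ejector mesh, which also plays on install.
; Held projectile fire loops Fire on a timer scaled by the passive's fire rate.
; Heavy attacks temporarily enlarge the particles, adding an upward burst at high charge; ConfettiBuild_BP spawning is unconnected.
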(event `self.LightAttack`
  (`parent.LightAttack`)
  (`KismetSystemLibrary.Delay` 0.1)
  (`self.Fire`))

(event `self.LightProjectileStop`
  (`parent.LightProjectileStop`)
  (`KismetSystemLibrary.K2_ClearAndInvalidateTimerHandle` (stale `self.LightProjectileStart` _returnvalue)))

(event `self.LightProjectileStart`
  (bind (_currentpassive_type _currentpassive_speedscale _currentpassive_dmgscale _currentpassive_firerate) (break `/Game/Resources/Characters/Modules/ModulePassive_Struct` (`/Game/Resources/Characters/Modules/ModuleManager_BPC.CurrentPassive` (`self.Manager`))))
  (`parent.LightProjectileStart`)
  (bind _returnvalue (`KismetSystemLibrary.K2_SetTimer` null "Fire" (* (`self.BaseFireRate`) _currentpassive_firerate) true))
  (`self.Fire`))

(event `self.HeavyAttack`
  (params (Charge :type "Float (double-precision)"))
  (bind _returnvalue (`SceneComponent.K2_GetComponentLocation` (`self.Arrow`)))
  (`parent.HeavyAttack` Charge)
  (set `self.ScaleParticle` (10.0 10.0 10.0))
  (`self.Fire`)
  (if (>= Charge 0.7)
    (`NiagaraFunctionLibrary.SpawnSystemAtLocation` "/Game/Resources/VFX/TestParticle/Confetti_NS.Confetti_NS" _returnvalue (`KismetMathLibrary.FindLookAtRotation` _returnvalue (+ _returnvalue (0.0 0.0 1000.0))) (`self.ScaleParticle`)))
  (`KismetSystemLibrary.Delay` 0.2)
  (set `self.ScaleParticle` (1.0 1.0 1.0)))

(event `self.On Installed`
  (bind (_direction _explode) (`Timeline|Timeline` :!via `PlayFromStart` :!label _label)
    (:`Update`
      (`SceneComponent.SetRelativeScale3D` (`self.ConfettiEjector`) (`KismetMathLibrary.MakeVector` 1.0 1.0 (`KismetMathLibrary.Lerp` 1.0 3.0 _explode))))))

(event `Fire`
  (bind _arrow (`self.Arrow`))
  (`NiagaraFunctionLibrary.SpawnSystemAtLocation` "/Game/Resources/VFX/TestParticle/Confetti_NS.Confetti_NS" (`SceneComponent.K2_GetComponentLocation` _arrow) (`SceneComponent.K2_GetComponentRotation` _arrow) (`self.ScaleParticle`))
  (`FMODBlueprintStatics.PlayEventAtLocation` "/Game/FMOD/Events/Sounds/Module/Confetti_Fire.Confetti_Fire" (`self.GetTransform`))
  (goto _label :!via `PlayFromStart`))

(fn `UserConstructionScript`
  (`parent.UserConstructionScript`))