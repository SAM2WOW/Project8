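; PrinterMod_BP is a ranged weapon module that fires PrinterCoin_BP projectiles, aimed at the locked target when one is valid.
; Light attack fires once, projectile mode loops on a timer scaled by the manager's passive fire rate, and heavy attack fires a short delayed burst.
; Each shot passes damage and the host's tag, plays audio and force feedback, and briefly stretches the cube.
; The scrap-consumption logic is disconnected.
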(event `self.LightAttack`
  (`parent.LightAttack`)
  (`self.Fire`))

(event `self.LightProjectileStop`
  (`parent.LightProjectileStop`)
  (`KismetSystemLibrary.K2_ClearAndInvalidateTimerHandle` (stale `self.LightProjectileStart` _returnvalue)))

(event `self.LightProjectileStart`
  (bind (_currentpassive_type _currentpassive_speedscale _currentpassive_dmgscale _currentpassive_firerate) (break `/Game/Resources/Characters/Modules/ModulePassive_Struct` (`/Game/Resources/Characters/Modules/ModuleManager_BPC.CurrentPassive` (`self.Manager`))))
  (`parent.LightProjectileStart`)
  (bind _returnvalue (`KismetSystemLibrary.K2_SetTimer` null "Fire" (* (`self.BaseFireRate`) _currentpassive_firerate) true))
  (`self.Fire`))

(event `self.HeavyAttack`
  (params (Charge :type "Float (double-precision)"))
  (`parent.HeavyAttack` Charge)
  (`/Game/Resources/Characters/Player/Blueprints/NewActorMacroLibrary.ForLoopWithDelay` 0 3 0.05
    (:`Loop Body`
      (`self.Fire`))))

(event `Fire`
  (bind (_returnvalue_location _returnvalue_rotation) (`KismetMathLibrary.BreakTransform` (`self.GetTransform`)))
  (bind _basedmg (`self.BaseDmg`))
  (bind _locked_target (`self.Locked Target`)
    (:`then`
      (`self.Spawn Bullet` _returnvalue_location (`KismetMathLibrary.FindLookAtRotation` (`self.K2_GetActorLocation` self) (`self.K2_GetActorLocation` _locked_target)) (1.0 1.0 1.0) _basedmg))
    (:`else`
      (`self.Spawn Bullet` _returnvalue_location _returnvalue_rotation (1.0 1.0 1.0) _basedmg)))
  (`SceneComponent.SetRelativeScale3D` (`self.Cube`) (0.206141 0.206141 0.60321))
  (`|ExecutionSequence`
    (:`then_1`
      (`KismetSystemLibrary.RetriggerableDelay` 0.2)
      (`SceneComponent.SetRelativeScale3D` (`self.Cube`) (0.206141 0.206141 0.206141)))))

(fn `Spawn Bullet`
  (params (Location :type "Vector Structure") (Rotation :type "Rotator Structure") (Scale :type "Vector Structure") (BaseDmg :type "Float (double-precision)"))
  (bind _tag (message `/Game/Resources/Characters/Modules/DamageOwner_BPInter.Get Tag` (`self.Host`)))
  (`|SpawnActorFromClass` "/Game/Resources/Characters/Modules/Printer/PrinterCoin_BP.PrinterCoin_BP_C" (`KismetMathLibrary.MakeTransform` Location Rotation Scale) "AdjustIfPossibleButAlwaysSpawn" "OverrideRootScale" null _tag BaseDmg null)
  (`FMODBlueprintStatics.PlayEventAtLocation` "/Game/FMOD/Events/Sounds/Module/Printer_Fire.Printer_Fire" (`KismetMathLibrary.MakeTransform` Location Rotation))
  (`GameplayStatics.SpawnForceFeedbackAttached` "/Game/Resources/Characters/Weapons/Sword/Feedbacks/Fire_Feed.Fire_Feed" (`self.Cube`) "None" (0.0 0.0 0.0) (struct) "SnapToTarget" false false (`KismetMathLibrary.RandomFloatInRange` 0.5 1.0) 0.0 null))

(fn `UserConstructionScript`
  (`parent.UserConstructionScript`))