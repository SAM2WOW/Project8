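; PrinterCoin is a coin actor for the Printer module that is drawn into whatever overlaps it and can damage that target.
; Its sphere collision turns on shortly after spawn, then an overlap starts a timeline that lerps the coin to the target's live location.
; On arrival it runs parent collect logic, damages and knocks back DamageOwner targets with a different tag, then destroys itself.
; The projectile bounce handler is empty.
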(event `self.ReceiveBeginPlay`
  (`KismetSystemLibrary.Delay` 0.8)
  (`PrimitiveComponent.SetCollisionEnabled` (`self.Sphere1`) "QueryAndPhysics"))

(event `self.Sphere1.OnComponentBeginOverlap`
  (params (OverlappedComponent :type "PrimitiveComponent Object Reference") (OtherActor :type "Actor Object Reference") (OtherComp :type "PrimitiveComponent Object Reference") (OtherBodyIndex :type Integer) (bFromSweep :type Boolean) (SweepResult :type "HitResult Structure (by ref)"))
  (set `self.TargetActor` OtherActor)
  (set `self.TempLocation` (`self.K2_GetActorLocation`))
  (bind (_direction _collect) (`Timeline|Timeline`)
    (:`Update`
      (`self.K2_SetActorLocation` (`KismetMathLibrary.VLerp` (`self.TempLocation`) (`self.K2_GetActorLocation` (`self.TargetActor`)) _collect)))
    (:`Finished`
      (`self.On Collect`)
      (`self.K2_DestroyActor`))))

(event `self.On Collect`
  (bind _targetactor (`self.TargetActor`))
  (`parent.On Collect`)
  (if (`KismetSystemLibrary.DoesImplementInterface` (`self.TargetActor`) "/Game/Resources/Characters/Modules/DamageOwner_BPInter.DamageOwner_BPInter_C")
    (bind _tag (message `/Game/Resources/Characters/Modules/DamageOwner_BPInter.Get Tag` (`self.TargetActor`)))
    (if (!= _tag (`self.Tag`))
      (`GameplayStatics.ApplyDamage` _targetactor (`self.Base Damage`) null self "/Script/Engine.DamageType")
      (message `/Game/Resources/Characters/Player/Blueprints/Knockback_BPInter.Apply Knockback` _targetactor self 100.0 50.0))))

(event `self.ProjectileMovement.OnProjectileBounce`
  (params (ImpactResult :type "HitResult Structure (by ref)") (ImpactVelocity :type "Vector Structure (by ref)")))

(fn `UserConstructionScript`
  (`parent.UserConstructionScript`))