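; Cutter weapon module for a host character, attacking with spinning blades that damage and knock back everything in a sphere around the module.
; Light attack fires once and projectile mode loops Fire on a timer; each hit pass enlarges and spins blades until a retriggerable delay resets them.
; Heavy attack extends the arm by charge on a timeline, widening the radius for stronger hits that notify the GameState.
; An attached sound's Hit parameter follows trace results.
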(event `self.ReceiveTick`
  (params (DeltaSeconds :type "Float (single-precision)"))
  (`parent.ReceiveTick` DeltaSeconds)
  (if (`self.Rotate`)
    (`SceneComponent.K2_AddLocalRotation` (`self.CutterPole`) (struct :`Yaw` 10.0) false false)))

(event `self.ReceiveBeginPlay`
  (`parent.ReceiveBeginPlay`)
  (bind _returnvalue (`FMODBlueprintStatics.PlayEventAttached` "/Game/FMOD/Events/Sounds/Module/Cutter_Fire.Cutter_Fire" (`self.CutterPole`) "None" (0.0 0.0 0.0) "SnapToTarget" true false false))
  (set `self.SoundEvent` _returnvalue))

(event `self.LightAttack`
  (`parent.LightAttack`)
  (`FMODAudioComponent.Play` (`self.SoundEvent`))
  (`KismetSystemLibrary.Delay` 0.1)
  (`self.Fire`)
  (`FMODAudioComponent.Stop` (`self.SoundEvent`)))

(event `self.LightProjectileStart`
  (`parent.LightProjectileStart`)
  (`FMODAudioComponent.Play` (`self.SoundEvent`))
  (bind _returnvalue (`KismetSystemLibrary.K2_SetTimer` null "Fire" 0.05 true)))

(event `self.LightProjectileStop`
  (`parent.LightProjectileStop`)
  (`FMODAudioComponent.Stop` (`self.SoundEvent`))
  (`KismetSystemLibrary.K2_ClearAndInvalidateTimerHandle` (stale `self.LightProjectileStart` _returnvalue)))

(event `Fire`
  (bind _returnvalue (`self.K2_GetActorLocation`))
  (bind _soundevent (`self.SoundEvent`))
  (set `self.Rotate` true)
  (`SceneComponent.SetRelativeScale3D` (`self.CutterBlade_001`) (1.0 1.0 1.0))
  (`SceneComponent.SetRelativeScale3D` (`self.CutterBlade_002`) (1.0 1.0 1.0))
  (`|ExecutionSequence`
    (:`then_0`
      (bind _channel (message `/Game/Resources/Characters/Modules/DamageOwner_BPInter.Get Trace Channel` (`self.Host`)))
      (bind (_outhits _returnvalue_2) (`KismetSystemLibrary.SphereTraceMulti` _returnvalue _returnvalue (`self.Radius`) _channel))
      (if _returnvalue_2
        (`FMODAudioComponent.SetParameter` _soundevent "Hit" 1.0)
        (for _array_element _outhits
          (`GameplayStatics.ApplyDamage` (`.HitActor` (`GameplayStatics.BreakHitResult` _array_element)) (`KismetMathLibrary.SelectFloat` 30.0 5.0 (>= (`self.Radius`) 140.0)) null (`self.Host`) "/Script/Engine.DamageType")
          (message `/Game/Resources/Characters/Player/Blueprints/Knockback_BPInter.Apply Knockback` (`.HitActor` (`GameplayStatics.BreakHitResult` _array_element)) self (`KismetMathLibrary.SelectFloat` 100.0 10.0 (>= (`self.Radius`) 140.0)) 4.0)
          (if (>= (`self.Radius`) 140.0)
            (bind _asnew_game_state_gs (cast `/Game/Resources/Characters/Player/Blueprints/NewGameState_GS` (`GameplayStatics.GetGameState`)))
            (`/Game/Resources/Characters/Player/Blueprints/NewGameState_GS.Enter Damange` _asnew_game_state_gs 0.6)))
        (else
          (`FMODAudioComponent.SetParameter` _soundevent "Hit" 0.0))))
    (:`then_1`
      (`KismetSystemLibrary.RetriggerableDelay` 0.2)
      (`SceneComponent.SetRelativeScale3D` (`self.CutterBlade_001`) (0.5 0.5 0.5))
      (`SceneComponent.SetRelativeScale3D` (`self.CutterBlade_002`) (0.5 0.5 0.5))
      (set `self.Rotate` false))))

(event `self.HeavyAttack`
  (params (Charge :type "Float (double-precision)"))
  (bind _arm (`self.Arm`))
  (`parent.HeavyAttack` Charge)
  (`FMODAudioComponent.Play` (`self.SoundEvent`))
  (`ActorComponent.SetActive` (`self.Trail_NS1`) true false)
  (set `self.Radius` 180.0)
  (bind (_direction _newtrack_0) (`Timeline|Heavy` :!via `PlayFromStart`)
    (:`Update`
      (bind _returnvalue (`KismetMathLibrary.Lerp` 0.0 (`KismetMathLibrary.Lerp` 0.0 200.0 Charge) _newtrack_0))
      (`SceneComponent.K2_SetRelativeLocation` (`self.CutterPole`) (`KismetMathLibrary.MakeVector` _returnvalue) false false)
      (`SceneComponent.SetRelativeScale3D` _arm (`KismetMathLibrary.MakeVector` _newtrack_0 0.271916 0.271916))
      (`SceneComponent.K2_SetRelativeLocation` _arm (`KismetMathLibrary.MakeVector` (/ _returnvalue 2.0)) false false))
    (:`Finished`
      (set `self.Radius` 80.0)
      (`FMODAudioComponent.Stop` (`self.SoundEvent`))
      (`ActorComponent.SetActive` (`self.Trail_NS1`) false false))
    (:`Trigger`
      (`self.Fire`))))

(event `self.Deploy`
  (`parent.Deploy`))

(fn `UserConstructionScript`
  (`parent.UserConstructionScript`))