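; Weapon module (CableMod) that heals the character holding the host weapon and uses Planter module meshes and animations.
; Light attack gives a fixed heal with a firing animation, repeating on a timer during projectile mode, while heavy attack heals by charge.
; Tick keeps a sphere on the wielder, install and uninstall play open and close animations, and CalculatePassive registers the module and increments its type count.
; Lock-on damage logic is left disconnected.
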(event `self.ReceiveTick`
  (params (DeltaSeconds :type "Float (single-precision)"))
  (`parent.ReceiveTick` DeltaSeconds)
  (`|ExecutionSequence`
    (:`then_0`
      (bind _asweapon_base_bp (cast `/Game/Resources/Characters/Weapons/WeaponBase_BP` (`self.Host`)))
      (`SceneComponent.K2_SetWorldLocation` (`self.Sphere1`) (`self.K2_GetActorLocation` (`/Game/Resources/Characters/Weapons/WeaponBase_BP.Host` _asweapon_base_bp)) false false))))

(event `self.LightAttack`
  (`self.Fire`))

(event `self.On Installed`
  (`SkeletalMeshComponent.PlayAnimation` (`self.SK_PlanterModule`) "/Game/Resources/Characters/Modules/Planter/SK_PlanterModule_Anim_PlanterArmature_PlanterStartUp.SK_PlanterModule_Anim_PlanterArmature_PlanterStartUp" false))

(event `self.LightProjectileStart`
  (bind _returnvalue (`KismetSystemLibrary.K2_SetTimer` null "Fire" 0.3 true)))

(event `self.On Uninstalled`
  (`SkeletalMeshComponent.PlayAnimation` (`self.SK_PlanterModule`) "/Game/Resources/Characters/Modules/Planter/SK_PlanterModule_Anim_PlanterArmature_PlanterCloseUp.SK_PlanterModule_Anim_PlanterArmature_PlanterCloseUp" false))

(event `self.LightProjectileStop`
  (`KismetSystemLibrary.K2_ClearAndInvalidateTimerHandle` (stale `self.LightProjectileStart` _returnvalue)))

(event `self.HeavyAttack`
  (params (Charge :type "Float (double-precision)"))
  (bind _asweapon_base_bp (cast `/Game/Resources/Characters/Weapons/WeaponBase_BP` (`self.Host`)))
  (message `/Game/Resources/Characters/Player/Blueprints/ApplyingStat_BPInter.Apply Healing` (`/Game/Resources/Characters/Weapons/WeaponBase_BP.Host` _asweapon_base_bp) (* Charge 100.0)))

(event `Fire`
  (bind _asweapon_base_bp (cast `/Game/Resources/Characters/Weapons/WeaponBase_BP` (`self.Host`)))
  (message `/Game/Resources/Characters/Player/Blueprints/ApplyingStat_BPInter.Apply Healing` (`/Game/Resources/Characters/Weapons/WeaponBase_BP.Host` _asweapon_base_bp) 10.0)
  (`SkeletalMeshComponent.PlayAnimation` (`self.SK_PlanterModule`) "/Game/Resources/Characters/Modules/Planter/SK_PlanterModule_Anim_PlanterArmature_PlanterFiring.SK_PlanterModule_Anim_PlanterArmature_PlanterFiring" false))

(fn `Calculate Passive`
  (params (`Old Passive` :type "/Game/Resources/Characters/Modules/ModulePassive_Struct Structure"))
  (returns (Passive :type "/Game/Resources/Characters/Modules/ModulePassive_Struct Structure"))
  (bind (_type _speedscale _dmgscale _firerate _passivefunctions _passivecount) (break `/Game/Resources/Characters/Modules/ModulePassive_Struct` `Old Passive`))
  (bind (_value _returnvalue) (`BlueprintMapLibrary.Map_Find` _passivecount (`self.Type`)))
  (`KismetArrayLibrary.Array_Add` _passivefunctions self)
  (if _returnvalue
    (`BlueprintMapLibrary.Map_Add` _passivecount (`self.Type`) (+ _value 1))
    (else
      (`BlueprintMapLibrary.Map_Add` _passivecount (`self.Type`) 1)))
  (return (make `/Game/Resources/Characters/Modules/ModulePassive_Struct` _type _speedscale _dmgscale _firerate _passivefunctions _passivecount)))

(fn `UserConstructionScript`
  (`parent.UserConstructionScript`))