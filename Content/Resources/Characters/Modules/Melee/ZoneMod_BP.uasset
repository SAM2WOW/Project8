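; Melee character module that damages everything in a sphere around itself, using the host's trace channel.
; Light attacks call Fire, repeated on a looping timer during light projectile mode, showing the sphere and dealing damage with slight upward knockback.
; Each Fire builds charge that grows radius, damage and visual scale, until a retriggerable delay resets it.
; Heavy attack makes one charge-scaled sphere hit with strong vertical knockback.
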(event `self.LightAttack`
  (`parent.LightAttack`)
  (`self.Fire`))

(event `self.LightProjectileStop`
  (`parent.LightProjectileStop`)
  (`KismetSystemLibrary.K2_ClearAndInvalidateTimerHandle` (stale `self.LightProjectileStart` _returnvalue)))

(event `self.LightProjectileStart`
  (`parent.LightProjectileStart`)
  (bind _returnvalue (`KismetSystemLibrary.K2_SetTimer` null "Fire" (`self.BaseFireRate`) true))
  (`self.Fire`))

(event `self.HeavyAttack`
  (params (Charge :type "Float (double-precision)"))
  (bind _returnvalue (`self.K2_GetActorLocation`))
  (`parent.HeavyAttack` Charge)
  (bind _channel (message `/Game/Resources/Characters/Modules/DamageOwner_BPInter.Get Trace Channel` (`self.Host`)))
  (bind (_outhits _returnvalue_2) (`KismetSystemLibrary.SphereTraceMulti` _returnvalue _returnvalue (`KismetMathLibrary.Lerp` 150.0 300.0 Charge) _channel))
  (if _returnvalue_2
    (for _array_element _outhits
      (`GameplayStatics.ApplyDamage` (`.HitActor` (`GameplayStatics.BreakHitResult` _array_element)) (`KismetMathLibrary.Lerp` 8.0 50.0 Charge) null (`self.Host`) "/Game/Resources/Characters/Weapons/Sword/Heavy_DamageType.Heavy_DamageType_C")
      (message `/Game/Resources/Characters/Player/Blueprints/Knockback_BPInter.Apply Knockback` (`.HitActor` (`GameplayStatics.BreakHitResult` _array_element)) self 0.0 400.0))))

(event `Fire`
  (bind _returnvalue (`self.K2_GetActorLocation`))
  (`SceneComponent.SetVisibility` (`self.Sphere`) true false)
  (bind _output_get (set `self.Charge` (`KismetMathLibrary.FMin` (+ (`self.Charge`) 0.04) 1.0)))
  (`SceneComponent.SetRelativeScale3D` (`self.Sphere`) (`KismetMathLibrary.VLerp` (3.0 3.0 3.0) (6.0 6.0 6.0) _output_get))
  (`|ExecutionSequence`
    (:`then_0`
      (bind _channel (message `/Game/Resources/Characters/Modules/DamageOwner_BPInter.Get Trace Channel` (`self.Host`)))
      (bind (_outhits _returnvalue_2) (`KismetSystemLibrary.SphereTraceMulti` _returnvalue _returnvalue (`KismetMathLibrary.Lerp` 150.0 300.0 (`self.Charge`)) _channel))
      (if _returnvalue_2
        (for _array_element _outhits
          (`GameplayStatics.ApplyDamage` (`.HitActor` (`GameplayStatics.BreakHitResult` _array_element)) (`KismetMathLibrary.Lerp` 2.0 15.0 (`self.Charge`)) null (`self.Host`) "/Script/Engine.DamageType")
          (message `/Game/Resources/Characters/Player/Blueprints/Knockback_BPInter.Apply Knockback` (`.HitActor` (`GameplayStatics.BreakHitResult` _array_element)) self 0.0 10.0))))
    (:`then_1`
      (`KismetSystemLibrary.RetriggerableDelay` 0.2)
      (`SceneComponent.SetVisibility` (`self.Sphere`) false false)
      (set `self.Charge` 0.0)
      (`SceneComponent.SetRelativeScale3D` (`self.Sphere`) (3.0 3.0 3.0)))))

(fn `UserConstructionScript`
  (`parent.UserConstructionScript`))