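; ModuleBase_BP is a base actor for character modules, with empty light, projectile and heavy attack events and a pass-through CalculatePassive.
; Tick counts Cooldown down to zero.
; Deploy looks up its Type in ModuleInfo_DT and spawns that row's Buildable at the module's location with the Host's yaw.
; The spawn receives the Host as parent, health from the row, the Passive value and a random reachable target near the Host.
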(event `self.ReceiveTick`
  (params (DeltaSeconds :type "Float (single-precision)"))
  ;[0 1 0.2031] Cooldown
  (if (> (`self.Cooldown`) 0.0)
    (bind _output_get (set `self.Cooldown` (`KismetMathLibrary.FMax` (- (`self.Cooldown`) DeltaSeconds))))))

(event `LightAttack`
  ;[0 1 0.6719] // Attacks
)

(event `LightProjectileStart`
  ;[0 1 0.6719] // Attacks
)

(event `LightProjectileStop`
  ;[0 1 0.6719] // Attacks
)

(event `HeavyAttack`
  (params (Charge :type "Float (double-precision)"))
  ;[0 1 0.6719] // Attacks
)

(event `Deploy`
  (bind _returnvalue_location (`KismetMathLibrary.BreakTransform` (`self.GetTransform`)))
  (bind _host (`self.Host`))
  (bind (_returnvalue_roll _returnvalue_pitch _returnvalue_yaw) (`KismetMathLibrary.BreakRotator` (`self.K2_GetActorRotation` _host)))
  ;[0 1 0.6719] // Attacks
  (bind _returnvalue (`|GetDataTableRow` "/Game/Resources/Characters/Modules/ModuleInfo_DT.ModuleInfo_DT" (`self.Type`))
    (:`then`
      (if (`KismetSystemLibrary.IsValidClass` (`.Buildable_12_952B647D4466188B0B8913A0526CC98B` (break `/Game/Resources/Characters/Modules/ModuleInfo_Struct` _returnvalue)))
        (`|SpawnActorFromClass` (`.Buildable_12_952B647D4466188B0B8913A0526CC98B` (break `/Game/Resources/Characters/Modules/ModuleInfo_Struct` _returnvalue)) (`KismetMathLibrary.MakeTransform` _returnvalue_location (`KismetMathLibrary.MakeRotator` 0.0 0.0 _returnvalue_yaw)) "AdjustIfPossibleButAlwaysSpawn" "OverrideRootScale" null (`self.Host`) (`.BuildableHealth_28_23B734B641FBF7FD67ADF0AFDE5ACAD4` (break `/Game/Resources/Characters/Modules/ModuleInfo_Struct` _returnvalue)) (`NavigationSystemV1.K2_GetRandomReachablePointInRadius` (`self.K2_GetActorLocation` _host) 500.0 null null) (`self.Passive`) null)))))

(fn `Calculate Passive`
  (params (`Old Passive` :type "/Game/Resources/Characters/Modules/ModulePassive_Struct Structure"))
  (returns (Passive :type "/Game/Resources/Characters/Modules/ModulePassive_Struct Structure"))
  (return `Old Passive`))

(fn `UserConstructionScript`)