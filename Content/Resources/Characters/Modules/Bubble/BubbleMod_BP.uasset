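; Bubble weapon module that shoots bullets at the locked target, or along its own facing when nothing is locked.
; Light attacks fire single shots or looping timer-driven two-shot bursts, while heavy attacks scale burst length with charge and enlarge the muzzle flash.
; SpawnBullet passes host, passives and damage to each bullet and plays flash and sound.
; Each shot also animates the bubble layer's scale and rumbles the controller for player hosts.
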(event `self.LightAttack`
  (`parent.LightAttack`)
  (`self.Fire`))

(event `self.LightProjectileStop`
  (`parent.LightProjectileStop`)
  (`KismetSystemLibrary.K2_ClearAndInvalidateTimerHandle` (stale `self.LightProjectileStart` _returnvalue)))

(event `self.LightProjectileStart`
  (`parent.LightProjectileStart`)
  (bind _returnvalue (`KismetSystemLibrary.K2_SetTimer` null "FireBubble" (`self.BaseFireRate`) true))
  (`self.Fire`)
  (`KismetSystemLibrary.PrintString` "FIRE!!!" true true (struct :`R` 1.0 :`B` 0.094325 :`A` 1.0)))

(event `FireBubble`
  (`/Game/Resources/Characters/Player/Blueprints/NewActorMacroLibrary.ForLoopWithDelay` 0 1 0.15
    (:`Loop Body`
      (`self.Fire`))))

(event `self.HeavyAttack`
  (params (Charge :type "Float (double-precision)"))
  (`parent.HeavyAttack` Charge)
  (set `self.ScaleParticle` (10.0 10.0 10.0))
  (`/Game/Resources/Characters/Player/Blueprints/NewActorMacroLibrary.ForLoopWithDelay` 0 (`KismetMathLibrary.Round` (`KismetMathLibrary.Lerp` 0.0 3.0 Charge)) 0.1
    (:`Loop Body`
      (`NiagaraFunctionLibrary.SpawnSystemAtLocation` "/Game/VFX_Pack/Niagara/NS_OverdriveHint.NS_OverdriveHint" (`SceneComponent.K2_GetComponentLocation` (`self.StaticBubble`)))
      (`self.Fire`))
    (:`Completed`
      (set `self.ScaleParticle` (1.0 1.0 1.0)))))

(event `Fire`
  (bind (_returnvalue_location _returnvalue_rotation) (`KismetMathLibrary.BreakTransform` (`self.GetTransform`)))
  (bind _basedmg (`self.BaseDmg`))
  (bind _locked_target (`self.Locked Target`)
    (:`then`
      (`self.Spawn Bullet` _returnvalue_location (`KismetMathLibrary.FindLookAtRotation` (`self.K2_GetActorLocation` self) (`self.K2_GetActorLocation` _locked_target)) (1.0 1.0 1.0) _basedmg))
    (:`else`
      (`self.Spawn Bullet` _returnvalue_location _returnvalue_rotation (1.0 1.0 1.0) _basedmg)))
  (`|ExecutionSequence`
    (:`then_0`
      (bind _tag (message `/Game/Resources/Characters/Modules/DamageOwner_BPInter.Get Tag` (`self.Host`)))
      (if (== _tag "Player")
        (`GameplayStatics.SpawnForceFeedbackAttached` "/Game/Resources/Characters/Weapons/Sword/Feedbacks/Fire_Feed.Fire_Feed" null "None" (0.0 0.0 0.0) (struct) "SnapToTarget" false false (`KismetMathLibrary.RandomFloatInRange` 0.3 0.8) 0.0 null)))
    (:`then_1`
      (bind (_direction _newtrack_0) (`Timeline|Shoot` :!via `PlayFromStart` :!label _label)
        (:`Update`
          (`SceneComponent.SetRelativeScale3D` (`self.StaticBubbleLayer`) (`KismetMathLibrary.MakeVector` 1.0 1.0 (`KismetMathLibrary.Lerp` 0.1 2.0 _newtrack_0))))))))

(event `self.On Installed`
  (goto _label :!via `PlayFromStart`))

(event `self.On Uninstalled`
  (goto _label :!via `PlayFromStart`))

(event `self.Deploy`
  (`parent.Deploy`))

(fn `Spawn Bullet`
  (params (Location :type "Vector Structure") (Rotation :type "Rotator Structure") (Scale :type "Vector Structure") (BaseDmg :type "Float (double-precision)"))
  (`|SpawnActorFromClass` (`self.BulletClass`) (`KismetMathLibrary.MakeTransform` Location Rotation Scale) "AlwaysSpawn" "OverrideRootScale" null (`self.Host`) (`/Game/Resources/Characters/Modules/ModuleManager_BPC.CurrentPassive` (`self.Manager`)) BaseDmg null)
  (`NiagaraFunctionLibrary.SpawnSystemAtLocation` "/Game/VFX_Pack/Niagara/NS_test_Flash_16.NS_test_Flash_16" Location Rotation (`self.ScaleParticle`))
  (`FMODBlueprintStatics.PlayEventAtLocation` "/Game/FMOD/Events/Sounds/Module/Bubble_Fire.Bubble_Fire" (`KismetMathLibrary.MakeTransform` Location Rotation Scale)))

(fn `UserConstructionScript`
  (`parent.UserConstructionScript`))