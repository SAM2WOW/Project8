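; VITA is the player's floating sword companion, performing light and heavy attacks, a projectile mode and a deploy move.
; Tick eases it toward a point chosen by Mode: idle socket, attack target, aim ahead of Host, or beside the camera.
; Attacks animate the swing with timelines and apply sphere-trace damage, scaled by charge for heavy hits, then idle after a timer.
; Attached modules receive attack, projectile, deploy and locked-target updates.
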(event `self.ReceiveTick`
  (params (DeltaSeconds :type "Float (single-precision)"))
  (bind _returnvalue (`GameplayStatics.GetWorldDeltaSeconds`))
  (bind (_returnvalue_location _returnvalue_rotation) (`KismetMathLibrary.BreakTransform` (`self.GetTransform`)))
  (bind _mode (`self.Mode`))
  (bind _host (`self.Host`))
  (bind _speed (`self.Speed`))
  (bind _returnvalue_2 (`self.K2_GetActorRotation` _host))
  (bind _asbp_player_character (cast `/Game/Resources/Characters/Player/Blueprints/BP_PlayerCharacter` (`GameplayStatics.GetPlayerPawn` 0) :!pure true))
  (bind _followcamera (`/Game/Resources/Characters/Player/Blueprints/BP_PlayerCharacter.FollowCamera` _asbp_player_character))
  (bind (_returnvalue_location_2 _returnvalue_rotation_2) (`KismetMathLibrary.BreakTransform` (`SceneComponent.K2_GetComponentToWorld` (`/Game/Resources/Characters/Player/Blueprints/BP_PlayerCharacter.Sword Idle ` _asbp_player_character))))
  (`self.K2_SetActorTransform` (`KismetMathLibrary.MakeTransform` (`KismetMathLibrary.VInterpTo` _returnvalue_location (select `/Game/Resources/Characters/Sword/SwordModes_Enum` _mode :`NewEnumerator0` _returnvalue_location_2 :`NewEnumerator1` (`self.TargetLoc`) :`NewEnumerator2` (+ (`self.K2_GetActorLocation` _host) (* (`KismetMathLibrary.GetForwardVector` _returnvalue_2) 300.0)) :`NewEnumerator3` (+ (`SceneComponent.K2_GetComponentLocation` _followcamera) (* (`SceneComponent.GetForwardVector` _followcamera) 200.0) (* (`SceneComponent.GetRightVector` _followcamera) -50.0))) _returnvalue _speed) (`KismetMathLibrary.RInterpTo` _returnvalue_rotation (select `/Game/Resources/Characters/Sword/SwordModes_Enum` _mode :`NewEnumerator0` _returnvalue_rotation_2 :`NewEnumerator1` (`self.TargetRot`) :`NewEnumerator2` (`KismetMathLibrary.MakeRotator` (+ (.roll _returnvalue_2) 90.0) (+ (.pitch _returnvalue_2) 90.0) (.yaw _returnvalue_2)) :`NewEnumerator3` (`SceneComponent.K2_GetComponentRotation` _followcamera)) _returnvalue _speed))))

(event `Light Attack`
  (params (Location :type "Vector Structure") (Rotation :type "Rotator Structure"))
  (bind _targetloc (`self.TargetLoc`))
  ;[0.8607 1 0] Light Attack
  (if (not (`self.Actioning`))
    (set `self.Actioning` true)
    (`KismetSystemLibrary.K2_ClearAndInvalidateTimerHandle` (`self.ReturnTimer`))
    (set `self.TargetLoc` (+ Location (* (`KismetMathLibrary.RandomUnitVector`) 20.0)))
    (set `self.TargetRot` Rotation)
    (set `self.Mode` "NewEnumerator1")
    (`|ExecutionSequence`
      (:`then_0`
        (bind (_direction _0) (`Timeline|Swinging` :!via `PlayFromStart`)
          (:`Update`
            (`SceneComponent.K2_SetRelativeRotation` (`self.sword`) (`KismetMathLibrary.MakeRotator` 180.0 (`KismetMathLibrary.Lerp` 320.0 0.0 _0) 90.0) false true)
            (`SceneComponent.K2_SetRelativeLocation` (`self.sword`) (`KismetMathLibrary.VLerp` (-200.0 0.0 0.0) (0.0 0.0 0.0) _0) false false)
            (set `self.Speed` (`KismetMathLibrary.Lerp` 40.0 5.0 _0)))
          (:`Finished`
            (set `self.Actioning` false)
            (bind _asbp_player_character (cast `/Game/Resources/Characters/Player/Blueprints/BP_PlayerCharacter` (`GameplayStatics.GetPlayerPawn` 0)))
            (bind _light_attack (`/Game/Resources/Characters/Player/Blueprints/BP_PlayerCharacter.Is Light Action?` _asbp_player_character))
            (if _light_attack
              (`self.Shoot`)
              (else
                (bind _returnvalue (`KismetSystemLibrary.K2_SetTimer` null "Finish Swing" (`self.ReturnTime`)))
                (set `self.ReturnTimer` _returnvalue))))))
      (:`then_1`
        (bind (_outhits _returnvalue_2) (`KismetSystemLibrary.SphereTraceMulti` :`Start` _targetloc :`End` _targetloc :`Radius` 150.0 :`TraceChannel` "TraceTypeQuery3" :`DrawDebugType` "ForOneFrame"))
        (if _returnvalue_2
          (for _array_element _outhits
            (`GameplayStatics.ApplyDamage` (`.HitActor` (`GameplayStatics.BreakHitResult` _array_element)) 80.0 null self "/Script/Engine.DamageType")
            (`GameplayStatics.SpawnForceFeedbackAttached` "/Game/Resources/Characters/Sword/Light_Feed.Light_Feed" (`self.sword`) "None" (0.0 0.0 0.0) (struct) "SnapToTarget" false false 1.0 0.0 null))))
      (:`then_2`
        (for _array_element_2 (`self.Modules`)
          (`/Game/Resources/Characters/Modules/ModuleBase_BP.LightAttack` _array_element_2))))))

(event `Heavy Attack`
  (params (Location :type "Vector Structure") (Rotation :type "Rotator Structure") (Charge :type "Float (double-precision)"))
  (bind _targetloc (`self.TargetLoc`))
  ;[1 0.6697 0] Light Attack
  (if (not (`self.Actioning`))
    (set `self.Actioning` true)
    (`KismetSystemLibrary.K2_ClearAndInvalidateTimerHandle` (`self.ReturnTimer`))
    (set `self.TargetLoc` Location)
    (set `self.TargetRot` Rotation)
    (set `self.Mode` "NewEnumerator1")
    (`|ExecutionSequence`
      (:`then_0`
        (bind (_direction _0) (`Timeline|Timeline` :!via `PlayFromStart`)
          (:`Update`
            (`SceneComponent.K2_SetRelativeRotation` (`self.sword`) (`KismetMathLibrary.MakeRotator` 180.0 (`KismetMathLibrary.Lerp` 359.0 0.0 _0) 90.0) false true)
            (`SceneComponent.K2_SetRelativeLocation` (`self.sword`) (`KismetMathLibrary.VLerp` (0.0 0.0 300.0) (0.0 0.0 0.0) _0) false false)
            (set `self.Speed` (`KismetMathLibrary.Lerp` 40.0 5.0 _0)))
          (:`Finished`
            (set `self.Actioning` false)
            (bind _returnvalue (`KismetSystemLibrary.K2_SetTimer` null "Finish Swing" (`self.ReturnTime`)))
            (set `self.ReturnTimer` _returnvalue))))
      (:`then_1`
        (bind (_outhits _returnvalue_2) (`KismetSystemLibrary.SphereTraceMulti` :`Start` _targetloc :`End` _targetloc :`Radius` 300.0 :`TraceChannel` "TraceTypeQuery3" :`DrawDebugType` "ForOneFrame"))
        (if _returnvalue_2
          (for _array_element _outhits
            (`GameplayStatics.ApplyDamage` (`.HitActor` (`GameplayStatics.BreakHitResult` _array_element)) (`KismetMathLibrary.Lerp` 100.0 300.0 Charge) null self "/Script/Engine.DamageType")
            (`GameplayStatics.SpawnForceFeedbackAttached` "/Game/Resources/Characters/Sword/Light_Feed.Light_Feed" (`self.sword`) "None" (0.0 0.0 0.0) (struct) "SnapToTarget" false false 1.0 0.0 null))))
      (:`then_2`
        (for _array_element_2 (`self.Modules`)
          (`/Game/Resources/Characters/Modules/ModuleBase_BP.HeavyAttack` _array_element_2))))))

(event `Finish Swing`
  ;[1 0.7091 0] Finish Swing
  (set `self.Mode` "NewEnumerator0"))

(event `LightAttack Completed`
  ;[1 0.4309 0] Finished Projectile Attack
  (if (`self.Shooting`)
    (set `self.Shooting` false)
    (for _array_element (`self.Modules`)
      (`/Game/Resources/Characters/Modules/ModuleBase_BP.LightProjectileStop` _array_element))
    (bind _returnvalue (`KismetSystemLibrary.K2_SetTimer` null "Finish Swing" (`self.ReturnTime`)))
    (set `self.ReturnTimer` _returnvalue)))

(event `Shoot`
  ;[1 0.1588 0] Start Projectile Mode
  (set `self.Shooting` true)
  (for _array_element (`self.Modules`)
    (`/Game/Resources/Characters/Modules/ModuleBase_BP.LightProjectileStart` _array_element))
  (set `self.Mode` "NewEnumerator2"))

(event `Deploy`
  (bind _asbp_player_character (cast `/Game/Resources/Characters/Player/Blueprints/BP_PlayerCharacter` (`GameplayStatics.GetPlayerPawn` 0) :!pure true))
  (bind _returnvalue (`self.K2_GetActorRotation` _asbp_player_character))
  (bind _returnvalue_2 (+ (`self.K2_GetActorLocation` _asbp_player_character) (* (`KismetMathLibrary.GetForwardVector` _returnvalue) 100.0)))
  ;[0.2188 0 1] Deploy
  (if (not (`self.Actioning`))
    (set `self.Actioning` true)
    (`KismetSystemLibrary.K2_ClearAndInvalidateTimerHandle` (`self.ReturnTimer`))
    (set `self.Speed` 40.0)
    (set `self.TargetLoc` (+ _returnvalue_2 (0.0 0.0 100.0)))
    (set `self.TargetRot` _returnvalue)
    (set `self.Mode` "NewEnumerator1")
    (`KismetSystemLibrary.Delay` 0.3)
    (set `self.Speed` 20.0)
    (set `self.TargetLoc` (+ _returnvalue_2 (0.0 0.0 -50.0)))
    (for _array_element (`self.Modules`)
      (`/Game/Resources/Characters/Modules/ModuleBase_BP.Deploy` _array_element))
    (`KismetSystemLibrary.Delay` 0.3)
    (set `self.Mode` "NewEnumerator0")
    (set `self.Actioning` false)))

(event `Attach Module`
  (params (Module :type "/Game/Resources/Characters/Modules/ModuleBase_BP Object Reference"))
  (bind (_origin _boxextent) (`KismetSystemLibrary.GetComponentBounds` (`self.Box`)))
  ;[0 0.5853 1] Attach
  (set `/Game/Resources/Characters/Modules/ModuleBase_BP.Host` self Module)
  (`self.K2_SetActorLocation` Module (`KismetMathLibrary.RandomPointInBoundingBox` _origin _boxextent) false false)
  (`self.K2_AttachToActor` Module self "None" "KeepWorld" "SnapToTarget" "KeepWorld" true)
  (`KismetArrayLibrary.Array_Add` (`self.Modules`) Module))

(event `Update Modules Target`
  (params (`New Target` :type "Actor Object Reference"))
  ;[1 0.1978 0.8982] Update Locked Targets
  (bind _output_get (set `self.Locked Target` `New Target`))
  (for _array_element (`self.Modules`)
    (set `/Game/Resources/Characters/Modules/ModuleBase_BP.Locked Target` _output_get _array_element)))

(fn `Remove Module`
  (params (Index :type "Integer (by ref)"))
  (returns (Output_Get :type "/Game/Resources/Characters/Modules/ModuleBase_BP Object Reference"))
  (locals (Temp :type "/Game/Resources/Characters/Modules/ModuleBase_BP Object Reference"))
  (bind _modules (`self.Modules`))
  (bind _output_get (set `local.Temp` (`|GetArrayItem` _modules Index)))
  (`self.K2_DetachFromActor` _output_get "KeepWorld" "KeepWorld" "KeepWorld")
  (`KismetArrayLibrary.Array_Remove` _modules Index)
  (return _output_get))

(fn `UserConstructionScript`)